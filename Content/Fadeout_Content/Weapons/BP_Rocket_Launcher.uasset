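; Rocket launcher weapon, a child Blueprint that adds a loaded-rocket display, restricted alt-fire and its own fire sound.
; Alt-fire passes to the parent only when the owner is BP_Char_Mouse, gated by CanDetonate.
; FakeRocket visibility updates every Tick from ammo, fire readiness, mesh visibility and cloaking, stays shown on the ground, and also refreshes on LastProjectileNotify.
; PlayFireSound layers two attenuated shots with random pitch.
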(event `self.OnAltFirePress`
  (set `self.canDetonate` false)
  (bind _asbp_player_character (cast `/Game/Fadeout_Content/Core/Characters/BP_PlayerCharacter` (`self.GetOwner`)))
  (cast `/Game/Fadeout_Content/Core/Characters/BP_Char_Mouse` _asbp_player_character
    (:`then`
      (set `self.canDetonate` true))
    (:`CastFailed`
      _))
  (if (`self.canDetonate`)
    (`parent.OnAltFirePress`)))

(event `/Game/Fadeout_Content/Core/Weapons/BP_ProjectileGun.Last Projectile Notify`
  (`parent.Last Projectile Notify`)
  (`SceneComponent.SetVisibility` (`self.fakeRocket`) (`self.CanFire?`) false))

(event `Check For Rocket Display`
  (bind _firecostmet (`self.AmmoCheckFunction`))
  (`SceneComponent.SetVisibility` (`self.fakeRocket`) (and _firecostmet (`self.CanFire?`) (`SceneComponent.bVisible` (`self.SkeletalMesh`)) (not (`self.cloaked`))) false))

(event `self.ReceiveTick`
  (params (DeltaSeconds :type "Float (single-precision)"))
  (if (`self.onGround?`)
    (`SceneComponent.SetVisibility` (`self.fakeRocket`) true false)
    (else
      (`self.Check For Rocket Display`))))

(fn `PlayFireSound`
  (bind _returnvalue (`self.K2_GetActorLocation`))
  (bind _returnvalue_2 (`KismetMathLibrary.RandomFloatInRange` 0.9 1.1))
  (`GameplayStatics.PlaySoundAtLocation` (`self.FireSound`) _returnvalue (struct) 1.0 _returnvalue_2 0.0 "/Game/Fadeout_Content/Core/Characters/GunshotAttenuation.GunshotAttenuation" null null)
  (`GameplayStatics.PlaySoundAtLocation` "/Game/Fadeout_Content/Core/Audio/Gun/Steampunk_Weapons_-_Grenade_Launcher_2_-_Shot_-_02.Steampunk_Weapons_-_Grenade_Launcher_2_-_Shot_-_02" _returnvalue (struct) 0.8 _returnvalue_2 0.0 "/Game/Fadeout_Content/Core/Characters/GunshotAttenuation.GunshotAttenuation" null null))

(fn `UserConstructionScript`
  (`parent.UserConstructionScript`))