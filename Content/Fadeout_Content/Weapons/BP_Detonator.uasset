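; BP_Detonator is a child weapon Blueprint for a detonator that displays how many projectiles its owning player has out.
; A looping timer refreshes a TextRender count from the player character's MyOwnedProjectiles while the weapon is not on the ground, hiding it when cloaked.
; Fire presses pass to the parent only when the ammo cost is met and CanFire is set, otherwise a no-ammo sound plays.
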(event `self.ReceiveBeginPlay`
  (`parent.ReceiveBeginPlay`)
  (`KismetSystemLibrary.K2_SetTimerDelegate` (delegate `Bomb Count Timer`) 0.5 true))

(event `self.onSwapOut`
  (`parent.onSwapOut`))

(event `self.onSwapIn`
  (`parent.onSwapIn`))

(event `Bomb Count Timer`
  (if (not (`self.onGround?`))
    (`self.update Bomb Count Text`)
    (`SceneComponent.SetVisibility` (`self.TextRender`) (not (`self.cloaked`)) false)))

(event `self.OnFirePress`
  (bind _firecostmet (`self.AmmoCheckFunction`))
  (if (and _firecostmet (`self.CanFire?`))
    (`parent.OnFirePress`)
    (else
      (`self.PlayNoAmmoSound`))))

(event `update Bomb Count Text`
  (bind _returnvalue (`self.GetOwner`))
  (`/Engine/EditorBlueprintResources/StandardMacros.IsValid` _returnvalue
    (:`Is Valid`
      (`/Engine/EditorBlueprintResources/StandardMacros.IsValid` (`self.TextRender`)
        (:`Is Valid`
          (bind _asbp_player_character (cast `/Game/Fadeout_Content/Core/Characters/BP_PlayerCharacter` _returnvalue)
            (:`then`
              (`TextRenderComponent.K2_SetText` (`self.TextRender`) (`KismetTextLibrary.Conv_IntToText` (`KismetArrayLibrary.Array_Length` (`/Game/Fadeout_Content/Core/Characters/BP_PlayerCharacter.myOwnedProjectiles` _asbp_player_character)) false true 2 3)))
            (:`CastFailed`
              (`TextRenderComponent.K2_SetText` (`self.TextRender`) (`KismetTextLibrary.Conv_IntToText` 0 false true 2 3)))))))))

(fn `UserConstructionScript`)