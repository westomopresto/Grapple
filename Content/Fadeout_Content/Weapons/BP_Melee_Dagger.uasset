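; Dagger melee weapon that lunges its wielder along the camera direction on each attack and rewards stealth strikes.
; Firing doubles damage if the owner is cloaked and out of combat, then replicates a short-delayed launch and grunt via server and multicast events.
; Hits at crit-level damage add a marker sound and spark burst, while hitting a non-character pops the wielder upward.
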(event `self.ReceiveBeginPlay`
  (`parent.ReceiveBeginPlay`)
  (set `self.BaseDamage` (`self.damage`)))

(event `Multicast Launch`
  (params (Target :type "/Game/Fadeout_Content/Core/Characters/BP_PlayerCharacter Object Reference") (Direction :type "Vector Structure"))
  (`/Engine/EditorBlueprintResources/StandardMacros.IsValid` Target
    (:`Is Valid`
      (`KismetSystemLibrary.Delay` 0.2)
      (`self.GruntSound`)
      (`Character.LaunchCharacter` Target (* (+ Direction (0.0 0.0 0.25)) 700.0) false false))))

(event `self.Melee Release Anim`
  (params (`Player Character` :type "/Game/Fadeout_Content/Core/Characters/BP_PlayerCharacter Object Reference"))
  (`/Game/Fadeout_Content/Core/Characters/BP_PlayerCharacter.Dagger Montage` `Player Character` "attack"))

(event `Server Launch`
  (params (Target :type "/Game/Fadeout_Content/Core/Characters/BP_PlayerCharacter Object Reference") (Direction :type "Vector Structure"))
  (`self.Multicast Launch` Target Direction))

(event `self.OnFirePress`
  ;[1 1 1] actually important lol
  (`parent.OnFirePress`)
  (bind _firecostmet (`self.AmmoCheckFunction`))
  (if _firecostmet
    (bind (_location _direction) (`self.CameraFVector`))
    (bind _asbp_char_bingo (cast `/Game/Fadeout_Content/Core/Characters/BP_Char_Bingo` (`self.GetOwner`))
      (:`then`
        (`self.MeleeCrit` (and (`/Game/Fadeout_Content/Core/Characters/BP_PlayerCharacter.isCloaked` _asbp_char_bingo) (not (`/Game/Fadeout_Content/Core/Characters/BP_PlayerCharacter.inCOMBAT` _asbp_char_bingo)))))
      (:`CastFailed`
        _))
    (`parent.OnFire`)
    (`/Engine/EditorBlueprintResources/ActorMacros.Switch Has Authority`
      (:`Authority`
        (`self.Multicast Launch` _asbp_char_bingo _direction))
      (:`Remote`
        (`self.Server Launch` _asbp_char_bingo _direction)))))

(event `MeleeCrit`
  (params (bPickA :type Boolean))
  (bind _basedamage (`self.BaseDamage`))
  (set `self.damage` (`KismetMathLibrary.SelectFloat` (* _basedamage 2.0) _basedamage bPickA)))

(event `self.Damaged Player Hit Event`
  (params (Location :type "Vector Structure") (Amount :type "Float (single-precision)"))
  (if (>= Amount (* (`self.BaseDamage`) 2.0))
    (`GameplayStatics.SpawnSoundAtLocation` "/Game/Fadeout_Content/Core/Audio/Weapon_SFX/CritMarker_V5.CritMarker_V5" Location (struct) 2.0 1.5 0.0 "/Game/Fadeout_Content/Core/Characters/BulletHit_Attenuation.BulletHit_Attenuation" "/Game/Fadeout_Content/Core/Characters/BulletHitConcurrency.BulletHitConcurrency")
    (`GameplayStatics.SpawnEmitterAttached` "/Game/AnimeFX/Particles/Parametric/PS_Spark_Burst.PS_Spark_Burst" (`self.trail_loc`))))

(event `self.Melee Damage Event`
  (params (DamagedActor :type "Actor Object Reference") (BaseDamage :type "Float (single-precision)") (EventInstigator :type "Controller Object Reference") (DamageCauser :type "Actor Object Reference") (DamageTypeClass :type "DamageType Class Reference") (`Impact Normal` :type "Vector Structure") (`Impact Point` :type "Vector Structure"))
  (`parent.Melee Damage Event` DamagedActor BaseDamage EventInstigator DamageCauser DamageTypeClass `Impact Normal` `Impact Point`)
  (cast `Character` DamagedActor
    (:`CastFailed`
      (bind _ascharacter (cast `Character` (`self.GetOwner`)))
      (`Character.LaunchCharacter` _ascharacter (0.0 0.0 200.0) false false))))

(fn `GruntSound`
  (`GameplayStatics.SpawnSoundAttached` "/Game/PunchSoundPack/BonusSounds/voice_male_effort_grunt_01_Cue.voice_male_effort_grunt_01_Cue" (`Actor.RootComponent` (`self.GetOwner`)) "None" (0.0 0.0 0.0) (struct) "KeepRelativeOffset" false 1.0 1.0 0.0 null null))

(fn `SpawnHitTrail`
  (bind _currenttrail (`self.currentTrail`))
  (`/Engine/EditorBlueprintResources/StandardMacros.IsValid` _currenttrail
    (:`Is Valid`
      (`ActorComponent.K2_DestroyComponent` _currenttrail))
    (:`Is Not Valid`
      _))
  (bind _returnvalue (`GameplayStatics.SpawnEmitterAttached` "/Game/Fadeout_Content/Core/FX/meleeTrail.meleeTrail" (`self.trail_loc`)))
  (set `self.currentTrail` _returnvalue))

(fn `UserConstructionScript`
  (`parent.UserConstructionScript`))