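; BP_TNT is a throwable TNT weapon that fires projectiles and can apply damage to the ones still active.
; Primary fire plays the player's throw montage, waits briefly, then spawns the projectile at the muzzle transform, with a flag blocking refire during the throw.
; Alt fire damages every active projectile, presumably to detonate them remotely.
; On BeginPlay or drop, the mesh switches between simulated and in-hand physics assets depending on ground state.
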(event `self.ReceiveBeginPlay`
  (`self.OnDropped`))

(event `self.OnDropped`
  (bind _mesh (`self.Mesh`))
  (if (`self.onGround?`)
    (`SkinnedMeshComponent.SetPhysicsAsset` _mesh "/Game/Fadeout_Content/Core/FBX/TNT/TNT_simulated.TNT_simulated" false)
    (else
      (`SkinnedMeshComponent.SetPhysicsAsset` _mesh "/Game/Fadeout_Content/Core/FBX/TNT/TNT_inhand.TNT_inhand" false))))

(event `self.OnFire`
  (if (`self.CanFire?`)
    (set `self.CanFire?` false)
    (`self.playThrowAnim`)
    (`KismetSystemLibrary.Delay` 0.4)
    (`self.Fire Projectile` (`self.ProjectileToFire`) true (`SceneComponent.K2_GetComponentToWorld` (`self.muzzle transform`)))
    (set `self.CanFire?` true)))

(event `self.OnAltFire`
  (params (`MoveCamera?` :type Boolean))
  (for _array_element (`self.ActiveProjectiles`)
    (`GameplayStatics.ApplyDamage` _array_element 1.0 (`self.GetInstigatorController`) self)))

(fn `playThrowAnim`
  (bind _asbp_player_character (cast `/Game/Fadeout_Content/Core/Characters/BP_PlayerCharacter` (`Controller.K2_GetPawn` (`self.GetInstigatorController`))))
  (`Character.PlayAnimMontage` _asbp_player_character "/Game/Fadeout_Content/Core/Characters/Kasparian_BP/Unarmed/inventory/itemThrow.itemThrow" 1.0 "Default"))

(fn `UserConstructionScript`
  (`parent.UserConstructionScript`))