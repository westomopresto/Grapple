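; BP_Barrel_Thrower_Weapon is a child weapon Blueprint that throws barrel projectiles and shows its readiness visually.
; Tick shows the barrel mesh when ammo cost and CanFire allow firing, otherwise a hologram whose dynamic material "shift" follows the normalized remaining cooldown.
; LastProjectileNotify registers each projectile with the owning player character and starts that cooldown timer, whose callback is empty.
; SpawnProjectileServer forwards spawn parameters to SpawnProjectile.
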(event `self.ReceiveTick`
  (params (DeltaSeconds :type "Float (single-precision)"))
  (bind _firecostmet (`self.AmmoCheckFunction`))
  (bind _returnvalue (and _firecostmet (`self.CanFire?`)))
  (`SceneComponent.SetVisibility` (`self.StaticMesh`) _returnvalue false)
  (bind _returnvalue_2 (not _returnvalue))
  (`SceneComponent.SetVisibility` (`self.hologram`) _returnvalue_2 false)
  (if _returnvalue_2
    (`MaterialInstanceDynamic.SetScalarParameterValue` (`self.barrelreload_mat`) "shift" (`KismetMathLibrary.NormalizeToRange` (`KismetSystemLibrary.K2_GetTimerRemainingTimeHandle` (`self.barrelCD`)) 0.0 (`self.Fire CoolDown`)))))

(event `self.Last Projectile Notify`
  (bind _lastprojectile (`self.LastProjectile`))
  (bind _canfire_ (`self.CanFire?`))
  (`|ExecutionSequence`
    (:`then_0`
      (`SceneComponent.SetVisibility` (`self.StaticMesh`) _canfire_ false)
      (`SceneComponent.SetVisibility` (`self.hologram`) (not _canfire_) false))
    (:`then_1`
      (`/Engine/EditorBlueprintResources/StandardMacros.IsValid` _lastprojectile
        (:`Is Valid`
          (`KismetSystemLibrary.PrintString` "valid" true true (struct :`R` 0.057249 :`G` 1.0 :`A` 1.0))
          (bind _asbp_player_character (cast `/Game/Fadeout_Content/Core/Characters/BP_PlayerCharacter` (`self.GetOwner`)))
          (`KismetArrayLibrary.Array_Add` (`/Game/Fadeout_Content/Core/Characters/BP_PlayerCharacter.myOwnedProjectiles` _asbp_player_character) _lastprojectile))))
    (:`then_2`
      (bind _returnvalue (`KismetSystemLibrary.K2_SetTimerDelegate` (delegate `FireCDDone`) (`self.Fire CoolDown`)))
      (set `self.barrelCD` _returnvalue))))

(event `self.Spawn Projectile Server`
  (params (SpawnTransform :type "Transform Structure") (OwningWeapon :type "/Game/Fadeout_Content/Core/Weapons/BP_weaponBase Object Reference") (RayHitActor :type "Actor Object Reference") (`Initial Speed Override` :type "Float (single-precision)") (`Override Speed` :type Boolean))
  (`self.Spawn Projectile` SpawnTransform OwningWeapon `Initial Speed Override` `Override Speed`))

(event `FireCDDone`)

(fn `UserConstructionScript`
  (`parent.UserConstructionScript`)
  (bind _returnvalue (`PrimitiveComponent.CreateDynamicMaterialInstance` (`self.hologram`) 0 "/Game/Fadeout_Content/Core/FBX/FlameThrower/M_barrel_reload.M_barrel_reload" "None"))
  (set `self.barrelreload_mat` _returnvalue))