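; Bow weapon in the Grapple_Gun folder that adds draw and fire visuals to its parent weapon's charge and post-shot events.
; Charge start plays the pull animation on the bow and restarts the owning player character's draw montage.
; A successful shot plays bow and character fire animations plus a muzzle particle, while a failed one stops the draw montage and plays the bow's shoot animation.
; Construction snaps HookDummy to the arrow socket.
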(event `self.Post Shot Mg`
  (params (Fired :type Boolean))
  (`parent.Post Shot Mg` Fired)
  (if Fired
    (`SkeletalMeshComponent.PlayAnimation` (`self.SkeletalMesh`) "/Game/Fadeout_Content/Core/FBX/Bow/Bow_Shoot.Bow_Shoot" false)
    (bind _asbp_player_character (cast `/Game/Fadeout_Content/Core/Characters/BP_PlayerCharacter` (`self.GetOwner`)))
    (`Character.PlayAnimMontage` _asbp_player_character (`/Game/Fadeout_Content/Core/Characters/BP_PlayerCharacter.bow_fire_montage` _asbp_player_character) 1.0 "Default")
    (`GameplayStatics.SpawnEmitterAttached` "/Game/AnimeFX/Particles/HandDrawn/PS_Circle02_01.PS_Circle02_01" (`self.SkeletalMesh`) "Muzzle")
    (else
      (bind _asbp_player_character_2 (cast `/Game/Fadeout_Content/Core/Characters/BP_PlayerCharacter` (`self.GetOwner`)))
      (`Character.StopAnimMontage` _asbp_player_character_2 (`/Game/Fadeout_Content/Core/Characters/BP_PlayerCharacter.bow_drawn_montage` _asbp_player_character_2))
      (`SkeletalMeshComponent.PlayAnimation` (`self.SkeletalMesh`) "/Game/Fadeout_Content/Core/FBX/Bow/Bow_Shoot.Bow_Shoot" false))))

(event `self.Charge Start Multicast`
  (`parent.Charge Start Multicast`)
  (bind _asbp_player_character (cast `/Game/Fadeout_Content/Core/Characters/BP_PlayerCharacter` (`self.GetOwner`)))
  (bind _bow_drawn_montage (`/Game/Fadeout_Content/Core/Characters/BP_PlayerCharacter.bow_drawn_montage` _asbp_player_character))
  (`Character.StopAnimMontage` _asbp_player_character _bow_drawn_montage)
  (`Character.PlayAnimMontage` _asbp_player_character _bow_drawn_montage 1.0 "Default")
  (`SkeletalMeshComponent.PlayAnimation` (`self.SkeletalMesh`) "/Game/Fadeout_Content/Core/FBX/Bow/Bow_Pull.Bow_Pull" false))

(fn `UserConstructionScript`
  (`parent.UserConstructionScript`)
  (`SceneComponent.K2_AttachToComponent` (`self.HookDummy`) (`self.SkeletalMesh`) "arrowSocket" "SnapToTarget" "SnapToTarget" "SnapToTarget" true))