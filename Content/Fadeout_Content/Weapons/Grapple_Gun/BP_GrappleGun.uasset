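; Grapple gun weapon that fires a hook projectile, blocked with a message while the player carries the flag.
; Press spends ammo, switches to aim cam and charges per tick (not delta-scaled); release fires at full charge, otherwise refunds ammo.
; Server/multicast events replicate charging and shot transform, while Returned blocks refiring and hides the dummy hook until the hook returns.
; It can also hold an attached target, dropped on charge or swap-out.
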(event `Charge Start Multicast`
  ;[1 1 1] Fire Press Multicast
  (`|ExecutionSequence`
    (:`then_0`
      (bind _asbp_player_character (cast `/Game/Fadeout_Content/Core/Characters/BP_PlayerCharacter` (`self.GetOwner`)))
      (`GameplayStatics.SpawnEmitterAttached` (`self.muzzleEmitter`) (`self.muzzleParticle`) "None" (0.0 0.0 0.0) (struct) (1.0 1.0 1.0) "SnapToTargetIncludingScale")
      (`self.PlayAltFireSound`)
      (`/Game/Fadeout_Content/Core/Characters/BP_PlayerCharacter.toAimCam` _asbp_player_character false false)
      (`/Engine/EditorBlueprintResources/ActorMacros.Switch Has Authority`
        (:`Authority`
          (`self.AmmoCostFunction` false)
          (set `self.TookAmmo` true))))
    (:`then_1`
      (set `/Game/Fadeout_Content/Core/Characters/BP_PlayerCharacter.canSwapTools?` false _asbp_player_character)
      (set `self.Is Charging` true)
      (`self.Drop Held Object`))))

(event `Charge Start Server`
  ;[1 1 1] Fire Press Multicast
  (`self.Charge Start Multicast`))

(event `ReturnedHookSERVER`
  (`self.ReturnedHook`))

(event `ReturnedHookEvent`
  (`/Engine/EditorBlueprintResources/ActorMacros.Switch Has Authority`
    (:`Authority`
      (`self.ReturnedHook`))
    (:`Remote`
      (`self.ReturnedHookSERVER`))))

(event `Post Shot Mg`
  ;[1 1 1] Shoot the hook
  (bind _hasflag_ (`self.Flag Check`))
  (if (not _hasflag_)
    (`|ExecutionSequence`
      (:`then_0`
        (`self.HideHookToggle` false)
        (bind _asbp_grapple_hook_projectile (cast `/Game/Fadeout_Content/Weapons/Projectiles/BP_GrappleHook_Projectile` (`self.LastProjectile`)))
        (bind _asbp_player_character (cast `/Game/Fadeout_Content/Core/Characters/BP_PlayerCharacter` (`self.GetOwner`)))
        (`/Game/Fadeout_Content/Weapons/Projectiles/BP_GrappleHook_Projectile.ignore actor` _asbp_grapple_hook_projectile (`/Game/Fadeout_Content/Core/Characters/BP_PlayerCharacter.actor attached` _asbp_player_character)))
      (:`then_1`
        (set `self.Returned` false))
      (:`then_2`
        (`self.PlayFireSound`)))))

(event `ReturnedHook`
  (bind _asbp_player_character (cast `/Game/Fadeout_Content/Core/Characters/BP_PlayerCharacter` (`self.GetOwner`)))
  (set `self.Returned` true)
  (set `/Game/Fadeout_Content/Core/Characters/BP_PlayerCharacter.canSwapTools?` true _asbp_player_character)
  (`/Game/Fadeout_Content/Core/Characters/BP_PlayerCharacter.Equipment Camera Check` _asbp_player_character)
  (`self.HideHookToggle` true))

(event `self.OnFirePress`
  (bind _returnvalue (not (`/Game/Fadeout_Content/Core/Characters/BP_PlayerCharacter.HasFlag?` (`self.playerCharacter`))))
  (`|ExecutionSequence`
    (:`then_0`
      (bind _asbp_player_character (cast `/Game/Fadeout_Content/Core/Characters/BP_PlayerCharacter` (`self.GetOwner`)))
      (set `self.playerCharacter` _asbp_player_character))
    (:`then_1`
      (bind _firecostmet (`self.AmmoCheckFunction`))
      ;[1 1 1] Check if we can fire
      (if (and (`self.CanFire?`) (`self.Returned`) _returnvalue _firecostmet)
        ;[1 1 1] Animation replicate
        (`/Engine/EditorBlueprintResources/ActorMacros.Switch Has Authority`
          (:`Authority`
            (`self.Charge Start Multicast`))
          (:`Remote`
            (`self.Charge Start Server`)))
        (else
          (`self.PlayNoAmmoSound`)
          (if (not _returnvalue)
            (`self.FlagErrorText`)))))))

(event `self.OnFireRelease`
  (params (`charged?` :type Boolean))
  (`|ExecutionSequence`
    (:`then_0`
      (bind _asbp_player_character (cast `/Game/Fadeout_Content/Core/Characters/BP_PlayerCharacter` (`self.GetOwner`)))
      (set `self.playerCharacter` _asbp_player_character))
    (:`then_1`
      (bind _hasflag_ (`self.FlagErrorText`))
      (if _hasflag_
        (bind _output_get (set `self.was charging` (`self.Is Charging`)))
        (set `self.Is Charging` false)
        (if _output_get
          (`self.Charge Fail Multicast`))
        (else
          (bind _shootfromtransform (`self.Calculate Projectile Position` (`self.RaycastAim`)))
          (`|ExecutionSequence`
            (:`then_0`
              (`/Engine/EditorBlueprintResources/ActorMacros.Switch Has Authority`
                (:`Authority`
                  (`self.Set Shoot Transform Multicast` _shootfromtransform))
                (:`Remote`
                  (`self.Set Shoot Transform Server` _shootfromtransform))))
            (:`then_1`
              (`self.Charge Check Server`))))))))

(event `self.ReceiveTick`
  (params (DeltaSeconds :type "Float (single-precision)"))
  ;[1 1 1] Event Tick
  (`parent.ReceiveTick` DeltaSeconds)
  (if (not (`self.onGround?`))
    (`|ExecutionSequence`
      (:`then_0`
        (if (`self.Is Charging`)
          (bind _output_get (set `self.Charge` (+ (`self.charge`) 10.0)))
          (set `self.charge` (`KismetMathLibrary.FClamp` _output_get 0.0 (`self.maxCharge`)))))
      (:`then_1`
        (if (`self.Returned`)
          (`SceneComponent.SetVisibility` (`self.HookDummy`) (not (`self.cloaked`)) false))))))

(event `Charge Check Server`
  ;[1 1 1] Charge Check Events
  (set `self.Is Charging` false)
  (if (`self.Returned`)
    (`/Engine/EditorBlueprintResources/StandardMacros.CompareFloat` (`self.charge`) (`self.maxCharge`)
      (:`>`
        (set `self.charge` 0.0 :!label _label)
        (`self.Spawn Projectile Server` (`self.Shoot Transform Client`) self)
        (`self.Post Shot Mg`))
      (:`==`
        (goto _label))
      (:`<`
        (set `self.charge` 0.0)
        (`self.PlayNoAmmoSound`)
        (`self.Charge Fail Multicast`)))))

(event `Set Shoot Transform Multicast`
  (params (`Shoot Transform Client` :type "Transform Structure"))
  (set `self.Shoot Transform Client` `Shoot Transform Client`))

(event `Set Shoot Transform Server`
  (params (`Shoot Transform Client` :type "Transform Structure"))
  (`self.Set Shoot Transform Multicast` `Shoot Transform Client`))

(event `Charge Fail Multicast`
  ;[1 1 1] Charge Failed
  (bind _asbp_player_character (cast `/Game/Fadeout_Content/Core/Characters/BP_PlayerCharacter` (`self.GetOwner`)))
  (set `/Game/Fadeout_Content/Core/Characters/BP_PlayerCharacter.canSwapTools?` true _asbp_player_character)
  (`/Game/Fadeout_Content/Core/Characters/BP_PlayerCharacter.toRearCam` _asbp_player_character false)
  (`/Engine/EditorBlueprintResources/ActorMacros.Switch Has Authority`
    (:`Authority`
      (if (`self.TookAmmo`)
        (`self.AmmoCostFunction` true)
        (set `self.TookAmmo` false)))))

(event `Drop Held Object`
  (bind _heldtarget (`self.heldTarget`))
  ;[1 1 1] Drop the held object
  (if (and (`self.holdingSomething`) (`KismetSystemLibrary.IsValid` _heldtarget))
    (`self.K2_DetachFromActor` _heldtarget "KeepWorld" "KeepWorld" "KeepWorld")
    (`|ExecutionSequence`
      (:`then_0`
        (bind _asbp_world_pickup_class (cast `/Game/Fadeout_Content/Core/Props/BP_WorldPickup_Class` _heldtarget))
        (`/Game/Fadeout_Content/Core/Props/BP_WorldPickup_Class.resetCollision` _asbp_world_pickup_class))
      (:`then_1`
        (set `self.heldTarget` null))
      (:`then_2`
        (set `self.holdingSomething` false)))))

(event `self.onSwapOut`
  ;[1 1 1] on SwapOut
  (`self.Drop Held Object`))

(event `Hold Target`
  (params (holdTarget :type "Actor Object Reference"))
  ;[1 1 1] Hold Object
  (bind _output_get (set `self.heldTarget` holdTarget))
  (`self.K2_AttachToActor` _output_get self "None" "KeepWorld" "KeepWorld" "KeepWorld" false)
  (set `self.holdingSomething` true)
  (bind _asbp_world_pickup_class (cast `/Game/Fadeout_Content/Core/Props/BP_WorldPickup_Class` _output_get))
  (`/Game/Fadeout_Content/Core/Props/BP_WorldPickup_Class.noCollision` _asbp_world_pickup_class))

(fn `Flag Check`
  (returns (`HasFlag?` :type Boolean))
  (bind _playercharacter (`self.playerCharacter`))
  (`/Engine/EditorBlueprintResources/StandardMacros.IsValid` _playercharacter
    (:`Is Valid`
      (if (`/Game/Fadeout_Content/Core/Characters/BP_PlayerCharacter.HasFlag?` _playercharacter)
        (return true)
        (else
          _)))
    (:`Is Not Valid`
      _))
  (return false))

(fn `FlagErrorText`
  (returns (`HasFlag?` :type Boolean))
  (bind _playercharacter (`self.playerCharacter`))
  (`/Engine/EditorBlueprintResources/StandardMacros.IsValid` _playercharacter
    (:`Is Valid`
      (if (`/Game/Fadeout_Content/Core/Characters/BP_PlayerCharacter.HasFlag?` _playercharacter)
        (bind _asfo_player_controller (cast `/Game/Fadeout_Content/Core/FO_PlayerController` (`self.GetInstigatorController` _playercharacter)))
        (`/Game/Fadeout_Content/Core/FO_PlayerController.ShowSystemMessage` _asfo_player_controller "Cannot Use Grapple with Flag" (struct :`R` 0.988034 :`G` 1.0 :`A` 1.0))
        (`/Game/Fadeout_Content/Core/Characters/BP_PlayerCharacter.StylishError` _playercharacter "Cannot Grapple with Flag")
        (return true)
        (else
          _)))
    (:`Is Not Valid`
      _))
  (return false))

(fn `GetMuzzleLocation`
  (returns (MuzzleLocation :type "Vector Structure") (MuzzleTransform :type "Transform Structure"))
  (bind _skeletalmesh (`self.SkeletalMesh`))
  (bind _muzzlesocket (`self.MuzzleSocket`))
  (return (`SceneComponent.GetSocketLocation` _skeletalmesh _muzzlesocket) (`SceneComponent.GetSocketTransform` _skeletalmesh _muzzlesocket "RTS_World")))

(fn `HideHookToggle`
  (params (visibility :type Boolean :default true))
  (`SceneComponent.SetVisibility` (`self.HookDummy`) visibility false)
  (return))

(fn `UserConstructionScript`
  (`parent.UserConstructionScript`))