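; BP_TheFinalCoil is a charge weapon that releases an area lightning attack on surrounding player characters.
; Charging grows ElecField and raises the sound pitch via server-to-multicast events.
; Firing sphere-traces at the field's size, keeps line-of-sight targets, then routes them through the server to a multicast applying damage, doubled for swimmers, and thunder effects.
; It extends a parent weapon's charge and shot events, destroying the inherited HookDummy.
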(event `Lightning scan client`
  (bind _elecfield (`self.ElecField`))
  (bind _ele_chargesound (`self.ele_chargeSound`))
  (bind (_returnvalue_x _returnvalue_y) (`KismetMathLibrary.BreakVector` (`SceneComponent.K2_GetComponentScale` _elecfield)))
  (bind _returnvalue (`SceneComponent.K2_GetComponentLocation` _elecfield))
  (bind _array (`|MakeArray` (`self.playerCharacter`) (`self.GetOwner`) :!type "Actor Object Reference"))
  (set `self.ele_damageRadius` (* _returnvalue_y 50.0))
  (`SceneComponent.SetWorldScale3D` (`self.ElecField`) (0.0 0.0 0.0))
  (`|ExecutionSequence`
    (:`then_0`
      (`/Engine/EditorBlueprintResources/StandardMacros.IsValid` _ele_chargesound
        (:`Is Valid`
          (`AudioComponent.FadeOut` _ele_chargesound 0.5 0.0 "Linear"))))
    (:`then_1`
      (bind _outhits (`KismetSystemLibrary.SphereTraceMultiForObjects` _returnvalue (+ _returnvalue 1.0) (`self.ele_damageRadius`) (`|MakeArray` "ObjectTypeQuery3" :!type "EObjectTypeQuery Enum") false _array "ForDuration"))
      (for _array_element _outhits
        (bind (_bblockinghit _binitialoverlap _time _distance _location _impactpoint _normal _impactnormal _physmat _hitactor) (`GameplayStatics.BreakHitResult` _array_element))
        (bind _asbp_player_character (cast `/Game/Fadeout_Content/Core/Characters/BP_PlayerCharacter` _hitactor))
        (bind (_outhit _returnvalue_2) (`KismetSystemLibrary.LineTraceSingle` _returnvalue _impactpoint "TraceTypeQuery1" false _array "ForDuration" true (struct :`G` 0.910388 :`B` 1.0 :`A` 1.0) (struct :`R` 1.0 :`G` 0.920735 :`A` 1.0) 9.0))
        (if (not _returnvalue_2)
          (`KismetArrayLibrary.Array_AddUnique` (`self.ele_damageActors`) _asbp_player_character)))
      (`self.Server Lightning Event` (`self.ele_damageActors`)))))

(event `Server Lightning Event`
  (params (Characters :type "Array of /Game/Fadeout_Content/Core/Characters/BP_PlayerCharacter Object Reference (by ref)"))
  (`self.Server Lightning Multicast` Characters))

(event `Server Lightning Multicast`
  (params (DmgChars :type "Array of /Game/Fadeout_Content/Core/Characters/BP_PlayerCharacter Object Reference"))
  (bind _ele_chargesound (`self.ele_chargeSound`))
  (bind _ele_damage (`self.ele_damage`))
  (for _array_element DmgChars
    (`GameplayStatics.ApplyDamage` _array_element (`KismetMathLibrary.SelectFloat` (* _ele_damage 2.0) _ele_damage (`/Game/Fadeout_Content/Core/Characters/BP_PlayerCharacter.isSwimmingNET` _array_element)) (`Pawn.GetController` (`self.PlayerOwner`)) null "/Game/Fadeout_Content/Core/Weapons/DamageTypes/DT_Rifle.DT_Rifle_C")
    (bind _returnvalue (`SceneComponent.K2_GetComponentLocation` (`Actor.RootComponent` _array_element)))
    (`GameplayStatics.SpawnEmitterAtLocation` "/Game/AnimeFX/Particles/HandDrawn/PS_Cast01_01.PS_Cast01_01" _returnvalue)
    (`GameplayStatics.SpawnSoundAtLocation` "/Game/Fadeout_Content/Weapons/Grapple_Gun/477840__josh74000mc__thunder4.477840__josh74000mc__thunder4" _returnvalue (struct) 1.0 1.0 0.0 null "/Game/Fadeout_Content/Core/Characters/ExplosionConcurrency.ExplosionConcurrency")
    (bind _outhit (`KismetSystemLibrary.LineTraceSingle` _returnvalue (+ _returnvalue (0.0 0.0 -200.0)) "TraceTypeQuery1" false (`|MakeArray` _array_element :!type "Actor Object Reference")))
    (`GameplayStatics.SpawnEmitterAtLocation` "/Game/VFX_Toolkit_V1/ParticleSystems/356Days/Par_Thundara_02.Par_Thundara_02" (`.Location` (`GameplayStatics.BreakHitResult` _outhit)) (struct) (0.5 0.5 0.5)))
  (`/Engine/EditorBlueprintResources/StandardMacros.IsValid` _ele_chargesound
    (:`Is Valid`
      (`AudioComponent.Stop` _ele_chargesound))))

(event `self.Charge Ticking`
  (`parent.Charge Ticking`)
  (`self.serverCharge` (`self.Charge`)))

(event `self.Post Shot Mg`
  (params (Fired :type Boolean))
  (`parent.Post Shot Mg` Fired)
  (`|ExecutionSequence`
    (:`then_0`
      (`KismetArrayLibrary.Array_Clear` (`self.ele_damageActors`))
      (if Fired
        (`self.Lightning scan client`)
        (else
          (bind _asbp_player_character (cast `/Game/Fadeout_Content/Core/Characters/BP_PlayerCharacter` (`self.GetOwner`)))
          (`Character.StopAnimMontage` _asbp_player_character (`/Game/Fadeout_Content/Core/Characters/BP_PlayerCharacter.bow_drawn_montage` _asbp_player_character)))))
    (:`then_1`
      (`SceneComponent.SetWorldScale3D` (`self.ElecField`) (0.298692 0.298692 0.298692)))))

(event `serverCharge`
  (params (A :type "Float (double-precision)"))
  (`self.multiCharge` A))

(event `multiCharge`
  (params (A :type "Float (double-precision)"))
  (bind _returnvalue (* A 0.01))
  (bind _ele_chargesound (`self.ele_chargeSound`))
  (bind _returnvalue_2 (`KismetMathLibrary.Lerp` 0.298692 32.0 _returnvalue))
  (`/Engine/EditorBlueprintResources/StandardMacros.IsValid` _ele_chargesound
    (:`Is Valid`
      (`AudioComponent.SetPitchMultiplier` _ele_chargesound (`KismetMathLibrary.Lerp` 1.0 2.0 _returnvalue)))
    (:`Is Not Valid`
      _))
  (`SceneComponent.SetWorldScale3D` (`self.ElecField`) (`KismetMathLibrary.MakeVector` _returnvalue_2 _returnvalue_2 _returnvalue_2)))

(event `self.Charge Start Multicast`
  (bind _ele_chargesound (`self.ele_chargeSound`))
  (`|ExecutionSequence`
    (:`then_0`
      (`SceneComponent.SetWorldScale3D` (`self.ElecField`) (0.0 0.0 0.0)))
    (:`then_1`
      (`/Engine/EditorBlueprintResources/StandardMacros.IsValid` _ele_chargesound
        (:`Is Valid`
          (`AudioComponent.Stop` _ele_chargesound))))
    (:`then_2`
      (bind _asbp_player_character (cast `/Game/Fadeout_Content/Core/Characters/BP_PlayerCharacter` (`self.GetOwner`)))
      (set `/Game/Fadeout_Content/Core/Characters/BP_PlayerCharacter.canSwapTools?` false _asbp_player_character)
      (bind _returnvalue (`GameplayStatics.SpawnSoundAttached` "/Game/Fadeout_Content/Weapons/Grapple_Gun/EnergyGun_Charge1.EnergyGun_Charge1" (`self.SkeletalMesh`) "None" (0.0 0.0 0.0) (struct) "KeepRelativeOffset" false 2.0 1.0 0.0 null null))
      (set `self.ele_chargeSound` _returnvalue))
    (:`then_3`
      (`self.Cloak Weapon` (`self.cloaked`)))))

(fn `UserConstructionScript`
  (`parent.UserConstructionScript`)
  (`ActorComponent.K2_DestroyComponent` (`self.HookDummy`)))