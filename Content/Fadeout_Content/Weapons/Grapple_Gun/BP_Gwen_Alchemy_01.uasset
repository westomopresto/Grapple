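; Gwen alchemy bow, a child weapon Blueprint that cycles four elements and sets a different projectile class for each.
; Charge start plays the bow pull animation and the owning player's draw montage.
; After a shot it plays the bow release, adding a fire montage and muzzle particles if fired, otherwise stopping the draw montage.
; The construction script snaps the inherited hook dummy to the bow's arrow socket.
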(event `self.Post Shot Mg`
  (params (Fired :type Boolean))
  (`parent.Post Shot Mg` Fired)
  (if Fired
    (`SkeletalMeshComponent.PlayAnimation` (`self.SkeletalMesh`) "/Game/Fadeout_Content/Core/FBX/Bow/Bow_Shoot.Bow_Shoot" false)
    (bind _asbp_player_character (cast `/Game/Fadeout_Content/Core/Characters/BP_PlayerCharacter` (`self.GetOwner`)))
    (`Character.PlayAnimMontage` _asbp_player_character (`/Game/Fadeout_Content/Core/Characters/BP_PlayerCharacter.bow_fire_montage` _asbp_player_character) 1.0 "Default")
    (`GameplayStatics.SpawnEmitterAttached` "/Game/AnimeFX/Particles/HandDrawn/PS_Circle02_01.PS_Circle02_01" (`self.SkeletalMesh`) "Muzzle")
    (else
      (bind _asbp_player_character_2 (cast `/Game/Fadeout_Content/Core/Characters/BP_PlayerCharacter` (`self.GetOwner`)))
      (`Character.StopAnimMontage` _asbp_player_character_2 (`/Game/Fadeout_Content/Core/Characters/BP_PlayerCharacter.bow_drawn_montage` _asbp_player_character_2))
      (`SkeletalMeshComponent.PlayAnimation` (`self.SkeletalMesh`) "/Game/Fadeout_Content/Core/FBX/Bow/Bow_Shoot.Bow_Shoot" false))))

(event `Switch Element`
  (bind _output_get (set `self.current_gwen_element` (select `/Game/Fadeout_Content/Core/Characters/Gwen/Gwen_Elements` (`self.current_gwen_element`) :`NewEnumerator0` "NewEnumerator1" :`NewEnumerator1` "NewEnumerator2" :`NewEnumerator2` "NewEnumerator3" :`NewEnumerator3` "NewEnumerator0" :!type "/Game/Fadeout_Content/Core/Characters/Gwen/Gwen_Elements Enum")))
  (set `self.ProjectileToFire` (select `/Game/Fadeout_Content/Core/Characters/Gwen/Gwen_Elements` _output_get :`NewEnumerator0` "/Game/Fadeout_Content/Core/Weapons/BP_Alchemic_Projectile.BP_Alchemic_Projectile_C" :`NewEnumerator1` "/Game/Fadeout_Content/Weapons/Projectiles/BP_TNT_Prox_Projectile.BP_TNT_Prox_Projectile_C" :`NewEnumerator2` "/Game/Fadeout_Content/Core/Weapons/BP_Arrow_Projectile.BP_Arrow_Projectile_C" :`NewEnumerator3` "/Game/Fadeout_Content/Weapons/Projectiles/BP_BrutalShot_Projectile.BP_BrutalShot_Projectile_C" :!type "/Game/Fadeout_Content/Core/Weapons/BP_ProjectileBase Class Reference")))

(event `self.Charge Start Multicast`
  (`parent.Charge Start Multicast`)
  (bind _asbp_player_character (cast `/Game/Fadeout_Content/Core/Characters/BP_PlayerCharacter` (`self.GetOwner`)))
  (bind _bow_drawn_montage (`/Game/Fadeout_Content/Core/Characters/BP_PlayerCharacter.bow_drawn_montage` _asbp_player_character))
  (`Character.StopAnimMontage` _asbp_player_character _bow_drawn_montage)
  (`Character.PlayAnimMontage` _asbp_player_character _bow_drawn_montage 1.0 "Default")
  (`SkeletalMeshComponent.PlayAnimation` (`self.SkeletalMesh`) "/Game/Fadeout_Content/Core/FBX/Bow/Bow_Pull.Bow_Pull" false))

(fn `UserConstructionScript`
  (`parent.UserConstructionScript`)
  (`SceneComponent.K2_AttachToComponent` (`self.HookDummy`) (`self.SkeletalMesh`) "arrowSocket" "SnapToTarget" "SnapToTarget" "SnapToTarget" true))