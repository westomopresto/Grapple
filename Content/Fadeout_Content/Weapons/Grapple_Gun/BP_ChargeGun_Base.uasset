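; Base charge-and-release weapon in the Grapple Gun folder that launches a projectile whose speed scales with charge, with aim-down-sights on alt fire.
; A looping timer builds Charge while fire is held; release fires above a minimum charge, costing ammo and starting a cooldown, otherwise cancels.
; Server and multicast events sync effects, dummy-hook visibility and tool-swap locking, while a server event spawns the replicated projectile.
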(event `Charge Start Multicast`
  ;[1 1 1] Fire Press Multicast
  (`|ExecutionSequence`
    (:`then_0`
      (bind _asbp_player_character (cast `/Game/Fadeout_Content/Core/Characters/BP_PlayerCharacter` (`self.GetOwner`)))
      (`GameplayStatics.SpawnEmitterAttached` (`self.muzzleEmitter`) (`self.muzzleParticle`) "None" (0.0 0.0 0.0) (struct) (1.0 1.0 1.0) "SnapToTargetIncludingScale")
      (`self.PlayAltFireSound`))
    (:`then_1`
      (set `/Game/Fadeout_Content/Core/Characters/BP_PlayerCharacter.canSwapTools?` false _asbp_player_character))
    (:`then_2`
      (`self.HideHookToggle` true)
      (`self.Cloak Weapon` (`self.cloaked`)))))

(event `Charge Start Server`
  ;[1 1 1] Fire Press Multicast
  (`self.Charge Start Multicast`))

(event `Post Shot Server`
  (params (Fired :type Boolean))
  (`self.Post Shot Mg` Fired))

(event `Post Shot Mg`
  (params (Fired :type Boolean))
  ;[1 1 1] Shoot the hook
  (`|ExecutionSequence`
    (:`then_0`
      (`self.HideHookToggle` false))
    (:`then_1`
      (if Fired
        (`self.PlayFireSound`)))
    (:`then_2`
      (bind _asbp_player_character (cast `/Game/Fadeout_Content/Core/Characters/BP_PlayerCharacter` (`self.GetOwner`)))
      (set `/Game/Fadeout_Content/Core/Characters/BP_PlayerCharacter.canSwapTools?` true _asbp_player_character))))

(event `self.Spawn Projectile Server`
  (params (SpawnTransform :type "Transform Structure") (OwningWeapon :type "/Game/Fadeout_Content/Core/Weapons/BP_weaponBase Object Reference") (RayHitActor :type "Actor Object Reference") (`Initial Speed Override` :type "Float (single-precision)") (`Override Speed` :type Boolean))
  ;[1 1 1] only spawn 1 arrow on the server, let replication handle the rest
  (`self.Spawn Projectile` SpawnTransform OwningWeapon `Initial Speed Override` `Override Speed`)
  (`self.ForceNetUpdate`))

(event `Charge Check`
  (bind _charge (`self.charge`))
  ;[1 1 1] Charge Check Events
  (set `self.Is Charging` false)
  (if (>= _charge 5.0)
    (set `self.speedOverride` (`KismetMathLibrary.Lerp` 0.5 3.0 (/ (+ _charge 0.01) (`self.maxCharge`))))
    (`self.Fire Projectile Event` true)
    (`self.Post Shot Server` true)
    (set `self.charge` 0.0)
    (set `self.CanFire?` false)
    (`self.AmmoCostServer`)
    (`self.FireCoolDown`)
    (else
      (set `self.charge` 0.0)
      (set `self.CanFire?` true)
      (`self.Post Shot Server` false))))

(event `self.FireCoolDown_Finish`
  ;[1 1 1] Comment
  (`parent.FireCoolDown_Finish`)
  (set `self.CanFire?` true))

(event `self.OnFirePress`
  (set `self.charge` 0.0)
  (if (and (`self.CanFire?`) (not (`self.Is Charging`)))
    (`|ExecutionSequence`
      (:`then_0`
        (bind _asbp_player_character (cast `/Game/Fadeout_Content/Core/Characters/BP_PlayerCharacter` (`self.GetOwner`)))
        (set `self.playerCharacter` _asbp_player_character))
      (:`then_1`
        (bind _firecostmet (`self.AmmoCheckFunction`))
        ;[1 1 1] Check if we can fire
        (if (and (`self.CanFire?`) _firecostmet)
          ;[1 1 1] Animation replicate
          (`|ExecutionSequence`
            (:`then_0`
              (`/Engine/EditorBlueprintResources/ActorMacros.Switch Has Authority`
                (:`Authority`
                  (`self.Charge Start Multicast`))
                (:`Remote`
                  (`self.Charge Start Server`))))
            (:`then_1`
              (set `self.Is Charging` true)))
          (else
            (`self.PlayNoAmmoSound`)))))))

(event `Charge Ticking`
  ;[1 1 1] Event Tick
  (if (`self.onGround?`)
    _
    (elif (`self.Is Charging`)
      (set `self.charge` (`KismetMathLibrary.FClamp` (+ (`self.charge`) 1.0) 0.0 (`self.maxCharge`)))
      (else
        (set `self.charge` 0.0)))))

(event `self.OnFireRelease`
  (params (`charged?` :type Boolean))
  (`|ExecutionSequence`
    (:`then_0`
      (bind _asbp_player_character (cast `/Game/Fadeout_Content/Core/Characters/BP_PlayerCharacter` (`self.GetOwner`)))
      (set `self.playerCharacter` _asbp_player_character))
    (:`then_1`
      (bind _firecostmet (`self.AmmoCheckFunction`))
      (if (and (`self.CanFire?`) _firecostmet)
        (`self.Charge Check `)
        (else
          (`self.PlayNoAmmoSound`)
          (bind _asbp_player_character_2 (cast `/Game/Fadeout_Content/Core/Characters/BP_PlayerCharacter` (`self.GetOwner`)))
          (set `/Game/Fadeout_Content/Core/Characters/BP_PlayerCharacter.canSwapTools?` true _asbp_player_character_2))))))

(event `self.ReceiveBeginPlay`
  ;[1 1 1] Event Tick
  (`parent.ReceiveBeginPlay`)
  (`KismetSystemLibrary.K2_SetTimerDelegate` (delegate `Charge Ticking`) 0.05 true))

(event `self.OnAltFirePress`
  ;[1 1 1] Alt Fire
  (if (`self.canAltFire?`)
    (bind _asbp_player_character (cast `/Game/Fadeout_Content/Core/Characters/BP_PlayerCharacter` (`self.GetOwner`)))
    (set `/Game/Fadeout_Content/Core/Characters/BP_PlayerCharacter.Player_is_ADS` true _asbp_player_character)
    (`/Game/Fadeout_Content/Core/Characters/BP_PlayerCharacter.toAimCam` _asbp_player_character true false)))

(event `self.AltFireRelease`
  ;[1 1 1] Alt Fire
  (if (`self.canAltFire?`)
    (bind _asbp_player_character (cast `/Game/Fadeout_Content/Core/Characters/BP_PlayerCharacter` (`self.GetOwner`)))
    (set `/Game/Fadeout_Content/Core/Characters/BP_PlayerCharacter.Player_is_ADS` false _asbp_player_character)
    (`/Game/Fadeout_Content/Core/Characters/BP_PlayerCharacter.Equipment Camera Check` _asbp_player_character)
    (`/Game/Fadeout_Content/Core/Characters/BP_PlayerCharacter.ZoomCamera` _asbp_player_character false false)
    (`/Game/Fadeout_Content/Core/Characters/BP_PlayerCharacter.Global CD` _asbp_player_character)))

(fn `Cloak Weapon`
  (params (cloaked :type Boolean))
  (bind _hookdummy (`self.HookDummy`))
  (`parent.Cloak Weapon` cloaked)
  (`/Engine/EditorBlueprintResources/StandardMacros.IsValid` _hookdummy
    (:`Is Valid`
      (`SceneComponent.SetVisibility` _hookdummy (not cloaked) false))))

(fn `GetMuzzleLocation`
  (returns (MuzzleLocation :type "Vector Structure") (MuzzleTransform :type "Transform Structure"))
  (bind _skeletalmesh (`self.SkeletalMesh`))
  (bind _muzzlesocket (`self.MuzzleSocket`))
  (return (`SceneComponent.GetSocketLocation` _skeletalmesh _muzzlesocket) (`SceneComponent.GetSocketTransform` _skeletalmesh _muzzlesocket "RTS_World")))

(fn `HideHookToggle`
  (params (visibility :type Boolean :default true))
  (`SceneComponent.SetVisibility` (`self.HookDummy`) visibility false)
  (return))

(fn `UserConstructionScript`
  (`parent.UserConstructionScript`))