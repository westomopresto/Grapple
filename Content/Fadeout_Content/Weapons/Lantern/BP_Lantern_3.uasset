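; Lantern weapon that toggles a point light and particle effect on fire press, burning the owning player's FuelAmmo while lit.
; Tick deducts FireCost each second unless mounted on a post, and a value-change watcher on HasFuel shuts the light off when fuel runs out.
; Setup starts post and menu-level lanterns lit, others off, adding blocking collision for ground ones.
; Light changes replicate through authority-checked server and multicast events.
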(event `Oil Tick`
  (params (`Delta Time` :type "Float (double-precision)"))
  (if (not (`self.onPost?`))
    (set `self.tickFloat` (+ (`self.tickFloat`) `Delta Time`))
    (if (>= (`self.tickFloat`) 1.0)
      (`self.UpdateInstigatorWeaponInfo`)
      (set `self.tickFloat` 0.0)
      (bind _value (`self.GetAmmo`))
      (`self.SetAmmo` (- _value (`self.FireCost`)))
      (bind _value_2 (`self.GetAmmo`))
      (if (<= _value_2 0)
        (`self.SetAmmo` 0)))))

(event `self.Initialize`
  (bind _skeletalmesh (`self.SkeletalMesh`))
  (`parent.Initialize`)
  (if (`self.onGround?`) :!label _label
    (`self.manualShutOff`)
    (`|ExecutionSequence`
      (:`then_0`
        (`PrimitiveComponent.SetCollisionResponseToChannel` _skeletalmesh "ECC_WorldStatic" "ECR_Block"))
      (:`then_1`
        (`PrimitiveComponent.SetCollisionResponseToChannel` _skeletalmesh "ECC_WorldDynamic" "ECR_Block"))
      (:`then_2`
        (`PrimitiveComponent.SetCollisionResponseToChannel` _skeletalmesh "ECC_GameTraceChannel5" "ECR_Block")))
    (elif (`self.onPost?`)
      (`self.turnOn`)
      (`SceneComponent.SetMobility` (`self.PointLight1`) "Stationary")
      (else
        (`self.manualShutOff`)
        (bind _returnvalue (`GameplayStatics.GetCurrentLevelName` true))
        (if (`KismetStringLibrary.Contains` _returnvalue "menu")
          (`self.turnOn`))))))

(event `self.ReceiveBeginPlay`
  (bind _hasfuel (`self.hasFuel`))
  (`parent.ReceiveBeginPlay`)
  (bind (_old_value _new_value) (`/Game/Fadeout_Content/Core/MacroLibrary.Value Changed` _hasfuel _hasfuel :!label _label_2)
    (:`Setup Complete`
      (goto _label))
    (:`Value changed`
      (if (not _new_value)
        (`self.turnOff`)))))

(event `self.ReceiveTick`
  (params (DeltaSeconds :type "Float (single-precision)"))
  (if (`self.lanternOn?`)
    (`self.Oil Tick` DeltaSeconds))
  (bind _value (`self.GetAmmo`))
  (set `self.hasFuel` (> _value 0))
  (goto _label_2 :!via `Check Change`))

(event `self.OnFirePress`
  (`/Engine/EditorBlueprintResources/StandardMacros.FlipFlop`
    (:`A`
      (set `self.lanternOn?` true)
      (bind _value (`self.GetAmmo`))
      (if (> _value 0)
        (`self.turnOn`)))
    (:`B`
      (set `self.lanternOn?` false :!label _label_3)
      (`self.turnOff`))))

(event `turnOnMulticast`
  (`LightComponent.SetIntensity` (`self.PointLight1`) (`self.onIntensity`))
  (`ActorComponent.Activate` (`self.ParticleSystem`) false))

(event `manualShutOff`
  (goto _label_3))

(event `turnOn`
  (`/Engine/EditorBlueprintResources/ActorMacros.Switch Has Authority`
    (:`Authority`
      (`self.turnOnMulticast`))
    (:`Remote`
      (`self.turnOnServer`))))

(event `turnOnServer`
  (`self.turnOnMulticast`))

(event `turnOffMulticast`
  (`LightComponent.SetIntensity` (`self.PointLight1`) 0.0)
  (`ActorComponent.Deactivate` (`self.ParticleSystem`)))

(event `turnOffServer`
  (`self.turnOffMulticast`))

(event `turnOff`
  (`/Engine/EditorBlueprintResources/ActorMacros.Switch Has Authority`
    (:`Authority`
      (`self.turnOffMulticast`))
    (:`Remote`
      (`self.turnOffServer`))))

(fn `GetAmmo`
  (returns (Value :type Integer))
  (bind _asbp_player_character (cast `/Game/Fadeout_Content/Core/Characters/BP_PlayerCharacter` (`self.GetOwner`)))
  (`/Engine/EditorBlueprintResources/StandardMacros.IsValid` _asbp_player_character
    (:`Is Valid`
      (if true
        (return (`.FuelAmmo_6_F2355AB6418103DADF4DA58B81C677A6` (break `/Game/Fadeout_Content/Core/Support/AmmoStruct` (`/Game/Fadeout_Content/Core/Characters/BP_PlayerCharacter.HeldAmmo` _asbp_player_character))))
        (else
          _)))
    (:`Is Not Valid`
      _))
  (return 0))

(fn `SetAmmo`
  (params (Value :type Integer))
  (bind _asbp_player_character (cast `/Game/Fadeout_Content/Core/Characters/BP_PlayerCharacter` (`self.GetOwner`)))
  (bind (_tntammo _pistolammo) (break `/Game/Fadeout_Content/Core/Support/AmmoStruct` (`/Game/Fadeout_Content/Core/Characters/BP_PlayerCharacter.HeldAmmo` _asbp_player_character)))
  (set `/Game/Fadeout_Content/Core/Characters/BP_PlayerCharacter.HeldAmmo` (make `/Game/Fadeout_Content/Core/Support/AmmoStruct` _tntammo _pistolammo Value) _asbp_player_character)
  (return))

(fn `UserConstructionScript`)