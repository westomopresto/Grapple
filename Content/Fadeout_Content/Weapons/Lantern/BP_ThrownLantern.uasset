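; Thrown lantern weapon Blueprint that uses the owning player's fuel reserve as its ammo.
; GetAmmo casts the owner to BP_PlayerCharacter and returns FuelAmmo from its HeldAmmo struct, with a zero fallback for an invalid reference.
; SetAmmo writes the new fuel value by rebuilding that struct, carrying the TNT and pistol counts over unchanged.
; The file holds only these accessors, with no throw logic.
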(fn `GetAmmo`
  (returns (Value :type Integer))
  (bind _asbp_player_character (cast `/Game/Fadeout_Content/Core/Characters/BP_PlayerCharacter` (`self.GetOwner`)))
  (`/Engine/EditorBlueprintResources/StandardMacros.IsValid` _asbp_player_character
    (:`Is Valid`
      (if true
        (return (`.FuelAmmo_6_F2355AB6418103DADF4DA58B81C677A6` (break `/Game/Fadeout_Content/Core/Support/AmmoStruct` (`/Game/Fadeout_Content/Core/Characters/BP_PlayerCharacter.HeldAmmo` _asbp_player_character))))
        (else
          _)))
    (:`Is Not Valid`
      _))
  (return 0))

(fn `SetAmmo`
  (params (Value :type Integer))
  (bind _asbp_player_character (cast `/Game/Fadeout_Content/Core/Characters/BP_PlayerCharacter` (`self.GetOwner`)))
  (bind (_tntammo _pistolammo) (break `/Game/Fadeout_Content/Core/Support/AmmoStruct` (`/Game/Fadeout_Content/Core/Characters/BP_PlayerCharacter.HeldAmmo` _asbp_player_character)))
  (set `/Game/Fadeout_Content/Core/Characters/BP_PlayerCharacter.HeldAmmo` (make `/Game/Fadeout_Content/Core/Support/AmmoStruct` _tntammo _pistolammo Value) _asbp_player_character)
  (return))

(fn `UserConstructionScript`)