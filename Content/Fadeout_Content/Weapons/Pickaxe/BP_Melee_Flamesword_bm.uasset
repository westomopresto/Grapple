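; Flamesword melee weapon Blueprint whose hits can bat projectiles along the player's aim.
; Its MeleeDamageEvent override launches struck flame balls with a minimum upward lift, boosts their stored damage and calls DelayExplode.
; Other projectiles are deflected faster with negligible damage, and their instigator and controller pass to the attacker.
; Other targets take normal parent melee damage, and OnFirePress forwards to the parent fire logic.
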(event `/Game/Fadeout_Content/Core/Weapons/BP_MeleeBase.Melee Damage Event`
  (params (DamagedActor :type "Actor Object Reference") (BaseDamage :type "Float (single-precision)") (EventInstigator :type "Controller Object Reference") (DamageCauser :type "Actor Object Reference") (DamageTypeClass :type "DamageType Class Reference") (`Impact Normal` :type "Vector Structure") (`Impact Point` :type "Vector Structure") (AimDirection :type "Vector Structure"))
  (bind _returnvalue (`self.K2_GetActorLocation` (`self.PlayerOwner`)))
  (bind _returnvalue_2 (`KismetMathLibrary.GetDirectionUnitVector` _returnvalue (+ _returnvalue AimDirection)))
  (bind _asbp_projectile_flame_ball (cast `/Game/Fadeout_Content/Core/Weapons/BP_Projectile_Flame_Ball` DamagedActor)
    (:`then`
      (set `MovementComponent.Velocity` (* (`KismetMathLibrary.Normal` (`KismetMathLibrary.MakeVector` (.x _returnvalue_2) (.y _returnvalue_2) (`KismetMathLibrary.FMax` (.z _returnvalue_2) 0.35))) 2500.0) (`/Game/Fadeout_Content/Core/Weapons/BP_ProjectileBase.ProjectileMovement` _asbp_projectile_flame_ball))
      (`parent.Melee Damage Event` DamagedActor 15.0 EventInstigator DamageCauser DamageTypeClass `Impact Normal` `Impact Point` AimDirection)
      (set `/Game/Fadeout_Content/Core/Weapons/BP_Projectile_Flame_Ball.StoredDamage` (* (`/Game/Fadeout_Content/Core/Weapons/BP_Projectile_Flame_Ball.StoredDamage` _asbp_projectile_flame_ball) 1.25) _asbp_projectile_flame_ball)
      (`/Game/Fadeout_Content/Core/Weapons/BP_Projectile_Flame_Ball.DelayExplode` _asbp_projectile_flame_ball))
    (:`CastFailed`
      (bind _asbp_projectile_base (cast `/Game/Fadeout_Content/Core/Weapons/BP_ProjectileBase` DamagedActor)
        (:`then`
          (set `MovementComponent.Velocity` (* (`KismetMathLibrary.MakeVector` (.x _returnvalue_2) (.y _returnvalue_2) (.z _returnvalue_2)) 3500.0) (`/Game/Fadeout_Content/Core/Weapons/BP_ProjectileBase.ProjectileMovement` _asbp_projectile_base))
          (`parent.Melee Damage Event` DamagedActor 0.1 EventInstigator DamageCauser DamageTypeClass `Impact Normal` `Impact Point` AimDirection)
          (set `Actor.Instigator` (`self.PlayerOwner`) DamagedActor)
          (set `/Game/Fadeout_Content/Core/Weapons/BP_ProjectileBase.Instigator Controller` EventInstigator _asbp_projectile_base))
        (:`CastFailed`
          (`parent.Melee Damage Event` DamagedActor BaseDamage EventInstigator DamageCauser DamageTypeClass `Impact Normal` `Impact Point` AimDirection))))))

(event `self.OnFirePress`
  ;[1 1 1] actually important lol
  (`parent.OnFire`))

(fn `UserConstructionScript`
  (`parent.UserConstructionScript`))