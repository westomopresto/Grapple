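; Bear trap projectile that roots and bleeds a player character caught in it.
; Box overlaps and hits feed the parent's hit event; the authority-side trigger pulls the victim to center, disables movement for a set duration and applies a bleed DoT.
; A periodically refreshed light shows red or green by whether it would trigger on the local player.
; Expiry or qualifying damage cancels the trap, restoring movement and shrinking it away.
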(event `self.CollisionSphere.OnComponentBeginOverlap`
  (params (OverlappedComponent :type "PrimitiveComponent Object Reference") (OtherActor :type "Actor Object Reference") (OtherComp :type "PrimitiveComponent Object Reference") (OtherBodyIndex :type Integer) (bFromSweep :type Boolean) (SweepResult :type "HitResult Structure (by ref)")))

(event `self.Box.OnComponentBeginOverlap`
  (params (OverlappedComponent :type "PrimitiveComponent Object Reference") (OtherActor :type "Actor Object Reference") (OtherComp :type "PrimitiveComponent Object Reference") (OtherBodyIndex :type Integer) (bFromSweep :type Boolean) (SweepResult :type "HitResult Structure (by ref)"))
  (bind _asbp_player_character (cast `/Game/Fadeout_Content/Core/Characters/BP_PlayerCharacter` OtherActor))
  (if (not (== (`self.Instigator Controller`) (`Pawn.GetController` _asbp_player_character)))
    (`self.OnProjectileHitEvent` OtherActor OtherComp SweepResult)))

(event `self.CollisionSphere.OnComponentHit`
  (params (HitComponent :type "PrimitiveComponent Object Reference") (OtherActor :type "Actor Object Reference") (OtherComp :type "PrimitiveComponent Object Reference") (NormalImpulse :type "Vector Structure") (Hit :type "HitResult Structure (by ref)")))

(event `self.Box.OnComponentHit`
  (params (HitComponent :type "PrimitiveComponent Object Reference") (OtherActor :type "Actor Object Reference") (OtherComp :type "PrimitiveComponent Object Reference") (NormalImpulse :type "Vector Structure") (Hit :type "HitResult Structure (by ref)"))
  (`self.OnProjectileHitEvent` OtherActor OtherComp Hit))

(event `Friend Light`
  (bind _triggered (`self.Would Trigger` (`Controller.K2_GetPawn` (`GameplayStatics.GetPlayerController` 0))))
  (`LightComponent.SetLightColor` (`self.Light`) (`KismetMathLibrary.SelectColor` (struct :`R` 1.0 :`A` 1.0) (struct :`G` 1.0 :`A` 1.0) _triggered) true))

(event `self.ReceiveBeginPlay`
  (`parent.ReceiveBeginPlay`)
  (`self.Friend Light`))

(event `/Game/Fadeout_Content/Weapons/Projectiles/BP_TNT_Projectile.TimedTNT`
  (`parent.TimedTNT`))

(event `Triggered Server`
  (`self.Trap Target`))

(event `self.Triggered`
  (`/Engine/EditorBlueprintResources/ActorMacros.Switch Has Authority`
    (:`Authority`
      (`self.Triggered Server`))))

(event `Trap Target`
  (bind _other_actor (`self.Other Actor`))
  (if (not (`self.Trapped`))
    (`/Engine/EditorBlueprintResources/StandardMacros.IsValid` _other_actor
      (:`Is Valid`
        (bind _asbp_player_character (cast `/Game/Fadeout_Content/Core/Characters/BP_PlayerCharacter` _other_actor))
        (set `self.Trapped` true)
        (`self.Lerp To Center` _asbp_player_character (`self.K2_GetActorLocation` _asbp_player_character))
        (`KismetSystemLibrary.Delay` 0.1)
        (`self.Apply Dot to Trapped1` _asbp_player_character)
        (bind _charactermovement (`Character.CharacterMovement` _asbp_player_character))
        (`CharacterMovementComponent.DisableMovement` _charactermovement)
        (`GameplayStatics.SpawnSoundAtLocation` "/Game/Fadeout_Content/Core/FBX/Trap/278203__thepriest909__bear-trap.278203__thepriest909__bear-trap" (`self.K2_GetActorLocation`) (struct) 1.0 1.0 0.0 null null)
        (`SkeletalMeshComponent.PlayAnimation` (`self.Trap`) "/Game/Fadeout_Content/Core/FBX/Trap/TrapAnim.TrapAnim" false)
        (`KismetSystemLibrary.Delay` (`self.Trap Duration`))
        (`CharacterMovementComponent.SetMovementMode` _charactermovement "MOVE_Walking" 0)
        (`self.Cancel Trap`)))))

(event `Notify Bleed`
  (params (add :type Boolean) (BP_Player :type "/Game/Fadeout_Content/Core/Characters/BP_PlayerCharacter Object Reference"))
  (bind _asbp_char_wolf (cast `/Game/Fadeout_Content/Core/Characters/BP_Char_Wolf` (`self.GetOwner`)))
  (`/Game/Fadeout_Content/Core/Characters/BP_Char_Wolf.Find Bleeding Enemy` _asbp_char_wolf BP_Player add))

(event `Lerp To Center`
  (params (Target :type "Actor Object Reference") (`Start Loc` :type "Vector Structure"))
  (bind (_direction _alpha) (`Timeline|Timeline_0` :!via `PlayFromStart`)
    (:`Update`
      (`self.K2_SetActorLocation` Target (`KismetMathLibrary.VLerp` `Start Loc` (`SceneComponent.K2_GetComponentLocation` (`self.CharacterLocator`)) _alpha) false false))))

(event `self.ReceiveTick`
  (params (DeltaSeconds :type "Float (single-precision)"))
  (`parent.ReceiveTick` DeltaSeconds)
  (bind _output_get (set `self.Friend Tick` (+ DeltaSeconds (`self.Friend Tick`))))
  (if (>= _output_get 2.0)
    (`self.Friend Light`)
    (set `self.Friend Tick` 0.0)))

(event `self.ReceiveAnyDamage`
  (params (Damage :type "Float (single-precision)") (DamageType :type "DamageType Object Reference") (InstigatedBy :type "Controller Object Reference") (DamageCauser :type "Actor Object Reference"))
  (if (> Damage 500.0)
    (`self.Cancel Trap`)
    (else
      (bind _asdamage_type_base (cast `/Game/Fadeout_Content/Core/Weapons/DamageTypes/DamageType_Base` DamageType)
        (:`then`
          (bind _damagetypes (`/Game/Fadeout_Content/Core/Weapons/DamageTypes/DamageType_Base.DamageTypes` _asdamage_type_base))
          (if (or (`|EnumEquality` _damagetypes "NewEnumerator4") (`|EnumEquality` _damagetypes "NewEnumerator14") (`|EnumEquality` _damagetypes "NewEnumerator10") (`|EnumEquality` _damagetypes "NewEnumerator16"))
            (`self.Cancel Trap`)))
        (:`CastFailed`
          (`self.Cancel Trap`))))))

(event `Cancel Trap`
  (set `self.Trapped` true)
  (bind _asbp_player_character (cast `/Game/Fadeout_Content/Core/Characters/BP_PlayerCharacter` (`self.Other Actor`))
    (:`then`
      (`CharacterMovementComponent.SetMovementMode` (`Character.CharacterMovement` _asbp_player_character) "MOVE_Walking" 0)
      (bind (_direction _alpha) (`Timeline|Scale Timeline` :!via `PlayFromStart` :!label _label)
        (:`Update`
          (`self.SetActorScale3D` (`KismetMathLibrary.VLerp` (1.0 1.0 1.0) (0.0 0.0 0.0) _alpha)))
        (:`Finished`
          (`self.K2_DestroyActor`))))
    (:`CastFailed`
      (goto _label :!via `PlayFromStart`))))

(fn `Apply Dot to Trapped1`
  (params (`BP Player Character` :type "/Game/Fadeout_Content/Core/Characters/BP_PlayerCharacter Object Reference"))
  (`/Engine/EditorBlueprintResources/ActorMacros.Switch Has Authority`
    (:`Authority`
      (`/Game/Fadeout_Content/Core/Characters/BP_PlayerCharacter.Attach DoT ` `BP Player Character` "/Game/Fadeout_Content/Core/Weapons/BP_Bleed_DOT.BP_Bleed_DOT_C" (`self.GetInstigator`))
      (return))
    (:`Remote`
      (return))))

(fn `UserConstructionScript`
  (`parent.UserConstructionScript`))