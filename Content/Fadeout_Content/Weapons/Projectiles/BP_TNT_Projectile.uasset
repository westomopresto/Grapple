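; Thrown TNT projectile that explodes shortly after taking any damage, either timed or tracked in the player's owned-projectile list.
; Timed charges run a beeping, blinking timeline that damages itself on finish; untimed ones remove themselves from the owner's list when detonated.
; Explosion applies full radial damage, plays effects, and uses a sphere trace to launch characters and physics-simulating TNT outward.
; Projectile movement hands over to physics simulation on first bounce or stop.
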(event `self.ReceiveAnyDamage`
  (params (Damage :type "Float (single-precision)") (DamageType :type "DamageType Object Reference") (InstigatedBy :type "Controller Object Reference") (DamageCauser :type "Actor Object Reference"))
  (bind _returnvalue (`self.K2_GetActorLocation`))
  (bind _pointlight (`self.PointLight`))
  (`KismetSystemLibrary.PrintString` (`KismetSystemLibrary.GetDisplayName` InstigatedBy))
  (set `self.Instigator` (`self.GetInstigator` DamageCauser))
  (`KismetSystemLibrary.Delay` 0.2)
  (`self.Explode`)
  (`GameplayStatics.SpawnEmitterAtLocation` "/Game/StarterContent/Particles/P_Explosion.P_Explosion" _returnvalue (struct) (2.0 2.0 2.0))
  (`LightComponentBase.SetCastShadows` _pointlight true)
  (`LightComponent.SetIntensity` _pointlight 8400.0)
  (`GameplayStatics.PlaySoundAtLocation` "/Game/Fadeout_Content/Core/Audio/Explosions/Explosion_5_W_Rubble_3.Explosion_5_W_Rubble_3" _returnvalue (struct) 1.25 (`KismetMathLibrary.RandomFloatInRange` 0.9 1.1) 0.0 "/Game/Fadeout_Content/Core/Characters/Footstep_Attenuation.Footstep_Attenuation" null null)
  (if (not (`self.timed`))
    (bind _asbp_player_character (cast `/Game/Fadeout_Content/Core/Characters/BP_PlayerCharacter` (`self.GetInstigator`)))
    (`KismetArrayLibrary.Array_RemoveItem` (`/Game/Fadeout_Content/Core/Characters/BP_PlayerCharacter.myOwnedProjectiles` _asbp_player_character) self))
  (`self.K2_DestroyActor`))

(event `self.ReceiveBeginPlay`
  (bind _returnvalue (`self.K2_GetActorLocation`))
  (bind _beeplight (`self.beepLight`))
  (if (`self.timed`)
    (`GameplayStatics.PlaySoundAtLocation` "/Game/Fadeout_Content/Core/Audio/Explosions/Tick_2.Tick_2" _returnvalue (struct) 1.0 1.0 0.0 "/Game/Fadeout_Content/Core/Props/Elevator_Attenuation.Elevator_Attenuation" null null)
    (`Timeline|timedExplode` :!via `PlayFromStart` :!label _label
      (:`Finished`
        (`GameplayStatics.ApplyDamage` self 1.0 (`Pawn.GetController` (`self.GetInstigator`)) self)
        (`LightComponent.SetLightColor` _beeplight (struct :`R` 1.0 :`A` 1.0) true))
      (:`beeps`
        (`LightComponent.SetLightColor` _beeplight (struct :`G` 1.0 :`B` 0.150592 :`A` 1.0) true)
        (`GameplayStatics.PlaySoundAtLocation` "/Game/Fadeout_Content/Core/Audio/Elevator/beep.beep" _returnvalue (struct) 1.0 1.0 0.0 null null null)
        (`KismetSystemLibrary.Delay` 0.1)
        (`LightComponent.SetLightColor` _beeplight (struct :`A` 1.0) true)))))

(event `interruptTimer`
  (goto _label :!via `Stop`))

(event `Explode`
  (bind _returnvalue (`self.K2_GetActorLocation`))
  (`self.RadialDamage`)
  (bind _outhits (`KismetSystemLibrary.SphereTraceMultiForObjects` :`Start` _returnvalue :`End` (+ _returnvalue (0.0 0.0 1.0)) :`Radius` 200.0 :`ObjectTypes` (`|MakeArray` "ObjectTypeQuery3" "ObjectTypeQuery7" :!type "EObjectTypeQuery Enum") :`bTraceComplex` true :`DrawTime` 1.0))
  (for _array_element _outhits
    (bind (_bblockinghit _binitialoverlap _time _distance _location _impactpoint _normal _impactnormal _physmat _hitactor) (`GameplayStatics.BreakHitResult` _array_element))
    (bind _ascharacter (cast `Character` _hitactor)
      (:`then`
        (`Character.LaunchCharacter` _ascharacter (* (`KismetMathLibrary.GetDirectionUnitVector` _returnvalue (`self.K2_GetActorLocation` _ascharacter)) 1200.0) false false))
      (:`CastFailed`
        (bind _asbp_tnt_projectile (cast `/Game/Fadeout_Content/Weapons/Projectiles/BP_TNT_Projectile` _hitactor))
        (bind _staticmesh (`/Game/Fadeout_Content/Weapons/Projectiles/BP_TNT_Projectile.StaticMesh` _asbp_tnt_projectile))
        (if (`SceneComponent.IsSimulatingPhysics` _staticmesh "None")
          (`PrimitiveComponent.AddImpulse` _staticmesh (* (`KismetMathLibrary.GetDirectionUnitVector` _returnvalue (`self.K2_GetActorLocation` _asbp_tnt_projectile)) 1200.0) "None" true)
          (`KismetSystemLibrary.PrintString` "IMPULSE"))))))

(event `self.ReceiveHit`
  (params (MyComp :type "PrimitiveComponent Object Reference") (Other :type "Actor Object Reference") (OtherComp :type "PrimitiveComponent Object Reference") (bSelfMoved :type Boolean) (HitLocation :type "Vector Structure") (HitNormal :type "Vector Structure") (NormalImpulse :type "Vector Structure") (Hit :type "HitResult Structure (by ref)")))

(event `self.ProjectileMovement1.OnProjectileStop`
  (params (ImpactResult :type "HitResult Structure (by ref)"))
  (`PrimitiveComponent.SetSimulatePhysics` (`self.StaticMesh`) true :!label _label_2))

(event `stopBouncing`
  (goto _label_2))

(event `self.ProjectileMovement1.OnProjectileBounce`
  (params (ImpactResult :type "HitResult Structure (by ref)") (ImpactVelocity :type "Vector Structure (by ref)"))
  (bind (_bblockinghit _binitialoverlap _time _distance _location _impactpoint) (`GameplayStatics.BreakHitResult` ImpactResult))
  (`KismetSystemLibrary.PrintString` "BOUNCED")
  (`GameplayStatics.PlaySoundAtLocation` "/Game/Fadeout_Content/Core/Audio/residue-sfx/emptyclip.emptyclip" _impactpoint (struct) 1.0 (`KismetMathLibrary.RandomFloatInRange` 0.9 1.1) 0.0 "/Game/Fadeout_Content/Core/Characters/Footstep_Attenuation.Footstep_Attenuation" null null)
  (`GameplayStatics.SpawnEmitterAtLocation` "/Game/Fadeout_Content/Core/FX/particle_footSmoke.particle_footSmoke" _impactpoint)
  (`self.stopBouncing`))

(fn `RadialDamage`
  (`GameplayStatics.ApplyRadialDamage` :`BaseDamage` (`self.Damage`) :`Origin` (`self.K2_GetActorLocation`) :`DamageRadius` 400.0 :`DamageTypeClass` "/Game/Fadeout_Content/Core/Weapons/DamageTypes/DT_TNT.DT_TNT_C" :`DamageCauser` self :`InstigatedByController` (`Pawn.GetController` (`self.GetInstigator`)) :`bDoFullDamage` true))

(fn `UserConstructionScript`)