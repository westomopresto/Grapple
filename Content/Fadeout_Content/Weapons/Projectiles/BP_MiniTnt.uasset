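; BP_MiniTnt is a mini TNT projectile Blueprint that builds on a parent class for its detonation behavior.
; After BeginPlay it waits on a fixed delay, then calls TimedTNT if PlantedGround is still false.
; Its Detonate event only forwards to the parent implementation.
; The construction script sets the mesh as the projectile movement's interpolated component, allowing smoothed visual motion.
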(event `self.Detonate`
  ;[1 1 1] Disable Detonation
  (`parent.Detonate`))

(event `self.ReceiveBeginPlay`
  (`parent.ReceiveBeginPlay`)
  (`KismetSystemLibrary.Delay` 20.0)
  (if (not (`self.planted_Ground`))
    (`self.TimedTNT`)))

(fn `UserConstructionScript`
  (`parent.UserConstructionScript`)
  (`ProjectileMovementComponent.SetInterpolatedComponent` (`self.ProjectileMovement`) (`self.Mesh`)))