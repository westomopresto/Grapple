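; Poison proximity TNT projectile, a child Blueprint that, once planted in the ground, is set off by players entering its Range component.
; WouldTrigger filters overlaps by comparing PlayerState teams and IDs against the Instigator, so only enemies, or anyone but the owner in FFA, qualify.
; Triggered applies pick-type damage to the TNT itself, leaving detonation and any poison effect to logic outside this Blueprint.
; The tnt_m_color override is empty, with its parent call disconnected.
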(event `self.Range.OnComponentBeginOverlap`
  (params (OverlappedComponent :type "PrimitiveComponent Object Reference") (OtherActor :type "Actor Object Reference") (OtherComp :type "PrimitiveComponent Object Reference") (OtherBodyIndex :type Integer) (bFromSweep :type Boolean) (SweepResult :type "HitResult Structure (by ref)"))
  (if (`self.planted_Ground`)
    (bind _triggered (`self.Would Trigger` OtherActor))
    (if _triggered
      (set `self.Other Actor` OtherActor)
      (`self.Triggered`))))

(event `Triggered`
  (bind _instigator (`self.Instigator`))
  (`GameplayStatics.ApplyDamage` self 50.0 (`self.GetInstigatorController` _instigator) _instigator "/Game/Fadeout_Content/Core/Weapons/DamageTypes/DT_Pick.DT_Pick_C"))

(fn `tnt_m_color`
  (params (Value :type "LinearColor Structure") (SourceMaterial :type "MaterialInterface Object Reference")))

(fn `UserConstructionScript`
  (`parent.UserConstructionScript`))

(fn `Would Trigger`
  (params (Object :type "Object Object Reference"))
  (returns (Triggered :type Boolean))
  (bind _playerstate (`Pawn.PlayerState` (`self.Instigator`)))
  (`/Engine/EditorBlueprintResources/StandardMacros.IsValid` (`self.Instigator`)
    (:`Is Valid`
      (bind _asbp_player_character (cast `/Game/Fadeout_Content/Core/Characters/BP_PlayerCharacter` Object))
      (bind _playerstate_2 (`Pawn.PlayerState` _asbp_player_character))
      (bind _asfo_player_state (cast `/Game/Fadeout_Content/Core/Support/Multiplayer_Support/FO_PlayerState` _playerstate_2)
        (:`then`
          (bind _asfo_player_state_2 (cast `/Game/Fadeout_Content/Core/Support/Multiplayer_Support/FO_PlayerState` _playerstate))
          (bind _team (`/Game/Fadeout_Content/Core/Support/Multiplayer_Support/FO_PlayerState.Team` _asfo_player_state))
          (if (`KismetStringLibrary.NotEqual_StrStr` _team "FFA")
            (bind _returnvalue (!= (`PlayerState.PlayerId` _playerstate_2) (`PlayerState.PlayerId` _playerstate)))
            (if (and (not (`KismetStringLibrary.EqualEqual_StrStr` _team (`/Game/Fadeout_Content/Core/Support/Multiplayer_Support/FO_PlayerState.Team` _asfo_player_state_2))) _returnvalue)
              _
              (else
                (bind _output_get (set `self.Triggerable` false :!label _label))
                (return _output_get)))
            (else
              ;[1 1 1] FFA
              (if _returnvalue
                _
                (else
                  (goto _label)))))
          (bind _output_get_2 (set `self.Triggerable` true))
          (return _output_get_2))
        (:`CastFailed`
          (return true))))
    (:`Is Not Valid`
      (return (`self.Triggerable`)))))