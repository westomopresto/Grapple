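; Explosive barrel that detonates when it takes any damage, crediting the damage instigator's pawn for the blast.
; After a short random delay it spawns explosion FX and sound, applies full radial TNT damage, then destroys itself.
; A smaller multi-sphere trace launches characters, reports damage events and triggers the player's AirSpin.
; The same hits pass through ApplyImpulse, which pushes movable, physics-simulating static and skeletal meshes.
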(event `self.ReceiveBeginPlay`)

(event `Detonate`
  (`KismetSystemLibrary.Delay` (`KismetMathLibrary.RandomFloatInRange` 0.1 0.3))
  (`self.Explode`))

(event `self.ReceiveAnyDamage`
  (params (Damage :type "Float (single-precision)") (DamageType :type "DamageType Object Reference") (InstigatedBy :type "Controller Object Reference") (DamageCauser :type "Actor Object Reference"))
  (`/Engine/EditorBlueprintResources/StandardMacros.IsValid` InstigatedBy
    (:`Is Valid`
      (set `self.Instigator` (`Controller.K2_GetPawn` InstigatedBy)))
    (:`Is Not Valid`
      _))
  (`self.Detonate`))

(event `Explode`
  (bind _returnvalue (`self.K2_GetActorLocation`))
  (`GameplayStatics.SpawnEmitterAtLocation` "/Game/Explosions/Particles/P_ImpactExplosion4.P_ImpactExplosion4" (`SceneComponent.K2_GetComponentLocation` (`self.explosionLoc`)) (struct) (0.7 0.7 0.7))
  (`GameplayStatics.PlaySoundAtLocation` "/Game/Fadeout_Content/Core/Audio/Explosions/Explosion_5_W_Rubble_3.Explosion_5_W_Rubble_3" (`self.K2_GetActorLocation`) (struct) 1.25 (`KismetMathLibrary.RandomFloatInRange` 0.9 1.1) 0.0 "/Game/Fadeout_Content/Core/Characters/Footstep_Attenuation.Footstep_Attenuation" null null)
  (`self.RadialDamage`)
  (bind (_outhits _returnvalue_2) (`KismetSystemLibrary.SphereTraceMultiForObjects` :`Start` _returnvalue :`End` (+ _returnvalue (0.0 0.0 1.0)) :`Radius` 400.0 :`ObjectTypes` (`|MakeArray` "ObjectTypeQuery3" "ObjectTypeQuery7" "ObjectTypeQuery2" "ObjectTypeQuery4" :!type "EObjectTypeQuery Enum") :`bTraceComplex` true :`DrawTime` 1.0))
  (if _returnvalue_2
    (for _array_element _outhits
      (`|ExecutionSequence`
        (:`then_0`
          (bind (_bblockinghit _binitialoverlap _time _distance _location _impactpoint _normal _impactnormal _physmat _hitactor _hitcomponent) (`GameplayStatics.BreakHitResult` _array_element))
          (bind _ascharacter (cast `Character` _hitactor))
          (bind _returnvalue_3 (* _impactnormal -1200.0))
          (`Character.LaunchCharacter` _ascharacter _returnvalue_3 false true)
          (`AISense_Damage.ReportDamageEvent` _hitactor (`self.GetInstigator`) (`self.Damage`) _location)
          (bind _asbp_player_character (cast `/Game/Fadeout_Content/Core/Characters/BP_PlayerCharacter` _ascharacter))
          (`/Game/Fadeout_Content/Core/Characters/BP_PlayerCharacter.air_Spin` _asbp_player_character))
        (:`then_1`
          (`self.applyImpulse` _hitcomponent _returnvalue_3)))))
  (`KismetSystemLibrary.Delay` 0.05)
  (`self.K2_DestroyActor`))

(fn `applyImpulse`
  (params (Object :type "PrimitiveComponent Object Reference") (InputPin :type "Vector Structure"))
  (bind _asstatic_mesh_component (cast `StaticMeshComponent` Object)
    (:`then`
      (if (and (`SceneComponent.IsSimulatingPhysics` _asstatic_mesh_component "None") (`|EnumEquality` (`SceneComponent.Mobility` _asstatic_mesh_component) "Movable"))
        (`PrimitiveComponent.AddImpulse` _asstatic_mesh_component InputPin "None" true)))
    (:`CastFailed`
      (bind _asskeletal_mesh_component (cast `SkeletalMeshComponent` Object))
      (if (and (`SceneComponent.IsSimulatingPhysics` _asskeletal_mesh_component "None") (`|EnumEquality` (`SceneComponent.Mobility` _asskeletal_mesh_component) "Movable"))
        (`PrimitiveComponent.AddImpulse` _asskeletal_mesh_component InputPin "None" true)))))

(fn `RadialDamage`
  (`GameplayStatics.ApplyRadialDamage` :`BaseDamage` (`self.Damage`) :`Origin` (`self.K2_GetActorLocation`) :`DamageRadius` 800.0 :`DamageTypeClass` "/Game/Fadeout_Content/Core/Weapons/DamageTypes/DT_TNT.DT_TNT_C" :`DamageCauser` self :`InstigatedByController` (`Pawn.GetController` (`self.Instigator`)) :`bDoFullDamage` true)
  (return))

(fn `UserConstructionScript`)