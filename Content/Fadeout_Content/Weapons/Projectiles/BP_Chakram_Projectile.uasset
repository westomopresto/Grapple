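; Chakram projectile that flies out, damages other players and homes back to the throwing player like a boomerang.
; After a brief plane-constrained flight toward its initial target, it switches homing to the owner, then releases the constraint.
; Each bounce doubles homing acceleration, and repeated bounces leave it only overlapping pawns so it passes through obstacles.
; An owner impact or looping proximity check notifies the chakram weapon of the return and destroys the projectile.
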(event `self.ProjectileMovement.OnProjectileBounce`
  (params (ImpactResult :type "HitResult Structure (by ref)") (ImpactVelocity :type "Vector Structure (by ref)"))
  (bind _collisionsphere (`self.CollisionSphere`))
  (bind _projectilemovement (`self.ProjectileMovement`))
  (set `ProjectileMovementComponent.HomingAccelerationMagnitude` (* (`ProjectileMovementComponent.HomingAccelerationMagnitude` _projectilemovement) 2.0) _projectilemovement)
  (`self.PlayImpactEffects` ImpactResult true)
  (bind _result (`/Engine/EditorBlueprintResources/StandardMacros.IncrementInt` (`self.bounces`))
    (:`  `
      (if (>= _result 2)
        (`PrimitiveComponent.SetCollisionResponseToAllChannels` _collisionsphere "ECR_Ignore")
        (`PrimitiveComponent.SetCollisionResponseToChannel` _collisionsphere "ECC_Pawn" "ECR_Overlap")))))

(event `self.ReceiveBeginPlay`
  (`|ExecutionSequence`
    (:`then_0`
      (`PrimitiveComponent.IgnoreActorWhenMoving` (`self.CollisionSphere`) (`self.GetOwner`) true)
      (set `self.Instigator Controller` (`self.GetInstigatorController`))
      (`KismetSystemLibrary.Delay` 0.1)
      (set `self.canhurtOwner` true))
    (:`then_1`
      (set `ProjectileMovementComponent.HomingTargetComponent` (`self.HomingTarget`) (`self.ProjectileMovement`))
      (`MovementComponent.SetPlaneConstraintNormal` (`self.ProjectileMovement`) (`SceneComponent.GetUpVector` (`self.Mesh`)))
      (`KismetSystemLibrary.Delay` 0.2)
      (bind _output_get (set `self.HomingTarget` (`Actor.RootComponent` (`self.GetOwner` (`self.OwningWeapon_NET`)))))
      (set `ProjectileMovementComponent.HomingTargetComponent` _output_get (`self.ProjectileMovement`))
      (set `ProjectileMovementComponent.HomingAccelerationMagnitude` 50000.0 (`self.ProjectileMovement`))
      (`KismetSystemLibrary.Delay` 0.2)
      (`MovementComponent.SetPlaneConstraintEnabled` (`self.ProjectileMovement`) false))
    (:`then_2`
      ;[1 1 1] Reset chakram when we're near our owner
      (`KismetSystemLibrary.K2_SetTimerDelegate` (delegate `EndCheck`) 0.05 true))))

(event `EndCheck`
  ;[1 1 1] Reset chakram when we're near our owner
  (`self.ResetChakramCD`))

(event `self.OnProjectileHitEvent`
  (params (OtherActor :type "Actor Object Reference") (OtherComponent :type "PrimitiveComponent Object Reference") (HitResult :type "HitResult Structure (by ref)"))
  (`KismetSystemLibrary.PrintString` (`KismetSystemLibrary.GetDisplayName` OtherActor))
  (bind _asbp_player_character (cast `/Game/Fadeout_Content/Core/Characters/BP_PlayerCharacter` OtherActor))
  (if (not (== _asbp_player_character (`self.GetOwner` (`self.OwningWeapon_NET`))))
    (`parent.OnProjectileHitEvent` OtherActor OtherComponent HitResult)))

(event `self.SurfaceImpactEvent`
  (params (HitResult :type "HitResult Structure") (`Hardsurface?` :type Boolean) (hitactor :type "Actor Object Reference"))
  (bind _asbp_player_character (cast `/Game/Fadeout_Content/Core/Characters/BP_PlayerCharacter` hitactor)
    (:`then`
      (if (== _asbp_player_character (`self.GetOwner` (`self.OwningWeapon_NET`)))
        (bind _asbp_chakram_weapon (cast `/Game/Fadeout_Content/Core/Weapons/BP_Chakram_Weapon` (`self.OwningWeapon_NET`)))
        (`/Game/Fadeout_Content/Core/Weapons/BP_Chakram_Weapon.Chakram Returned` _asbp_chakram_weapon)
        (`self.K2_DestroyActor`)))
    (:`CastFailed`
      (`parent.SurfaceImpactEvent` HitResult `Hardsurface?` hitactor))))

(fn `ResetChakramCD`
  (if (and (<= (`KismetMathLibrary.Vector_Distance` (`self.K2_GetActorLocation` (`self.GetOwner` (`self.OwningWeapon_NET`))) (`self.K2_GetActorLocation`)) 75.0) (`self.canhurtOwner`))
    (bind _asbp_chakram_weapon (cast `/Game/Fadeout_Content/Core/Weapons/BP_Chakram_Weapon` (`self.OwningWeapon_NET`)))
    (`/Game/Fadeout_Content/Core/Weapons/BP_Chakram_Weapon.Chakram Returned` _asbp_chakram_weapon)
    (`self.K2_DestroyActor`)))

(fn `UserConstructionScript`
  (`parent.UserConstructionScript`))