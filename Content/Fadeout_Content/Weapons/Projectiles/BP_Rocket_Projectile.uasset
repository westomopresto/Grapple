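; Rocket projectile Blueprint that deals damage and explodes on impact, with optional acceleration and a detachable trail.
; On BeginPlay it ignores its owner, can spawn and attach a separate trail actor, and can run a timeline that multiplies velocity each update.
; Hits kill the trail, then the server applies damage and explodes once while clients destroy their copy.
; Taking damage also kills the trail before passing to parent logic.
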(event `self.ReceiveBeginPlay`
  (bind _projectilemovement (`self.ProjectileMovement`))
  (`PrimitiveComponent.IgnoreActorWhenMoving` (`self.CollisionSphere`) (`self.GetOwner`) true)
  (`parent.ReceiveBeginPlay`)
  (if (`self.detachTrail`)
    (bind _returnvalue (`|SpawnActorFromClass` "/Game/Fadeout_Content/Weapons/Detach_Trail.Detach_Trail_C" (`SceneComponent.K2_GetComponentToWorld` (`self.trail`)) "AlwaysSpawn" "OverrideRootScale" null null))
    (bind _output_get (set `self.RocketTrail` _returnvalue))
    (`self.K2_AttachToActor` _returnvalue self "None" "KeepWorld" "KeepWorld" "KeepWorld" true)
    (`self.K2_AttachToActor` _output_get self "None" "KeepWorld" "KeepWorld" "KeepWorld" true))
  (if (`self.accelerate`)
    (`Timeline|Timeline_0` :!via `PlayFromStart`
      (:`Update`
        (set `MovementComponent.Velocity` (* (`MovementComponent.Velocity` _projectilemovement) 1.3) _projectilemovement)))))

(event `Multicast Kill Trail`
  (bind _rockettrail (`self.RocketTrail`))
  (`/Engine/EditorBlueprintResources/StandardMacros.IsValid` _rockettrail
    (:`Is Valid`
      (`/Game/Fadeout_Content/Weapons/Detach_Trail.Kill` _rockettrail))))

(event `self.OnProjectileHitEvent`
  (params (OtherActor :type "Actor Object Reference") (OtherComponent :type "PrimitiveComponent Object Reference") (HitResult :type "HitResult Structure (by ref)") (fromHit :type Boolean))
  (bind _rockettrail (`self.RocketTrail`))
  (`/Engine/EditorBlueprintResources/StandardMacros.IsValid` _rockettrail
    (:`Is Valid`
      (`/Game/Fadeout_Content/Weapons/Detach_Trail.Kill` _rockettrail))
    (:`Is Not Valid`
      _))
  (`/Engine/EditorBlueprintResources/ActorMacros.Switch Has Authority`
    (:`Authority`
      (`/Engine/EditorBlueprintResources/StandardMacros.DoOnce` false
        (:`Completed`
          (`GameplayStatics.ApplyDamage` OtherActor (`self.Damage`) (`self.Instigator Controller`) self (`self.DamageType`))
          (`self.Explode`))))
    (:`Remote`
      (`self.K2_DestroyActor`))))

(event `self.ReceiveAnyDamage`
  (params (Damage :type "Float (single-precision)") (DamageType :type "DamageType Object Reference") (InstigatedBy :type "Controller Object Reference") (DamageCauser :type "Actor Object Reference"))
  (`self.Multicast Kill Trail`)
  (`parent.ReceiveAnyDamage` Damage DamageType InstigatedBy DamageCauser))

(fn `tnt_m_color`
  (params (Value :type "LinearColor Structure") (SourceMaterial :type "MaterialInterface Object Reference")))

(fn `UserConstructionScript`
  (`parent.UserConstructionScript`))