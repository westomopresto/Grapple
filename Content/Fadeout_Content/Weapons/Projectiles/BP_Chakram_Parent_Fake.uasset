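; BP_Chakram_Parent_Fake is a short-lived stand-in projectile that splits into two BP_Chakram_Projectile actors.
; On BeginPlay, the authority spawns one chakram at each of its two arrow components, passing along owner, instigator and owning weapon.
; Both chakrams receive the same target point, far along the parent's forward vector.
; The authority copy destroys itself after a brief delay, while remote copies destroy themselves immediately.
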(event `self.ReceiveBeginPlay`
  (bind _returnvalue (+ (.location (`self.GetTransform`)) (* (`KismetMathLibrary.GetForwardVector` (.rotation (`self.GetTransform`))) 4000.0)))
  (`parent.ReceiveBeginPlay`)
  (`/Engine/EditorBlueprintResources/ActorMacros.Switch Has Authority`
    (:`Authority`
      (`self.Spawn Chakram` (`SceneComponent.K2_GetComponentToWorld` (`self.Arrow1`)) _returnvalue)
      (`self.Spawn Chakram` (`SceneComponent.K2_GetComponentToWorld` (`self.Arrow`)) _returnvalue)
      (`KismetSystemLibrary.Delay` 0.05)
      (`self.K2_DestroyActor`))
    (:`Remote`
      (`self.K2_DestroyActor`))))

(fn `Spawn Chakram`
  (params (SpawnTransform :type "Transform Structure") (DummyLOC :type "Vector Structure"))
  (bind _owningweapon (`self.OwningWeapon`))
  (`|SpawnActorFromClass` "/Game/Fadeout_Content/Weapons/Projectiles/BP_Chakram_Projectile.BP_Chakram_Projectile_C" SpawnTransform "Undefined" "OverrideRootScale" (`self.GetOwner`) _owningweapon DummyLOC _owningweapon 1.0 false (`self.Instigator`)))

(fn `UserConstructionScript`
  (`parent.UserConstructionScript`))