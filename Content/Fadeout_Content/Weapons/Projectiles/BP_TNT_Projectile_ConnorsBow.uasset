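; TNT projectile for Connor's bow that sticks to player characters it hits, is destroyed on other hits, and explodes on a timer or when damaged.
; A beeping, color-flashing timeline starts at spawn or after DeathTime, then self-damages to trigger detonation through AnyDamage.
; The explosion sphere-traces for physics impulses, once-per-actor damage with optional distance falloff, and character knockback.
; An owner wearing the Jester Camille outfit swaps the mesh.
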(event `Detonate`
  (set `self.death` true)
  (`KismetSystemLibrary.Delay` (`KismetMathLibrary.RandomFloatInRange` 0.05 0.1))
  (`self.Explode`))

(event `self.ReceiveAnyDamage`
  (params (Damage :type "Float (single-precision)") (DamageType :type "DamageType Object Reference") (InstigatedBy :type "Controller Object Reference") (DamageCauser :type "Actor Object Reference"))
  (if (>= Damage 1.0)
    (if (`self.death`)
      (`KismetSystemLibrary.Delay` 3.0)
      (`self.K2_DestroyActor`)
      (else
        (`/Engine/EditorBlueprintResources/StandardMacros.IsValid` InstigatedBy
          (:`Is Valid`
            (set `self.Instigator` (`Controller.K2_GetPawn` InstigatedBy)))
          (:`Is Not Valid`
            _))
        (`self.Detonate`)))))

(event `Attach`
  (params (NewTransform :type "Transform Structure (by ref)") (ParentActor :type "Actor Object Reference"))
  ;[1 1 1] Attachment
  (`self.K2_SetActorRotation` (.rotation NewTransform) true)
  (`self.K2_AddActorLocalOffset` (0.0 0.0 -15.0) false true)
  (`self.K2_AttachToActor` ParentActor "None" "KeepWorld" "KeepWorld" "KeepWorld")
  (`self.ForceNetUpdate`)
  (set `self.NetUpdateFrequency` 2.0))

(event `TimedTNT`
  (`GameplayStatics.SpawnSoundAttached` "/Game/Fadeout_Content/Core/Audio/Connors/flak_beeps_connors.flak_beeps_connors" (`self.CollisionSphere`) "None" (0.0 0.0 0.0) (struct) "SnapToTarget" true 1.0 1.0 0.0 "/Game/Fadeout_Content/Core/Characters/GunshotAttenuation.GunshotAttenuation" null)
  (`Timeline|timedExplode` :!via `PlayFromStart` :!label _label
    (:`Finished`
      (`GameplayStatics.ApplyDamage` self 999.0 (`Pawn.GetController` (`self.GetInstigator`)) self "/Game/Fadeout_Content/Core/Weapons/DamageTypes/DT_TNT.DT_TNT_C")
      (`self.tnt_m_color` (struct :`R` 1.0 :`A` 1.0) (`PrimitiveComponent.GetMaterial` (`self.Mesh`) 0)))
    (:`beeps`
      (`self.tnt_m_color` (struct :`G` 1.0 :`B` 0.14996 :`A` 1.0) (`PrimitiveComponent.GetMaterial` (`self.Mesh`) 0))
      (`GameplayStatics.SpawnSoundAttached` "/Game/Fadeout_Content/Core/Audio/short_beep.short_beep" (`self.CollisionSphere`) "None" (0.0 0.0 0.0) (struct) "SnapToTarget" true 1.0 1.0 0.0 "/Game/Fadeout_Content/Core/Characters/GunshotAttenuation.GunshotAttenuation" null)
      (`KismetSystemLibrary.Delay` 0.1)
      (`self.tnt_m_color` (struct :`A` 1.0)))))

(event `interruptTimer`
  (goto _label :!via `Stop`))

(event `self.ReceiveBeginPlay`
  (`parent.ReceiveBeginPlay`)
  (`|ExecutionSequence`
    (:`then_0`
      (if (`self.timed`)
        (`self.TimedTNT`)
        (else
          (`KismetSystemLibrary.Delay` (`self.DeathTime`))
          (`self.TimedTNT`))))
    (:`then_1`
      (`KismetSystemLibrary.Delay` 0.5)
      (`PrimitiveComponent.SetCollisionResponseToChannel` (`self.CollisionSphere`) "ECC_Pawn" "ECR_Block"))
    (:`then_2`
      (bind _asbp_char_mouse (cast `/Game/Fadeout_Content/Core/Characters/BP_Char_Mouse` (`self.GetOwner`)))
      (switch `/Game/Fadeout_Content/Core/UI/Customize/Camille_Outfits` (cast `/Game/Fadeout_Content/Core/UI/Customize/Camille_Outfits` (`/Game/Fadeout_Content/Core/Characters/BP_PlayerCharacter.current_outfit` _asbp_char_mouse))
        (:`NewEnumerator5`
          (`StaticMeshComponent.SetStaticMesh` (`self.Mesh`) "/Game/Fadeout_Content/Core/FBX/TNT/jester_TNT_skin.jester_TNT_skin"))))))

(event `Explode`
  (bind _returnvalue (`self.K2_GetActorLocation`))
  (bind _returnvalue_2 (`self.GetOwner`))
  (bind _damageradius (`self.DamageRadius`))
  (bind _radialdamageamount (`self.radialDamageAmount`))
  (`GameplayStatics.SpawnEmitterAtLocation` (`self.ImpactVFX`) (`self.K2_GetActorLocation`) (struct) (`self.ExplosionVFXscale`))
  (`GameplayStatics.PlaySoundAtLocation` "/Game/Fadeout_Content/Core/Audio/Explosions/Explosion_5_W_Rubble_3.Explosion_5_W_Rubble_3" (`self.K2_GetActorLocation`) (struct) 1.25 (`KismetMathLibrary.RandomFloatInRange` 0.9 1.1) 0.0 "/Game/Fadeout_Content/Core/Characters/Footstep_Attenuation.Footstep_Attenuation" null null)
  (bind (_outhits _returnvalue_3) (`KismetSystemLibrary.SphereTraceMultiForObjects` :`Start` _returnvalue :`End` (+ _returnvalue (0.0 0.0 1.0)) :`Radius` (`self.DamageRadius`) :`ObjectTypes` (`|MakeArray` "ObjectTypeQuery3" "ObjectTypeQuery7" "ObjectTypeQuery2" "ObjectTypeQuery4" :!type "EObjectTypeQuery Enum") :`DrawDebugType` "ForDuration" :`TraceColor` (struct :`R` 0.993276 :`B` 1.0 :`A` 1.0) :`TraceHitColor` (struct :`G` 0.859794 :`B` 1.0 :`A` 1.0)))
  (if _returnvalue_3
    (for _array_element _outhits
      (`|ExecutionSequence`
        (:`then_0`
          (bind (_bblockinghit _binitialoverlap _time _distance _location _impactpoint _normal _impactnormal _physmat _hitactor _hitcomponent _hitbonename _hititem _faceindex _tracestart) (`GameplayStatics.BreakHitResult` _array_element))
          (bind _returnvalue_4 (* _impactnormal (`self.KnockbackPower`)))
          (`self.applyImpulse` _hitcomponent _returnvalue_4))
        (:`then_1`
          (if (not (`KismetArrayLibrary.Array_Contains` (`self.uniqueDamage`) _hitactor))
            ;[1 1 1] Distance fall off damage
            (`GameplayStatics.ApplyDamage` _hitactor (`KismetMathLibrary.SelectFloat` (`KismetMathLibrary.Lerp` _radialdamageamount (* _radialdamageamount 0.75) (/ (`KismetMathLibrary.FClamp` (`KismetMathLibrary.Vector_Distance` _tracestart _impactpoint) 1.0 _damageradius) _damageradius)) (`self.radialDamageAmount`) (`self.distanceFalloff`)) (`self.Instigator Controller`) self (`self.AOEDamageType`))))
        (:`then_2`
          (`KismetArrayLibrary.Array_AddUnique` (`self.uniqueDamage`) _hitactor)
          (bind _asbp_player_character (cast `/Game/Fadeout_Content/Core/Characters/BP_PlayerCharacter` _hitactor))
          (if (`Actor.bCanBeDamaged` _asbp_player_character)
            (`Character.LaunchCharacter` _asbp_player_character _returnvalue_4 false (not (>= (.z (`self.GetVelocity` _asbp_player_character)) 0.1)))
            (if (> (`KismetMathLibrary.VSize` _returnvalue_4) 40.0)
              (`/Engine/EditorBlueprintResources/ActorMacros.Switch Has Authority`
                (:`Authority`
                  (`/Game/Fadeout_Content/Core/Characters/BP_PlayerCharacter.air_Spin` _asbp_player_character)))))))))
  (`KismetSystemLibrary.Delay` 0.05)
  (`/Engine/EditorBlueprintResources/StandardMacros.IsValid` _returnvalue_2
    (:`Is Valid`
      (bind _asbp_player_character_2 (cast `/Game/Fadeout_Content/Core/Characters/BP_PlayerCharacter` _returnvalue_2))
      (`KismetArrayLibrary.Array_RemoveItem` (`/Game/Fadeout_Content/Core/Characters/BP_PlayerCharacter.myOwnedProjectiles` _asbp_player_character_2) self)
      (`self.K2_DestroyActor`))
    (:`Is Not Valid`
      (`self.K2_DestroyActor`))))

(event `self.OnProjectileHitEvent`
  (params (OtherActor :type "Actor Object Reference") (OtherComponent :type "PrimitiveComponent Object Reference") (HitResult :type "HitResult Structure (by ref)") (fromHit :type Boolean))
  (`/Engine/EditorBlueprintResources/ActorMacros.Switch Has Authority`
    (:`Authority`
      (`self.TNT Hit Event` HitResult OtherActor))))

(event `TNT Hit Event`
  (params (HitResult :type "HitResult Structure (by ref)") (HitActor :type "Actor Object Reference"))
  (bind _returnvalue (`self.GetOwner`))
  (bind (_bblockinghit _binitialoverlap _time _distance _location _impactpoint _normal _impactnormal) (`GameplayStatics.BreakHitResult` HitResult))
  (bind _returnvalue_2 (`self.K2_GetActorLocation`))
  (bind _collisionsphere (`self.CollisionSphere`))
  (if (not (`self.planted_Ground`))
    (cast `/Game/Fadeout_Content/Core/Characters/BP_PlayerCharacter` HitActor
      (:`then`
        (`ProjectileMovementComponent.StopSimulating` (`self.ProjectileMovement`) HitResult)
        (`PrimitiveComponent.SetCollisionResponseToAllChannels` _collisionsphere "ECR_Ignore")
        (`PrimitiveComponent.SetCollisionResponseToChannel` _collisionsphere "ECC_GameTraceChannel7" "ECR_Overlap")
        (`PrimitiveComponent.SetCollisionResponseToChannel` _collisionsphere "ECC_GameTraceChannel1" "ECR_Overlap")
        (`GameplayStatics.PlaySoundAtLocation` "/Game/Fadeout_Content/Core/Audio/residue-sfx/emptyclip.emptyclip" _returnvalue_2 (struct) 1.0 (`KismetMathLibrary.RandomFloatInRange` 0.9 1.1) 0.0 "/Game/Fadeout_Content/Core/Characters/Footstep_Attenuation.Footstep_Attenuation" null null)
        (`GameplayStatics.SpawnEmitterAtLocation` "/Game/Fadeout_Content/Core/FX/particle_footSmoke.particle_footSmoke" _returnvalue_2)
        (`PrimitiveComponent.SetCollisionResponseToChannel` (`self.CollisionSphere`) "ECC_PhysicsBody" "ECR_Ignore")
        (`PrimitiveComponent.SetCollisionResponseToChannel` (`self.CollisionSphere`) "ECC_Visibility" "ECR_Block")
        (`self.Attach` (`KismetMathLibrary.MakeTransform` (+ _impactpoint (* _impactnormal 10.0)) (`KismetMathLibrary.ComposeRotators` (`KismetMathLibrary.MakeRotator` 0.0 0.0 (.yaw (`self.K2_GetActorRotation`))) (`KismetMathLibrary.MakeRotFromZ` _impactnormal))) HitActor)
        (set `self.planted_Ground` true)
        (`self.tnt_m_color` (struct :`R` 0.904661 :`B` 1.0 :`A` 1.0)))
      (:`CastFailed`
        ;[1 1 1] Destroys projectile
        (`KismetSystemLibrary.Delay` 0.05)
        (`/Engine/EditorBlueprintResources/StandardMacros.IsValid` _returnvalue
          (:`Is Valid`
            (bind _asbp_player_character (cast `/Game/Fadeout_Content/Core/Characters/BP_PlayerCharacter` _returnvalue))
            (`KismetArrayLibrary.Array_RemoveItem` (`/Game/Fadeout_Content/Core/Characters/BP_PlayerCharacter.myOwnedProjectiles` _asbp_player_character) self)
            (`self.K2_DestroyActor`))
          (:`Is Not Valid`
            (`self.K2_DestroyActor`)))))))

(fn `applyImpulse`
  (params (Object :type "Object Object Reference") (InputPin :type "Vector Structure"))
  (bind _asstatic_mesh_component (cast `StaticMeshComponent` Object)
    (:`then`
      (if (and (`SceneComponent.IsSimulatingPhysics` _asstatic_mesh_component "None") (`|EnumEquality` (`SceneComponent.Mobility` _asstatic_mesh_component) "Movable") (not (`PrimitiveComponent.bIgnoreRadialImpulse` _asstatic_mesh_component)))
        (`PrimitiveComponent.AddImpulse` _asstatic_mesh_component InputPin "None" true)))
    (:`CastFailed`
      (bind _asskeletal_mesh_component (cast `SkeletalMeshComponent` Object))
      (if (and (`SceneComponent.IsSimulatingPhysics` _asskeletal_mesh_component "None") (`|EnumEquality` (`SceneComponent.Mobility` _asskeletal_mesh_component) "Movable"))
        (`PrimitiveComponent.AddImpulse` _asskeletal_mesh_component InputPin "None" true)
        (`KismetSystemLibrary.PrintString` (`KismetSystemLibrary.GetDisplayName` Object))))))

(fn `OnRep_Impact Normal Var`)

(fn `RadialDamage`
  (`/Engine/EditorBlueprintResources/ActorMacros.Switch Has Authority`
    (:`Authority`
      (`GameplayStatics.ApplyRadialDamage` :`BaseDamage` (`self.radialDamageAmount`) :`Origin` (`self.K2_GetActorLocation`) :`DamageRadius` (`self.DamageRadius`) :`DamageTypeClass` (`self.AOEDamageType`) :`DamageCauser` self :`InstigatedByController` (`self.Instigator Controller`) :`bDoFullDamage` (`self.AoeFullDamage`)))
    (:`Remote`
      _))
  (return))

(fn `tnt_m_color`
  (params (Value :type "LinearColor Structure") (SourceMaterial :type "MaterialInterface Object Reference"))
  (`/Engine/EditorBlueprintResources/StandardMacros.IsValid` (`self.tnt_dynamic`)
    (:`Is Valid`
      _)
    (:`Is Not Valid`
      (bind _returnvalue (`PrimitiveComponent.CreateDynamicMaterialInstance` (`self.Mesh`) 0 SourceMaterial "None"))
      (bind _output_get (set `self.tnt_dynamic` _returnvalue))))
  (`MaterialInstanceDynamic.SetVectorParameterValue` _output_get "fcolor" Value))

(fn `UserConstructionScript`
  (`parent.UserConstructionScript`)
  (`ProjectileMovementComponent.SetInterpolatedComponent` (`self.ProjectileMovement`) (`self.Mesh`)))