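; Menu game mode for Fadeout with a function that sets up local multiplayer players and their characters.
; SpawnPlayersFunction reads the player count from Fadeout_GameInstance and creates that many local players, spawning controllers for all but the first.
; A second loop spawns a BP_PlayerCharacter near the origin for each index, passes it as PlayerInt, and has the matching controller possess it.
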(fn `spawnPlayersFunction`
  (bind _asfadeout_game_instance (cast `/Game/Fadeout_GameInstance` (`GameplayStatics.GetGameInstance`)))
  (bind _returnvalue (- (`/Game/Fadeout_GameInstance.numberOfPlayers` _asfadeout_game_instance) 1))
  (for _index (range (+ _returnvalue 1))
    (`GameplayStatics.CreatePlayer` _index (not (== _index 0))))
  (for _index_2 (range (+ _returnvalue 1))
    (bind _returnvalue_2 (`|SpawnActorFromClass` :`Class` "/Game/Fadeout_Content/Core/Characters/BP_PlayerCharacter.BP_PlayerCharacter_C" :`SpawnTransform` (`KismetMathLibrary.MakeTransform` (0.0 0.0 1.0)) :`CollisionHandlingOverride` "Undefined" :`TransformScaleMethod` "OverrideRootScale" :`PlayerInt` _index_2 :`Instigator` null))
    (`Controller.Possess` (`GameplayStatics.GetPlayerController` _index_2) _returnvalue_2)))

(fn `UserConstructionScript`)