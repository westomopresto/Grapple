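; Lobby game mode for Fadeout that provides local multiplayer player setup, with BeginPlay left empty.
; SpawnPlayersFunction creates players from the game instance's player count, then possesses existing Allied-tagged BP_PlayerCharacters or spawns and possesses new ones if none are found.
; A helper maps allies to their RescueState and returns an escaped count.
; Online session create, find and join nodes are present but never run.
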(event `self.ReceiveBeginPlay`)

(fn `getAllyCountbyState`
  (returns (alliesAndStates :type "Map of /Game/Fadeout_Content/Core/Characters/BP_Ally Object Reference to /Game/Fadeout_Content/Core/Characters/RescueStates Enum") (escapedSince :type Integer))
  (locals (alliesAndState :type "Map of /Game/Fadeout_Content/Core/Characters/BP_Ally Object Reference to /Game/Fadeout_Content/Core/Characters/RescueStates Enum") (amountEscaped :type Integer))
  (for _array_element _
    (`/Engine/EditorBlueprintResources/StandardMacros.IsValid` _array_element
      (:`Is Valid`
        (`BlueprintMapLibrary.Map_Add` (`local.alliesAndState`) _array_element (`/Game/Fadeout_Content/Core/Characters/BP_Ally.RescueState` _array_element)))))
  (bind _values (`BlueprintMapLibrary.Map_Values` (`local.alliesAndState`)))
  (set `local.amountEscaped` 0)
  (for _array_element_2 _values
    (if (`|EnumEquality` _array_element_2 "NewEnumerator5")
      (`/Engine/EditorBlueprintResources/StandardMacros.IncrementInt` (`local.amountEscaped`))))
  (return (`local.alliesAndState`) (`local.amountEscaped`)))

(fn `spawnPlayersFunction`
  (bind _asfadeout_game_instance (cast `/Game/Fadeout_GameInstance` (`GameplayStatics.GetGameInstance`)))
  (bind _returnvalue (- (`/Game/Fadeout_GameInstance.numberOfPlayers` _asfadeout_game_instance) 1))
  (for _index (range (+ _returnvalue 1))
    (`GameplayStatics.CreatePlayer` _index (not (== _index 0))))
  (bind _outactors (`BlueprintGameplayTagLibrary.GetAllActorsOfClassMatchingTagQuery` "/Game/Fadeout_Content/Core/Characters/BP_PlayerCharacter.BP_PlayerCharacter_C" (`BlueprintGameplayTagLibrary.MakeGameplayTagQuery` (struct :`TagDictionary` (struct :`(TagName` "allied") :`(TagName` "player")) :`QueryTokenStream` "(0,1,2,2,0,1)" :`AutoDescription` " ALL( allied, player )"))))
  (if (> (`KismetArrayLibrary.Array_Length` _outactors) 0)
    (for (_array_element _array_index) _outactors
      (bind _aspawn (cast `Pawn` _array_element))
      (`Controller.Possess` (`GameplayStatics.GetPlayerController` _array_index) _aspawn))
    (else
      (for _index_2 (range (+ _returnvalue 1))
        (bind _returnvalue_2 (`|SpawnActorFromClass` "/Game/Fadeout_Content/Core/Characters/BP_PlayerCharacter.BP_PlayerCharacter_C" (`KismetMathLibrary.MakeTransform` (0.0 0.0 1.0)) "Undefined" "OverrideRootScale" null _index_2 null))
        (`Controller.Possess` (`GameplayStatics.GetPlayerController` _index_2) _returnvalue_2)))))

(fn `UserConstructionScript`)