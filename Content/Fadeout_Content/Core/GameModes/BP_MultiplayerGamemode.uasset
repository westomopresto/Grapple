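; Multiplayer game mode for Fadeout that runs timed rounds and switches between game types such as FFA, TDM and CTF.
; On login it assigns or balances teams, then spawns the selected character at team-tagged PlayerStarts.
; StartRound resets scores, flags and timer; EndRound moves players to spectator and scoreboard, optionally restarting.
; It also handles announcer sounds, chat lookups, cheats, per-tick Steam server updates and older VaRest master-server registration.
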(event `update Server Info`
  ;[0.1268 1 0.5965 1 40] OLD MULTIPLAYER
  (`KismetSystemLibrary.Delay` 0.5)
  (`self.Get Player Names`)
  (`self.Get Level Name`)
  (`self.Get Server Name`))

(event `Add game to Master Server`
  ;[0.1268 1 0.5965 1 40] OLD MULTIPLAYER
  (`self.update Server Info`)
  (`KismetSystemLibrary.Delay` 2.0)
  (`self.POST Event` "AddGame"))

(event `POST Event`
  (params (command :type String))
  ;[0.1268 1 0.5965 1 40] OLD MULTIPLAYER
  ;;[1 1 1] Post Command
  (`VaRestSubsystem.CallURL` (subsystem `VaRestSubsystem`) (`KismetStringLibrary.Concat_StrStr` (`self.MatchMakeServer`) command) "POST" "x_www_form_urlencoded_url" null (delegate `Post Game Callback`)))

(event `Remove game on Master Server`
  ;[0.1268 1 0.5965 1 40] OLD MULTIPLAYER
  (`self.POST Event` "RemoveGame"))

(event `Update game on Master Server`
  ;[0.1268 1 0.5965 1 40] OLD MULTIPLAYER
  (`self.update Server Info`)
  (`KismetSystemLibrary.Delay` 2.0)
  (`self.POST Event` "UpdateGame"))

(event `Post Game Callback`
  (params (Request :type "VaRestRequestJSON Object Reference"))
  ;[0.1268 1 0.5965 1 40] OLD MULTIPLAYER
  ;;[1 1 1] Post Command
  (bind _output_get (set `self.AddGameReturn` (`VaRestRequestJSON.GetResponseObject` Request)))
  (`VaRestJsonObject.DecodeJson` _output_get (`VaRestJsonObject.EncodeJsonToSingleString` _output_get) true)
  (bind _output_get_2 (set `self.AddGameSuccess` (`VaRestJsonObject.GetBoolField` _output_get "success")))
  (`KismetSystemLibrary.PrintString` (`KismetStringLibrary.Concat_StrStr` (stale `POST Event` command) (`KismetStringLibrary.Conv_BoolToString` _output_get_2)) true true (struct :`G` 0.66 :`B` 1.0 :`A` 1.0) 5.0))

(event `Get Servers IP`
  (bind _returnvalue (subsystem `VaRestSubsystem`))
  ;[0.1268 1 0.5965 1 40] OLD MULTIPLAYER
  ;;[1 1 1] Get IP
  (bind _returnvalue_2 (`VaRestSubsystem.ConstructVaRestJsonObject` _returnvalue))
  (`VaRestSubsystem.CallURL` _returnvalue (`KismetStringLibrary.Concat_StrStr` (`self.MatchMakeServer`) "GetMyIP") "GET" "x_www_form_urlencoded_url" _returnvalue_2 (delegate `Response`)))

(event `Response`
  (params (Request :type "VaRestRequestJSON Object Reference"))
  ;[0.1268 1 0.5965 1 40] OLD MULTIPLAYER
  ;;[1 1 1] Get IP
  (bind _output_get (set `self.IP Json` (`VaRestRequestJSON.GetResponseObject` Request)))
  (`VaRestJsonObject.DecodeJson` _output_get (`VaRestJsonObject.EncodeJsonToSingleString` _output_get) true)
  (bind _returnvalue (`VaRestJsonObject.GetStringField` _output_get "ip_address"))
  (`KismetSystemLibrary.PrintString` _returnvalue)
  (set `self.serverIP` _returnvalue)
  (bind _output_get_2 (set `self.IPSuccess` (`VaRestJsonObject.GetBoolField` _output_get "success")))
  (if _output_get_2
    (`self.Add game to Master Server`)
    (`KismetSystemLibrary.PrintString` (`KismetStringLibrary.Concat_StrStr` "GetMyIP: " (`KismetStringLibrary.Conv_BoolToString` _output_get_2)) true true (struct :`G` 0.66 :`B` 1.0 :`A` 1.0) 5.0)
    (else
      (`KismetSystemLibrary.PrintString` "IP FETCH FAILED" true true (struct :`R` 1.0 :`B` 0.013159 :`A` 1.0) 500.0))))

(event `Flag Event`
  (params (SoundToPlay :type "SoundBase Object Reference"))
  (`/Engine/EditorBlueprintResources/StandardMacros.DoOnce` false :!label _label
    (:`Completed`
      (`|SpawnActorFromClass` "/Game/Fadeout_Content/Core/Support/Multiplayer_Support/KillSounds/KillSounder.KillSounder_C" (`KismetMathLibrary.MakeTransform` (0.0 0.0 0.0)) "AlwaysSpawn" "OverrideRootScale" null SoundToPlay null)
      (`KismetSystemLibrary.Delay` 5.0)
      (goto _label :!via `Reset`))))

(event `Gametype Voice Announce`
  (params (gametype :type "/Game/Fadeout_Content/Core/Support/Multiplayer_Support/DM_GameType Enum" :default "NewEnumerator0"))
  (bind _fo_announcer (`self.FO_Announcer`))
  (switch `/Game/Fadeout_Content/Core/Support/Multiplayer_Support/DM_GameType` gametype
    (:`NewEnumerator0`
      (`/Engine/EditorBlueprintResources/StandardMacros.IsValid` (`self.FO_Announcer`)
        (:`Is Valid`
          (`KismetSystemLibrary.Delay` 0.5)
          (`/Game/Fadeout_Content/Core/Support/Multiplayer_Support/FO_Announcer.Say FREE FOR ALL` _fo_announcer)
          (`self.Start Round`))))
    (:`NewEnumerator1`
      (`/Engine/EditorBlueprintResources/StandardMacros.IsValid` _fo_announcer
        (:`Is Valid`
          (`KismetSystemLibrary.Delay` 0.5)
          (`/Game/Fadeout_Content/Core/Support/Multiplayer_Support/FO_Announcer.Say Team DM` _fo_announcer)
          (`self.Start Round`))))
    (:`NewEnumerator2`
      (`/Engine/EditorBlueprintResources/StandardMacros.IsValid` _fo_announcer
        (:`Is Valid`
          (`KismetSystemLibrary.Delay` 0.5)
          (`/Game/Fadeout_Content/Core/Support/Multiplayer_Support/FO_Announcer.Say CAPTURE THE FLAG` _fo_announcer)
          (`self.Start Round`))))))

(event `Round Timer`
  ;[1 1 1] Round Timer
  (`KismetSystemLibrary.K2_ClearAndInvalidateTimerHandle` (`self.RoundCountdown`))
  (set `self.RoundTimeRemaining` (`self.MaxRoundTime`))
  (bind _returnvalue (`KismetSystemLibrary.K2_SetTimerDelegate` (delegate `TimeDecrement`) 1.0 true))
  (set `self.RoundCountdown` _returnvalue))

(event `TimeDecrement`
  ;[1 1 1] Round Timer
  (bind _result (`/Engine/EditorBlueprintResources/StandardMacros.DecrementInt` (`self.RoundTimeRemaining`))
    (:`  `
      (bind _asmultiplayer_game_state (cast `/Game/Fadeout_Content/Core/Support/Multiplayer_Support/Multiplayer_GameState` (`GameplayStatics.GetGameState`)))
      (bind _output_get (set `/Game/Fadeout_Content/Core/Support/Multiplayer_Support/Multiplayer_GameState.RoundTimeLeft` _result _asmultiplayer_game_state))
      (if (<= _output_get 0)
        (`KismetSystemLibrary.K2_ClearAndInvalidateTimerHandle` (`self.RoundCountdown`))
        (`self.End Round` true)))))

(event `self.ReceiveEndPlay`
  (params (EndPlayReason :type "EEndPlayReason Enum" :default "Destroyed"))
  ;[1 1 1] End Play
  (switch `EEndPlayReason` EndPlayReason
    (:`Destroyed`
      _)
    (:`LevelTransition`
      _)
    (:`EndPlayInEditor`
      _)
    (:`RemovedFromWorld`
      _)
    (:`Quit`
      _))
  (bind _asfadeout_game_instance (cast `/Game/Fadeout_GameInstance` (`GameplayStatics.GetGameInstance`)))
  (`/Game/Fadeout_GameInstance.End Session` _asfadeout_game_instance))

(event `Player Initialize`
  (params (InputPin :type "Controller Object Reference"))
  (switch `/Game/Fadeout_Content/Core/Support/Multiplayer_Support/DM_GameType` (`self.GameType`)
    (:`NewEnumerator0`
      (`self.Change Player Team` InputPin "FFA"))
    (:`NewEnumerator1`
      (`self.Team Balance` InputPin))
    (:`NewEnumerator2`
      (`self.Team Balance` InputPin))
    (:`NewEnumerator3`
      (`self.Team Balance` InputPin))
    (:`NewEnumerator4`
      (`self.Team Balance` InputPin))
    (:`NewEnumerator5`
      (`self.Team Balance` InputPin))))

(event `SET Teamscore`
  (params (redScore :type Integer) (blueScore :type Integer))
  ;[1 1 1] Team Score
  (bind _asmultiplayer_game_state (cast `/Game/Fadeout_Content/Core/Support/Multiplayer_Support/Multiplayer_GameState` (`GameplayStatics.GetGameState`)))
  (bind _output_get (set `/Game/Fadeout_Content/Core/Support/Multiplayer_Support/Multiplayer_GameState.redScore` redScore _asmultiplayer_game_state))
  (bind _output_get_2 (set `/Game/Fadeout_Content/Core/Support/Multiplayer_Support/Multiplayer_GameState.blueScore` blueScore _asmultiplayer_game_state))
  (set `self.redTeamScore` _output_get)
  (set `self.blueTeamScore` _output_get_2))

(event `PlayKillSound`
  (params (KillStreak :type Integer))
  (bind _returnvalue (`KismetMathLibrary.MakeTransform` (0.0 0.0 0.0)))
  ;[1 1 1] Kill Streak
  (`KismetSystemLibrary.Delay` 0.5)
  (switch `int` KillStreak
    (:`Default`
      (if (>= KillStreak 6)
        (`|SpawnActorFromClass` "/Game/Fadeout_Content/Core/Support/Multiplayer_Support/KillSounds/KillSounder.KillSounder_C" _returnvalue "AlwaysSpawn" "OverrideRootScale" null "/Game/Fadeout_Content/Core/Support/Multiplayer_Support/KillSounds/Fadeout_KillSounds/holy_shit.holy_shit" null)))
    (:`2`
      (`|SpawnActorFromClass` "/Game/Fadeout_Content/Core/Support/Multiplayer_Support/KillSounds/KillSounder.KillSounder_C" _returnvalue "AlwaysSpawn" "OverrideRootScale" null "/Game/Fadeout_Content/Core/Support/Multiplayer_Support/KillSounds/Fadeout_KillSounds/double_kill.double_kill" null))
    (:`3`
      (`|SpawnActorFromClass` "/Game/Fadeout_Content/Core/Support/Multiplayer_Support/KillSounds/KillSounder.KillSounder_C" _returnvalue "AlwaysSpawn" "OverrideRootScale" null "/Game/Fadeout_Content/Core/Support/Multiplayer_Support/KillSounds/Fadeout_KillSounds/triple_kill.triple_kill" null))
    (:`4`
      (`|SpawnActorFromClass` "/Game/Fadeout_Content/Core/Support/Multiplayer_Support/KillSounds/KillSounder.KillSounder_C" _returnvalue "AlwaysSpawn" "OverrideRootScale" null "/Game/Fadeout_Content/Core/Support/Multiplayer_Support/KillSounds/Fadeout_KillSounds/dominating.dominating" null))
    (:`5`
      (`|SpawnActorFromClass` "/Game/Fadeout_Content/Core/Support/Multiplayer_Support/KillSounds/KillSounder.KillSounder_C" _returnvalue "AlwaysSpawn" "OverrideRootScale" null "/Game/Fadeout_Content/Core/Support/Multiplayer_Support/KillSounds/Fadeout_KillSounds/monster_kill.monster_kill" null))))

(event `Add Teamscore`
  (params (redTeamScore :type Integer) (blueTeamScore :type Integer))
  ;[1 1 1] Team Score
  (set `self.redTeamScore` (+ (`self.redTeamScore`) redTeamScore))
  (set `self.blueTeamScore` (+ (`self.blueTeamScore`) blueTeamScore))
  (bind _asmultiplayer_game_state (cast `/Game/Fadeout_Content/Core/Support/Multiplayer_Support/Multiplayer_GameState` (`GameplayStatics.GetGameState`)))
  (set `/Game/Fadeout_Content/Core/Support/Multiplayer_Support/Multiplayer_GameState.redScore` (`self.redTeamScore`) _asmultiplayer_game_state)
  (set `/Game/Fadeout_Content/Core/Support/Multiplayer_Support/Multiplayer_GameState.blueScore` (`self.blueTeamScore`) _asmultiplayer_game_state))

(event `self.ReceiveTick`
  (params (DeltaSeconds :type "Float (single-precision)"))
  ;[0 1 0.171 1 50] EVENT TICK
  (bind _asfadeout_game_instance (cast `/Game/Fadeout_GameInstance` (`GameplayStatics.GetGameInstance`)))
  (`/Game/Fadeout_GameInstance.Update Steam Server` _asfadeout_game_instance))

(event `self.K2_PostLogin`
  (params (NewPlayer :type "PlayerController Object Reference"))
  ;[1 1 1] Post Login
  (`self.Player Initialize` NewPlayer)
  ;[1 1 1] Add player to PlayersConnected array
  (`/Engine/EditorBlueprintResources/ActorMacros.Switch Has Authority`
    (:`Authority`
      (`/Engine/EditorBlueprintResources/StandardMacros.IsValid` NewPlayer
        (:`Is Valid`
          (bind _returnvalue (`KismetArrayLibrary.Array_AddUnique` (`self.ConnectedPlayers`) NewPlayer))
          (message `/Game/AntizeChatSystem/Blueprints/BP_AntizeChatInterface.MSG_SetPlayerID` NewPlayer _returnvalue)
          (bind _asfo_player_controller (cast `/Game/Fadeout_Content/Core/FO_PlayerController` NewPlayer))
          (`/Game/Fadeout_Content/Core/FO_PlayerController.CreateChat` _asfo_player_controller)
          (bind _asfo_player_state (cast `/Game/Fadeout_Content/Core/Support/Multiplayer_Support/FO_PlayerState` (`Controller.PlayerState` _asfo_player_controller)))
          (set `self.connectingPlayersName` (`/Game/Fadeout_Content/Core/Support/Multiplayer_Support/FO_PlayerState.CustomName` _asfo_player_state))
          (for _array_element (`self.ConnectedPlayers`)
            (bind _asfo_player_controller_2 (cast `/Game/Fadeout_Content/Core/FO_PlayerController` _array_element))
            (`/Game/Fadeout_Content/Core/FO_PlayerController.ShowSystemMessage` _asfo_player_controller_2 (`KismetTextLibrary.Conv_StringToText` (`KismetStringLibrary.Concat_StrStr` (`KismetTextLibrary.Conv_TextToString` (`self.connectingPlayersName`)) " Has Joined the Server")) (struct :`G` 1.0 :`B` 0.107029 :`A` 1.0))))))))

(event `Change Game Type`
  (params (`Game Type` :type "/Game/Fadeout_Content/Core/Support/Multiplayer_Support/DM_GameType Enum" :default "NewEnumerator0"))
  ;[1 1 1] Change Game type
  (bind _output_get (set `self.GameType` `Game Type`))
  (`self.GameType to M_Gamestate` _output_get)
  (for _array_element (`self.ConnectedPlayers`)
    (`self.Player Initialize` _array_element))
  (`self.Gametype Voice Announce` _output_get)
  (bind _outactors (`GameplayStatics.GetAllActorsOfClass` "/Game/Fadeout_Content/Core/Characters/BP_Turret.BP_Turret_C"))
  (for _array_element_2 _outactors
    (`GameplayStatics.ApplyDamage` _array_element_2 999.0)))

(event `Start Round`
  ;[1 1 1] Rounds
  (if (`self.RoundActive?`)
    (`self.End Round` false)
    (`KismetSystemLibrary.Delay` 1.0))
  (set `self.canSpawn?` true)
  (for _array_element (`self.ConnectedPlayers`)
    (bind _asfo_player_controller (cast `/Game/Fadeout_Content/Core/FO_PlayerController` _array_element))
    (set `/Game/Fadeout_Content/Core/FO_PlayerController.CanRespawn` true _asfo_player_controller)
    (`/Game/Fadeout_Content/Core/FO_PlayerController.RequestSpawn` _asfo_player_controller)
    (`/Game/Fadeout_Content/Core/FO_PlayerController.StartSpawnTime` _asfo_player_controller)
    (bind _asfo_player_state (cast `/Game/Fadeout_Content/Core/Support/Multiplayer_Support/FO_PlayerState` (`Controller.PlayerState` _array_element)))
    (set `/Game/Fadeout_Content/Core/Support/Multiplayer_Support/FO_PlayerState.FO_Score` 0 _asfo_player_state)
    (`/Game/Fadeout_Content/Core/FO_PlayerController.Hide Scoreboard` _asfo_player_controller))
  (`|ExecutionSequence`
    (:`then_0`
      (set `self.RoundActive?` true)
      (`self.SET Teamscore` 0)
      (bind _outactors (`GameplayStatics.GetAllActorsOfClass` "/Game/Fadeout_Content/Core/Props/GameModeSupport/BP_Flag.BP_Flag_C"))
      (for _array_element_2 _outactors
        (`GameplayStatics.ApplyDamage` _array_element_2 99999.0)))
    (:`then_1`
      (bind _outactors_2 (`GameplayStatics.GetAllActorsOfClass` "/Game/Fadeout_Content/Core/Props/GameModeSupport/BP_FlagStand.BP_FlagStand_C"))
      (for _array_element_3 _outactors_2
        (switch `/Game/Fadeout_Content/Core/Support/Multiplayer_Support/DM_GameType` (`self.GameType`)
          (:`NewEnumerator0`
            (set `/Game/Fadeout_Content/Core/Props/GameModeSupport/BP_FlagStand.canSpawnFlag?` false _array_element_3 :!label _label_2))
          (:`NewEnumerator1`
            (goto _label_2))
          (:`NewEnumerator2`
            (set `/Game/Fadeout_Content/Core/Props/GameModeSupport/BP_FlagStand.canSpawnFlag?` true _array_element_3))
          (:`NewEnumerator3`
            (goto _label_2))
          (:`NewEnumerator4`
            (goto _label_2))
          (:`NewEnumerator5`
            (goto _label_2)))))
    (:`then_2`
      (`self.Round Timer`))))

(event `self.K2_OnLogout`
  (params (ExitingController :type "Controller Object Reference"))
  ;[1 1 1] Remove player from PlayersConnected array
  (`|ExecutionSequence`
    (:`then_0`
      (`/Engine/EditorBlueprintResources/ActorMacros.Switch Has Authority`
        (:`Authority`
          (`KismetArrayLibrary.Array_RemoveItem` (`self.ConnectedPlayers`) ExitingController))))))

(event `self.ReceiveBeginPlay`
  ;[1 1 1] Begin Play
  (`|ExecutionSequence`
    (:`then_0`
      (`self.GameType to M_Gamestate` (`self.GameType`)))
    (:`then_1`
      (`parent.ReceiveBeginPlay`)
      (bind _outactors (`GameplayStatics.GetAllActorsOfClass` "/Script/Engine.PlayerStart"))
      (bind _output_get (set `self.All_PlayerStarts` _outactors))
      (for _array_element _output_get
        (switch `name` (`PlayerStart.PlayerStartTag` _array_element)
          (:`red`
            (`KismetArrayLibrary.Array_Add` (`self.red_PlayerStarts`) _array_element))
          (:`blue`
            (`KismetArrayLibrary.Array_Add` (`self.blue_PlayerStarts`) _array_element))
          (:`spec`
            (set `self.spectatorStart` _array_element))
          (:`FFA`
            (`KismetArrayLibrary.Array_Add` (`self.FFA_PlayerStarts`) _array_element)))))
    (:`then_2`
      (bind _outactors_2 (`GameplayStatics.GetAllActorsOfClass` "/Game/Fadeout_Content/Core/Support/Multiplayer_Support/FO_Announcer.FO_Announcer_C"))
      (set `self.FO_Announcer` (`|GetArrayItem` _outactors_2)))
    (:`then_3`
      (`KismetSystemLibrary.Delay` 1.0)
      (bind _asfadeout_game_instance (cast `/Game/Fadeout_GameInstance` (`GameplayStatics.GetGameInstance`)))
      (`/Game/Fadeout_GameInstance.Update Steam Server` _asfadeout_game_instance)
      (`KismetSystemLibrary.Delay` 1.0)
      (`self.Start Round`))))

(event `maxammo`
  ;[1 1 1] Cheats
  (for _array_element (`self.ConnectedPlayers`)
    (bind _asbp_player_character (cast `/Game/Fadeout_Content/Core/Characters/BP_PlayerCharacter` (`Controller.K2_GetPawn` _array_element)))
    (set `/Game/Fadeout_Content/Core/Characters/BP_PlayerCharacter.HeldAmmo` (`/Game/Fadeout_Content/Core/Characters/BP_PlayerCharacter.MaxHeldAmmo` _asbp_player_character) _asbp_player_character)
    (`KismetSystemLibrary.PrintString` "CHEAT: Max Ammo" true true (struct :`R` 1.0 :`G` 0.971415 :`A` 1.0) 5.0)))

(event `End Round`
  (params (`AutoStartNextRound?` :type Boolean))
  ;[1 1 1] Rounds
  (`KismetSystemLibrary.K2_ClearAndInvalidateTimerHandle` (`self.RoundCountdown`))
  (`|ExecutionSequence`
    (:`then_0`
      (for _array_element (`self.ConnectedPlayers`)
        (bind _asfo_player_controller (cast `/Game/Fadeout_Content/Core/FO_PlayerController` _array_element))
        (set `/Game/Fadeout_Content/Core/FO_PlayerController.CanRespawn` false _asfo_player_controller)
        (bind _asbp_player_character (cast `/Game/Fadeout_Content/Core/Characters/BP_PlayerCharacter` (`Controller.K2_GetPawn` _asfo_player_controller)))
        (`self.Spawn Spectator` (`self.GetTransform` (`self.spectatorStart`)) _asfo_player_controller)
        (`/Game/Fadeout_Content/Core/Characters/BP_PlayerCharacter.Drop All Tools Multicast` _asbp_player_character true)
        (`self.K2_DestroyActor` _asbp_player_character)
        (`/Game/Fadeout_Content/Core/FO_PlayerController.DeadSpectator` _asfo_player_controller)
        (`KismetSystemLibrary.Delay` 1.0)
        (`/Game/Fadeout_Content/Core/FO_PlayerController.Menu Action` _asfo_player_controller "NewEnumerator4")
        (`/Game/Fadeout_Content/Core/FO_PlayerController.Show ScoreBoard` _asfo_player_controller)
        (`/Game/Fadeout_Content/Core/FO_PlayerController.ShowSystemMessage` _asfo_player_controller "NEXT ROUND STARTS IN 8 SECONDS" (struct :`R` 1.0 :`G` 0.966016 :`A` 1.0))
        (`/Game/Fadeout_Content/Core/FO_PlayerController.ShowSystemMessage` _asfo_player_controller "NEXT ROUND STARTS IN 8 SECONDS" (struct :`R` 1.0 :`G` 0.966016 :`A` 1.0)))
      (set `self.canSpawn?` false)
      (set `self.RoundActive?` false))
    (:`then_1`
      (`|SpawnActorFromClass` "/Game/Fadeout_Content/Core/Support/Multiplayer_Support/KillSounds/KillSounder.KillSounder_C" (`KismetMathLibrary.MakeTransform` (0.0 0.0 0.0)) "AlwaysSpawn" "OverrideRootScale" null "/Game/Fadeout_Content/Core/Audio/Multiplayer_Sounds/Buzzer-SoundBible_com-188422102.Buzzer-SoundBible_com-188422102" null)
      (if `AutoStartNextRound?`
        (`KismetSystemLibrary.Delay` 8.0)
        (`self.Start Round`)))))

(event `flamethrower`
  ;[1 1 1] Cheats
  (for _array_element (`self.ConnectedPlayers`)
    (`|SpawnActorFromClass` "/Game/Fadeout_Content/Core/Weapons/BP_FlameThrower.BP_FlameThrower_C" (`KismetMathLibrary.Conv_VectorToTransform` (`self.K2_GetActorLocation` (`Controller.K2_GetPawn` _array_element))) "AlwaysSpawn" "OverrideRootScale" null "/Game/Fadeout_Content/Core/Weapons/BP_Projectile_Flame.BP_Projectile_Flame_C" true null)
    (`KismetSystemLibrary.PrintString` "CHEAT: Flame Thrower" true true (struct :`R` 1.0 :`G` 0.971415 :`A` 1.0) 5.0)))

(event `Spawn Player`
  (params (Controller :type "Controller Object Reference") (`spectator Override` :type Boolean))
  (bind _all_playerstarts (`self.All_PlayerStarts`))
  (bind _red_playerstarts (`self.red_PlayerStarts`))
  (bind _blue_playerstarts (`self.blue_PlayerStarts`))
  (bind _spectatorstart (`self.spectatorStart`))
  (bind _ffa_playerstarts (`self.FFA_PlayerStarts`))
  (bind _asfo_player_state (cast `/Game/Fadeout_Content/Core/Support/Multiplayer_Support/FO_PlayerState` (`Controller.PlayerState` Controller) :!pure true))
  (bind _output (`|GetArrayItem` _ffa_playerstarts (`KismetMathLibrary.RandomIntegerInRange` 0 (- (`KismetArrayLibrary.Array_Length` _ffa_playerstarts) 1))))
  (bind _returnvalue (`self.GetTransform` (`|GetArrayItem` _all_playerstarts (`KismetMathLibrary.RandomIntegerInRange` 0 (- (`KismetArrayLibrary.Array_Length` _all_playerstarts) 1)))))
  (if `spectator Override`
    (`|ExecutionSequence` :!label _label_3
      (:`then_0`
        ;[1 1 1] Assigns spawn location based on team or tag
        (switch `string` (`/Game/Fadeout_Content/Core/Support/Multiplayer_Support/FO_PlayerState.Team` (cast `/Game/Fadeout_Content/Core/Support/Multiplayer_Support/FO_PlayerState` (`Controller.PlayerState` Controller) :!pure true))
          (:`Default`
            (set `self.SpawnTransform` _returnvalue))
          (:`red`
            (set `self.SpawnTransform` (`self.GetTransform` (`|GetArrayItem` _red_playerstarts (`KismetMathLibrary.RandomIntegerInRange` 0 (- (`KismetArrayLibrary.Array_Length` _red_playerstarts) 1))))))
          (:`blue`
            (set `self.SpawnTransform` (`self.GetTransform` (`|GetArrayItem` _blue_playerstarts (`KismetMathLibrary.RandomIntegerInRange` 0 (- (`KismetArrayLibrary.Array_Length` _blue_playerstarts) 1))))))
          (:`spec`
            (`/Engine/EditorBlueprintResources/StandardMacros.IsValid` _spectatorstart
              (:`Is Valid`
                (set `self.SpawnTransform` (`self.GetTransform` _spectatorstart)))
              (:`Is Not Valid`
                (set `self.SpawnTransform` (`KismetMathLibrary.MakeTransform` (0.0 0.0 0.0))))))
          (:`FFA`
            (`/Engine/EditorBlueprintResources/StandardMacros.IsValid` _output
              (:`Is Valid`
                (set `self.SpawnTransform` (`self.GetTransform` _output)))
              (:`Is Not Valid`
                (set `self.SpawnTransform` _returnvalue))))))
      (:`then_1`
        (`KismetSystemLibrary.PrintString` (`|GetEnumeratorNameAsString` (`/Game/Fadeout_Content/Core/Support/Multiplayer_Support/FO_PlayerState.SelectedCharacter` _asfo_player_state)) true true (struct :`R` 0.989392 :`G` 1.0 :`A` 1.0) 12.0)
        (switch `string` (`/Game/Fadeout_Content/Core/Support/Multiplayer_Support/FO_PlayerState.Team` _asfo_player_state)
          (:`Default`
            (`self.Character Spawning` Controller _asfo_player_state :!label _label_4))
          (:`red`
            (goto _label_4))
          (:`blue`
            (goto _label_4))
          (:`spec`
            (bind _returnvalue_2 (`|SpawnActorFromClass` "/Game/Fadeout_Content/Core/Characters/BP_Spectator_Player.BP_Spectator_Player_C" (`self.SpawnTransform`) "AdjustIfPossibleButAlwaysSpawn" "OverrideRootScale" null 0 "NewEnumerator2" null))
            (`Controller.Possess` Controller _returnvalue_2)))))
    (elif (`self.canSpawn?`)
      (goto _label_3))))

(event `SwitchCharacter`
  (params (SelectedCharacter :type "/Game/Fadeout_Content/Core/Support/Multiplayer_Support/CharactersSelected Enum" :default "NewEnumerator0") (`Character Controller` :type "PlayerController Object Reference"))
  (bind _asfo_player_state (cast `/Game/Fadeout_Content/Core/Support/Multiplayer_Support/FO_PlayerState` (`Controller.PlayerState` `Character Controller`) :!pure true))
  ;[1 1 1] Switch Character
  (set `/Game/Fadeout_Content/Core/Support/Multiplayer_Support/FO_PlayerState.SelectedCharacter` SelectedCharacter _asfo_player_state)
  (`KismetSystemLibrary.PrintString` (`KismetStringLibrary.Concat_StrStr` (`KismetTextLibrary.Conv_TextToString` (`/Game/Fadeout_Content/Core/Support/Multiplayer_Support/FO_PlayerState.CustomName` _asfo_player_state)) (`|GetEnumeratorNameAsString` (`/Game/Fadeout_Content/Core/Support/Multiplayer_Support/FO_PlayerState.SelectedCharacter` _asfo_player_state))) true true (struct :`R` 1.0 :`G` 0.086574 :`A` 1.0) 4.0))

(event `Change Player Team`
  (params (`Player Controller` :type "Controller Object Reference") (Team :type String))
  ;[1 1 1] Change Team
  (bind _asfo_player_state (cast `/Game/Fadeout_Content/Core/Support/Multiplayer_Support/FO_PlayerState` (`Controller.PlayerState` `Player Controller`)))
  (set `/Game/Fadeout_Content/Core/Support/Multiplayer_Support/FO_PlayerState.Team` Team _asfo_player_state))

(event `Spawn Spectator`
  (params (SpawnTransform :type "Transform Structure") (Target :type "Controller Object Reference"))
  ;[1 1 1] Assigns spawn location based on team or tag
  (`/Engine/EditorBlueprintResources/StandardMacros.IsValid` Target
    (:`Is Valid`
      (bind _returnvalue (`|SpawnActorFromClass` "/Game/Fadeout_Content/Core/Characters/BP_Spectator_Player.BP_Spectator_Player_C" SpawnTransform "Undefined" "OverrideRootScale" null 0 "NewEnumerator4" null))
      (`Controller.Possess` Target _returnvalue))))

(fn `Character Spawning`
  (params (Controller :type "Controller Object Reference") (FO_PlayerState :type "/Game/Fadeout_Content/Core/Support/Multiplayer_Support/FO_PlayerState Object Reference"))
  (switch `/Game/Fadeout_Content/Core/Support/Multiplayer_Support/CharactersSelected` (`/Game/Fadeout_Content/Core/Support/Multiplayer_Support/FO_PlayerState.SelectedCharacter` FO_PlayerState)
    (:`NewEnumerator0`
      (bind _returnvalue (`|SpawnActorFromClass` :`Class` "/Game/Fadeout_Content/Core/Characters/BP_Char_Mouse.BP_Char_Mouse_C" :`SpawnTransform` (`self.SpawnTransform`) :`CollisionHandlingOverride` "AdjustIfPossibleButAlwaysSpawn" :`TransformScaleMethod` "OverrideRootScale" :`current_outfit` (`KismetMathLibrary.Conv_ByteToInt` (`/Game/Fadeout_Content/Core/Support/Multiplayer_Support/FO_PlayerState.fav-outfit_Camille` FO_PlayerState)) :`Instigator` null))
      (`Controller.Possess` Controller _returnvalue))
    (:`NewEnumerator1`
      (bind _returnvalue_2 (`|SpawnActorFromClass` :`Class` "/Game/Fadeout_Content/Core/Characters/BP_Char_Snek.BP_Char_Snek_C" :`SpawnTransform` (`self.SpawnTransform`) :`CollisionHandlingOverride` "AdjustIfPossibleButAlwaysSpawn" :`TransformScaleMethod` "OverrideRootScale" :`current_outfit` (`KismetMathLibrary.Conv_ByteToInt` (`/Game/Fadeout_Content/Core/Support/Multiplayer_Support/FO_PlayerState.fav-outfit_Dalton` FO_PlayerState)) :`Instigator` null))
      (`Controller.Possess` Controller _returnvalue_2))
    (:`NewEnumerator2`
      (bind _returnvalue_3 (`|SpawnActorFromClass` :`Class` "/Game/Fadeout_Content/Core/Characters/BP_Char_Bunn.BP_Char_Bunn_C" :`SpawnTransform` (`self.SpawnTransform`) :`CollisionHandlingOverride` "AdjustIfPossibleButAlwaysSpawn" :`TransformScaleMethod` "OverrideRootScale" :`current_outfit` (`KismetMathLibrary.Conv_ByteToInt` (`/Game/Fadeout_Content/Core/Support/Multiplayer_Support/FO_PlayerState.fav-outfit_Friday` FO_PlayerState)) :`Instigator` null))
      (`Controller.Possess` Controller _returnvalue_3))
    (:`NewEnumerator3`
      (bind _returnvalue_4 (`|SpawnActorFromClass` :`Class` "/Game/Fadeout_Content/Core/Characters/BP_Char_Raccoon.BP_Char_Raccoon_C" :`SpawnTransform` (`self.SpawnTransform`) :`CollisionHandlingOverride` "AdjustIfPossibleButAlwaysSpawn" :`TransformScaleMethod` "OverrideRootScale" :`Instigator` null))
      (`Controller.Possess` Controller _returnvalue_4))))

(fn `GameType to M_Gamestate`
  (params (`Game Type` :type "/Game/Fadeout_Content/Core/Support/Multiplayer_Support/DM_GameType Enum" :default "NewEnumerator0"))
  (bind _asmultiplayer_game_state (cast `/Game/Fadeout_Content/Core/Support/Multiplayer_Support/Multiplayer_GameState` (`GameplayStatics.GetGameState`)))
  (bind _output_get (set `/Game/Fadeout_Content/Core/Support/Multiplayer_Support/Multiplayer_GameState.ModeType` `Game Type` _asmultiplayer_game_state))
  (switch `/Game/Fadeout_Content/Core/Support/Multiplayer_Support/DM_GameType` _output_get
    (:`NewEnumerator0`
      (set `/Game/Fadeout_Content/Core/Support/Multiplayer_Support/Multiplayer_GameState.ModeName` "Free For All" _asmultiplayer_game_state))
    (:`NewEnumerator1`
      (set `/Game/Fadeout_Content/Core/Support/Multiplayer_Support/Multiplayer_GameState.ModeName` "Team Deathmatch" _asmultiplayer_game_state))
    (:`NewEnumerator2`
      (set `/Game/Fadeout_Content/Core/Support/Multiplayer_Support/Multiplayer_GameState.ModeName` "Capture The Flag" _asmultiplayer_game_state))))

(fn `Get Level Name`
  (bind _returnvalue (`GameplayStatics.GetCurrentLevelName` true))
  (set `self.levelName` _returnvalue))

(fn `Get Player Names`
  (`KismetArrayLibrary.Array_Clear` (`self.playerNames`))
  (for _array_element (`self.ConnectedPlayers`)
    (bind _asfo_player_state (cast `/Game/Fadeout_Content/Core/Support/Multiplayer_Support/FO_PlayerState` (`Controller.PlayerState` _array_element)))
    (`KismetArrayLibrary.Array_Add` (`self.playerNames`) (`KismetTextLibrary.Conv_TextToString` (`/Game/Fadeout_Content/Core/Support/Multiplayer_Support/FO_PlayerState.CustomName` _asfo_player_state))))
  (return))

(fn `Get Server Name`
  (bind _asfadeout_game_instance (cast `/Game/Fadeout_GameInstance` (`GameplayStatics.GetGameInstance`)))
  (set `self.serverName` (`KismetStringLibrary.Concat_StrStr` (`KismetTextLibrary.Conv_TextToString` (`/Game/Fadeout_GameInstance.MultiplayerName` _asfadeout_game_instance)) "s" " Server"))
  (return))

(fn `getAllyCountbyState`
  (returns (alliesAndStates :type "Map of /Game/Fadeout_Content/Core/Characters/BP_Ally Object Reference to /Game/Fadeout_Content/Core/Characters/RescueStates Enum") (escapedSince :type Integer))
  (locals (alliesAndState :type "Map of /Game/Fadeout_Content/Core/Characters/BP_Ally Object Reference to /Game/Fadeout_Content/Core/Characters/RescueStates Enum") (amountEscaped :type Integer))
  (for _array_element _
    (`/Engine/EditorBlueprintResources/StandardMacros.IsValid` _array_element
      (:`Is Valid`
        (`BlueprintMapLibrary.Map_Add` (`local.alliesAndState`) _array_element (`/Game/Fadeout_Content/Core/Characters/BP_Ally.RescueState` _array_element)))))
  (bind _values (`BlueprintMapLibrary.Map_Values` (`local.alliesAndState`)))
  (set `local.amountEscaped` 0)
  (for _array_element_2 _values
    (if (`|EnumEquality` _array_element_2 "NewEnumerator5")
      (`/Engine/EditorBlueprintResources/StandardMacros.IncrementInt` (`local.amountEscaped`))))
  (return (`local.alliesAndState`) (`local.amountEscaped`)))

(fn `GetPlayerName`
  (params (Object :type "Object Object Reference"))
  (returns (ReturnValue :type String) (`AsFO Player Controller` :type "/Game/Fadeout_Content/Core/FO_PlayerController Object Reference"))
  (bind _asfo_player_controller (cast `/Game/Fadeout_Content/Core/FO_PlayerController` Object))
  (bind _asfo_player_state (cast `/Game/Fadeout_Content/Core/Support/Multiplayer_Support/FO_PlayerState` (`Controller.PlayerState` _asfo_player_controller)))
  (return (`KismetStringLibrary.Concat_StrStr` (`KismetTextLibrary.Conv_TextToString` (`/Game/Fadeout_Content/Core/Support/Multiplayer_Support/FO_PlayerState.CustomName` _asfo_player_state)) " has joined the server.") _asfo_player_controller))

(fn `MSG_GetConnectedPlayers`
  (returns (Players :type "Array of Controller Object Reference"))
  (return (`self.ConnectedPlayers`)))

(fn `MSG_GetPlayerID`
  (returns (PlayerID :type Integer))
  (return 0))

(fn `MSG_GetPlayerIDFromUsername`
  (params (Username :type Text))
  (returns (PlayerID :type Integer))
  (locals (Local_PlayerID :type Integer))
  (for _array_element (`self.ConnectedPlayers`)
    (bind (_success_ _username) (message `/Game/AntizeChatSystem/Blueprints/BP_AntizeChatInterface.MSG_GetUsername` _array_element))
    (if _success_
      (if (`KismetTextLibrary.EqualEqual_TextText` _username Username)
        (bind _playerid (message `/Game/AntizeChatSystem/Blueprints/BP_AntizeChatInterface.MSG_GetPlayerID` _array_element))
        (set `local.Local_PlayerID` _playerid)
        (break))))
  (return (`local.Local_PlayerID`)))

(fn `MSG_GetTeamID`
  (returns (TeamID :type Integer))
  (return 0))

(fn `MSG_GetUsername`
  (returns (`Success?` :type Boolean) (Username :type Text))
  (return false ""))

(fn `MSG_RequestPrivateMessage`
  (params (Request :type "/Game/AntizeChatSystem/Logics/E_PrivateMEssage Enum" :default "NewEnumerator1") (ToPlayerID :type Integer) (Username :type Text) (Message :type Text))
  (returns (`Online?` :type Boolean))
  (locals (`Local_Online?` :type Boolean))
  (if (>= ToPlayerID 0)
    (switch `/Game/AntizeChatSystem/Logics/E_PrivateMEssage` Request
      (:`NewEnumerator1`
        _)
      (:`NewEnumerator3`
        _)
      (:`NewEnumerator0`
        (for _array_element (`self.ConnectedPlayers`)
          (bind _playerid (message `/Game/AntizeChatSystem/Blueprints/BP_AntizeChatInterface.MSG_GetPlayerID` _array_element))
          (if (== _playerid ToPlayerID)
            (set `local.Local_Online?` true)
            (break)))
        (return (`local.Local_Online?`)))
      (:`NewEnumerator4`
        _))
    (return (`local.Local_Online?`))
    (else
      (return (`local.Local_Online?`)))))

(fn `ReadyToEndMatch`
  (returns (ReturnValue :type Boolean))
  (return false))

(fn `ReadyToStartMatch`
  (returns (ReturnValue :type Boolean))
  (return true))

(fn `Team Balance`
  (params (PlayerController :type "Controller Object Reference"))
  (bind _asfo_player_state (cast `/Game/Fadeout_Content/Core/Support/Multiplayer_Support/FO_PlayerState` (`Controller.PlayerState` PlayerController)))
  (bind _asmultiplayer_game_state (cast `/Game/Fadeout_Content/Core/Support/Multiplayer_Support/Multiplayer_GameState` (`GameplayStatics.GetGameState`)))
  (`/Game/Fadeout_Content/Core/Support/Multiplayer_Support/Multiplayer_GameState.updatePlayerTeam` _asmultiplayer_game_state)
  (`/Engine/EditorBlueprintResources/StandardMacros.CompareInt` (`KismetArrayLibrary.Array_Length` (`/Game/Fadeout_Content/Core/Support/Multiplayer_Support/Multiplayer_GameState.RedPlayers` _asmultiplayer_game_state)) (`KismetArrayLibrary.Array_Length` (`/Game/Fadeout_Content/Core/Support/Multiplayer_Support/Multiplayer_GameState.BluePlayers` _asmultiplayer_game_state))
    (:`>`
      (set `/Game/Fadeout_Content/Core/Support/Multiplayer_Support/FO_PlayerState.Team` "blue" _asfo_player_state))
    (:`==`
      (set `/Game/Fadeout_Content/Core/Support/Multiplayer_Support/FO_PlayerState.Team` "red" _asfo_player_state))
    (:`<`
      (set `/Game/Fadeout_Content/Core/Support/Multiplayer_Support/FO_PlayerState.Team` "red" _asfo_player_state))))

(fn `UserConstructionScript`)