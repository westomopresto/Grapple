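; Game mode for Fadeout that spawns local players, applies startup display settings and tracks whether enemies have detected anyone.
; On BeginPlay it creates a player per the game instance's player count, possesses a spawned character for each, forces windowed resolution and caches checkpoints.
; Every tick it rebuilds the alerted enemy list by checking each tagged enemy's blackboard TargetActor, prints the count and sets a DANGER flag.
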(event `Spawn Players Event`
  (`self.spawnPlayersFunction`)
  (`WidgetBlueprintLibrary.SetInputMode_GameOnly` (`GameplayStatics.GetPlayerController` 0)))

(event `self.ReceiveBeginPlay`
  (`self.Spawn Players Event`)
  (bind _returnvalue (`GameUserSettings.GetGameUserSettings`))
  (`GameUserSettings.SetScreenResolution` _returnvalue (make `IntPoint` 1280 720))
  (`GameUserSettings.SetFullscreenMode` _returnvalue "Windowed")
  (`GameUserSettings.ApplySettings` _returnvalue true)
  (bind _outactors (`GameplayStatics.GetAllActorsOfClass` "/Game/Fadeout_Content/Core/Props/BP_Checkpoint.BP_Checkpoint_C"))
  (set `self.checkPoints` _outactors))

(event `self.ReceiveTick`
  (params (DeltaSeconds :type "Float (single-precision)"))
  (`KismetArrayLibrary.Array_Clear` (`self.alertedEnemies`))
  (bind _outactors (`BlueprintGameplayTagLibrary.GetAllActorsOfClassMatchingTagQuery` "/Game/Fadeout_Content/Core/Characters/BP_Enemy.BP_Enemy_C" (`BlueprintGameplayTagLibrary.MakeGameplayTagQuery` (struct :`TagDictionary` (struct :`(TagName` "enemy")) :`QueryTokenStream` "(0,1,1,1,0)" :`AutoDescription` " ANY( enemy )"))))
  (for _array_element _outactors
    (bind _asbp_enemy (cast `/Game/Fadeout_Content/Core/Characters/BP_Enemy` _array_element))
    (`/Engine/EditorBlueprintResources/StandardMacros.IsValid` (`BlackboardComponent.GetValueAsObject` (`AIBlueprintHelperLibrary.GetBlackboard` _asbp_enemy) "TargetActor")
      (:`Is Valid`
        (`KismetArrayLibrary.Array_AddUnique` (`self.alertedEnemies`) _array_element))))
  (bind _output_get (set `self.alertedCount` (`KismetArrayLibrary.Array_Length` (`self.alertedEnemies`))))
  (`KismetSystemLibrary.PrintString` (`KismetStringLibrary.BuildString_Int` "" "" _output_get "Enemies see you") true true (struct :`G` 0.66 :`B` 1.0 :`A` 1.0) 0.01)
  (if (> _output_get 0)
    (set `self.DANGER?` true)
    (else
      (set `self.DANGER?` false))))

(fn `spawnPlayersFunction`
  (bind _asfadeout_game_instance (cast `/Game/Fadeout_GameInstance` (`GameplayStatics.GetGameInstance`)))
  (bind _returnvalue (- (`/Game/Fadeout_GameInstance.numberOfPlayers` _asfadeout_game_instance) 1))
  (for _index (range (+ _returnvalue 1))
    (`GameplayStatics.CreatePlayer` _index (not (== _index 0))))
  (for _index_2 (range (+ _returnvalue 1))
    (bind _returnvalue_2 (`|SpawnActorFromClass` "/Game/Fadeout_Content/Core/Characters/BP_PlayerCharacter.BP_PlayerCharacter_C" (`KismetMathLibrary.MakeTransform` (0.0 0.0 1.0)) "Undefined" "OverrideRootScale" null _index_2 null))
    (`Controller.Possess` (`GameplayStatics.GetPlayerController` _index_2) _returnvalue_2)))

(fn `UserConstructionScript`)