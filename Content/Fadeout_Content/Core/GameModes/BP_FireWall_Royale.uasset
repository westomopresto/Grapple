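; BP_FireWall_Royale is the safe-zone boundary for a royale game mode, damaging players who leave its cylinder.
; Cylinder overlap events maintain an UnsafePlayers list, adding a BP_PlayerCharacter on exit and removing it on entry.
; A looping one-second timer applies fixed damage with DT_BrushOff to each valid listed player, passing that player's own controller as instigator.
; The Blueprint contains no movement or shrinking logic.
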(event `self.ReceiveBeginPlay`
  (`KismetSystemLibrary.K2_SetTimerDelegate` (delegate `Player Check`) 1.0 true 1.0))

(event `Player Check`
  (for _array_element (`self.Unsafe Players`)
    (`/Engine/EditorBlueprintResources/StandardMacros.IsValid` _array_element
      (:`Is Valid`
        (`GameplayStatics.ApplyDamage` _array_element 40.0 (`Pawn.GetController` _array_element) self "/Game/Fadeout_Content/Core/Weapons/DamageTypes/DT_BrushOff.DT_BrushOff_C")))))

(event `self.Cylinder.OnComponentBeginOverlap`
  (params (OverlappedComponent :type "PrimitiveComponent Object Reference") (OtherActor :type "Actor Object Reference") (OtherComp :type "PrimitiveComponent Object Reference") (OtherBodyIndex :type Integer) (bFromSweep :type Boolean) (SweepResult :type "HitResult Structure (by ref)"))
  (bind _asbp_player_character (cast `/Game/Fadeout_Content/Core/Characters/BP_PlayerCharacter` OtherActor))
  (`KismetArrayLibrary.Array_RemoveItem` (`self.Unsafe Players`) _asbp_player_character))

(event `self.Cylinder.OnComponentEndOverlap`
  (params (OverlappedComponent :type "PrimitiveComponent Object Reference") (OtherActor :type "Actor Object Reference") (OtherComp :type "PrimitiveComponent Object Reference") (OtherBodyIndex :type Integer))
  (bind _asbp_player_character (cast `/Game/Fadeout_Content/Core/Characters/BP_PlayerCharacter` OtherActor))
  (`KismetArrayLibrary.Array_AddUnique` (`self.Unsafe Players`) _asbp_player_character))

(fn `UserConstructionScript`)