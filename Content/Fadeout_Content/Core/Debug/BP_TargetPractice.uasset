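; BP_TargetPractice is a debug moving target that displays the damage dealt to it.
; A looping Movement timeline, with play rate set by Speed, moves the Offset component to local-space positions along the Spline.
; Any damage spawns a BP_FloatingDamageNumber at Offset with the truncated amount, owned by the damage instigator.
; The construction script detaches the Spline, keeping its world transform.
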(event `self.ReceiveBeginPlay`
  (`|ExecutionSequence`
    (:`then_0`
      (`TimelineComponent.SetPlayRate` (`self.Movement`) (`self.Speed`)))
    (:`then_1`
      (bind (_direction _timealpha) (`Timeline|Movement` :!via `PlayFromStart` :!label _label)
        (:`Update`
          (`SceneComponent.K2_SetRelativeLocation` (`self.Offset`) (.location (`SplineComponent.GetTransformAtTime` (`self.Spline`) _timealpha "Local" false false)) false false))
        (:`Finished`
          (goto _label :!via `PlayFromStart`))))))

(event `self.ReceiveAnyDamage`
  (params (Damage :type "Float (single-precision)") (DamageType :type "DamageType Object Reference") (InstigatedBy :type "Controller Object Reference") (DamageCauser :type "Actor Object Reference"))
  (bind _returnvalue (`SceneComponent.K2_GetComponentToWorld` (`self.Offset`)))
  (`|SpawnActorFromClass` "/Game/Fadeout_Content/Core/Support/BP_FloatingDamageNumber.BP_FloatingDamageNumber_C" _returnvalue "Undefined" "OverrideRootScale" InstigatedBy (.location _returnvalue) (`KismetMathLibrary.FTrunc` Damage) (`Actor.Instigator` DamageCauser)))

(fn `UserConstructionScript`
  (`SceneComponent.K2_DetachFromComponent` (`self.Spline`) "KeepWorld" "KeepWorld" "KeepWorld" true))