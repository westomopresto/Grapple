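; Tutorial barrier that checks whether the player character has a specific weapon.
; Its CheckforPlayerProperty event searches the character's Equipment for an item whose class exactly matches WeaponClass, stopping at the first match.
; A match calls CheckSucceeded, and the Blueprint contains no other active logic.
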(event `self.Check for Player Property`
  (params (`BP Player Character` :type "/Game/Fadeout_Content/Core/Characters/BP_PlayerCharacter Object Reference"))
  (for _array_element (`/Game/Fadeout_Content/Core/Characters/BP_PlayerCharacter.equipment` `BP Player Character`)
    (bind _output_get (set `self.found` (== (`GameplayStatics.GetObjectClass` _array_element) (`self.Weapon Class`))))
    (if _output_get
      (break)))
  (if (`self.found`)
    (`self.Check Succeeded`)))

(fn `UserConstructionScript`
  (`parent.UserConstructionScript`))