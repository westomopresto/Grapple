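; Tutorial check that succeeds once a required number of NPCs from its assigned spawners have been killed.
; On BeginPlay it binds to the NPC death event of each spawner in NPCSpawners.
; Each death increments the kill count, turns off CanSpawn on the object passed by the event, and calls CheckSucceeded once RequiredKills is reached.
; The CheckforPlayerProperty event is left empty, so progress is driven only by death events.
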(event `self.ReceiveBeginPlay`
  (for _array_element (`self.NPC_Spawners`)
    (add `/Game/Fadeout_Content/Core/Props/NPC_Spawner.SpawnerNPC_Died` _array_element (delegate `SpawnerNPC_Died`))))

(event `SpawnerNPC_Died`
  (params (NewParam :type "/Game/Fadeout_Content/Core/Props/NPC_Spawner Object Reference"))
  (bind _result (`/Engine/EditorBlueprintResources/StandardMacros.IncrementInt` (`self.NPCsKilled`))
    (:`  `
      (set `/Game/Fadeout_Content/Core/Props/NPC_Spawner.CanSpawn` false NewParam)
      (if (>= _result (`self.RequiredKills`))
        (`self.Check Succeeded`)))))

(event `self.Check for Player Property`
  (params (`BP Player Character` :type "/Game/Fadeout_Content/Core/Characters/BP_PlayerCharacter Object Reference")))

(fn `UserConstructionScript`
  (`parent.UserConstructionScript`))