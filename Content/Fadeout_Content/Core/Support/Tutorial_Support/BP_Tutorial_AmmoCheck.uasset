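; Tutorial check that passes when the player character is carrying full pistol and rifle ammo.
; Its CheckforPlayerProperty event compares the character's held ammo to the maximum for both types.
; It calls CheckSucceeded only when both are at or above their limits.
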(event `self.Check for Player Property`
  (params (`BP Player Character` :type "/Game/Fadeout_Content/Core/Characters/BP_PlayerCharacter Object Reference"))
  (bind (_tntammo _pistolammo _fuelammo _rifleammo) (break `/Game/Fadeout_Content/Core/Support/AmmoStruct` (`/Game/Fadeout_Content/Core/Characters/BP_PlayerCharacter.MaxHeldAmmo` `BP Player Character`)))
  (bind (_tntammo_2 _pistolammo_2 _fuelammo_2 _rifleammo_2) (break `/Game/Fadeout_Content/Core/Support/AmmoStruct` (`/Game/Fadeout_Content/Core/Characters/BP_PlayerCharacter.HeldAmmo` `BP Player Character`)))
  (if (and (>= _pistolammo_2 _pistolammo) (>= _rifleammo_2 _rifleammo))
    (`self.Check Succeeded`)))

(fn `UserConstructionScript`
  (`parent.UserConstructionScript`))