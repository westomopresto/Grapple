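; World-placed tutorial button prompt actor that shows the key or button bound to a configurable ActionName through its widget component.
; On BeginPlay it binds to FO_PlayerController's gamepad-notify dispatcher.
; Each notification switches the Widget_Tutorial_Button label between gamepad and keyboard key groups, sets the action and refreshes it.
; The construction script writes ActionName into a TextRender component.
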(event `self.ReceiveBeginPlay`
  (bind _asfo_player_controller (cast `/Game/Fadeout_Content/Core/FO_PlayerController` (`GameplayStatics.GetPlayerController` 0)))
  (add `/Game/Fadeout_Content/Core/FO_PlayerController.Gamepad Notify Dispatcher` _asfo_player_controller (delegate `ButtonPressCheck`)))

(event `ButtonPressCheck`
  (params (bGamepad :type Boolean))
  (bind _aswidget_tutorial_button (cast `/Game/Fadeout_Content/Core/Support/Tutorial_Support/Widget_Tutorial_Button` (`WidgetComponent.GetUserWidgetObject` (`self.Widget`))))
  (bind _defaultactionlabel (`/Game/Fadeout_Content/Core/Support/Tutorial_Support/Widget_Tutorial_Button.DefaultActionLabel` _aswidget_tutorial_button))
  (set `InputLabel.MappingGroup` -1 _defaultactionlabel)
  (set `InputLabel.KeyGroup` (select `bool` bGamepad :`false` (struct :`TagName` "Keyboard Group") :`true` (struct :`TagName` "Gamepad Buttons") :!type "GameplayTag Structure") _defaultactionlabel)
  (set `ActionLabel.ActionName` (`self.ActionName`) _defaultactionlabel)
  (`InputLabel.UpdateLabel` _defaultactionlabel))

(fn `UserConstructionScript`
  (`TextRenderComponent.K2_SetText` (`self.TextRender`) (`KismetTextLibrary.Conv_NameToText` (`self.ActionName`))))