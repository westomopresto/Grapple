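; Tutorial barrier actor that only opens when the player character hits it while rolling.
; On a hit against its Cube, it casts to BP_PlayerCharacter and checks whether the current montage's object name contains "roll".
; On success it switches the Cube to a green hologram material, plays a wrench hit sound and disables collision so the player can pass.
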(event `Check for Player Property`
  (params (`BP Player Character` :type "/Game/Fadeout_Content/Core/Characters/BP_PlayerCharacter Object Reference"))
  (bind _returnvalue (`Character.GetCurrentMontage` `BP Player Character`))
  (if (`KismetStringLibrary.Contains` (`KismetSystemLibrary.GetObjectName` _returnvalue) "roll")
    (`self.Check Succeeded`)))

(event `Check Succeeded`
  (bind _cube (`self.Cube`))
  (`PrimitiveComponent.SetMaterial` _cube 0 "/Game/Fadeout_Content/Core/Props/Capture_Points/M_Holo_Green.M_Holo_Green")
  (`GameplayStatics.PlaySound2D` "/Game/Fadeout_Content/Core/FBX/Wrench/wrenchHit.wrenchHit" 1.0 1.0 0.0 null null)
  (`PrimitiveComponent.SetCollisionEnabled` _cube "NoCollision"))

(event `self.Cube.OnComponentHit`
  (params (HitComponent :type "PrimitiveComponent Object Reference") (OtherActor :type "Actor Object Reference") (OtherComp :type "PrimitiveComponent Object Reference") (NormalImpulse :type "Vector Structure") (Hit :type "HitResult Structure (by ref)"))
  (bind _asbp_player_character (cast `/Game/Fadeout_Content/Core/Characters/BP_PlayerCharacter` OtherActor))
  (`self.Check for Player Property` _asbp_player_character))

(fn `UserConstructionScript`)