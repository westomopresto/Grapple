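; Tutorial step actor that runs one voiced, on-screen instruction between a start trigger and an end trigger.
; The player overlapping Start_Trigger once starts voice lines through BP_Tutorial_Persist, shows a speaking widget, and binds a retry line to player death.
; The step completes via End_Trigger or when a looping timer finds no objectives remaining.
; Completion fires StepCompleted, clears the timer, resets the count, and gives praise.
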(event `Start Step`
  (bind _tutorial_persist (`self.Tutorial_Persist`))
  ;[1 1 1] Step
  (`/Game/Fadeout_Content/Core/Support/Tutorial_Support/BP_Tutorial_Persist.Play Tutorial Voice Lines` _tutorial_persist (`self.VoiceLine`))
  (add `/Game/Fadeout_Content/Core/Support/Tutorial_Support/BP_Tutorial_Persist.LastLineSpokenFinished` _tutorial_persist (delegate `Line Spoken Finished Event`))
  (`self.Start Watching`)
  (`self.PushMessage` (`self.tutorialStep`)))

(event `Line Spoken Finished Event`
  ;[1 1 1] Step
)

(event `Start Watching`
  (add `/Game/Fadeout_Content/Core/Characters/BP_PlayerCharacter.OnDeath` (`self.PlayerPawn`) (delegate `Died`))
  (bind _returnvalue (`KismetSystemLibrary.K2_SetTimerDelegate` (delegate `ObjectiveTick`) 0.2 true))
  (set `self.objectiveTimer` _returnvalue))

(event `Died`
  (params (`Killer Actor` :type "Actor Object Reference") (`Death location` :type "Transform Structure") (`Damage Type` :type "/Game/Fadeout_Content/Core/Weapons/DamageTypes Enum" :default "NewEnumerator0"))
  (`/Game/Fadeout_Content/Core/Support/Tutorial_Support/BP_Tutorial_Persist.Play Tutorial Voice Lines` (`self.Tutorial_Persist`) "/Game/Fadeout_Content/Core/Support/Tutorial_Support/Abby_Tutorial_lines/retry_Oops.retry_Oops"))

(event `Step Complete`
  (bind _tutorial_widget (`self.tutorial_widget`)
    (:`then`
      (`Widget.RemoveFromParent` _tutorial_widget))
    (:`else`
      _))
  (`self.Step Completed`)
  (`KismetSystemLibrary.K2_ClearAndInvalidateTimerHandle` (`self.objectiveTimer`))
  (set `self.objectivesRemain` (`self.objectiveAmount`))
  (`self.PushMessage` "nicejob")
  (`/Game/Fadeout_Content/Core/Support/Tutorial_Support/BP_Tutorial_Persist.Play Tutorial Voice Lines` (`self.Tutorial_Persist`) "/Game/Fadeout_Content/Core/Support/Tutorial_Support/Abby_Tutorial_lines/NiceJob_01_Cue.NiceJob_01_Cue"))

(event `ObjectiveTick`
  (if (<= (`self.objectivesRemain`) 0)
    (`self.Step Complete`)))

(event `self.End_Trigger.OnActorBeginOverlap`
  (params (OverlappedActor :type "Actor Object Reference") (OtherActor :type "Actor Object Reference"))
  (bind _asbp_player_character (cast `/Game/Fadeout_Content/Core/Characters/BP_PlayerCharacter` OtherActor))
  (if (== (`self.PlayerPawn`) _asbp_player_character)
    (`/Engine/EditorBlueprintResources/StandardMacros.DoOnce` false :!label _label
      (:`Completed`
        (`self.Step Complete`)))))

(event `self.End_Trigger.OnActorEndOverlap`
  (params (OverlappedActor :type "Actor Object Reference") (OtherActor :type "Actor Object Reference"))
  (bind _asbp_player_character (cast `/Game/Fadeout_Content/Core/Characters/BP_PlayerCharacter` OtherActor))
  (if (== (`self.PlayerPawn`) _asbp_player_character)
    (goto _label)))

(event `self.Start_Trigger.OnActorBeginOverlap`
  (params (OverlappedActor :type "Actor Object Reference") (OtherActor :type "Actor Object Reference"))
  (bind _asbp_player_character (cast `/Game/Fadeout_Content/Core/Characters/BP_PlayerCharacter` OtherActor))
  (if (== (`self.PlayerPawn`) _asbp_player_character)
    (`/Engine/EditorBlueprintResources/StandardMacros.DoOnce` false :!label _label_2
      (:`Completed`
        (`self.Start Step`)))))

(event `self.Start_Trigger.OnActorEndOverlap`
  (params (OverlappedActor :type "Actor Object Reference") (OtherActor :type "Actor Object Reference"))
  (bind _asbp_player_character (cast `/Game/Fadeout_Content/Core/Characters/BP_PlayerCharacter` OtherActor))
  (if (== (`self.PlayerPawn`) _asbp_player_character)
    (goto _label_2)))

(event `self.ReceiveBeginPlay`
  (`KismetSystemLibrary.K2_SetTimerDelegate` (delegate `GetPlayerPawn`) 0.1 true)
  (`self.GetPlayerPawn`)
  (set `self.objectivesRemain` (`self.objectiveAmount`)))

(event `GetPlayerPawn`
  (`self.PlayerPawn`
    (:`then`)
    (:`else`
      (bind _asbp_player_character (cast `/Game/Fadeout_Content/Core/Characters/BP_PlayerCharacter` (`GameplayStatics.GetPlayerPawn` 0)))
      (set `self.PlayerPawn` _asbp_player_character))))

(fn `PushMessage`
  (params (tutorial_step :type Name))
  (bind _returnvalue (`|CreateWidget` "/Game/Fadeout_Content/Core/Support/Tutorial_Support/Widget_Tutorial_Speaking.Widget_Tutorial_Speaking_C" (`GameplayStatics.GetPlayerController` 0) tutorial_step))
  (set `self.tutorial_widget` _returnvalue)
  (bind _tutorial_widget (`self.tutorial_widget`)
    (:`then`
      (`UserWidget.AddToViewport` _tutorial_widget 99))
    (:`else`)))

(fn `UserConstructionScript`
  (bind _outactors (`GameplayStatics.GetAllActorsOfClass` "/Game/Fadeout_Content/Core/Support/Tutorial_Support/BP_Tutorial_Persist.BP_Tutorial_Persist_C"))
  (set `self.Tutorial_Persist` (`|GetArrayItem` _outactors)))