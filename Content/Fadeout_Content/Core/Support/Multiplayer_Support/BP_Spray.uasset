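; BP_Spray is a spray-paint decal actor that displays a texture where it is placed or spawned.
; Its construction script calls SetSpray, which creates a dynamic instance of M_Spray_inst, feeds the Texture variable into it and applies it to the Decal component.
; On BeginPlay it spawns a scaled-up smoke emitter and plays a spray can sound at its location.
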(event `self.ReceiveBeginPlay`
  (bind _returnvalue (`self.K2_GetActorLocation`))
  (`GameplayStatics.SpawnEmitterAtLocation` "/Game/Fadeout_Content/Core/FX/particle_footSmoke.particle_footSmoke" _returnvalue (struct) (5.0 5.0 5.0))
  (`GameplayStatics.PlaySoundAtLocation` "/Game/Fadeout_Content/Core/Audio/SprayCan_SFX/spraycan_01_Cue.spraycan_01_Cue" _returnvalue (struct) 1.0 1.0 0.0 null null null))

(fn `SetSpray`
  (bind _returnvalue (`KismetMaterialLibrary.CreateDynamicMaterialInstance` "/Game/Fadeout_Content/Core/Decals/M_Spray_inst.M_Spray_inst"))
  (`MaterialInstanceDynamic.SetTextureParameterValue` _returnvalue "Texture" (`self.texture`))
  (`DecalComponent.SetDecalMaterial` (`self.Decal`) _returnvalue))

(fn `UserConstructionScript`
  (`self.SetSpray`))