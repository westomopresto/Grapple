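; Character select preview actor in the multiplayer support content that shows a dummy of the selected character (Mouse, Snek or Bunn).
; SpawnCharacter destroys any existing dummy, then passes the selection to the spawn event.
; That event switches on the selection, spawns the matching dummy Blueprint at the SpawnPoint transform regardless of collisions, and stores it in Char for later replacement.
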(event `Spawn Character`
  (params (selected :type "/Game/Fadeout_Content/Core/Support/Multiplayer_Support/CharactersSelected Enum" :default "NewEnumerator0"))
  (bind _char (`self.char`))
  (`/Engine/EditorBlueprintResources/StandardMacros.IsValid` _char
    (:`Is Valid`
      (`self.K2_DestroyActor` _char))
    (:`Is Not Valid`
      _))
  (`self.spawn` selected))

(event `spawn`
  (params (Selection :type "/Game/Fadeout_Content/Core/Support/Multiplayer_Support/CharactersSelected Enum" :default "NewEnumerator0"))
  (bind _returnvalue (`SceneComponent.K2_GetComponentToWorld` (`self.spawn point`)))
  (switch `/Game/Fadeout_Content/Core/Support/Multiplayer_Support/CharactersSelected` Selection
    (:`NewEnumerator0`
      (bind _returnvalue_2 (`|SpawnActorFromClass` "/Game/Fadeout_Content/Core/Characters/dummies/BP_mouse_dummy.BP_mouse_dummy_C" _returnvalue "AlwaysSpawn" "OverrideRootScale" null 0 null))
      (set `self.char` _returnvalue_2))
    (:`NewEnumerator1`
      (bind _returnvalue_3 (`|SpawnActorFromClass` "/Game/Fadeout_Content/Core/Characters/dummies/BP_snek_dummy.BP_snek_dummy_C" _returnvalue "AlwaysSpawn" "OverrideRootScale" null 0 null))
      (set `self.char` _returnvalue_3))
    (:`NewEnumerator2`
      (bind _returnvalue_4 (`|SpawnActorFromClass` "/Game/Fadeout_Content/Core/Characters/dummies/BP_bunn_dummy.BP_bunn_dummy_C" _returnvalue "AlwaysSpawn" "OverrideRootScale" null 0 null))
      (set `self.char` _returnvalue_4))))

(fn `UserConstructionScript`)