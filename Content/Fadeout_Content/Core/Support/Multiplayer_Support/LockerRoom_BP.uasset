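; LockerRoom_BP is a locker room actor that displays a dummy character for the selected species: Mouse, Snek or Bunn.
; It shows Mouse on BeginPlay, and SpawnCharacter destroys the current dummy before spawning the requested one at SpawnPoint.
; Each dummy spawns with the unarmed starter weapon and a NameManager call with a blank name and Spawn off.
; Only Snek also calls EquipItemFunction after spawning.
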(event `self.ReceiveBeginPlay`
  (`self.Spawn Character` "NewEnumerator0"))

(event `Spawn Character`
  (params (selected :type "/Game/Fadeout_Content/Core/Support/Multiplayer_Support/CharactersSelected Enum" :default "NewEnumerator0"))
  (bind _char (`self.char`))
  (`/Engine/EditorBlueprintResources/StandardMacros.IsValid` _char
    (:`Is Valid`
      (`self.K2_DestroyActor` _char))
    (:`Is Not Valid`
      _))
  (`self.spawn` selected))

(event `spawn`
  (params (Selection :type "/Game/Fadeout_Content/Core/Support/Multiplayer_Support/CharactersSelected Enum" :default "NewEnumerator0"))
  (bind _returnvalue (`SceneComponent.K2_GetComponentToWorld` (`self.spawn point`)))
  (switch `/Game/Fadeout_Content/Core/Support/Multiplayer_Support/CharactersSelected` Selection
    (:`NewEnumerator0`
      (bind _returnvalue_2 (`|SpawnActorFromClass` "/Game/Fadeout_Content/Core/Characters/dummies/BP_mouse_dummy.BP_mouse_dummy_C" _returnvalue "AlwaysSpawn" "OverrideRootScale" null (`|MakeArray` "/Game/Fadeout_Content/Core/Weapons/BP_Unarmed.BP_Unarmed_C" :!type "/Game/Fadeout_Content/Core/Weapons/BP_weaponBase Class Reference") 0 true null))
      (bind _output_get (set `self.char` _returnvalue_2))
      (`/Game/Fadeout_Content/Core/Characters/BP_PlayerCharacter.name manager` _output_get false ""))
    (:`NewEnumerator1`
      (bind _returnvalue_3 (`|SpawnActorFromClass` "/Game/Fadeout_Content/Core/Characters/dummies/BP_snek_dummy.BP_snek_dummy_C" _returnvalue "AlwaysSpawn" "OverrideRootScale" null (`|MakeArray` "/Game/Fadeout_Content/Core/Weapons/BP_Unarmed.BP_Unarmed_C" :!type "/Game/Fadeout_Content/Core/Weapons/BP_weaponBase Class Reference") 0 true null))
      (bind _output_get_2 (set `self.char` _returnvalue_3))
      (`/Game/Fadeout_Content/Core/Characters/BP_PlayerCharacter.name manager` _output_get_2 false "")
      (`/Game/Fadeout_Content/Core/Characters/BP_PlayerCharacter.EquipItemFunction` _output_get_2 0))
    (:`NewEnumerator2`
      (bind _returnvalue_4 (`|SpawnActorFromClass` "/Game/Fadeout_Content/Core/Characters/dummies/BP_bunn_dummy.BP_bunn_dummy_C" _returnvalue "AlwaysSpawn" "OverrideRootScale" null (`|MakeArray` "/Game/Fadeout_Content/Core/Weapons/BP_Unarmed.BP_Unarmed_C" :!type "/Game/Fadeout_Content/Core/Weapons/BP_weaponBase Class Reference") 0 true null))
      (bind _output_get_3 (set `self.char` _returnvalue_4))
      (`/Game/Fadeout_Content/Core/Characters/BP_PlayerCharacter.name manager` _output_get_3 false ""))))

(fn `UserConstructionScript`)