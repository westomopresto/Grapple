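; Floating nameplate actor showing a player's name in team or custom color, destroying itself on dedicated servers and for the local player.
; Tick always shows non-FFA teammates with a health bar; others need camera distance and line-of-sight checks.
; Outside teammate mode, a cloaked BP_Char_Bingo stays hidden unless in combat.
; Name and team refresh every few seconds, destroying the actor if the instigator's PlayerState is invalid.
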(event `Check Name`
  (bind _playerstate (`self.playerstate`))
  (`/Engine/EditorBlueprintResources/StandardMacros.IsValid` (`Pawn.PlayerState` (`self.GetInstigator`))
    (:`Is Valid`
      (`/Engine/EditorBlueprintResources/StandardMacros.IsValid` _playerstate
        (:`Is Valid`
          (set `self.name` (`/Game/Fadeout_Content/Core/Support/Multiplayer_Support/FO_PlayerState.CustomName` _playerstate))
          (set `self.team` (`/Game/Fadeout_Content/Core/Support/Multiplayer_Support/FO_PlayerState.Team` _playerstate)))
        (:`Is Not Valid`
          _))
      (bind _asname_widget (cast `/Game/Fadeout_Content/Core/Support/Name_Widget` (`WidgetComponent.GetUserWidgetObject` (`self.NameUI`)) :!label _label))
      (set `/Game/Fadeout_Content/Core/Support/Name_Widget.name` (`self.name`) _asname_widget)
      (set `/Game/Fadeout_Content/Core/Support/Name_Widget.nameColor` (`self.color`) _asname_widget)
      (switch `string` (`self.team`)
        (:`FFA`
          (`/Engine/EditorBlueprintResources/StandardMacros.IsValid` (`self.playerstate`)
            (:`Is Valid`
              (set `/Game/Fadeout_Content/Core/Support/Name_Widget.nameColor` (make `SlateColor` (`KismetMathLibrary.Conv_ColorToLinearColor` (`/Game/Fadeout_Content/Core/Support/Multiplayer_Support/FO_PlayerState.CustomColor` _playerstate))) _asname_widget))
            (:`Is Not Valid`
              (set `/Game/Fadeout_Content/Core/Support/Name_Widget.nameColor` (make `SlateColor` (struct :`R` 1.0 :`G` 1.0 :`B` 1.0 :`A` 1.0)) _asname_widget))))
        (:`blue`
          (set `/Game/Fadeout_Content/Core/Support/Name_Widget.nameColor` (make `SlateColor` (struct :`G` 0.375397 :`B` 1.0 :`A` 1.0)) _asname_widget))
        (:`red`
          (set `/Game/Fadeout_Content/Core/Support/Name_Widget.nameColor` (make `SlateColor` (struct :`R` 1.0 :`B` 0.020101 :`A` 1.0)) _asname_widget))))
    (:`Is Not Valid`
      (`self.K2_DestroyActor`))))

(event `self.ReceiveBeginPlay`
  (goto _label))

(event `Check name event`
  (params (deltaTime :type "Float (double-precision)"))
  (bind _output_get (set `self.nametime` (+ deltaTime (`self.nametime`))))
  (if (> _output_get 3.0)
    (set `self.nametime` 0.0)
    (`self.Check Name`)))

(event `self.ReceiveTick`
  (params (DeltaSeconds :type "Float (single-precision)"))
  (if (`KismetSystemLibrary.IsDedicatedServer`)
    (`self.K2_DestroyActor`)
    (else
      (`/Engine/EditorBlueprintResources/StandardMacros.IsValid` (`GameplayStatics.GetPlayerController` 0)
        (:`Is Valid`
          (bind _your_own_name (`self.Own Name Check`))
          (if _your_own_name
            (`self.K2_DestroyActor`)
            (else
              (`|ExecutionSequence`
                (:`then_0`
                  (`self.Make HP Visible` false))
                (:`then_1`
                  (bind (_ffa_ _same_team_) (`self.Team Check`))
                  (if _same_team_
                    (if _ffa_
                      ;[1 1 1] FFA mode
                      (bind _closerange (`self.Distance Check` 1500.0))
                      (if _closerange
                        (bind _blocked (`self.CameraVisible`))
                        (`self.Make Name Visible` (not _blocked))
                        (else
                          (`self.Make Name Visible` _closerange)))
                      (else
                        ;[1 1 1] Teammate mode
                        (`self.Make Name Visible` true true)
                        (`self.Make HP Visible` true)
                        (`self.Set Health Bar`)))
                    (else
                      ;[1 1 1] Regular Distance Mode
                      (bind _closerange_2 (`self.Distance Check` 1500.0))
                      (if _closerange_2
                        (bind _blocked_2 (`self.CameraVisible`))
                        (`self.Make Name Visible` (not _blocked_2))
                        (else
                          (`self.Make Name Visible` _closerange_2))))))
                (:`then_2`
                  (`self.Check name event` DeltaSeconds))))))))))

(event `Set Health Bar`
  (bind _playerstate (`Pawn.PlayerState` (`self.GetInstigator`)))
  (`/Engine/EditorBlueprintResources/StandardMacros.IsValid` _playerstate
    (:`Is Valid`
      (bind _asbp_player_character (cast `/Game/Fadeout_Content/Core/Characters/BP_PlayerCharacter` (`PlayerState.PawnPrivate` _playerstate)))
      (set `/Game/Fadeout_Content/Core/Support/Name_Widget.healthNormalized` (/ (`/Game/Fadeout_Content/Core/Characters/BP_PlayerCharacter.health` _asbp_player_character) (`/Game/Fadeout_Content/Core/Characters/BP_PlayerCharacter.maxHealth` _asbp_player_character)) (cast `/Game/Fadeout_Content/Core/Support/Name_Widget` (`WidgetComponent.GetUserWidgetObject` (`self.NameUI`)) :!pure true)))))

(fn `CameraVisible`
  (returns (Blocked :type Boolean))
  (bind _playercameramanager (`PlayerController.PlayerCameraManager` (`GameplayStatics.GetPlayerController` 0)))
  (`/Engine/EditorBlueprintResources/StandardMacros.IsValid` _playercameramanager
    (:`Is Valid`
      (bind (_outhit _returnvalue) (`KismetSystemLibrary.LineTraceSingle` :`Start` (`self.K2_GetActorLocation` self) :`End` (`PlayerCameraManager.GetCameraLocation` _playercameramanager) :`TraceChannel` "TraceTypeQuery1" :`DrawDebugType` "ForOneFrame"))
      (return _returnvalue))))

(fn `Distance Check`
  (params (Distance :type "Float (double-precision)" :default 1500.0))
  (returns (CloseRange :type Boolean))
  (return (< (`KismetMathLibrary.Vector_Distance` (`self.K2_GetActorLocation` self) (`PlayerCameraManager.GetCameraLocation` (`PlayerController.PlayerCameraManager` (`GameplayStatics.GetPlayerController` 0)))) Distance)))

(fn `Make HP Visible`
  (params (`Visible?` :type Boolean))
  (bind _nameui (`self.NameUI`))
  (bind _hpbar (`/Game/Fadeout_Content/Core/Support/Name_Widget.hpbar` (cast `/Game/Fadeout_Content/Core/Support/Name_Widget` (`WidgetComponent.GetUserWidgetObject` _nameui) :!pure true)))
  (`/Engine/EditorBlueprintResources/StandardMacros.IsValid` _nameui
    (:`Is Valid`
      (if `Visible?`
        (`Widget.SetVisibility` _hpbar "HitTestInvisible")
        (return)
        (else
          (`Widget.SetVisibility` _hpbar "Hidden")
          (return))))
    (:`Is Not Valid`
      (return))))

(fn `Make Name Visible`
  (params (`Name Visible` :type Boolean) (`TeamMode?` :type Boolean))
  (bind _nameui (`self.NameUI`))
  (bind _asbp_char_bingo (cast `/Game/Fadeout_Content/Core/Characters/BP_Char_Bingo` (`self.GetInstigator`))
    (:`then`
      (if `TeamMode?`
        (`SceneComponent.SetVisibility` _nameui `Name Visible` false :!label _label)
        (else
          (`SceneComponent.SetVisibility` _nameui (and (or (`/Game/Fadeout_Content/Core/Characters/BP_PlayerCharacter.inCOMBAT` _asbp_char_bingo) (not (`/Game/Fadeout_Content/Core/Characters/BP_PlayerCharacter.isCloaked` _asbp_char_bingo))) `Name Visible`) false))))
    (:`CastFailed`
      (goto _label))))

(fn `Own Name Check`
  (returns (`Your own name` :type Boolean))
  (bind _returnvalue (`self.GetInstigator`))
  (bind _returnvalue_2 (`GameplayStatics.GetPlayerController` 0))
  (if (and (`KismetSystemLibrary.IsValid` _returnvalue) (`KismetSystemLibrary.IsValid` (`Pawn.PlayerState` _returnvalue)) (`KismetSystemLibrary.IsValid` _returnvalue_2) (`KismetSystemLibrary.IsValid` (`Controller.PlayerState` _returnvalue_2)))
    (return (== (`PlayerState.PlayerId` (`Pawn.PlayerState` (`self.GetInstigator`))) (`PlayerState.PlayerId` (`Controller.PlayerState` (`GameplayStatics.GetPlayerController` 0)))))))

(fn `Team Check`
  (returns (`FFA?` :type Boolean) (`Same Team?` :type Boolean))
  (bind _asfo_player_state (cast `/Game/Fadeout_Content/Core/Support/Multiplayer_Support/FO_PlayerState` (`Controller.PlayerState` (`GameplayStatics.GetPlayerController` 0))))
  (bind _team (`/Game/Fadeout_Content/Core/Support/Multiplayer_Support/FO_PlayerState.Team` _asfo_player_state))
  (return (`KismetStringLibrary.EqualEqual_StrStr` _team "FFA") (`KismetStringLibrary.EqualEqual_StrStr` _team (`self.team`))))

(fn `UserConstructionScript`)