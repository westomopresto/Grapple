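; BP_FloatingDamageNumber is a world actor that shows a damage number rising and fading, then destroys itself.
; Each update pushes damage and stack count to its DamageNumber_Widget, restarts the Move timeline and sets the expiry timer.
; Refreshnumber accumulates further damage into the same number, passing a stack level capped at three.
; A short timer clears Updateable to close the stacking window, though this graph never checks that flag itself.
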(event `self.ReceiveBeginPlay`
  (`self.DamageUpdate` (`self.damage`)))

(event `Close Updates`
  ;[1 1 1] Stop being able to be updated after 0.2 seconds
  (set `self.Updateable` false))

(event `DamageUpdate`
  (params (damage :type Integer) (stack :type Integer))
  (bind _startloc (`self.startloc`))
  (bind _asdamage_number_widget (cast `/Game/Fadeout_Content/Core/Support/DamageNumber_Widget` (`WidgetComponent.GetUserWidgetObject` (`self.DamageUI`))))
  (set `/Game/Fadeout_Content/Core/Support/DamageNumber_Widget.damage` damage _asdamage_number_widget)
  (set `/Game/Fadeout_Content/Core/Support/DamageNumber_Widget.StackNumber` stack _asdamage_number_widget)
  (`/Game/Fadeout_Content/Core/Support/DamageNumber_Widget.Update Number` _asdamage_number_widget)
  ;[1 1 1] Stop being able to be updated after 0.2 seconds
  (`KismetSystemLibrary.K2_SetTimerDelegate` (delegate `Close Updates`) 0.2)
  (bind _returnvalue (`KismetSystemLibrary.K2_SetTimerDelegate` (delegate `Expire Damage Number`) 1.5))
  (set `self.ExpireTimer` _returnvalue)
  (bind (_direction _alpha) (`Timeline|move` :!via `PlayFromStart`)
    (:`Update`
      (`self.K2_SetActorLocation` (`KismetMathLibrary.VLerp` _startloc (+ _startloc (0.0 0.0 50.0)) _alpha))
      (set `/Game/Fadeout_Content/Core/Support/DamageNumber_Widget.textAlpha` (`KismetMathLibrary.Lerp` 1.0 0.0 _alpha) _asdamage_number_widget)
      (`/Game/Fadeout_Content/Core/Support/DamageNumber_Widget.Update Number` _asdamage_number_widget))))

(event `Expire Damage Number`
  (`self.Kill`))

(event `Refresh number`
  (params (`Updated Damage` :type Integer))
  (bind _output_get (set `self.stackCounter` (+ (`self.stackCounter`) 1)))
  (bind _output_get_2 (set `self.damage` (+ `Updated Damage` (`self.damage`))))
  (`self.DamageUpdate` _output_get_2 (`KismetMathLibrary.Clamp` _output_get 0 3)))

(event `Kill`
  (`FOCleanupLibrary.DestroyObject` (`WidgetComponent.GetUserWidgetObject` (`self.DamageUI`)))
  (`self.K2_DestroyActor`))

(event `self.ReceiveEndPlay`
  (params (EndPlayReason :type "EEndPlayReason Enum" :default "Destroyed"))
  (`self.Kill`))

(fn `UserConstructionScript`)