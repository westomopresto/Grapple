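; Actor that drops a set of weapons in a ring around itself on BeginPlay, spawning one Death_weapon_spawner per WeaponClasses entry.
; CircleSpawners spaces directions evenly around the Z axis and line-traces outward on Visibility from the root.
; Each spawn point is the trace end, or is pulled back from the hit when blocked, keeping drops out of obstacles.
; BeginPlay passes each weapon class to its spawner as SpawnersItem.
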(event `self.ReceiveBeginPlay`
  (bind _locations1 (`self.CircleSpawners`))
  (for (_array_element _array_index) _locations1
    (`|SpawnActorFromClass` "/Game/Fadeout_Content/Core/Props/death_weapon_spawner.death_weapon_spawner_C" (`KismetMathLibrary.MakeTransform` _array_element) "Undefined" "OverrideRootScale" null (`|GetArrayItem` (`self.WeaponClasses`) _array_index) 0 (struct) null)))

(fn `CircleSpawners`
  (returns (Locations1 :type "Array of Vector Structure"))
  (locals (Locations :type "Array of Vector Structure"))
  (bind _defaultsceneroot (`self.DefaultSceneRoot`))
  (bind _locations (`local.Locations`))
  (bind _returnvalue (`KismetArrayLibrary.Array_Length` (`self.WeaponClasses`)))
  (bind _returnvalue_2 (`SceneComponent.K2_GetComponentLocation` _defaultsceneroot))
  (for _index (range 1 (+ _returnvalue 1))
    (bind _returnvalue_3 (`KismetMathLibrary.RotateAngleAxis` (`SceneComponent.GetForwardVector` _defaultsceneroot) (* _index (/ 360.0 (`KismetMathLibrary.Conv_IntToDouble` _returnvalue))) (0.0 0.0 1.0)))
    (bind _outhit (`KismetSystemLibrary.LineTraceSingle` _returnvalue_2 (+ _returnvalue_2 (* _returnvalue_3 250.0)) "TraceTypeQuery1"))
    (bind (_bblockinghit _binitialoverlap _time _distance _location _impactpoint _normal _impactnormal _physmat _hitactor _hitcomponent _hitbonename _hititem _faceindex _tracestart _traceend) (`GameplayStatics.BreakHitResult` _outhit))
    (if _bblockinghit
      (`KismetArrayLibrary.Array_Add` _locations (- _location (* _returnvalue_3 50.0)))
      (else
        (`KismetArrayLibrary.Array_Add` _locations _traceend))))
  (return (`local.Locations`)))

(fn `UserConstructionScript`)