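; Server-driven director for Wave mode that runs a mission's waves of enemy bursts, with break times between waves and a victory once the last is cleared.
; A looping timer spawns bursts at unoccupied starts using a pre-spawned AI controller pool, scaling counts by human players and difficulty.
; Game mode events start rounds, spawn survivor bots and initialize player gold and UI.
; Multicasts toggle safe rooms and combat music.
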(event `Win MIssion Multicast`
  ;[1 1 1] Win Mission
  (bind _asfadeout_game_instance (cast `/Game/Fadeout_GameInstance` (`GameplayStatics.GetGameInstance`)))
  (`/Game/Fadeout_GameInstance.ProgressAchievement` _asfadeout_game_instance 301 1))

(event `Win Mission`
  ;[1 1 1] Win Mission
  (set `self.RoundOver` true)
  (`KismetSystemLibrary.K2_PauseTimerHandle` (`self.burstTicker`))
  (bind _asbp_multiplayer_gamemode (cast `/Game/Fadeout_Content/Core/GameModes/BP_MultiplayerGamemode` (`GameplayStatics.GetGameMode`)))
  (`/Game/Fadeout_Content/Core/GameModes/BP_MultiplayerGamemode.Broadcast` _asbp_multiplayer_gamemode "Victory!" (struct :`G` 1.0 :`B` 0.610038 :`A` 1.0) "/Game/PunchSoundPack/BonusSounds/ui_menu_button_click_01.ui_menu_button_click_01" true 15.0)
  (`self.Music Multi` false)
  (`self.Win MIssion Multicast`)
  (`/Game/Fadeout_Content/Core/GameModes/BP_MultiplayerGamemode.WaveMode_GameOver` _asbp_multiplayer_gamemode 15.0))

(event `Mission Start`
  ;[1 1 1] start
  (`self.Safe Room Event` false)
  (`self.Music Event` true)
  (set `self.MissionCopy` (`self.Mission`))
  (`KismetSystemLibrary.K2_ClearAndInvalidateTimerHandle` (`self.burstTicker`))
  (bind _returnvalue (`KismetSystemLibrary.K2_SetTimerDelegate` (delegate `Wave Updater`) 5.0 true 1.0))
  (set `self.burstTicker` _returnvalue)
  (bind _output_get (set `self.currentBurst` (`|GetArrayItem` (`.Waves_22_5717ED0D4CE58C058903A5BABD8BC61B` (break `/Game/Fadeout_Content/Core/Support/Wave_Support/STR_Waves` (`|GetArrayItem` (`self.MissionCopy`) (`self.current wave`)))) (`self.current burst`))))
  (`self.GetConnectedPlayersScaling` _output_get))

(event `Safe Room Multi`
  (params (SafeRoomEnable :type Boolean))
  ;[1 1 1] Multicasts
  (`self.RemoveSafeRooms` SafeRoomEnable))

(event `Safe Room Event`
  (params (safeRoomEnabled :type Boolean))
  ;[1 1 1] Multicasts
  (`/Engine/EditorBlueprintResources/ActorMacros.Switch Has Authority`
    (:`Authority`
      (bind _output_get (set `self.safeRoomEnabled` safeRoomEnabled))
      (`self.Safe Room Multi` _output_get))
    (:`Remote`
      (`self.RemoveSafeRooms` (`self.safeRoomEnabled`)))))

(event `Music Event`
  (params (combat :type Boolean))
  ;[1 1 1] Multicasts
  (`/Engine/EditorBlueprintResources/ActorMacros.Switch Has Authority`
    (:`Authority`
      (bind _output_get (set `self.combat` combat))
      (`self.Music Multi` _output_get))
    (:`Remote`
      (`self.Music Toggle` (`self.combat`)))))

(event `Wave Updater`
  (bind ((`burstComplete_22_0F843122496F073CD7EB169C44466E62` _burstcomplete)) (break `/Game/Fadeout_Content/Core/Support/Wave_Support/STR_WaveBurst` (`self.currentBurst`)))
  (bind _waves (break `/Game/Fadeout_Content/Core/Support/Wave_Support/STR_Waves` (`|GetArrayItem` (`self.Mission`) (`self.current wave`))))
  (if (`self.RoundOver`)
    _
    (elif (`self.wavesPaused`)
      _
      (elif _burstcomplete
        (`KismetSystemLibrary.PrintString` (`KismetStringLibrary.BuildString_Bool` "" "Wave Complete: " _burstcomplete))
        (if (>= (+ (`self.current burst`) 1) (`KismetArrayLibrary.Array_Length` _waves))
          (bind _remaining_alive_enemies (`self.Update Alive Enemies`))
          (if (== _remaining_alive_enemies 0)
            (if (>= (+ (`self.current wave`) 1) (`KismetArrayLibrary.Array_Length` (`self.Mission`)))
              (`KismetSystemLibrary.PrintString` "GAME OVER YOU WON" true true (struct :`R` 0.988024 :`G` 1.0 :`A` 1.0) 5.0)
              (`self.Win Mission`)
              (else
                (bind _output_get (set `self.current wave` (+ (`self.current wave`) 1)))
                (bind _output_get_2 (set `self.current burst` 0))
                (set `self.currentBurst` (`|GetArrayItem` (`.Waves_22_5717ED0D4CE58C058903A5BABD8BC61B` (break `/Game/Fadeout_Content/Core/Support/Wave_Support/STR_Waves` (`|GetArrayItem` (`self.Mission`) _output_get))) _output_get_2))
                (`KismetSystemLibrary.PrintString` "ADVANCING WAVE" true true (struct :`R` 0.172036 :`G` 1.0 :`A` 1.0) 5.0)
                (`self.BreakTimeStart` (`self.BreakTime`))
                (if (`self.GiveLivesBackBetweenRounds`)
                  (`/Game/Fadeout_Content/Core/GameModes/BP_MultiplayerGamemode.SetLives` (`self.GameMode`) 99 true))))
            (else
              (`KismetSystemLibrary.PrintString` "ENEMIES STILL ALIVE" true true (struct :`R` 0.916948 :`B` 1.0 :`A` 1.0) 5.0)))
          (else
            (set `self.current burst` (+ (`self.current burst`) 1))
            (bind (_count _structout) (`self.GetConnectedPlayersScaling` (`|GetArrayItem` _waves (`self.current burst`))))
            (set `self.currentBurst` _structout)
            (`KismetSystemLibrary.PrintString` "ADVANCING Burst" true true (struct :`G` 1.0 :`B` 0.557249 :`A` 1.0) 5.0)))
        (else
          (`self.Burst Spawn`))))))

(event `Music Multi`
  (params (Combat :type Boolean))
  ;[1 1 1] Multicasts
  (`self.Music Toggle` Combat))

(event `Update Players UI`
  (`/Game/Fadeout_Content/Core/GameModes/BP_MultiplayerGamemode.WaveCountUpdate` (`self.GameMode`) (`self.current wave`) (`KismetArrayLibrary.Array_Length` (`self.Mission`)) (`self.CurrentPhase`) (`self.difficulty`)))

(event `self.ReceiveBeginPlay`
  ;[1 0.863 0] disable begin play
  ;[0.1295 1 0.1096] Begin Play
  (if (not (`self.disabled`))
    (`|ExecutionSequence`
      (:`then_0`
        (`KismetSystemLibrary.Delay` 3.0)
        (`self.Safe Room Event` true)
        (`self.Music Event` false))
      (:`then_1`
        (if (`self.HasAuthority`)
          (bind _asbp_multiplayer_gamemode (cast `/Game/Fadeout_Content/Core/GameModes/BP_MultiplayerGamemode` (`GameplayStatics.GetGameMode`)))
          (bind _output_get (set `self.GameMode` _asbp_multiplayer_gamemode))
          (add `/Game/Fadeout_Content/Core/GameModes/BP_MultiplayerGamemode.GameTypeChanged` _output_get (delegate `GameTypeChanged`))
          (add `/Game/Fadeout_Content/Core/GameModes/BP_MultiplayerGamemode.RoundStarted` _output_get (delegate `RoundStart`))
          (add `/Game/Fadeout_Content/Core/GameModes/BP_MultiplayerGamemode.PlayerLoggedIn` _output_get (delegate `InitiPlayer`))
          (bind _asfadeout_game_instance (cast `/Game/Fadeout_GameInstance` (`GameplayStatics.GetGameInstance`)))
          (set `self.difficulty` (`/Game/Fadeout_GameInstance.waveModeDifficulty` _asfadeout_game_instance)))))))

(event `Music Toggle`
  (params (Condition :type Boolean))
  ;[1 1 1] Multicasts
  ;;[1 1 1] music function
  (if Condition
    (`/Game/Fadeout_Content/Core/Audio/BP_GlobalMusic.combatMusic` (`self.Music`) 2)
    (else
      (`/Game/Fadeout_Content/Core/Audio/BP_GlobalMusic.normalMusic` (`self.Music`) 3))))

(event `RoundStart`
  (`self.Mission Start`))

(event `GameTypeChanged`
  (params (`Game Type` :type "/Game/Fadeout_Content/Core/Support/Multiplayer_Support/DM_GameType Enum" :default "NewEnumerator0"))
  (bind _gamemode (`self.GameMode`))
  (switch `/Game/Fadeout_Content/Core/Support/Multiplayer_Support/DM_GameType` `Game Type`
    (:`NewEnumerator0`
      (for _array_element (`self.aiPool`) :!label _label
        (`self.K2_DestroyActor` _array_element)))
    (:`NewEnumerator1`
      (goto _label))
    (:`NewEnumerator2`
      (goto _label))
    (:`NewEnumerator3`
      (goto _label))
    (:`NewEnumerator4`
      (goto _label))
    (:`NewEnumerator5`
      (goto _label))
    (:`NewEnumerator7`
      (goto _label))
    (:`NewEnumerator8`
      (goto _label))
    (:`NewEnumerator10`
      (`|ExecutionSequence`
        (:`then_0`
          (`/Engine/EditorBlueprintResources/StandardMacros.DoOnce` false
            (:`Completed`
              (`self.Initialize Wave Director`))))
        (:`then_1`
          (for _array_element_2 (`/Game/Fadeout_Content/Core/GameModes/BP_MultiplayerGamemode.ConnectedPlayers` _gamemode)
            ;[1 1 1] might need to change this if we add friendly NPCs
            (if (`Controller.IsPlayerController` _array_element_2)
              (bind _asfo_player_controller (cast `/Game/Fadeout_Content/Core/FO_PlayerController` _array_element_2))
              (`/Game/Fadeout_Content/Core/FO_PlayerController.Wave Mode Inits` _asfo_player_controller (`self.STARTINGGOLD`))))
          (`/Game/Fadeout_Content/Core/GameModes/BP_MultiplayerGamemode.WaveCountUpdate` _gamemode (`self.current wave`) (`KismetArrayLibrary.Array_Length` (`self.Mission`)) (`self.CurrentPhase`) (`self.difficulty`))
          (`self.Update Players UI`))))))

(event `InitiPlayer`
  (params (PlayerController :type "PlayerController Object Reference"))
  (bind _asfo_player_controller (cast `/Game/Fadeout_Content/Core/FO_PlayerController` PlayerController))
  ;[1 1 1] might need to change this if we add friendly NPCs
  (if (`Controller.IsPlayerController` _asfo_player_controller)
    (`/Game/Fadeout_Content/Core/FO_PlayerController.Wave Mode Inits` _asfo_player_controller (`self.STARTINGGOLD`))
    (`/Game/Fadeout_Content/Core/FO_PlayerController.Current Wave Client` _asfo_player_controller (`self.current wave`) (`KismetArrayLibrary.Array_Length` (`self.Mission`)) (`self.CurrentPhase`) (`self.difficulty`))))

(event `BreakTimeStart`
  (params (Time :type "Float (double-precision)" :default 60.0))
  ;[1 1 1] Breaktime
  (`self.Music Event` false)
  (set `self.CurrentPhase` "Break Time")
  (`self.Update Players UI`)
  (set `self.wavesPaused` true)
  (bind _returnvalue (`KismetSystemLibrary.K2_SetTimerDelegate` (delegate `BreakTimeOver`) Time))
  (set `self.BreakTimer` _returnvalue)
  (bind _asbp_multiplayer_gamemode (cast `/Game/Fadeout_Content/Core/GameModes/BP_MultiplayerGamemode` (`GameplayStatics.GetGameMode`)))
  (`/Game/Fadeout_Content/Core/GameModes/BP_MultiplayerGamemode.Broadcast` _asbp_multiplayer_gamemode (`KismetTextLibrary.Conv_StringToText` (`KismetStringLibrary.BuildString_Double` "" "Break Time: " Time " seconds")) (struct :`G` 1.0 :`B` 0.506271 :`A` 1.0) null true 10.0))

(event `BreakTimeOver`
  (bind _gamemode (`self.GameMode`))
  ;[1 1 1] Breaktime
  (set `self.wavesPaused` false)
  (`/Game/Fadeout_Content/Core/GameModes/BP_MultiplayerGamemode.SetLives` _gamemode 1 true)
  (`/Game/Fadeout_Content/Core/GameModes/BP_MultiplayerGamemode.Broadcast` _gamemode "Breaktime Over!" (struct :`G` 1.0 :`B` 0.506271 :`A` 1.0) null true 5.0)
  (set `self.CurrentPhase` "Waves Incoming")
  (`self.Update Players UI`)
  (`self.Music Event` true))

(event `Initialize Wave Director`
  (`self.AI Pool Initialize`)
  (`KismetSystemLibrary.Delay` 2.0)
  (`self.Spawn Friendly Bots`))

(event `Spawn Friendly Bots`
  (if (>= (`self.survivorBots`) 1)
    (`/Game/Fadeout_Content/Core/GameModes/BP_MultiplayerGamemode.SpawnBots` (`self.GameMode`) (`self.survivorBots`) true "NewEnumerator10" true "survivor" false)))

(fn `AI Pool Initialize`
  (for _ (range (`self.aiPoolSize`))
    (bind _returnvalue (`|SpawnActorFromClass` "/Game/Fadeout_Content/Core/FO_TeamAIController.FO_TeamAIController_C" (`KismetMathLibrary.MakeTransform` (0.0 0.0 0.0)) "Undefined" "OverrideRootScale" null null))
    (bind _asfo_player_state (cast `/Game/Fadeout_Content/Core/Support/Multiplayer_Support/FO_PlayerState` (`Controller.PlayerState` _returnvalue)))
    (set `/Game/Fadeout_Content/Core/Support/Multiplayer_Support/FO_PlayerState.Team` "wavespawn" _asfo_player_state)
    (`KismetArrayLibrary.Array_Add` (`self.aiPool`) _returnvalue))
  (return))

(fn `AiPoolFree`
  (returns (`Available Ai Controllers` :type "Array of /Game/Fadeout_Content/Core/FO_TeamAIController Object Reference"))
  (locals (freedAis :type "Array of /Game/Fadeout_Content/Core/FO_TeamAIController Object Reference"))
  (for _array_element (`self.aiPool`)
    (`/Engine/EditorBlueprintResources/StandardMacros.IsValid` (`Controller.K2_GetPawn` _array_element)
      (:`Is Not Valid`
        (`KismetArrayLibrary.Array_Add` (`local.freedAis`) _array_element))))
  (return (`local.freedAis`)))

(fn `Burst Spawn`
  (locals (WaveSpawners :type "Array of PlayerStart Object Reference"))
  (bind _currentburst (`self.currentBurst`))
  (bind _gamemode (`self.GameMode`))
  (bind ((`Quantity_11_5717ED0D4CE58C058903A5BABD8BC61B` _quantity) (`EnemyType_3_E817DEA743587EB819C3138CE1E87CE9` _enemytype) (`Loadout_7_6F3E99BA4059F429D6839D8EC9D4C416` _loadout) (`HealthMultiplier_15_68DA6A114CCF05B64A363DB86EB616C1` _healthmultiplier)) (break `/Game/Fadeout_Content/Core/Support/Wave_Support/STR_WaveBurst` (`self.currentBurst`)))
  (bind _returnvalue (- _quantity 1))
  (`/Engine/EditorBlueprintResources/ActorMacros.Switch Has Authority`
    (:`Authority`
      (`/Engine/EditorBlueprintResources/StandardMacros.IsValid` _gamemode
        (:`Is Valid`
          (set `local.WaveSpawners` (`/Game/Fadeout_Content/Core/GameModes/BP_MultiplayerGamemode.wavespawn_starts` _gamemode))
          (bind _available_ai_controllers (`self.AiPoolFree`))
          (for _array_element _available_ai_controllers
            (if (>= _quantity 1)
              (`/Engine/EditorBlueprintResources/StandardMacros.IsValid` _array_element
                (:`Is Valid`
                  (bind _safespawns (`self.empty spawn scan` (`local.WaveSpawners`)))
                  (bind _returnvalue_2 (`|SpawnActorFromClass` :`Class` _enemytype :`SpawnTransform` (`self.GetTransform` (`|GetArrayItem` _safespawns (`KismetMathLibrary.RandomIntegerInRange` 0 (- (`KismetArrayLibrary.Array_Length` _safespawns) 1)))) :`CollisionHandlingOverride` "Undefined" :`TransformScaleMethod` "OverrideRootScale" :`starterWeapons` _loadout :`Name Visibility` false :`bBot` true :`Instigator` null))
                  (bind _output_get (set `/Game/Fadeout_Content/Core/Characters/BP_PlayerCharacter.maxHealth` (* _healthmultiplier (`/Game/Fadeout_Content/Core/Characters/BP_PlayerCharacter.maxHealth` _returnvalue_2)) _returnvalue_2))
                  (set `/Game/Fadeout_Content/Core/Characters/BP_PlayerCharacter.health` _output_get _returnvalue_2)
                  (`Controller.Possess` _array_element _returnvalue_2)
                  (`KismetSystemLibrary.PrintString` (`KismetStringLibrary.Conv_IntToString` _returnvalue) true true (struct :`R` 0.013375 :`G` 1.0 :`A` 1.0))
                  (setmembers `/Game/Fadeout_Content/Core/Support/Wave_Support/STR_WaveBurst` :`StructRef` (`self.currentBurst`) :`Quantity` _returnvalue)
                  (`/Game/Fadeout_Content/Core/Characters/BP_PlayerCharacter.WaveSpawn Initialize` _returnvalue_2)
                  (`KismetArrayLibrary.Array_Add` (`self.SpawnedEnemies`) _returnvalue_2)
                  (`KismetArrayLibrary.Array_Add` (`/Game/Fadeout_Content/Core/Characters/BP_PlayerCharacter.itemsToDropOnDeath` _returnvalue_2) "/Game/Fadeout_Content/Core/Props/Pickups/BP_GoldBars.BP_GoldBars_C")
                  (bind _asbp_char_bingo (cast `/Game/Fadeout_Content/Core/Characters/BP_Char_Bingo` _returnvalue_2))
                  (`/Game/Fadeout_Content/Core/Characters/BP_Char_Bingo.Cloak Toggle` _asbp_char_bingo true))
                (:`Is Not Valid`
                  (`KismetSystemLibrary.PrintString` "Ran out of Controllers, Waiting" true true (struct :`G` 0.66 :`B` 1.0 :`A` 1.0) 5.0)
                  (break)))
              (else
                (`KismetSystemLibrary.PrintString` "No More Enemies In Wave" true true (struct :`G` 0.66 :`B` 1.0 :`A` 1.0) 5.0)
                (break))))
          (setmembers `/Game/Fadeout_Content/Core/Support/Wave_Support/STR_WaveBurst` :`StructRef` _currentburst :`burstComplete` (<= (`.Quantity_11_5717ED0D4CE58C058903A5BABD8BC61B` (break `/Game/Fadeout_Content/Core/Support/Wave_Support/STR_WaveBurst` _currentburst)) 0))
          (return))
        (:`Is Not Valid`
          _)))
    (:`Remote`
      _))
  (return))

(fn `empty spawn scan`
  (params (PlayerStarts :type "Array of PlayerStart Object Reference"))
  (returns (safeSpawns :type "Array of PlayerStart Object Reference") (foundSome :type Boolean))
  (locals (emptySpawns :type "Array of PlayerStart Object Reference"))
  (for _array_element PlayerStarts
    (bind _returnvalue (`self.K2_GetActorLocation` _array_element))
    (bind (_outhit _returnvalue_2) (`KismetSystemLibrary.SphereTraceSingleForObjects` :`Start` _returnvalue :`End` (+ _returnvalue 1.0) :`Radius` 125.0 :`ObjectTypes` (`|MakeArray` "ObjectTypeQuery3" :!type "EObjectTypeQuery Enum") :`TraceColor` (struct :`G` 1.0 :`B` 0.920606 :`A` 1.0) :`TraceHitColor` (struct :`R` 1.0 :`G` 0.538916 :`A` 1.0) :`DrawTime` 15.0))
    (if (not _returnvalue_2)
      (`KismetArrayLibrary.Array_Add` (`local.emptySpawns`) _array_element)))
  (if (> (`KismetArrayLibrary.Array_Length` (`local.emptySpawns`)) 0)
    (return (`local.emptySpawns`) true)
    (else
      (return PlayerStarts false))))

(fn `GetAliveSurvivors`
  (returns (Success :type Boolean) (_Locations :type "Array of Vector Structure"))
  (locals (Locations :type "Array of Vector Structure"))
  (bind _asmultiplayer_game_state (cast `/Game/Fadeout_Content/Core/Support/Multiplayer_Support/Multiplayer_GameState` (`GameplayStatics.GetGameState`))
    (:`then`
      (for _array_element (`/Game/Fadeout_Content/Core/Support/Multiplayer_Support/Multiplayer_GameState.AllAlive_Players` _asmultiplayer_game_state)
        (`KismetArrayLibrary.Array_Add` (`local.Locations`) (`self.K2_GetActorLocation` _array_element)))
      (return true (`local.Locations`)))
    (:`CastFailed`
      (return false (`|MakeArray` (0.0 0.0 0.0) :!type "Vector Structure")))))

(fn `GetConnectedPlayersScaling`
  (params (Burst :type "/Game/Fadeout_Content/Core/Support/Wave_Support/STR_WaveBurst Structure (by ref)"))
  (returns (Count :type Integer) (StructOut :type "/Game/Fadeout_Content/Core/Support/Wave_Support/STR_WaveBurst Structure (by ref)"))
  (locals (players :type Integer))
  (for _array_element (`/Game/Fadeout_Content/Core/GameModes/BP_MultiplayerGamemode.ConnectedPlayers` (`self.GameMode`))
    (if (not (`PlayerState.bIsABot` (`Controller.PlayerState` _array_element)))
      (`/Engine/EditorBlueprintResources/StandardMacros.IncrementInt` (`local.players`))))
  (bind _output_get (set `local.players` (`KismetMathLibrary.Clamp` (`local.players`) 1 8)))
  (bind _structout (setmembers `/Game/Fadeout_Content/Core/Support/Wave_Support/STR_WaveBurst` :`StructRef` Burst :`Quantity` (* (* (`.Quantity_11_5717ED0D4CE58C058903A5BABD8BC61B` (break `/Game/Fadeout_Content/Core/Support/Wave_Support/STR_WaveBurst` Burst)) (select `int` _output_get :`0` 1 :`1` 1 :`2` 1 :`3` 2 :`4` 2 :`5` 3 :`6` 3 :`7` 4 :`8` 4)) (`self.difficulty`))))
  (`KismetSystemLibrary.PrintString` (`KismetStringLibrary.BuildString_Int` "" "Scaling: " (`.Quantity_11_5717ED0D4CE58C058903A5BABD8BC61B` (break `/Game/Fadeout_Content/Core/Support/Wave_Support/STR_WaveBurst` _structout))))
  (return _output_get _structout))

(fn `RemoveSafeRooms`
  (params (enable :type Boolean))
  (for _array_element (`self.SafeRoom`)
    (for _array_element_2 (`self.K2_GetComponentsByClass` _array_element "/Script/Engine.PrimitiveComponent")
      (`PrimitiveComponent.SetCollisionEnabled` _array_element_2 (select `bool` enable :`false` "NoCollision" :`true` "QueryAndPhysics" :!type "ECollisionEnabled Enum")))
    (`self.SetActorHiddenInGame` _array_element (not enable))))

(fn `Update Alive Enemies`
  (returns (`Remaining Alive Enemies` :type Integer))
  (locals (aliveEnemies :type "Array of /Game/Fadeout_Content/Core/Characters/BP_PlayerCharacter Object Reference"))
  (for _array_element (`self.SpawnedEnemies`)
    (`/Engine/EditorBlueprintResources/StandardMacros.IsValid` _array_element
      (:`Is Valid`
        (if (`/Game/Fadeout_Content/Core/Characters/BP_PlayerCharacter.alive?` _array_element)
          (`KismetArrayLibrary.Array_Add` (`local.aliveEnemies`) _array_element)))))
  (bind _output_get (set `self.SpawnedEnemies` (`local.aliveEnemies`)))
  (return (`KismetArrayLibrary.Array_Length` _output_get)))

(fn `UserConstructionScript`)