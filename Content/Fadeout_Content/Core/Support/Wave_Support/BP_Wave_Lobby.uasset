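; Wave mode lobby actor that loads the orchard wave map once all connected players stand in its trigger volume.
; On the server, overlap events rescan the volume for player-controlled characters and multicast the ready count to a text render.
; A full count starts timers for a broadcast countdown and map change, which are cleared when the count drops.
; A looping timer keeps every player's lives topped up while waiting.
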(event `LivesRefresh`
  ;[1 1 1] Lives Refresh
  (for _array_element (`/Game/Fadeout_Content/Core/GameModes/BP_MultiplayerGamemode.ConnectedPlayers` (`self.GameMode`))
    (bind _asfo_player_controller (cast `/Game/Fadeout_Content/Core/FO_PlayerController` _array_element))
    (bind _asfo_player_state (cast `/Game/Fadeout_Content/Core/Support/Multiplayer_Support/FO_PlayerState` (`Controller.PlayerState` _asfo_player_controller)))
    (set `/Game/Fadeout_Content/Core/Support/Multiplayer_Support/FO_PlayerState.Lives` 999 _asfo_player_state)))

(event `self.ReceiveBeginPlay`
  (bind _triggervolume (`self.TriggerVolume`))
  ;[1 1 1] Begin Play
  (bind _asbp_multiplayer_gamemode (cast `/Game/Fadeout_Content/Core/GameModes/BP_MultiplayerGamemode` (`GameplayStatics.GetGameMode`)))
  (set `self.GameMode` _asbp_multiplayer_gamemode)
  (if (`self.HasAuthority`)
    (add `self.OnActorBeginOverlap` _triggervolume (delegate `TriggerFired`))
    (add `self.OnActorEndOverlap` _triggervolume (delegate `TriggerFired`))
    (`KismetSystemLibrary.K2_SetTimerDelegate` (delegate `LivesRefresh`) 2.0 true)
    (`self.First Scan`)))

(event `Multicast ReadyCheck`
  (params (Pready :type Integer) (Nplayers :type Integer))
  ;[1 1 1] Mulicast Text Update (Players Ready)
  (`TextRenderComponent.K2_SetText` (`TextRenderActor.TextRender` (`self.textRender`)) (`KismetTextLibrary.Conv_StringToText` (`KismetStringLibrary.Concat_StrStr` (`KismetStringLibrary.Conv_IntToString` Pready) "/" (`KismetStringLibrary.Conv_IntToString` Nplayers)))))

(event `TriggerFired` :!signature `self.OnActorBeginOverlap`
  (params (OverlappedActor :type "Actor Object Reference") (OtherActor :type "Actor Object Reference"))
  ;[1 1 1] Ready Trigger Fired
  (cast `/Game/Fadeout_Content/Core/Characters/BP_PlayerCharacter` OtherActor)
  (bind (__readyplayers _readycount) (`self.ScanOverlap` (`self.TriggerVolume`) :!label _label))
  (set `self.PlayersReady` _readycount)
  (set `self.NumPlayers` (`KismetArrayLibrary.Array_Length` (`/Game/Fadeout_Content/Core/GameModes/BP_MultiplayerGamemode.ConnectedPlayers` (`self.GameMode`))))
  (`self.Multicast ReadyCheck` (`self.PlayersReady`) (`self.NumPlayers`))
  (`self.Ready Check`))

(event `First Scan`
  ;[1 1 1] Ready Trigger Fired
  (goto _label))

(event `Load Level`
  ;[1 1 1] Ready Check & Loadlevel
  (`KismetSystemLibrary.Delay` 1.0)
  (`/Game/Fadeout_Content/Core/GameModes/BP_MultiplayerGamemode.Change Map` (`self.GameMode`) "wave_orchard_base" 0.5 "Map Loading!"))

(event `Ready Check`
  (bind _numplayers (`self.NumPlayers`))
  (bind _playersready (`self.PlayersReady`))
  ;[1 1 1] Ready Check & Loadlevel
  (if (and (>= _playersready 0) (>= _playersready _numplayers) (>= _numplayers 0))
    (bind _returnvalue (`KismetSystemLibrary.K2_SetTimerDelegate` (delegate `Load Level`) 5.0))
    (set `self.LevelLoadCountDown` _returnvalue)
    (set `self.textCd` 5)
    (bind _returnvalue_2 (`KismetSystemLibrary.K2_SetTimerDelegate` (delegate `Announce`) 1.0 true))
    (set `self.countdown` _returnvalue_2)
    (else
      (`KismetSystemLibrary.K2_ClearAndInvalidateTimerHandle` (`self.LevelLoadCountDown`))
      (`KismetSystemLibrary.K2_ClearAndInvalidateTimerHandle` (`self.countdown`)))))

(event `Announce`
  ;[1 1 1] Ready Check & Loadlevel
  (bind _output_get (set `self.textCd` (- (`self.textCd`) 1)))
  (bind _returnvalue (`KismetMathLibrary.Clamp` (+ _output_get 1) -1 999))
  (if (>= _returnvalue 0)
    (`/Game/Fadeout_Content/Core/GameModes/BP_MultiplayerGamemode.Broadcast` (`self.GameMode`) (`KismetTextLibrary.Conv_IntToText` _returnvalue) (struct :`G` 1.0 :`B` 0.073314 :`A` 1.0) "/Game/PunchSoundPack/BonusSounds/ui_menu_button_click_02.ui_menu_button_click_02" true)))

(fn `ScanOverlap`
  (params (Volume :type "TriggerSphere Object Reference"))
  (returns (_ReadyPlayers :type "Array of /Game/Fadeout_Content/Core/Characters/BP_PlayerCharacter Object Reference") (ReadyCount :type Integer))
  (locals (ReadyPlayers :type "Array of /Game/Fadeout_Content/Core/Characters/BP_PlayerCharacter Object Reference"))
  (bind _readyplayers (`local.ReadyPlayers`))
  (for _array_element (`self.GetOverlappingActors` Volume "/Game/Fadeout_Content/Core/Characters/BP_PlayerCharacter.BP_PlayerCharacter_C")
    (bind _asbp_player_character (cast `/Game/Fadeout_Content/Core/Characters/BP_PlayerCharacter` _array_element))
    (if (`Pawn.IsPlayerControlled` _asbp_player_character)
      (`KismetArrayLibrary.Array_AddUnique` (`local.ReadyPlayers`) _asbp_player_character)))
  (return _readyplayers (`KismetArrayLibrary.Array_Length` _readyplayers)))

(fn `UserConstructionScript`)