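; Tractor Nexus is the wave mode objective, the "Tractor of Hope", whose destruction means defeat.
; It ignores damage instigated by player controllers, clamps health on other damage, and updates its name widget's health bar locally and through a multicast event.
; At zero health it broadcasts DEFEAT once through the multiplayer game mode and triggers the wave game over.
; The construction script enables custom depth stencil on its mesh.
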(event `MultiCast Update Health`
  (set `/Game/Fadeout_Content/Core/Support/Name_Widget.healthNormalized` (/ (`self.Health`) (`self.MaxHealth`)) (`self.nameHud`)))

(event `self.ReceiveBeginPlay`
  (bind _asname_widget (cast `/Game/Fadeout_Content/Core/Support/Name_Widget` (`WidgetComponent.GetUserWidgetObject` (`self.Widget`))))
  (set `/Game/Fadeout_Content/Core/Support/Name_Widget.name` "Tractor of Hope" _asname_widget)
  (set `self.nameHud` _asname_widget)
  (set `/Game/Fadeout_Content/Core/Support/Name_Widget.healthNormalized` (/ (`self.Health`) (`self.MaxHealth`)) (`self.nameHud`)))

(event `self.ReceiveAnyDamage`
  (params (Damage :type "Float (single-precision)") (DamageType :type "DamageType Object Reference") (InstigatedBy :type "Controller Object Reference") (DamageCauser :type "Actor Object Reference"))
  (cast `/Game/Fadeout_Content/Core/FO_PlayerController` InstigatedBy
    (:`CastFailed`
      (bind _output_get (set `self.Health` (`KismetMathLibrary.FClamp` (- (`self.Health`) Damage) 0.0 100000000.0)))
      (`|ExecutionSequence`
        (:`then_0`
          (set `/Game/Fadeout_Content/Core/Support/Name_Widget.healthNormalized` (/ _output_get (`self.MaxHealth`)) (`self.nameHud`))
          (`self.MultiCast Update Health`))
        (:`then_1`
          (if (<= (`self.Health`) 0.0)
            (`/Engine/EditorBlueprintResources/StandardMacros.DoOnce` false
              (:`Completed`
                (bind _asbp_multiplayer_gamemode (cast `/Game/Fadeout_Content/Core/GameModes/BP_MultiplayerGamemode` (`GameplayStatics.GetGameMode`)))
                (`/Game/Fadeout_Content/Core/GameModes/BP_MultiplayerGamemode.Broadcast` _asbp_multiplayer_gamemode "DEFEAT" (struct :`R` 1.0 :`B` 0.027276 :`A` 1.0) "/Game/PunchSoundPack/BonusSounds/ui_menu_button_beep_01.ui_menu_button_beep_01" true 10.0)
                (`/Game/Fadeout_Content/Core/GameModes/BP_MultiplayerGamemode.WaveMode_GameOver` _asbp_multiplayer_gamemode 5.0)))))))))

(fn `UserConstructionScript`
  (bind _staticmesh (`self.StaticMesh`))
  (`PrimitiveComponent.SetRenderCustomDepth` _staticmesh true)
  (`PrimitiveComponent.SetCustomDepthStencilValue` _staticmesh 2))