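; Purchasable slot machine for wave mode that sells the player a choice of three random powers.
; Interaction passes a short cooldown and an authority check into WaveModeBuySys, which triggers either an error beep or the purchase.
; A purchase opens Widget_3Powers with shuffled picks, then async-loads and spawns the chosen Action_Base for the player's pawn.
; Multicast effects spin material-driven reels on a timeline, unrelated to the offered powers; older weapon/buff spawning is unused.
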(event `DoActionOnServer`
  (params (ActionBaseClass :type "/Game/Fadeout_Content/PraxisStyleAction/Action_Base Soft Class Reference") (Instigator :type "Pawn Object Reference"))
  (bind _class (`|LoadAssetClass` ActionBaseClass)
    (:`Completed`
      (bind _asaction_base (castclass `/Game/Fadeout_Content/PraxisStyleAction/Action_Base` _class))
      (`|SpawnActorFromClass` _asaction_base (`self.GetTransform`) "AlwaysSpawn" "OverrideRootScale" Instigator Instigator))))

(event `ClientBought`
  (params (`FO Player Controller` :type "/Game/Fadeout_Content/Core/FO_PlayerController Object Reference"))
  (bind _actions (`self.RandomThreeActions`))
  (bind _returnvalue (`|CreateWidget` "/Game/Fadeout_Content/Core/UI/CasinoUI/Widget_3Powers.Widget_3Powers_C" `FO Player Controller` _actions self))
  (`UserWidget.AddToPlayerScreen` _returnvalue 1)
  (`/Game/Fadeout_Content/Core/FO_PlayerController.Menu Mode` `FO Player Controller` true)
  (add `/Game/Fadeout_Content/Core/UI/CasinoUI/Widget_3Powers.PowerChosen` _returnvalue (delegate `PowerChosenEvent`)))

(event `self.ReceiveBeginPlay`
  (bind _wavemode_buysys (`self.WaveMode_BuySys`))
  (`|ExecutionSequence`
    (:`then_0`
      (bind _aswm_cost_widget (cast `/Game/Fadeout_Content/Core/Support/Wave_Support/WM_CostWidget` (`WidgetComponent.GetUserWidgetObject` (`self.Widget`))))
      (set `/Game/Fadeout_Content/Core/Support/Wave_Support/WM_CostWidget.Cost` (`/Game/Fadeout_Content/Core/Support/Wave_Support/WaveMode_BuySys.CostOfThing` _wavemode_buysys) _aswm_cost_widget)
      (set `/Game/Fadeout_Content/Core/Support/Wave_Support/WM_CostWidget.Flavor Text` (`self.FlavorText`) _aswm_cost_widget))
    (:`then_1`
      (add `/Game/Fadeout_Content/Core/Support/Wave_Support/WaveMode_BuySys.PurchaseFail` _wavemode_buysys (delegate `Purchase Fail`))
      (add `/Game/Fadeout_Content/Core/Support/Wave_Support/WaveMode_BuySys.PurchaseSuccess` _wavemode_buysys (delegate `Spawn Weapon`)))
    (:`then_2`
      (bind _returnvalue (`KismetMaterialLibrary.CreateDynamicMaterialInstance` "/Game/Fadeout_Content/Core/Maps/wave_casino/SlotMachine/MM_SlotScroll.MM_SlotScroll"))
      (bind _output_get (set `self.SlotScrollDyn` _returnvalue))
      (`PrimitiveComponent.SetMaterial` (`self.Cube`) 1 _output_get))))

(event `PowerChosenEvent`
  (params (FOPlayerController :type "/Game/Fadeout_Content/Core/FO_PlayerController Object Reference") (ActionBaseClass :type "/Game/Fadeout_Content/PraxisStyleAction/Action_Base Soft Class Reference"))
  (`/Game/Fadeout_Content/Core/FO_PlayerController.Menu Mode` FOPlayerController false)
  (`self.DoActionOnServer` ActionBaseClass (`Controller.K2_GetPawn` FOPlayerController)))

(event `Purchase Fail`
  (`self.Error multicast`))

(event `Spawn Weapon`
  (params (`FO Player` :type "/Game/Fadeout_Content/Core/FO_PlayerController Object Reference"))
  (`self.SetOwner` `FO Player`)
  (`self.ClientBought` `FO Player`)
  (`self.PurchaseServer`))

(event `Error multicast`
  ;[1 1 1] Purchase Error
  (`GameplayStatics.PlaySoundAtLocation` "/Game/Fadeout_Content/Core/Audio/short_beep.short_beep" (`self.K2_GetActorLocation`) (struct) 2.0 1.0 0.0 null null null))

(event `PurchaseServer`
  (`self.PurchaseMulticast`))

(event `/Game/Fadeout_Content/Core/Support/Wave_Support/BPI_WaveModePurchases.AttemptPurchase`
  (params (`FO Player` :type "/Game/Fadeout_Content/Core/FO_PlayerController Object Reference"))
  ;[1 1 1] Purchase interface
  (if (`KismetSystemLibrary.K2_IsTimerActiveHandle` (`self.InteractCooldown`))
    (`self.Error multicast`)
    (else
      (bind _returnvalue (`KismetSystemLibrary.K2_SetTimerDelegate` (delegate `Cooldown Over`) 3.0))
      (set `self.InteractCooldown` _returnvalue)
      (`/Engine/EditorBlueprintResources/ActorMacros.Switch Has Authority`
        (:`Authority`
          (`/Game/Fadeout_Content/Core/Support/Wave_Support/BPI_WaveModePurchases.AttemptPurchase` (`self.WaveMode_BuySys`) `FO Player`))))))

(event `PurchaseMulticast`
  (`GameplayStatics.SpawnSoundAtLocation` "/Game/Fadeout_Content/Core/Audio/UI_Sound/184438__capslok__cash-register-fake.184438__capslok__cash-register-fake" (`self.K2_GetActorLocation`) (struct) 1.0 1.0 0.0 null null)
  (`self.RollEffects`))

(event `Cooldown Over`
  ;[1 1 1] Purchase interface
)

(event `RollEffects`
  (bind _slotscrolldyn (`self.SlotScrollDyn`))
  (set `self.ATarget` (+ (`self.SpinnerA`) (`KismetMathLibrary.SelectFloat` 0.5 1.0 (`KismetMathLibrary.RandomBool`))))
  (set `self.BTarget` (+ (`self.SpinnerB`) (`KismetMathLibrary.SelectFloat` 2.0 2.5 (`KismetMathLibrary.RandomBool`))))
  (set `self.CTarget` (+ (`self.SpinnerC`) (`KismetMathLibrary.SelectFloat` 0.5 1.0 (`KismetMathLibrary.RandomBool`))))
  (bind (_direction _spinnera _spinnerb _spinnerc) (`Timeline|SlotMachineRoll` :!via `PlayFromStart`)
    (:`Update`
      (`MaterialInstanceDynamic.SetScalarParameterValue` _slotscrolldyn "RollA" (`KismetMathLibrary.Lerp` (`self.SpinnerA`) (`self.ATarget`) _spinnera))
      (`MaterialInstanceDynamic.SetScalarParameterValue` _slotscrolldyn "RollB" (`KismetMathLibrary.Lerp` (`self.SpinnerB`) (`self.BTarget`) _spinnerb))
      (`MaterialInstanceDynamic.SetScalarParameterValue` _slotscrolldyn "RollC" (`KismetMathLibrary.Lerp` (`self.SpinnerC`) (`self.CTarget`) _spinnerc)))
    (:`Finished`
      (set `self.SpinnerA` (`self.ATarget`))
      (set `self.SpinnerB` (`self.BTarget`))
      (set `self.SpinnerC` (`self.CTarget`)))
    (:`Ding`
      (`GameplayStatics.PlaySoundAtLocation` "/Game/Fadeout_Content/Core/FBX/Trap/278203__thepriest909__bear-trap.278203__thepriest909__bear-trap" (`self.K2_GetActorLocation`) (struct) 2.0 1.5 0.0 "/Game/Fadeout_Content/Core/Characters/Footstep_Attenuation.Footstep_Attenuation" null null))))

(event `/Game/Fadeout_Content/Core/Support/Wave_Support/BPI_WaveModePurchases.PurchasedTrigger`
  ;[1 1 1] Purchase interface
  (`/Engine/EditorBlueprintResources/ActorMacros.Switch Has Authority`
    (:`Authority`
      (`/Game/Fadeout_Content/Core/Support/Wave_Support/BPI_WaveModePurchases.PurchasedTrigger` (`self.WaveMode_BuySys`)))))

(fn `UserConstructionScript`)