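; BP_BrickCar is a map hazard car that loops along a PatrolPath spline, forward or reversed, and runs over players.
; A fast looping timer advances spline distance and interpolates position at fixed height, facing travel.
; Box overlaps launch players, play a health-dependent horn and deal max-health-scaled damage, once per player until a five-second timer clears the hit list.
; That timer also multicasts server distance to resync clients.
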(event `ResetPlayerArray`
  (`KismetArrayLibrary.Array_Clear` (`self.hitPlayers`))
  (`/Engine/EditorBlueprintResources/ActorMacros.Switch Has Authority`
    (:`Authority`
      (`self.Multicast_Distance Sync` (`self.Current Distance`)))))

(event `Multicast_Distance Sync`
  (params (`Current Distance` :type "Float (double-precision)"))
  (`KismetSystemLibrary.K2_PauseTimerHandle` (`self.moveTimer`))
  (set `self.Current Distance` `Current Distance`)
  (`KismetSystemLibrary.K2_UnPauseTimerHandle` (`self.moveTimer`)))

(event `self.ReceiveBeginPlay`
  (bind _returnvalue (`self.K2_GetActorLocation`))
  (set `self.lastLoc` _returnvalue)
  (set `self.Z_Loc` (.z _returnvalue))
  (bind _returnvalue_2 (`KismetSystemLibrary.K2_SetTimerDelegate` (delegate `UpdateLocation`) 0.015 true))
  (set `self.moveTimer` _returnvalue_2)
  (set `self.SplineLength` (`SplineComponent.GetSplineLength` (`/Game/Fadeout_Content/Core/Characters/BP_PatrolPath.Spline` (`self.PatrolPath`))))
  (`KismetSystemLibrary.K2_SetTimerDelegate` (delegate `ResetPlayerArray`) 5.0 true))

(event `UpdateLocation`
  (bind _returnvalue (`GameplayStatics.GetWorldDeltaSeconds`))
  (bind _returnvalue_2 (+ (* (`self.Speed`) (`KismetMathLibrary.SelectFloat` -1.0 1.0 (`self.Reverse?`))) (`self.Current Distance`)))
  (bind _returnvalue_3 (`KismetMathLibrary.SelectFloat` (`KismetMathLibrary.SelectFloat` (`self.SplineLength`) _returnvalue_2 (<= _returnvalue_2 0.0)) (`KismetMathLibrary.SelectFloat` 0.0 _returnvalue_2 (>= _returnvalue_2 (`self.SplineLength`))) (`self.Reverse?`)))
  (bind _returnvalue_4 (`SplineComponent.GetLocationAtDistanceAlongSpline` (`/Game/Fadeout_Content/Core/Characters/BP_PatrolPath.Spline` (`self.PatrolPath`)) _returnvalue_3 "World"))
  (bind _returnvalue_5 (`KismetMathLibrary.VInterpTo` (`self.K2_GetActorLocation`) (`KismetMathLibrary.MakeVector` (.x _returnvalue_4) (.y _returnvalue_4) (`self.Z_Loc`)) _returnvalue 60.0))
  (`self.K2_SetActorLocationAndRotation` _returnvalue_5 (`KismetMathLibrary.RInterpTo` (`self.K2_GetActorRotation`) (`KismetMathLibrary.FindLookAtRotation` (`KismetMathLibrary.MakeVector` (.x (`self.K2_GetActorLocation`)) (.y (`self.K2_GetActorLocation`))) (`KismetMathLibrary.MakeVector` (.x _returnvalue_4) (.y _returnvalue_4))) _returnvalue 60.0))
  (set `self.Current Distance` _returnvalue_3)
  (set `self.lastLoc` _returnvalue_5))

(event `Hit_Player`
  (params (Player :type "/Game/Fadeout_Content/Core/Characters/BP_PlayerCharacter Object Reference") (Direction :type "Vector Structure"))
  (bind _returnvalue (* (`/Game/Fadeout_Content/Core/Characters/BP_PlayerCharacter.maxHealth` Player) 1.8))
  (if (not (`KismetArrayLibrary.Array_Contains` (`self.hitPlayers`) Player))
    (`Character.LaunchCharacter` Player Direction true true)
    (`|ExecutionSequence`
      (:`then_0`
        (`GameplayStatics.SpawnSoundAttached` (select `bool` (<= (`/Game/Fadeout_Content/Core/Characters/BP_PlayerCharacter.health` Player) (* _returnvalue 0.5)) :`false` "/Game/Fadeout_Content/Core/Maps/map_brickadia_support/Brickadia_BP/car_horn.car_horn" :`true` "/Game/Fadeout_Content/Core/Audio/Multiplayer_Sounds/Air_Horn-SoundBible_com-964603082.Air_Horn-SoundBible_com-964603082" :!type "SoundBase Object Reference") (`Character.Mesh` Player) "None" (0.0 0.0 0.0) (struct) "KeepRelativeOffset" true 2.0 1.0 0.0 "/Game/Fadeout_Content/Core/Props/Elevator_Attenuation.Elevator_Attenuation" null))
      (:`then_1`
        (`GameplayStatics.ApplyDamage` Player _returnvalue (`Pawn.GetController` Player) self "/Game/Fadeout_Content/Core/Weapons/DamageTypes/DT_Wrench.DT_Wrench_C")
        (`KismetArrayLibrary.Array_AddUnique` (`self.hitPlayers`) Player)))))

(event `self.Box.OnComponentBeginOverlap`
  (params (OverlappedComponent :type "PrimitiveComponent Object Reference") (OtherActor :type "Actor Object Reference") (OtherComp :type "PrimitiveComponent Object Reference") (OtherBodyIndex :type Integer) (bFromSweep :type Boolean) (SweepResult :type "HitResult Structure (by ref)"))
  (bind _asbp_player_character (cast `/Game/Fadeout_Content/Core/Characters/BP_PlayerCharacter` OtherActor))
  (`self.Hit_Player` _asbp_player_character (* (`KismetMathLibrary.Normal` (+ (`.Normal` (`GameplayStatics.BreakHitResult` SweepResult)) (0.0 0.0 -0.4))) -1500.0)))

(fn `UserConstructionScript`
  (`KismetSystemLibrary.DrawDebugSphere` (`SplineComponent.GetLocationAtDistanceAlongSpline` (`/Game/Fadeout_Content/Core/Characters/BP_PatrolPath.Spline` (`self.PatrolPath`)) (`self.Current Distance`) "World") 300.0 12 (struct :`R` 1.0 :`G` 1.0 :`B` 1.0 :`A` 1.0) 2.0))