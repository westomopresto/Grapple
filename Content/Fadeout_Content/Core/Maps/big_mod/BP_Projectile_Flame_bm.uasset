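; Flame projectile that grows after spawning and burns actors entering its BurnRadius, extending a parent projectile Blueprint.
; Overlaps apply damage once per actor via BurnVictims and skip the instigator unless CanHurtOwnerNow, which a spawn timeline event sets false despite its "Can Collide" name.
; On hit, it detaches Trail and BurnRadius, briefly delays removing the burn area, then scales the trail by timeline before destroying itself.
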(event `self.BurnRadius.OnComponentBeginOverlap`
  (params (OverlappedComponent :type "PrimitiveComponent Object Reference") (OtherActor :type "Actor Object Reference") (OtherComp :type "PrimitiveComponent Object Reference") (OtherBodyIndex :type Integer) (bFromSweep :type Boolean) (SweepResult :type "HitResult Structure (by ref)"))
  (`KismetSystemLibrary.PrintString` (`KismetSystemLibrary.GetDisplayName` OtherActor))
  (if (or (!= (`self.Instigator`) OtherActor) (`self.CanHurtOwnerNow`))
    (if (not (`KismetArrayLibrary.Array_Contains` (`self.BurnVictims`) OtherActor))
      (`GameplayStatics.ApplyDamage` OtherActor 3.0 (`self.Instigator Controller`) self (`self.DamageType`))
      (`KismetArrayLibrary.Array_Add` (`self.BurnVictims`) OtherActor))))

(event `self.OnProjectileHitEvent`
  (params (OtherActor :type "Actor Object Reference") (OtherComponent :type "PrimitiveComponent Object Reference") (HitResult :type "HitResult Structure (by ref)") (fromHit :type Boolean))
  (`self.K2_SetActorRotation` (struct :`Pitch` 270.0))
  (`SceneComponent.K2_DetachFromComponent` (`self.trail`) "KeepWorld" "KeepWorld" "KeepWorld" true)
  (`SceneComponent.K2_DetachFromComponent` (`self.BurnRadius`) "KeepWorld" "KeepWorld" "KeepWorld" true)
  (`KismetSystemLibrary.Delay` 0.2)
  (`ActorComponent.K2_DestroyComponent` (`self.BurnRadius`))
  (`KismetSystemLibrary.Delay` 0.2)
  (bind (_direction _scale) (`Timeline|Scale Over Time` :`NewTime` 1.0)
    (:`Update`
      (`SceneComponent.SetRelativeScale3D` (`self.trail`) (`KismetMathLibrary.Conv_DoubleToVector` _scale)))
    (:`Finished`
      (`self.K2_DestroyActor`))))

(event `self.ReceiveBeginPlay`
  (`parent.ReceiveBeginPlay`)
  (bind (_direction _scalealpha_start) (`Timeline|Timeline_0` :!via `PlayFromStart`)
    (:`Update`
      (`self.SetActorScale3D` (`KismetMathLibrary.Conv_DoubleToVector` _scalealpha_start)))
    (:`CanCollideWithOwnerNow`
      (set `self.CanHurtOwnerNow` false))))

(fn `UserConstructionScript`
  (`parent.UserConstructionScript`))