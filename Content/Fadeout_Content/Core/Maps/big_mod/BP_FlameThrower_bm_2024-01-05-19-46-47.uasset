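; Flamethrower weapon Blueprint that starts and stops a flame particle effect and looping sound on fire press and release.
; Pressing fire starts the flame only if the owner is not swimming and the ammo cost is met; releasing or dropping stops it.
; State replicates via multicast on authority or through a server event on remotes, with the attached loop sound fading out before being destroyed.
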(event `self.OnDropped`
  (bind _currentflamesound (`self.currentFlameSound`))
  (`parent.OnDropped`)
  (`parent.OnFireRelease` false :!label _label)
  (`self.Fire Release FlameThrower`)
  (`/Engine/EditorBlueprintResources/StandardMacros.IsValid` _currentflamesound
    (:`Is Valid`
      (`ActorComponent.K2_DestroyComponent` _currentflamesound))))

(event `self.OnDroppedNPC`
  (`parent.OnDroppedNPC`)
  (goto _label))

(event `self.OnFirePress`
  (`parent.OnFirePress`)
  (bind _firecostmet (`self.AmmoCheckFunction`))
  (if (and (not (`/Game/Fadeout_Content/Core/Characters/BP_PlayerCharacter.isSwimmingNET` (`self.PlayerOwner`))) _firecostmet)
    (`/Engine/EditorBlueprintResources/ActorMacros.Switch Has Authority`
      (:`Authority`
        (`self.Multicast_Flame` true))
      (:`Remote`
        (`self.server_flame` true)))
    (else
      (`/Engine/EditorBlueprintResources/ActorMacros.Switch Has Authority`
        (:`Authority`
          (`self.Multicast_Flame` false))
        (:`Remote`
          (`self.server_flame` false))))))

(event `Fire Release FlameThrower`
  (`/Engine/EditorBlueprintResources/ActorMacros.Switch Has Authority` :!label _label_2
    (:`Authority`
      (`self.Multicast_Flame` false))
    (:`Remote`
      (`self.server_flame` false))))

(event `Multicast_Flame`
  (params (start :type Boolean))
  (bind _currentflamesound (`self.currentFlameSound`))
  (bind _currentflamesound_2 (`self.currentFlameSound`))
  (if start
    (`self.PlayFireSound`)
    (`/Engine/EditorBlueprintResources/StandardMacros.IsValid` (`self.currentFlameSound`)
      (:`Is Valid`
        (`ActorComponent.Activate` (`self.ParticleSystem`) false))
      (:`Is Not Valid`
        (bind _returnvalue (`GameplayStatics.SpawnSoundAttached` "/Game/Fadeout_Content/Core/Audio/Weapon_SFX/Flame/Flame_Loop.Flame_Loop" (`self.SkeletalMesh`) "None" (0.0 0.0 0.0) (struct) "KeepRelativeOffset" false 1.0 1.0 0.0 null null))
        (`/Engine/EditorBlueprintResources/StandardMacros.IsValid` _currentflamesound
          (:`Is Valid`
            (`ActorComponent.K2_DestroyComponent` _currentflamesound))
          (:`Is Not Valid`
            _))
        (set `self.currentFlameSound` _returnvalue)
        (`ActorComponent.Activate` (`self.ParticleSystem`) false)))
    (else
      (`ActorComponent.Deactivate` (`self.ParticleSystem`))
      (`/Engine/EditorBlueprintResources/StandardMacros.IsValid` (`self.currentFlameSound`)
        (:`Is Valid`
          (`AudioComponent.FadeOut` _currentflamesound_2 1.0 0.0 "Linear")
          (`KismetSystemLibrary.Delay` 1.0)
          (`/Engine/EditorBlueprintResources/StandardMacros.IsValid` _currentflamesound_2
            (:`Is Valid`
              (`ActorComponent.K2_DestroyComponent` _currentflamesound_2))))))))

(event `self.OnFireRelease`
  (params (`charged?` :type Boolean))
  (`parent.OnFireRelease` `charged?`)
  (goto _label_2))

(event `server_flame`
  (params (start :type Boolean))
  (`self.Multicast_Flame` start))

(fn `UserConstructionScript`
  (`parent.UserConstructionScript`))