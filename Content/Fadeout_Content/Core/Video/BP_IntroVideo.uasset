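; BP_IntroVideo is an actor that plays a fullscreen intro video with sound.
; On BeginPlay it opens the media source, then on success shows a VideoFullscreen widget at high Z-order, starts playback and boosts the volume.
; End of playback, a skip from the widget, or any open or play failure leads to StopVideo, which closes the player, removes the widget, calls VideoFinished and destroys the actor.
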(event `Stop Video`
  (`MediaPlayer.Close` (`self.MediaPlayer`))
  (`Widget.RemoveFromParent` (`self.FullScreenVideo`))
  (`self.VideoFinished`)
  (`self.K2_DestroyActor`))

(event `self.ReceiveBeginPlay`
  (bind _mediaplayer (`self.MediaPlayer`))
  (add `MediaPlayer.OnMediaOpenFailed` _mediaplayer (delegate `Media Failed`))
  (add `MediaPlayer.OnMediaOpened` _mediaplayer (delegate `Media Opened`))
  (bind _returnvalue (`MediaPlayer.OpenSource` _mediaplayer (`self.VideoSource`)))
  (if (not _returnvalue)
    (`self.Stop Video`)))

(event `Media Opened`
  (params (OpenedUrl :type String))
  (bind _mediaplayer (`self.MediaPlayer`))
  (bind _returnvalue (`|CreateWidget` "/Game/Fadeout_Content/Core/Video/VideoFullscreen_Widget.VideoFullscreen_Widget_C"))
  (bind _output_get (set `self.FullScreenVideo` _returnvalue))
  (`UserWidget.AddToPlayerScreen` _output_get 999)
  (bind _returnvalue_2 (`MediaPlayer.Play` _mediaplayer))
  (if _returnvalue_2
    (add `MediaPlayer.OnEndReached` _mediaplayer (delegate `Video Finished Event`))
    (add `/Game/Fadeout_Content/Core/Video/VideoFullscreen_Widget.Skipped` _output_get (delegate `Video Finished Event`))
    (`SynthComponent.SetVolumeMultiplier` (`self.MediaSound`) 3.0)
    (else
      (`self.Stop Video`))))

(event `Media Failed`
  (params (FailedUrl :type String))
  (`self.Stop Video`))

(event `Video Finished Event`
  (`self.Stop Video`))

(fn `UserConstructionScript`)