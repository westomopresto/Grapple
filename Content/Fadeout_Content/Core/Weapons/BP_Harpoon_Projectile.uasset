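; Harpoon weapon projectile that impales an enemy player and pins them to world geometry with a cable.
; A team-checked player hit stores the victim and bends the projectile downward.
; On hard-surface impact, it syncs position, rotates to the surface, attaches the cable and timeline-drags a nearby victim to a capsule-traced spot.
; The server then applies bleed and slow; straying too far after a delay snaps the cable and reverts the slow.
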(event `self.ReceiveTick`
  (params (DeltaSeconds :type "Float (single-precision)"))
  (bind _heldplayers (`self.HeldPlayers`))
  (bind _harpoonslow (`self.HarpoonSlow`))
  (bind _returnvalue (`self.K2_GetActorLocation` _heldplayers))
  ;[1 1 1] Snap cable
  (`|ExecutionSequence`
    (:`then_0`
      ;[1 1 1] Rotate into position
      (if (`self.stuck`)
        (set `self.snapRotTimelimit` (+ DeltaSeconds (`self.snapRotTimelimit`)))
        (`self.K2_SetActorRotation` (`KismetMathLibrary.RInterpTo` (`self.K2_GetActorRotation`) (`KismetMathLibrary.MakeRotFromX` (* (`self.impactNormal`) -1.0)) DeltaSeconds 5.0) true)
        (if (>= (`self.snapRotTimelimit`) 0.2)
          (set `self.stuck` false))))
    (:`then_1`
      (if (and (`self.holdingSomeone`) (`KismetSystemLibrary.IsValid` _heldplayers) (not (`self.snapped`)))
        (if (and (>= (`KismetMathLibrary.Vector_Distance` _returnvalue (`self.K2_GetActorLocation`)) 1300.0) (`self.canSnap`))
          (set `self.snapped` true)
          (set `CableComponent.bAttachEnd` false (`self.Cable`))
          (`GameplayStatics.PlaySoundAtLocation` "/Game/Fadeout_Content/Core/Audio/Harpoon/ropeSnap_cue.ropeSnap_cue" _returnvalue (struct) 1.0 1.0 0.0 null null null)
          (`/Engine/EditorBlueprintResources/StandardMacros.IsValid` _harpoonslow
            (:`Is Valid`
              (`/Game/Fadeout_Content/Core/Weapons/BP_DoT_Effect_Damage_Over_Time.Revert Weakness` _harpoonslow))))))))

(event `Correct Position Multicast`
  (params (NewLocation :type "Vector Structure"))
  ;[1 1 1] Position correction
  (`self.K2_SetActorLocation` NewLocation false true))

(event `Hit Multi`
  (params (impactNormal :type "Vector Structure") (Location :type "Vector Structure"))
  (bind _cable (`self.Cable`))
  (bind _returnvalue (`SceneComponent.K2_GetComponentLocation` (`self.AttachEmpty`)))
  ;[1 1 1] Is a player close enough to impale
  (set `self.impactNormal` impactNormal)
  (`self.Correct Position Authority`)
  (set `self.stuck` true)
  (if (`KismetSystemLibrary.IsValid` (`self.HeldPlayers`))
    (if (<= (`KismetMathLibrary.Vector_Distance` Location (`self.playerHitLoc`)) 5000.0)
      (set `CableComponent.bAttachEnd` true _cable)
      (`CableComponent.SetAttachEndToComponent` _cable (`/Game/Fadeout_Content/Core/Characters/BP_PlayerCharacter.healFX` (`self.HeldPlayers`)) "None")
      (set `self.holdingSomeone` true)
      ;[1 1 1] Find safe place for player to be
      (bind (_outhit _returnvalue_2) (`KismetSystemLibrary.CapsuleTraceSingleForObjects` :`Start` (+ _returnvalue (* (`self.GetActorForwardVector`) -100.0) (* (`self.GetActorUpVector`) 100.0)) :`End` _returnvalue :`Radius` 56.0 :`HalfHeight` 96.0 :`ObjectTypes` (`|MakeArray` "ObjectTypeQuery1" :!type "EObjectTypeQuery Enum") :`bTraceComplex` true :`DrawDebugType` "ForDuration" :`TraceColor` (struct :`R` 0.239295 :`B` 1.0 :`A` 1.0)))
      ;[1 1 1] Drag the player
      (bind (_direction _lerp0_to_1) (`Timeline|Timeline_1` :`NewTime` 1.0 :!via `PlayFromStart`)
        (:`Update`
          (`self.K2_SetActorLocation` (`self.HeldPlayers`) (`KismetMathLibrary.VLerp` (`self.K2_GetActorLocation` (`self.HeldPlayers`)) (`KismetMathLibrary.SelectVector` (`.Location` (`GameplayStatics.BreakHitResult` _outhit)) (+ (`SceneComponent.K2_GetComponentLocation` (`self.AttachEmpty`)) (0.0 0.0 96.0)) _returnvalue_2) _lerp0_to_1) false false))
        (:`Finished`
          (`/Engine/EditorBlueprintResources/ActorMacros.Switch Has Authority`
            (:`Authority`
              (`self.Trap Target`))))))))

(event `self.SurfaceImpactEvent`
  (params (HitResult :type "HitResult Structure") (`Hardsurface?` :type Boolean) (hitactor :type "Actor Object Reference"))
  (bind (_bblockinghit _binitialoverlap _time _distance _location _impactpoint _normal _impactnormal) (`GameplayStatics.BreakHitResult` HitResult))
  (`AudioComponent.FadeOut` (`self.Audio`) 0.25 0.0 "Linear")
  (`/Engine/EditorBlueprintResources/ActorMacros.Switch Has Authority`
    (:`Authority`
      (`/Engine/EditorBlueprintResources/StandardMacros.IsValid` hitactor
        (:`Is Valid`
          (if `Hardsurface?`
            ;[1 1 1] Is a player close enough to impale
            (`parent.SurfaceImpactEvent` HitResult `Hardsurface?` hitactor)
            (`self.Hit Multi` _impactnormal _location)
            (else
              ;[1 1 1] Set Player var
              (bind _asbp_player_character (cast `/Game/Fadeout_Content/Core/Characters/BP_PlayerCharacter` hitactor))
              (`self.Multi cast Soft hit` _asbp_player_character (`.Location` (`GameplayStatics.BreakHitResult` HitResult))))))))
    (:`Remote`
      (`self.PlayImpactEffects` HitResult `Hardsurface?`))))

(event `Multi cast Soft hit`
  (params (`BP Character` :type "/Game/Fadeout_Content/Core/Characters/BP_PlayerCharacter Object Reference") (playerHitLoc :type "Vector Structure"))
  ;[1 1 1] Set Player var
  (bind _triggered (`self.Would Trigger` `BP Character`))
  (if (and _triggered (not (`/Game/Fadeout_Content/Core/Characters/BP_PlayerCharacter.CCd` `BP Character`)))
    (set `self.playerHitLoc` playerHitLoc)
    (set `self.HeldPlayers` `BP Character`)
    (set `ProjectileMovementComponent.ProjectileGravityScale` 7.0 (`self.ProjectileMovement`))
    (`ProjectileMovementComponent.SetVelocityInLocalSpace` (`self.ProjectileMovement`) (* (1.0 0.0 -0.5) (`ProjectileMovementComponent.InitialSpeed` (`self.ProjectileMovement`))))
    (`ProjectileMovementComponent.SetVelocityInLocalSpace` (`self.ProjectileMovement`) (* (1.0 0.0 -0.5) (`ProjectileMovementComponent.InitialSpeed` (`self.ProjectileMovement`))))))

(event `Trap Target`
  (bind _heldplayers (`self.HeldPlayers`))
  ;[1 1 1] Trap
  (if (not (`self.Trapped`))
    (`/Engine/EditorBlueprintResources/StandardMacros.IsValid` _heldplayers
      (:`Is Valid`
        (set `self.Trapped` true)
        (`/Game/Fadeout_Content/Core/Characters/BP_PlayerCharacter.Attach DoT ` _heldplayers "/Game/Fadeout_Content/Core/Weapons/BP_Bleed_DOT.BP_Bleed_DOT_C" (`self.GetInstigator`) false false)
        (bind _applied_dot (`/Game/Fadeout_Content/Core/Characters/BP_PlayerCharacter.Attach DoT ` (`self.HeldPlayers`) "/Game/Fadeout_Content/Core/Weapons/BP_Harpoon_Slow_DOT.BP_Harpoon_Slow_DOT_C" null false false))
        (set `self.HarpoonSlow` _applied_dot)
        (`GameplayStatics.SpawnSoundAtLocation` "/Game/Fadeout_Content/Core/Audio/Harpoon/pierce_cue.pierce_cue" (`self.K2_GetActorLocation`) (struct) 1.0 1.0 0.0 null null)
        (`self.ForceNetUpdate`)
        (`KismetSystemLibrary.Delay` 1.0)
        (set `self.canSnap` true)))))

(fn `Correct Position Authority`
  (if (`self.HasAuthority`)
    (`self.Correct Position Multicast` (`self.K2_GetActorLocation`))
    (return)
    (else
      (return))))

(fn `UserConstructionScript`)

(fn `Would Trigger`
  (params (InputPin :type "/Game/Fadeout_Content/Core/Characters/BP_PlayerCharacter Object Reference"))
  (returns (Triggered :type Boolean))
  (bind _playerstate (`Pawn.PlayerState` InputPin))
  (bind _playerstate_2 (`Pawn.PlayerState` (`self.Instigator`)))
  (bind _returnvalue (!= (`PlayerState.PlayerId` _playerstate) (`PlayerState.PlayerId` _playerstate_2)))
  (`/Engine/EditorBlueprintResources/StandardMacros.IsValid` (`self.Instigator`)
    (:`Is Valid`
      (bind _asfo_player_state (cast `/Game/Fadeout_Content/Core/Support/Multiplayer_Support/FO_PlayerState` _playerstate)
        (:`then`
          (bind _asfo_player_state_2 (cast `/Game/Fadeout_Content/Core/Support/Multiplayer_Support/FO_PlayerState` _playerstate_2))
          (bind _team (`/Game/Fadeout_Content/Core/Support/Multiplayer_Support/FO_PlayerState.Team` _asfo_player_state))
          (if (`KismetStringLibrary.NotEqual_StrStr` _team "ffa")
            (if (and (not (`KismetStringLibrary.EqualEqual_StrStr` _team (`/Game/Fadeout_Content/Core/Support/Multiplayer_Support/FO_PlayerState.Team` _asfo_player_state_2))) _returnvalue)
              _
              (else
                (return false)))
            (else
              ;[1 1 1] FFA
              (if _returnvalue
                _
                (else
                  (return false)))))
          (return true))
        (:`CastFailed`
          (return true))))
    (:`Is Not Valid`
      (return false))))