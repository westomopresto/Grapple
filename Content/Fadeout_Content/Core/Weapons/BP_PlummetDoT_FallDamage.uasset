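; Plummet weakness effect that deals fall damage to an airborne player when they land.
; On the server it ends at once if the player is grounded, otherwise it stores the activation location and binds to the player's landed and jumped dispatchers.
; Landing applies damage scaled by straight-line distance from that location, not just height, then ends the effect; jumping cancels it.
; Debug sphere and text show the start point and damage.
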(event `self.Apply Weakness Event`
  (bind _player (`self.Player`))
  (bind _player_2 (`self.Player`))
  (`/Engine/EditorBlueprintResources/ActorMacros.Switch Has Authority`
    (:`Authority`
      (if (`NavMovementComponent.IsMovingOnGround` (`Character.CharacterMovement` _player_2))
        (`self.earlyEnd`)
        (else
          (add `/Game/Fadeout_Content/Core/Characters/BP_PlayerCharacter.onLandedDispatch` _player (delegate `LandedWhileActive`))
          (add `/Game/Fadeout_Content/Core/Characters/BP_PlayerCharacter.onJumpDispatch` _player (delegate `JumpedWhileActive`))
          (bind _output_get (set `self.LocationOnActivate` (`self.K2_GetActorLocation` _player_2)))
          (`KismetSystemLibrary.DrawDebugSphere` _output_get 100.0 6 (struct :`R` 1.0 :`B` 0.075233 :`A` 1.0) 10.0 2.0))))))

(event `LandedWhileActive`
  (bind _returnvalue (`self.K2_GetActorLocation` (`self.Player`)))
  (bind _returnvalue_2 (* (`KismetMathLibrary.Vector_Distance` (`self.LocationOnActivate`) _returnvalue) 0.05))
  (`KismetSystemLibrary.DrawDebugString` _returnvalue (`KismetStringLibrary.Concat_StrStr` "Fall damage: " (`KismetStringLibrary.Conv_DoubleToString` _returnvalue_2)) null (struct :`R` 1.0 :`G` 0.018015 :`A` 1.0) 9.0)
  (`GameplayStatics.ApplyDamage` (`self.Player`) _returnvalue_2 (`self.Instigator Controller`) (`self.Damage Causer`) (`self.Damage Type`))
  (`self.earlyEnd`))

(event `JumpedWhileActive`
  (if (`KismetSystemLibrary.IsValid` self)
    (`self.earlyEnd`)))

(fn `UserConstructionScript`
  (`parent.UserConstructionScript`))