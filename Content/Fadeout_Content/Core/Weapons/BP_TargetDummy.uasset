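; BP_TargetDummy is a damageable test target that reports its state through a text render.
; On any damage it subtracts the amount from its Health and shows the remaining value after a "Damage:" label.
; Once Health reaches zero or below, the text changes to "Cube Is Dead", and nothing else happens to the actor.
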(event `self.ReceiveAnyDamage`
  (params (Damage :type "Float (single-precision)") (DamageType :type "DamageType Object Reference") (InstigatedBy :type "Controller Object Reference") (DamageCauser :type "Actor Object Reference"))
  (bind _textrender (`self.TextRender`))
  (bind _output_get (set `self.Health` (- (`self.Health`) Damage)))
  (if (<= _output_get 0.0)
    (`TextRenderComponent.K2_SetText` _textrender "Cube Is Dead")
    (else
      (`TextRenderComponent.K2_SetText` _textrender (`KismetTextLibrary.Conv_StringToText` (`KismetStringLibrary.BuildString_Double` "" " Damage: " _output_get))))))

(fn `UserConstructionScript`)