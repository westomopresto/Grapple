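; BP_Bingo_Revolver is a revolver weapon Blueprint whose headshot multiplier grows with its level.
; BeginPlay runs the parent logic, then caches the inherited headshot multiplier as a base value.
; RevolverLevelUpEvent stores the given level, rebuilds the weapon name to show it, and adds a linear per-level bonus to that base.
; The separate RevolverlevelUp function is empty.
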(event `self.ReceiveBeginPlay`
  (`parent.ReceiveBeginPlay`)
  (set `self.headshotmult_base` (`self.headShotMultiplier`)))

(event `RevolverLevelUpEvent`
  (params (InInt :type Integer))
  (bind _level (`self.Level`))
  (set `self.Level` InInt)
  (set `self.Name` (`KismetStringLibrary.Conv_StringToName` (`KismetStringLibrary.BuildString_Int` "" "Revolver lvl. " _level)))
  (set `self.headShotMultiplier` (+ (`self.headshotmult_base`) (* (`KismetMathLibrary.Conv_IntToDouble` _level) 0.2))))

(fn `RevolverlevelUp`)

(fn `UserConstructionScript`
  (`parent.UserConstructionScript`))