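; Dalton rifle weapon Blueprint that adds scoped alt-fire aiming on top of its parent weapon logic.
; Alt-fire press and release toggle the CameraToCameraAiming flag with debug prints, and swapping in or out clears it.
; When alt fire is allowed, the multicast press blocks tool swapping and moves the owning BP_PlayerCharacter to a scoped aim camera, with optional zoom.
; Dropping the rifle destroys the actor.
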(event `self.onSwapIn`
  (`parent.onSwapIn`)
  (set `self.CameraToCameraAiming` false))

(event `self.onSwapOut`
  (`parent.onSwapOut`)
  (set `self.CameraToCameraAiming` false))

(event `self.AltFireRelease`
  (`parent.AltFireRelease`)
  (bind _output_get (set `self.CameraToCameraAiming` false))
  (`KismetSystemLibrary.PrintString` (`KismetStringLibrary.Conv_BoolToString` _output_get)))

(event `self.OnAltFirePress`
  (`parent.OnAltFirePress`)
  (bind _output_get (set `self.CameraToCameraAiming` true))
  (`KismetSystemLibrary.PrintString` (`KismetStringLibrary.Conv_BoolToString` _output_get)))

(event `self.Alt Fire Press Multicast`
  (if (`self.canAltFire?`)
    (bind _asbp_player_character (cast `/Game/Fadeout_Content/Core/Characters/BP_PlayerCharacter` (`self.GetOwner`)))
    (set `/Game/Fadeout_Content/Core/Characters/BP_PlayerCharacter.canSwapTools?` false _asbp_player_character)
    (`/Game/Fadeout_Content/Core/Characters/BP_PlayerCharacter.toAimCam` _asbp_player_character (`self.ZoomOnSight?`) true)))

(event `self.OnDropped`
  (`self.K2_DestroyActor`))

(fn `UserConstructionScript`
  (`parent.UserConstructionScript`))