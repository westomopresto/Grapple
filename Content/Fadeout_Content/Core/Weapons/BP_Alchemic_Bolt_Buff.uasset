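; BP_Alchemic_Bolt_Buff is a weapon buff that replenishes the player's ammo over damage ticks.
; On each DamageTick, it checks whether held Energy ammo is below the player's maximum.
; If so, it grants a fixed ammo reward through the player's item pickup function with the OverrideForAbby flag set.
; The tick event is its only active logic, with no custom setup.
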(event `self.Damage Tick`
  (bind _player (`self.Player`))
  (if (< (`.Energy_18_2D8D75E04E1979C951FEA185FE1A6270` (break `/Game/Fadeout_Content/Core/Support/AmmoStruct` (`/Game/Fadeout_Content/Core/Characters/BP_PlayerCharacter.HeldAmmo` _player))) (`.Energy_18_2D8D75E04E1979C951FEA185FE1A6270` (break `/Game/Fadeout_Content/Core/Support/AmmoStruct` (`/Game/Fadeout_Content/Core/Characters/BP_PlayerCharacter.MaxHeldAmmo` _player))))
    (`/Game/Fadeout_Content/Core/Characters/BP_PlayerCharacter.PickUpItemBase _ USE` _player null 0 (make `/Game/Fadeout_Content/Core/Support/AmmoStruct` :`Energy` 30) true)))

(fn `UserConstructionScript`
  (`parent.UserConstructionScript`))