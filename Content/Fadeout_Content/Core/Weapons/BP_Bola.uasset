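; BP_Bola is a thrown projectile weapon that builds on its parent weapon's equip and fire logic.
; After firing, it blocks further fire, hides its mesh after the fire delay to mimic the throw, then restores both when the cooldown ends.
; Swapping out forces a fire release, and dropping the weapon destroys it.
; An unconnected leftover would deal half the projectile's damage to the owning player as vamp damage.
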(event `self.ReceiveBeginPlay`
  (`parent.ReceiveBeginPlay`))

(event `self.onSwapIn`
  (`parent.onSwapIn`))

(event `self.onSwapOut`
  (`parent.onSwapOut`)
  (`self.OnFireRelease` false))

(event `self.OnDropped`
  (`self.K2_DestroyActor`))

(event `self.Success Fire`
  (`parent.Success Fire`))

(event `self.Fire Projectile Event`
  (bind _skeletalmesh (`self.SkeletalMesh`))
  (`parent.Fire Projectile Event`)
  (set `self.CanFire?` false)
  (`KismetSystemLibrary.Delay` (`self.Fire Delay`))
  (`SceneComponent.SetVisibility` _skeletalmesh false true)
  (`KismetSystemLibrary.Delay` (- (`self.Fire CoolDown`) (`self.Fire Delay`)))
  (`SceneComponent.SetVisibility` _skeletalmesh true true)
  (set `self.CanFire?` true))

(event `self.OnFirePress`
  (`parent.OnFirePress`))

(fn `UserConstructionScript`
  (`parent.UserConstructionScript`))