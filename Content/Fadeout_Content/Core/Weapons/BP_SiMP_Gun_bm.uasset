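; BP_SiMP_Gun_bm is a burst-fire projectile gun built on a parent weapon Blueprint.
; On fire press it sizes the burst to available ammo, capped at MaxFire, and sets FireCost to that count before calling the parent.
; When firing is allowed, a looping timer spawns a projectile and plays the fire sound per tick, then clears itself once the burst completes.
; The shell-eject emitter is unwired and SpawnProjectileServer is empty.
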(event `Burst`
  (bind _returnvalue (`KismetSystemLibrary.K2_SetTimerDelegate` (delegate `Burst Window`) (`self.TimebetweenShots_Burst`) true))
  (set `self.BurstTimer` _returnvalue))

(event `Burst Window`
  (`self.Spawn Projectile` (stale `self.Spawn Projectile Server` SpawnTransform) (stale `self.Spawn Projectile Server` OwningWeapon) (stale `self.Spawn Projectile Server` `Initial Speed Override`) (stale `self.Spawn Projectile Server` `Override Speed`))
  (`self.PlayFireSound`)
  (`/Engine/EditorBlueprintResources/StandardMacros.IncrementInt` (`self.Current Fire`)
    (:`  `
      (if (>= (`self.Current Fire`) (`self.Current Burst`))
        (`KismetSystemLibrary.K2_ClearAndInvalidateTimerHandle` (`self.BurstTimer`))
        (set `self.Current Fire` 0)))))

(event `self.Spawn Projectile Server`
  (params (SpawnTransform :type "Transform Structure") (OwningWeapon :type "/Game/Fadeout_Content/Core/Weapons/BP_weaponBase Object Reference") (RayHitActor :type "Actor Object Reference") (`Initial Speed Override` :type "Float (single-precision)") (`Override Speed` :type Boolean)))

(event `self.Fire Projectile Event`
  (params (skipDelays :type Boolean) (customSpread :type Boolean) (spreadTransform :type "Transform Structure"))
  (if (`self.CanFire?`)
    (`self.Burst`)))

(event `self.OnFirePress`
  (bind (_firecostmet _ammowehave) (`self.AmmoCheckFunction`))
  (`self.Server current burst` _ammowehave)
  (`parent.OnFirePress`))

(event `Server current burst`
  (params (`Ammo We have` :type Integer))
  (if (< `Ammo We have` (`self.maxFire`))
    (set `self.Current Burst` (`KismetMathLibrary.Clamp` `Ammo We have` 1 99))
    (else
      (set `self.Current Burst` (`self.maxFire`))))
  (set `self.FireCost` (`self.Current Burst`)))

(fn `UserConstructionScript`
  (`parent.UserConstructionScript`))