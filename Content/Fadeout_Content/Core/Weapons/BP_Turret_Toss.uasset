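; BP_Turret_Toss is a weapon Blueprint, by its name for tossing turrets, that fires a projectile on press and destroys itself when dropped.
; A fire press checks CanFire and ammo cost, then either fires, deducts ammo and updates the instigator's weapon info, or plays a no-ammo sound.
; CanFire is set true both before and after the 0.2-second delay, so this graph never blocks repeat fire.
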(event `self.OnFirePress`
  (if (`self.CanFire?`)
    (set `self.CanFire?` true)
    (bind _firecostmet (`self.AmmoCheckFunction`))
    (if _firecostmet
      (`self.Fire Projectile Event` false)
      (`self.AmmoCostFunction` false)
      (`self.UpdateInstigatorWeaponInfo`)
      (else
        (`self.PlayNoAmmoSound`)))
    (`KismetSystemLibrary.Delay` 0.2)
    (set `self.CanFire?` true)))

(event `self.OnDropped`
  ;[1 1 1] Kill on dropped
  (`parent.OnDropped`)
  (`self.K2_DestroyActor`))

(fn `UserConstructionScript`
  (`parent.UserConstructionScript`))