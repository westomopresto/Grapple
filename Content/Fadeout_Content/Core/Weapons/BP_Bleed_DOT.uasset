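; Bleed damage-over-time effect that the Wolf character inflicts on a player, extending a parent effect class.
; On begin play it expires immediately on turrets; otherwise it registers the victim with the instigating Wolf as a bleeding enemy.
; It reveals its Trail only when the first local player controller belongs to the victim or the Wolf.
; On expiry it removes the victim from the Wolf's tracking before running parent cleanup.
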(event `Set Bleed Trail Visibility`
  (`SceneComponent.SetVisibility` (`self.Trail`) true false))

(event `self.ReceiveBeginPlay`
  (bind _instigator (`self.Instigator`))
  (bind _player (`self.Player`))
  (bind _playerstate (`Controller.PlayerState` (`GameplayStatics.GetPlayerController` 0)))
  (`parent.ReceiveBeginPlay`)
  (cast `/Game/Fadeout_Content/Core/Characters/BP_Turret` (`self.Player`)
    (:`then`
      (`self.Expire`))
    (:`CastFailed`
      (bind _asbp_char_wolf (cast `/Game/Fadeout_Content/Core/Characters/BP_Char_Wolf` _instigator))
      (`/Game/Fadeout_Content/Core/Characters/BP_Char_Wolf.Find Bleeding Enemy` _asbp_char_wolf _player true)
      (`|ExecutionSequence`
        (:`then_0`
          (if (== _playerstate (`Pawn.PlayerState` _player))
            (`self.Set Bleed Trail Visibility`)))
        (:`then_1`
          (if (== _playerstate (`Pawn.PlayerState` _instigator))
            (`self.Set Bleed Trail Visibility`)))))))

(event `self.Expire`
  (bind _player (`self.Player`))
  (bind _asbp_char_wolf (cast `/Game/Fadeout_Content/Core/Characters/BP_Char_Wolf` (`self.Instigator`))
    (:`then`
      (`/Engine/EditorBlueprintResources/StandardMacros.IsValid` _player
        (:`Is Valid`
          (`/Engine/EditorBlueprintResources/StandardMacros.IsValid` _asbp_char_wolf
            (:`Is Valid`
              (`/Game/Fadeout_Content/Core/Characters/BP_Char_Wolf.Find Bleeding Enemy` _asbp_char_wolf _player false))
            (:`Is Not Valid`
              _)))
        (:`Is Not Valid`
          _)))
    (:`CastFailed`
      _))
  (`parent.Expire`))

(fn `UserConstructionScript`
  (`parent.UserConstructionScript`))