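; BP_Slow_DOT is a weapon status effect that slows the affected player and weakens their jump.
; ApplyWeaknessEvent sets the player's SpeedMod to SpeedReductionMod, calls ToSprintMulticast, then caches and halves the jump Z velocity.
; RevertWeakness resets SpeedMod to normal, calls the same multicast and restores the cached jump velocity.
; Neither event contains timing or damage logic.
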(event `self.Apply Weakness Event`
  (bind _player (`self.Player`))
  (bind _charactermovement (`Character.CharacterMovement` _player))
  (bind _output_get (set `/Game/Fadeout_Content/Core/Characters/BP_PlayerCharacter.SpeedMod` (`self.SpeedReductionMod`) _player))
  (`/Game/Fadeout_Content/Core/Characters/BP_PlayerCharacter.toSprint Multicast` _player)
  (bind _output_get_2 (set `self.OriginalJumpHeight` (`CharacterMovementComponent.JumpZVelocity` _charactermovement)))
  (set `CharacterMovementComponent.JumpZVelocity` (/ _output_get_2 2.0) _charactermovement))

(event `self.Revert Weakness`
  (bind _player (`self.Player`))
  (set `/Game/Fadeout_Content/Core/Characters/BP_PlayerCharacter.SpeedMod` 1.0 _player)
  (`/Game/Fadeout_Content/Core/Characters/BP_PlayerCharacter.toSprint Multicast` _player)
  (set `CharacterMovementComponent.JumpZVelocity` (`self.OriginalJumpHeight`) (`Character.CharacterMovement` _player)))

(fn `UserConstructionScript`
  (`parent.UserConstructionScript`))