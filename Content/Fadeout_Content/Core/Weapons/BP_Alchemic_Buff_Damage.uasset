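; Alchemy effect that temporarily modifies a player's damage buffs, extending a parent effect's timer, damage tick and weakness events.
; On apply, the server adds each BUFFSLIST value to the player's DamageBuffs map, overwriting entries that are negative.
; On revert, it subtracts the same values from non-negative entries.
; The inherited damage tick is skipped when the affected player is the damage causer.
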(event `self.Damage Tick`
  (if (!= (`self.Player`) (`self.Damage Causer`))
    (`parent.Damage Tick`)))

(event `self.Timer`
  (`parent.Timer`))

(event `self.Apply Weakness Event`
  (bind _buffs_list (`self.BUFFS_LIST`))
  (bind _damagebuffs (`/Game/Fadeout_Content/Core/Characters/BP_PlayerCharacter.DamageBuffs` (`self.Player`)))
  (`parent.Apply Weakness Event`)
  (`/Engine/EditorBlueprintResources/ActorMacros.Switch Has Authority`
    (:`Authority`
      (bind _keys (`BlueprintMapLibrary.Map_Keys` _buffs_list))
      (for _array_element _keys
        (bind (_value _returnvalue) (`BlueprintMapLibrary.Map_Find` _buffs_list _array_element))
        (if _returnvalue
          (bind _value_2 (`BlueprintMapLibrary.Map_Find` _damagebuffs _array_element))
          (if (>= _value_2 0.0)
            (`BlueprintMapLibrary.Map_Add` _damagebuffs _array_element (+ _value_2 _value))
            (else
              (`BlueprintMapLibrary.Map_Add` _damagebuffs _array_element _value))))))))

(event `self.Revert Weakness`
  (bind _buffs_list (`self.BUFFS_LIST`))
  (bind _damagebuffs (`/Game/Fadeout_Content/Core/Characters/BP_PlayerCharacter.DamageBuffs` (`self.Player`)))
  (`parent.Revert Weakness`)
  (`/Engine/EditorBlueprintResources/ActorMacros.Switch Has Authority`
    (:`Authority`
      (bind _keys (`BlueprintMapLibrary.Map_Keys` _buffs_list))
      (for _array_element _keys
        (bind (_value _returnvalue) (`BlueprintMapLibrary.Map_Find` _buffs_list _array_element))
        (if _returnvalue
          (bind _value_2 (`BlueprintMapLibrary.Map_Find` _damagebuffs _array_element))
          (if (>= _value_2 0.0)
            (`BlueprintMapLibrary.Map_Add` _damagebuffs _array_element (- _value_2 _value))))))))

(fn `UserConstructionScript`
  (`parent.UserConstructionScript`))