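; Base Blueprint for pickup items and weapons, handling drop, pickup and timed despawn.
; Dropping re-checks the outline, calls an empty Initialize hook and starts a server-only Timeline that destroys the actor when finished; pickup stops it and forces a net update.
; Firing events refresh the owning BP_PlayerCharacter's weapon details after a short delay.
; Items flagged FromDeath run the drop logic on BeginPlay.
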(event `self.ReceiveBeginPlay`
  (`self.Initialize`)
  (if (`self.fromDeath`)
    (`self.OnDropped`)))

(event `UpdateInstigatorWeaponInfo`
  (`KismetSystemLibrary.Delay` 0.1)
  (bind _asbp_player_character (cast `/Game/Fadeout_Content/Core/Characters/BP_PlayerCharacter` (`self.GetOwner`)))
  (`/Game/Fadeout_Content/Core/Characters/BP_PlayerCharacter.updateWeaponDetails` _asbp_player_character))

(event `DespawnTimer`
  (if (`self.HasAuthority`)
    (bind (_direction _time) (`Timeline|Timeline_0` :!via `PlayFromStart` :!label _label)
      (:`Finished`
        (`self.K2_DestroyActor`)))))

(event `CancelDespawn`
  (if (`self.HasAuthority`)
    (goto _label :!via `Stop`)))

(event `OnPickUp`
  (params (setOwner :type "Actor Object Reference") (Instigator :type "Pawn Object Reference"))
  (`self.CancelDespawn`)
  (`self.ForceNetUpdate`))

(event `OnDroppedNPC`
  (`/Game/Fadeout_Content/Weapons/outline_controller.outlineCheck` (`self.outline_controller`) :!label _label_2)
  (`self.Initialize`)
  (`self.DespawnTimer`))

(event `Initialize`)

(event `OnFirePress`
  (`self.UpdateInstigatorWeaponInfo`))

(event `OnDropped`
  (goto _label_2))

(event `FireWeapon`
  (`self.UpdateInstigatorWeaponInfo`))

(fn `UserConstructionScript`)