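; Base weapon Blueprint for the player's weapons, with empty fire, alt-fire and swap-out events.
; Pickup sets owner, instigator and Player reference; pickup and drop run Initialize, which switches between ground and in-hand physics assets via OnGround.
; Helpers check durability, deduct FireCost from the player's ammo map when at least one round remains, and play fire or empty sounds.
; A timeline blends the player's aiming animation, and dropping also refreshes the outline.
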(event `self.ReceiveBeginPlay`
  (`self.Initialize`))

(event `UpdateInstigatorWeaponInfo`
  (`/Game/Fadeout_Content/Core/Characters/BP_PlayerCharacter.updateWeaponDetails` (`self.Player`)))

(event `OnPickUp`
  (params (setOwner :type "Actor Object Reference") (Instigator :type "Pawn Object Reference"))
  (`|ExecutionSequence`
    (:`then_0`
      (`self.SetOwner` setOwner))
    (:`then_1`
      (set `self.Instigator` Instigator)
      (`/Engine/EditorBlueprintResources/StandardMacros.IsValid` setOwner
        (:`Is Valid`
          (bind _asbp_player_character (cast `/Game/Fadeout_Content/Core/Characters/BP_PlayerCharacter` setOwner))
          (bind _output_get (set `self.Player` _asbp_player_character))
          (`KismetSystemLibrary.PrintString` (`KismetStringLibrary.BuildString_Object` "" "Setting owner as: " _output_get) true true (struct :`G` 0.66 :`B` 1.0 :`A` 1.0) 30.0))))
    (:`then_2`
      (set `self.onGround?` false))
    (:`then_3`
      (`self.Initialize`))))

(event `OnAltFire`)

(event `AltFireRelease`)

(event `OnFireRelease`
  (params (`charged?` :type Boolean)))

(event `OnDroppedNPC`
  (`/Game/Fadeout_Content/Weapons/outline_controller.outlineCheck` (`self.outline_controller`) :!label _label)
  (`self.Initialize`))

(event `Initialize`
  (bind _skeletalmesh (`self.SkeletalMesh`))
  (if (`self.onGround?`)
    (`SkinnedMeshComponent.SetPhysicsAsset` _skeletalmesh (`self.GroundPhysAsset`) false)
    (else
      (`SkinnedMeshComponent.SetPhysicsAsset` _skeletalmesh (`self.InHandPhysAsset`) false))))

(event `OnDropped`
  (goto _label))

(event `OnFire`)

(event `onSwapOut`)

(event `aimBlender`
  (params (In :type Boolean))
  (if In
    (bind (_direction _aimtime) (`Timeline|Timeline_0` :!via `PlayFromStart` :!label _label_2)
      (:`Update`
        (`/Game/Fadeout_Content/Core/Characters/BP_PlayerCharacter.setAimingAnimation` (`self.Player`) true _aimtime)))
    (else
      (goto _label_2 :!via `ReverseFromEnd`))))

(fn `CanWeaponFire`
  (returns (CanFire :type Boolean))
  (if (> (`self.Durability`) 0.0)
    (return true)
    (else
      (return false))))

(fn `PlayFireSound`
  (`GameplayStatics.PlaySoundAtLocation` (`self.FireSound`) (`self.K2_GetActorLocation`) (struct) 1.0 (`KismetMathLibrary.RandomFloatInRange` 0.9 1.1) 0.0 "/Game/Fadeout_Content/Core/Characters/Footstep_Attenuation.Footstep_Attenuation" "/Game/Fadeout_Content/Core/Characters/FootStepConcurrency.FootStepConcurrency" null))

(fn `PlayNoAmmoSound`
  (`GameplayStatics.PlaySoundAtLocation` (`self.NoAmmoSound`) (`self.K2_GetActorLocation`) (struct) 1.0 1.0 0.0 null null null))

(fn `UserConstructionScript`)

(fn `WeaponAmmoEvent`
  (returns (fireCostMet :type Boolean))
  (bind _weaponsammotype (`self.WeaponsAmmoType`))
  (bind _player (`self.Player`))
  (if (>= (`BlueprintMapLibrary.Map_Find` (`/Game/Fadeout_Content/Core/Characters/BP_PlayerCharacter.Ammo` _player) _weaponsammotype) 1)
    (`BlueprintMapLibrary.Map_Add` (`/Game/Fadeout_Content/Core/Characters/BP_PlayerCharacter.Ammo` _player) _weaponsammotype (- (`BlueprintMapLibrary.Map_Find` (`/Game/Fadeout_Content/Core/Characters/BP_PlayerCharacter.Ammo` _player) (`self.WeaponsAmmoType`)) (`self.FireCost`)))
    (return true)
    (else
      (return false))))