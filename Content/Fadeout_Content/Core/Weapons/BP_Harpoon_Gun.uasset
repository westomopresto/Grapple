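; BP_Harpoon_Gun is a harpoon weapon child Blueprint that adds an optional projectile-follow camera to its parent's firing logic.
; When Follow is set, the last projectile becomes player 0's blended view target, returning to the pawn a second after its hit event.
; Server projectile spawns force a net update.
; Follow toggling and cable attachment logic are disconnected, and AdditionalDamage checks teams without applying anything.
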(event `/Game/Fadeout_Content/Core/Weapons/BP_weaponBase.AltFireRelease`
  (`parent.AltFireRelease`))

(event `Set View to`
  (params (NewViewTarget :type "Actor Object Reference"))
  (`KismetSystemLibrary.Delay` 0.1)
  (if (`self.follow`)
    (`PlayerController.SetViewTargetWithBlend` (`GameplayStatics.GetPlayerController` 0) NewViewTarget 0.25 "VTBlend_Linear" 0.0 false)))

(event `/Game/Fadeout_Content/Core/Weapons/BP_weaponBase.OnAltFirePress`
  (`parent.OnAltFirePress`))

(event `Set View to Player`
  (`PlayerController.SetViewTargetWithBlend` (`GameplayStatics.GetPlayerController` 0) (`Controller.K2_GetPawn` (`GameplayStatics.GetPlayerController` 0)) 0.2 "VTBlend_Linear" 0.0 false))

(event `self.Last Projectile Notify`
  (`parent.Last Projectile Notify`)
  (`/Engine/EditorBlueprintResources/StandardMacros.IsValid` (`self.LastProjectile`)
    (:`Is Valid`
      (if (`self.follow`)
        (`self.Client projectile`)))))

(event `Client projectile`
  (bind _lastprojectile (`self.LastProjectile`))
  (`/Engine/EditorBlueprintResources/StandardMacros.IsValid` _lastprojectile
    (:`Is Valid`
      (`KismetSystemLibrary.PrintString` (`KismetSystemLibrary.GetDisplayName` _lastprojectile))
      (`self.Set View to` _lastprojectile)
      (add `/Game/Fadeout_Content/Core/Weapons/BP_ProjectileBase.onProjectileHit` _lastprojectile (delegate `Return View`)))))

(event `Return View`
  (`KismetSystemLibrary.Delay` 1.0)
  (`self.Set View to Player`))

(event `self.Additional Damage`
  (params (DamagedActor :type "Actor Object Reference") (BaseDamage :type "Float (single-precision)") (EventInstigator :type "Controller Object Reference") (DamageCauser :type "Actor Object Reference") (DamageTypeClass :type "DamageType Class Reference"))
  (bind _asbp_player_character (cast `/Game/Fadeout_Content/Core/Characters/BP_PlayerCharacter` DamagedActor))
  (bind (_sameteam _ffa_ _valid) (`/Game/Fadeout_Content/Core/Characters/BP_PlayerCharacter.CheckTeamDamage` _asbp_player_character (`self.GetInstigatorController`)))
  (if (and (or (not _sameteam) _ffa_) _valid)
    _))

(event `self.Spawn Projectile Server`
  (params (SpawnTransform :type "Transform Structure") (OwningWeapon :type "/Game/Fadeout_Content/Core/Weapons/BP_weaponBase Object Reference") (RayHitActor :type "Actor Object Reference"))
  (`parent.Spawn Projectile SERVER_ONLY` SpawnTransform OwningWeapon)
  (`self.ForceNetUpdate`))

(fn `UserConstructionScript`
  (`parent.UserConstructionScript`))