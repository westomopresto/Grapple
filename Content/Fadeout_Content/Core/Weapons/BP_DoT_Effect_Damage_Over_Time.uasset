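; Damage-over-time effect actor owned by a player character, dealing repeated damage ticks before destroying itself.
; SlowDot and 10SecDot select a 3, 6 or 10 second timeline, whose event track applies damage and multicasts the particle update.
; BeginPlay always overrides one of the player's damage resistances, but restores the saved map at timeline end only if ApplyWeakness is set.
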(event `self.ReceiveBeginPlay`
  (`SceneComponent.SetRelativeScale3D` (`self.ParticleSystem`) (`self.Particle Scale`))
  (bind _asbp_player_character (cast `/Game/Fadeout_Content/Core/Characters/BP_PlayerCharacter` (`self.GetOwner`)))
  (bind _output_get (set `self.Player` _asbp_player_character))
  (if true
    (bind _output_get_2 (set `self.Original Resist` (`/Game/Fadeout_Content/Core/Characters/BP_PlayerCharacter.DamageResistances` _output_get)))
    (set `self.New Resists` _output_get_2)
    (`BlueprintMapLibrary.Map_Add` (`self.New Resists`) (`self.Resist to Reduce`) (`self.Resist Reduction`))
    (set `/Game/Fadeout_Content/Core/Characters/BP_PlayerCharacter.DamageResistances` (`self.New Resists`) (`self.Player`)))
  (if (`self.SlowDot?`)
    (if (`self.10 sec dot`)
      (`self.10 second dot`)
      (else
        (`self.6 second dot`)))
    (else
      (`self.3 Second Dot`))))

(event `multicast particle`
  (if (`self.Particle?`)
    (`ParticleSystemComponent.SetTemplate` (`self.ParticleSystem`) (`self.Particle`))
    (else
      (`SceneComponent.SetVisibility` (`self.ParticleSystem`) false false))))

(event `Damage Tick`
  (`GameplayStatics.ApplyDamage` (`self.Player`) (`self.DamagePerTick`) (`Pawn.GetController` (`self.Instigator`)) (`self.Damage Causer`) (`self.Damage Type`))
  (`self.multicast particle`))

(event `10 second dot`
  (`Timeline|10 sec` :!via `PlayFromStart`
    (:`Finished`
      (if (`self.Apply Weakness`) :!label _label
        ;[1 1 1] Revert weakness
        (set `/Game/Fadeout_Content/Core/Characters/BP_PlayerCharacter.DamageResistances` (`self.Original Resist`) (`self.Player`)))
      (`KismetSystemLibrary.Delay` 1.0)
      (`self.Expire`))
    (:`Poison Tick`
      (`self.Damage Tick`))))

(event `6 second dot`
  (`Timeline|Timeline_0` :!via `PlayFromStart`
    (:`Finished`
      (goto _label))
    (:`Poison Tick`
      (`self.Damage Tick`))))

(event `3 Second Dot`
  (`Timeline|Poison Duration` :!via `PlayFromStart`
    (:`Finished`
      (goto _label))
    (:`Poison Tick`
      (`self.Damage Tick`))))

(event `Expire`
  (`self.K2_DestroyActor`))

(fn `UserConstructionScript`)