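; BP_Poison_DOT is a poison damage-over-time actor that afflicts the BP_PlayerCharacter that owns it.
; On BeginPlay it saves the player's damage resistances, applies a negative resistance entry and starts the PoisonDuration timeline.
; Each timeline tick deals DT_Poison damage and calls a multicast that sets the particle template to P_FireChunk.
; When the timeline finishes, it restores the saved resistances and destroys itself after a short delay.
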(event `multicast particle`
  (`ParticleSystemComponent.SetTemplate` (`self.ParticleSystem`) "/Game/2dFX_Pack/Particles/P_FireChunk.P_FireChunk"))

(event `self.ReceiveBeginPlay`
  (bind _asbp_player_character (cast `/Game/Fadeout_Content/Core/Characters/BP_PlayerCharacter` (`self.GetOwner`)))
  (bind _output_get (set `self.Player` _asbp_player_character))
  (bind _output_get_2 (set `self.Original Resist` (`/Game/Fadeout_Content/Core/Characters/BP_PlayerCharacter.DamageResistances` _output_get)))
  (set `self.New Resists` _output_get_2)
  (`BlueprintMapLibrary.Map_Add` (`self.New Resists`) "NewEnumerator10" -150.0)
  (set `/Game/Fadeout_Content/Core/Characters/BP_PlayerCharacter.DamageResistances` (`self.New Resists`) _asbp_player_character)
  (`Timeline|Poison Duration` :!via `PlayFromStart`
    (:`Finished`
      (set `/Game/Fadeout_Content/Core/Characters/BP_PlayerCharacter.DamageResistances` (`self.Original Resist`) (`self.Player`))
      (`KismetSystemLibrary.Delay` 1.0)
      (`self.K2_DestroyActor`))
    (:`Poison Tick`
      (`GameplayStatics.ApplyDamage` (`self.Player`) 11.0 (`Pawn.GetController` (`self.Instigator`)) (`self.Damage Causer`) "/Game/Fadeout_Content/Core/Weapons/DamageTypes/DT_Poison.DT_Poison_C")
      (`self.multicast particle`))))

(fn `UserConstructionScript`)