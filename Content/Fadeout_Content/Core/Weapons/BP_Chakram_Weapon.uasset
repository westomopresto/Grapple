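; Chakram weapon that shows a pair of chakrams in the player's hands and throws them as returning projectiles.
; On swap-in it attaches a spawned static mesh as the fake offhand, and a looping timer maintains the idle montage.
; Firing hides both meshes and locks tool swapping until the authority counts two returns, then cooldown resets and the attack montage reverses as a catch.
; HideChakrams is inverted: true means visible.
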(event `self.onSwapIn`
  (`parent.onSwapIn`)
  (`self.Start Idle Timer`)
  (set `self.ChakramCounter` 0)
  (`self.Play Idle Anim`)
  (`self.KillFakeOffhand`)
  (bind _returnvalue (`|SpawnActorFromClass` "/Script/Engine.StaticMeshActor" (`KismetMathLibrary.MakeTransform` (0.0 0.0 0.0)) "AlwaysSpawn" "OverrideRootScale" null null))
  (bind _output_get (set `self.fake_offhand` _returnvalue))
  (`StaticMeshActor.SetMobility` _output_get "Movable")
  (`StaticMeshComponent.SetStaticMesh` (`StaticMeshActor.StaticMeshComponent` _output_get) "/Game/Fadeout_Content/Core/FBX/Chakram/SM_Chakram_Projectile.SM_Chakram_Projectile")
  (bind _asbp_player_character (cast `/Game/Fadeout_Content/Core/Characters/BP_PlayerCharacter` (`self.GetOwner`)))
  (`/Game/Fadeout_Content/Core/Characters/BP_PlayerCharacter.AttachMeshSocket` _asbp_player_character "hand_sp_l" _output_get)
  (`self.HideChakrams` true))

(event `self.ReceiveBeginPlay`
  (`parent.ReceiveBeginPlay`)
  (`self.Start Idle Timer`))

(event `Start Idle Timer`
  (bind _returnvalue (`KismetSystemLibrary.K2_SetTimerDelegate` (delegate `Check Idling`) 1.0 true))
  (set `self.IdlingTimer` _returnvalue))

(event `Check Idling`
  (if (not (`self.onGround?`))
    (bind _asbp_player_character (cast `/Game/Fadeout_Content/Core/Characters/BP_PlayerCharacter` (`self.GetOwner`)))
    (if (== (`/Game/Fadeout_Content/Core/Characters/BP_PlayerCharacter.CurrentWeapon` _asbp_player_character) self)
      (if (and (`self.ChakramHidden`) (`Character.HasAnyRootMotion` _asbp_player_character))
        (`self.Stop Idle` :!label _label)
        (else
          (`self.Play Idle Anim`)))
      (else
        (goto _label)))))

(event `self.OnDropped`
  (`parent.OnDropped`)
  (`self.KillFakeOffhand` :!label _label_2)
  (`self.HideChakrams` true)
  (set `self.ChakramCounter` 0)
  (`self.Stop Idle`)
  (`KismetSystemLibrary.K2_ClearAndInvalidateTimerHandle` (`self.IdlingTimer`)))

(event `self.onSwapOut`
  (`parent.onSwapOut`)
  (goto _label_2))

(event `self.Success Fire`
  (`parent.Success Fire`)
  (`self.Multicast Fire`))

(event `Multicast Fire`
  (`self.HideChakrams` false)
  (set `self.ChakramCounter` 0)
  (bind _asbp_player_character (cast `/Game/Fadeout_Content/Core/Characters/BP_PlayerCharacter` (`self.GetOwner`)))
  (set `/Game/Fadeout_Content/Core/Characters/BP_PlayerCharacter.canSwapTools?` false _asbp_player_character))

(event `self.ReceiveEndPlay`
  (params (EndPlayReason :type "EEndPlayReason Enum" :default "Destroyed"))
  (`parent.ReceiveEndPlay` EndPlayReason)
  (`self.KillFakeOffhand`))

(event `Chakram Returned`
  ;[1 1 1] Resets Fire CD
  (`/Engine/EditorBlueprintResources/ActorMacros.Switch Has Authority`
    (:`Authority`
      (bind _result (`/Engine/EditorBlueprintResources/StandardMacros.IncrementInt` (`self.ChakramCounter`))
        (:`  `
          (if (>= _result 2)
            (`self.Chakram Return Multi`)))))))

(event `Chakram Return Multi`
  ;[1 1 1] Resets Fire CD
  (`KismetSystemLibrary.K2_ClearAndInvalidateTimerHandle` (`self.FireCoolDownTimer`))
  (`self.FireCoolDown_Finish`)
  (`self.HideChakrams` true)
  (set `self.ChakramCounter` 0)
  (bind _asbp_player_character (cast `/Game/Fadeout_Content/Core/Characters/BP_PlayerCharacter` (`self.GetOwner`)))
  (`Character.PlayAnimMontage` _asbp_player_character (`/Game/Fadeout_Content/Core/Characters/BP_PlayerCharacter.chakram_Atk_montage` _asbp_player_character) -2.0 "attack")
  (`KismetSystemLibrary.Delay` 0.1)
  (`self.Play Idle Anim`)
  (set `/Game/Fadeout_Content/Core/Characters/BP_PlayerCharacter.canSwapTools?` true _asbp_player_character))

(event `self.Spawn Projectile Server`
  (params (SpawnTransform :type "Transform Structure") (OwningWeapon :type "/Game/Fadeout_Content/Core/Weapons/BP_weaponBase Object Reference") (RayHitActor :type "Actor Object Reference") (`Initial Speed Override` :type "Float (single-precision)") (`Override Speed` :type Boolean))
  (`self.Spawn Projectile` SpawnTransform OwningWeapon))

(fn `Cloak Weapon`
  (params (cloaked :type Boolean))
  (bind _fake_offhand (`self.fake_offhand`))
  (`parent.Cloak Weapon` cloaked)
  (`/Engine/EditorBlueprintResources/StandardMacros.IsValid` _fake_offhand
    (:`Is Valid`
      (`PrimitiveComponent.SetMaterial` (`StaticMeshActor.StaticMeshComponent` _fake_offhand) 0 (select `bool` cloaked :`false` (`self.OriginalWeapon_Material`) :`true` (`self.Cloaked_material`) :!type "MaterialInterface Object Reference")))))

(fn `HideChakrams`
  (params (bNewVisibility :type Boolean))
  (bind _fake_offhand (`self.fake_offhand`))
  (bind _output_get (set `self.ChakramHidden` bNewVisibility))
  (`SceneComponent.SetVisibility` (`self.SkeletalMesh`) _output_get false)
  (`/Engine/EditorBlueprintResources/StandardMacros.IsValid` _fake_offhand
    (:`Is Valid`
      (`SceneComponent.SetVisibility` (`Actor.RootComponent` _fake_offhand) _output_get false))
    (:`Is Not Valid`
      _))
  (return))

(fn `KillFakeOffhand`
  (bind _fake_offhand (`self.fake_offhand`))
  (`/Engine/EditorBlueprintResources/StandardMacros.IsValid` _fake_offhand
    (:`Is Valid`
      (`self.K2_DestroyActor` _fake_offhand))
    (:`Is Not Valid`
      _))
  (return))

(fn `Play Idle Anim`
  (bind _asbp_player_character (cast `/Game/Fadeout_Content/Core/Characters/BP_PlayerCharacter` (`self.GetOwner`)))
  (if (`Character.IsPlayingRootMotion` _asbp_player_character)
    (return)
    (else
      (`Character.StopAnimMontage` _asbp_player_character null)
      (`Character.PlayAnimMontage` _asbp_player_character (`/Game/Fadeout_Content/Core/Characters/BP_PlayerCharacter.chakram_Idle_montage` _asbp_player_character) 1.0 "default")
      (return))))

(fn `Stop Idle`
  (bind _asbp_player_character (cast `/Game/Fadeout_Content/Core/Characters/BP_PlayerCharacter` (`self.GetOwner`)))
  (`Character.StopAnimMontage` _asbp_player_character (`/Game/Fadeout_Content/Core/Characters/BP_PlayerCharacter.chakram_Idle_montage` _asbp_player_character))
  (return))

(fn `UserConstructionScript`
  (`parent.UserConstructionScript`))