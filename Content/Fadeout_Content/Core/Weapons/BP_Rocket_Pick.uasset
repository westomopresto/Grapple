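; Rocket Pick, a charged melee weapon that winds up while fire is held and unleashes a player spin attack with a trace.
; Press and release route through server and multicast events; a looping timer grows light and flame with an alarm, and a horn signals full charge.
; Releasing early cancels with a fail sound, while overcharging periodically damages the owner unless disabled.
; The attack temporarily locks dodge roll, limits yaw and swaps hand sockets.
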(event `self.Effect Multicast`
  (bind _currenttrail (`self.currentTrail`))
  ;[1 1 1] Effect multicast
  (set `self.CanFire?` false)
  (`GameplayStatics.SpawnSoundAttached` "/Game/Fadeout_Content/Core/Audio/Train_SFX/Train_Horn.Train_Horn" (`self.SkeletalMesh`) "None" (0.0 0.0 0.0) (struct) "KeepRelativeOffset" false 1.0 1.0 0.0 null null)
  (`KismetArrayLibrary.Array_Clear` (`self.HitActors`))
  (bind _asbp_player_character (cast `/Game/Fadeout_Content/Core/Characters/BP_PlayerCharacter` (`self.GetOwner`)))
  (set `/Game/Fadeout_Content/Core/Characters/BP_PlayerCharacter.canDodgeRoll` false _asbp_player_character)
  (set `/Game/Fadeout_Content/Core/Characters/BP_PlayerCharacter.YawLimit` true _asbp_player_character)
  (`/Game/Fadeout_Content/Core/Characters/BP_PlayerCharacter.Enter_Combat` _asbp_player_character)
  (set `self.handSocket` "2hsocket")
  (`/Game/Fadeout_Content/Core/Characters/BP_PlayerCharacter.attachToSocket` _asbp_player_character self false)
  (`self.WeaponFiredEvent`)
  (`self.PlayFireSound_0`)
  (`self.SpawnHitTrail` (`self.trail`))
  (`self.Trace`)
  (`/Game/Fadeout_Content/Core/Characters/BP_PlayerCharacter.meleeSpinAttack` _asbp_player_character)
  (`KismetSystemLibrary.Delay` 0.05)
  (`KismetSystemLibrary.Delay` (`self.TraceDuration`))
  (set `self.CanFire?` true)
  (set `self.handSocket` "MeleeSocket")
  (set `/Game/Fadeout_Content/Core/Characters/BP_PlayerCharacter.canDodgeRoll` true _asbp_player_character)
  (set `/Game/Fadeout_Content/Core/Characters/BP_PlayerCharacter.YawLimit` false _asbp_player_character)
  (if (`/Game/Fadeout_Content/Core/Characters/BP_PlayerCharacter.alive?` _asbp_player_character)
    (`/Game/Fadeout_Content/Core/Characters/BP_PlayerCharacter.attachToSocket` _asbp_player_character self false))
  (set `/Game/Fadeout_Content/Core/Characters/BP_PlayerCharacter.canSwapTools?` true _asbp_player_character)
  (`LightComponent.SetIntensity` (`self.PointLight`) 0.0)
  (`/Engine/EditorBlueprintResources/StandardMacros.IsValid` _currenttrail
    (:`Is Valid`
      (`ActorComponent.Deactivate` _currenttrail))))

(event `Start Charge`
  (bind _returnvalue (`KismetSystemLibrary.K2_SetTimerDelegate` (delegate `Charging`) 0.1 true))
  (set `self.Charging Timer` _returnvalue)
  (set `self.Is Charging` true)
  (`LightComponent.SetIntensity` (`self.PointLight`) 0.0)
  (`SceneComponent.SetRelativeScale3D` (`self.chargeFire`) (0.0 0.0 0.0))
  (`self.stopAlarm`)
  (bind _returnvalue_2 (`GameplayStatics.SpawnSoundAttached` "/Game/Fadeout_Content/Core/Audio/Train_SFX/Alarm.Alarm" (`self.SkeletalMesh`) "None" (0.0 0.0 0.0) (struct) "KeepRelativeOffset" false 1.0 1.0 0.0 null null))
  (set `self.alarmsound` _returnvalue_2))

(event `Charge Start Multicast`
  ;[1 1 1] Fire Press Multicast
  (`|ExecutionSequence`
    (:`then_0`
      (`self.PlayAltFireSound`))
    (:`then_1`
      (bind _asbp_player_character (cast `/Game/Fadeout_Content/Core/Characters/BP_PlayerCharacter` (`self.GetOwner`)))
      (set `/Game/Fadeout_Content/Core/Characters/BP_PlayerCharacter.canSwapTools?` false _asbp_player_character)
      (`/Game/Fadeout_Content/Core/Characters/BP_PlayerCharacter.altMeleeWindup` _asbp_player_character))
    (:`then_2`
      (`ActorComponent.Activate` (`self.chargeFire`) false)
      (`self.Start Charge`))))

(event `Charging`
  (bind _returnvalue (`self.GetOwner`))
  (if (`self.onGround?`)
    (`KismetSystemLibrary.K2_ClearAndInvalidateTimerHandle` (`self.Charging Timer`))
    (set `self.Is Charging` false)
    (`self.stopAlarm`)
    (else
      (bind _output_get (set `self.Charge` (+ (`self.charge`) 3.34)))
      (set `self.OverCharge` (+ (`self.OverCharge`) 3.34))
      (bind _output_get_2 (set `self.charge` (`KismetMathLibrary.FClamp` _output_get 0.0 (`self.maxCharge`))))
      (`LightComponent.SetIntensity` (`self.PointLight`) (`KismetMathLibrary.MapRangeClamped` _output_get_2 0.0 100.0 0.0 10000.0))
      (`SceneComponent.SetRelativeScale3D` (`self.chargeFire`) (`KismetMathLibrary.VLerp` (0.0 0.0 0.0) (1.0 1.0 1.0) (`KismetMathLibrary.NormalizeToRange` _output_get_2 0.0 100.0)))
      (`|ExecutionSequence`
        (:`then_0`
          (if (>= _output_get_2 (`self.maxCharge`))
            (`/Engine/EditorBlueprintResources/StandardMacros.DoOnce` false :!label _label
              (:`Completed`
                (`GameplayStatics.SpawnSoundAttached` "/Game/Fadeout_Content/Core/Audio/Train_SFX/Train_Horn.Train_Horn" (`self.SkeletalMesh`) "None" (0.0 0.0 0.0) (struct) "KeepRelativeOffset" false 1.0 1.0 0.0 null null)))
            (else
              (goto _label :!via `Reset`))))
        (:`then_1`
          (if (`self.disableSelfDamage`)
            _
            (elif (>= (`self.OverCharge`) 125.0)
              (`/Engine/EditorBlueprintResources/StandardMacros.FlipFlop`
                (:`A`
                  (bind _asbp_player_character (cast `/Game/Fadeout_Content/Core/Characters/BP_PlayerCharacter` _returnvalue))
                  (`GameplayStatics.ApplyDamage` _returnvalue (* (`/Game/Fadeout_Content/Core/Characters/BP_PlayerCharacter.maxHealth` _asbp_player_character) 0.1) (`self.GetInstigatorController`) self "/Game/Fadeout_Content/Core/Weapons/DamageTypes/DT_Rocket_Pick.DT_Rocket_Pick_C"))))))))))

(event `Charge Start Server`
  ;[1 1 1] Fire Press Multicast
  (`self.Charge Start Multicast`))

(event `self.OnFirePress`
  ;[1 1 1] actually important lol
  (if (`self.CanFire?`)
    ;[1 1 1] Animation replicate
    (`/Engine/EditorBlueprintResources/ActorMacros.Switch Has Authority`
      (:`Authority`
        (`self.Charge Start Multicast`))
      (:`Remote`
        (`self.Charge Start Server`)))))

(event `Multi Charge Check`
  ;[1 1 1] Charge Check
  (set `self.Is Charging` false)
  (`KismetSystemLibrary.K2_ClearAndInvalidateTimerHandle` (`self.Charging Timer`))
  (`self.stopAlarm`)
  (`/Engine/EditorBlueprintResources/StandardMacros.CompareFloat` (`self.charge`) (`self.maxCharge`)
    (:`>`
      (set `self.OverCharge` 0.0 :!label _label_2)
      (set `self.charge` 0.0)
      (`parent.OnFire`)
      (`ActorComponent.Deactivate` (`self.chargeFire`)))
    (:`==`
      (goto _label_2))
    (:`<`
      (set `self.OverCharge` 0.0)
      (set `self.charge` 0.0)
      (`self.PlayNoAmmoSound`)
      (`self.Charge Fail Multicast`)
      (`LightComponent.SetIntensity` (`self.PointLight`) 0.0))))

(event `self.OnFireRelease`
  (params (`charged?` :type Boolean))
  (if (`self.CanFire?`)
    (`self.Charge Check Server`)))

(event `Charge Check Server`
  ;[1 1 1] Charge Check
  (`self.Multi Charge Check`))

(event `self.ReceiveBeginPlay`
  (`parent.ReceiveBeginPlay`)
  (`ActorComponent.Deactivate` (`self.chargeFire`))
  (`self.stopAlarm`))

(event `Charge Fail Multicast`
  ;[1 1 1] Charge Failed
  (bind _asbp_player_character (cast `/Game/Fadeout_Content/Core/Characters/BP_PlayerCharacter` (`self.GetOwner`)))
  (set `/Game/Fadeout_Content/Core/Characters/BP_PlayerCharacter.canSwapTools?` true _asbp_player_character)
  (`Character.StopAnimMontage` _asbp_player_character null)
  (`ActorComponent.Deactivate` (`self.chargeFire`)))

(event `self.Initialize`
  (`parent.Initialize`)
  (`self.stopAlarm`)
  (`ActorComponent.Deactivate` (`self.chargeFire`))
  (set `self.CanFire?` true))

(event `self.OnDropped`
  (`parent.OnDropped`)
  (`self.stopAlarm`))

(fn `stopAlarm`
  (bind _alarmsound (`self.alarmsound`))
  (`/Engine/EditorBlueprintResources/StandardMacros.IsValid` _alarmsound
    (:`Is Valid`
      (`AudioComponent.Stop` _alarmsound))))

(fn `UserConstructionScript`
  (`parent.UserConstructionScript`))