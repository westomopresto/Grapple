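; Harpoon weapon debuff that slows its owning player character and suppresses jump height.
; On BeginPlay it flags the player as crowd-controlled and runs a timeline that eases sprint speed modifier and jump velocity back up from their reduced values.
; Completion or RevertWeakness restores the player, deactivates the particles and expires after a delay.
; A separate event drains player energy through a server call, with no caller in this graph.
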(event `self.ReceiveBeginPlay`
  (set `self.Instigator Controller` (`self.GetInstigatorController`))
  (`SceneComponent.SetRelativeScale3D` (`self.ParticleSystem`) (`self.Particle Scale`))
  (bind _asbp_player_character (cast `/Game/Fadeout_Content/Core/Characters/BP_PlayerCharacter` (`self.GetOwner`)))
  (set `self.Player` _asbp_player_character)
  (`self.Apply Weakness Event`))

(event `Apply Energy Loss`
  (`/Game/Fadeout_Content/Core/Characters/BP_PlayerCharacter.EnergyCostServer` (`self.Player`) 15 false))

(event `self.Apply Weakness Event`
  (bind _player (`self.Player`))
  (bind _originaljumpheight (`/Game/Fadeout_Content/Core/Characters/BP_PlayerCharacter.OriginalJumpHeight` _player))
  (bind _charactermovement (`Character.CharacterMovement` _player))
  (set `/Game/Fadeout_Content/Core/Characters/BP_PlayerCharacter.CCd` true (`self.Player`))
  (`TimelineComponent.SetPlayRate` (`self.Timeline_1`) 0.5)
  (bind (_direction _alpha) (`Timeline|Timeline_1` :!via `PlayFromStart` :!label _label)
    (:`Update`
      (set `/Game/Fadeout_Content/Core/Characters/BP_PlayerCharacter.SpeedMod` (`KismetMathLibrary.Lerp` (`self.SpeedReductionMod`) 0.5 _alpha) _player)
      (`/Game/Fadeout_Content/Core/Characters/BP_PlayerCharacter.toSprint Multicast` _player)
      (set `CharacterMovementComponent.JumpZVelocity` (* _originaljumpheight (`KismetMathLibrary.Lerp` 0.1 1.0 _alpha)) _charactermovement))
    (:`Finished`
      (set `/Game/Fadeout_Content/Core/Characters/BP_PlayerCharacter.SpeedMod` 1.0 _player :!label _label_2)
      (`/Game/Fadeout_Content/Core/Characters/BP_PlayerCharacter.toSprint Multicast` _player)
      (set `CharacterMovementComponent.JumpZVelocity` _originaljumpheight _charactermovement)
      (set `/Game/Fadeout_Content/Core/Characters/BP_PlayerCharacter.CCd` false _player)
      (set `self.Ending` true)
      (`ActorComponent.Deactivate` (`self.ParticleSystem`))
      (`ActorComponent.Deactivate` (`self.Trail`))
      (`KismetSystemLibrary.Delay` 5.0)
      (`self.Expire`))))

(event `self.Revert Weakness`
  (`|ExecutionSequence`
    (:`then_0`
      (goto _label :!via `Stop`))
    (:`then_1`
      (goto _label_2))))

(fn `UserConstructionScript`
  (`parent.UserConstructionScript`))