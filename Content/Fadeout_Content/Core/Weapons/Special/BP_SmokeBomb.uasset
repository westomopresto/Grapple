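; Smoke bomb special weapon actor that shows a smoke sphere, tinted through a team-aware material, until it expires.
; BeginPlay creates a dynamic smoke material and grows the sphere from zero to full size on a timeline.
; The team check sets the material's OnTeam parameter from whether the bomb is hostile to the local player.
; On expiry, the same timeline reverses to shrink the sphere, then destroys the actor.
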(event `self.ReceiveBeginPlay`
  (bind _returnvalue (`PrimitiveComponent.CreateDynamicMaterialInstance` (`self.Sphere`) 0 "/Game/Fadeout_Content/Core/Weapons/Special/MM_SmokeBomb.MM_SmokeBomb" "None"))
  (set `self.SmokeMaterialDyn` _returnvalue)
  (`parent.ReceiveBeginPlay`)
  (`self.GrowShrink` true))

(event `self.CheckClientTeam`
  (`parent.CheckClientTeam`)
  (`MaterialInstanceDynamic.SetScalarParameterValue` (`self.SmokeMaterialDyn`) "OnTeam" (`KismetMathLibrary.Conv_BoolToDouble` (not (`self.HostileToYou`)))))

(event `GrowShrink`
  (params (bIntro :type Boolean))
  (if bIntro
    (bind (_direction _newtrack_0) (`Timeline|Timeline_0` :!via `PlayFromStart` :!label _label)
      (:`Update`
        (`SceneComponent.SetRelativeScale3D` (`self.Sphere`) (`KismetMathLibrary.VLerp` (0.0 0.0 0.0) (`self.FullSize`) _newtrack_0)))
      (:`Finished`
        (if (not bIntro)
          (`self.K2_DestroyActor`))))
    (else
      (goto _label :!via `ReverseFromEnd`))))

(event `self.ExpiredMulti`
  (`parent.ExpiredMulti`)
  (`self.GrowShrink` false))

(fn `UserConstructionScript`
  (`parent.UserConstructionScript`))