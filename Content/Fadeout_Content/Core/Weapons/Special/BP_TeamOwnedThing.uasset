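; Base actor for team-owned objects that tracks whether its Instigator is hostile to the local player.
; On BeginPlay, except on dedicated servers, it compares the first player controller's PlayerState with the Instigator's and stores HostileToYou and OwnersTeam.
; In FFA any other player counts as an enemy, while team modes also require a different team.
; It binds to the local PlayerState's team-change event to re-run the check.
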(event `CheckClientTeam`
  (bind _playerstate (`Controller.PlayerState` (`GameplayStatics.GetPlayerController` 0)))
  (`/Engine/EditorBlueprintResources/StandardMacros.IsValid` _playerstate
    (:`Is Valid`
      (bind _asfo_player_state (cast `/Game/Fadeout_Content/Core/Support/Multiplayer_Support/FO_PlayerState` _playerstate))
      (bind (_triggered _team) (`self.IsEnemyToLocal` _asfo_player_state))
      (set `self.OwnersTeam` _team)
      (add `/Game/Fadeout_Content/Core/Support/Multiplayer_Support/FO_PlayerState.TeamsChanged` _asfo_player_state (delegate `TeamChanged`))
      (set `self.HostileToYou` _triggered))))

(event `TeamChanged`
  (params (Team :type String))
  (`self.CheckClientTeam`))

(event `self.ReceiveBeginPlay`
  (`parent.ReceiveBeginPlay`)
  (if (not (`KismetSystemLibrary.IsDedicatedServer`))
    (`self.CheckClientTeam`)))

(fn `IsEnemyToLocal`
  (params (`FO Player State` :type "/Game/Fadeout_Content/Core/Support/Multiplayer_Support/FO_PlayerState Object Reference"))
  (returns (Triggered :type Boolean) (Team :type String))
  (bind _team (`/Game/Fadeout_Content/Core/Support/Multiplayer_Support/FO_PlayerState.Team` `FO Player State`))
  (bind _playerstate (`Pawn.PlayerState` (`self.Instigator`)))
  (bind _returnvalue (!= (`PlayerState.PlayerId` `FO Player State`) (`PlayerState.PlayerId` _playerstate)))
  (`/Engine/EditorBlueprintResources/StandardMacros.IsValid` (`self.Instigator`)
    (:`Is Valid`
      (`/Engine/EditorBlueprintResources/StandardMacros.IsValid` `FO Player State`
        (:`Is Valid`
          (bind _asfo_player_state (cast `/Game/Fadeout_Content/Core/Support/Multiplayer_Support/FO_PlayerState` _playerstate))
          (if (`KismetStringLibrary.NotEqual_StrStr` _team "FFA")
            (bind _team_2 (`/Game/Fadeout_Content/Core/Support/Multiplayer_Support/FO_PlayerState.Team` _asfo_player_state))
            (if (and (not (`KismetStringLibrary.EqualEqual_StrStr` _team _team_2)) _returnvalue)
              _
              (else
                (return false _team_2)))
            (else
              ;[1 1 1] FFA
              (if _returnvalue
                _
                (else
                  (return false _team_2)))))
          (return true _team_2))))
    (:`Is Not Valid`
      (return false ""))))

(fn `UserConstructionScript`)