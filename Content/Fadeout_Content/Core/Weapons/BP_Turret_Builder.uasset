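; Toolbox weapon that throws deployable BP_Turret actors for its raccoon character owner.
; Fire checks ammo, calls SpawnTurretServer to spawn and launch a turret along the camera direction, multicasts the throw animation and sounds, then runs a reload cooldown.
; The toolbox is tinted to the owner's helmet color and destroys itself when dropped.
; Hologram placement preview logic remains but is disconnected, and alt-fire is empty.
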(event `Spawn Turret Server`
  (params (SpawnTransform :type "Transform Structure") (Direction :type "Vector Structure"))
  (`self.AmmoCostFunction` false)
  (bind _returnvalue (`|SpawnActorFromClass` :`Class` "/Game/Fadeout_Content/Core/Characters/BP_Turret.BP_Turret_C" :`SpawnTransform` SpawnTransform :`CollisionHandlingOverride` "AdjustIfPossibleButAlwaysSpawn" :`TransformScaleMethod` "OverrideRootScale" :`Instigator` (`self.GetInstigator`)))
  (`self.Update Instigator Weapon Info`)
  (`Character.LaunchCharacter` _returnvalue (* Direction 1200.0) true true))

(event `Cast Hologram`)

(event `self.OnPickUp`
  (params (setOwner :type "Actor Object Reference") (Instigator :type "Pawn Object Reference"))
  (`parent.OnPickUp` setOwner Instigator)
  (bind _asbp_char_raccoon (cast `/Game/Fadeout_Content/Core/Characters/BP_Char_Raccoon` Instigator))
  (switch `/Game/Fadeout_Content/Core/UI/Customize/Abigail_Outfits` (cast `/Game/Fadeout_Content/Core/UI/Customize/Abigail_Outfits` (`/Game/Fadeout_Content/Core/Characters/BP_PlayerCharacter.current_outfit` _asbp_char_raccoon))
    (:`NewEnumerator3`
      (set `self.backSocket` "backtoolbox2"))))

(event `self.Throw Animation Multicast`
  (`self.Play fire anim 2`)
  (`self.PlayFireSound`)
  (bind _asbp_char_raccoon (cast `/Game/Fadeout_Content/Core/Characters/BP_Char_Raccoon` (`self.GetOwner`)))
  (`/Game/Fadeout_Content/Core/Characters/BP_Char_Raccoon.Play Deploy Sound` _asbp_char_raccoon))

(event `self.OnFirePress`
  (bind _returnvalue (`self.GetOwner`))
  (if (`self.CanFire?`)
    (set `self.CanFire?` false)
    (bind _firecostmet (`self.AmmoCheckFunction`))
    (if _firecostmet
      (bind (_locationvec _directionvec) (`self.getInstigatorCameraFVector`))
      (`self.Spawn Turret Server` (`KismetMathLibrary.MakeTransform` (+ (* (`self.GetActorForwardVector` _returnvalue) 20.0) (.location (`self.GetTransform` _returnvalue)) (20.0 0.0 90.0)) (.rotation (`self.GetTransform` _returnvalue)) (.scale (`self.GetTransform` _returnvalue))) _directionvec)
      (`|ExecutionSequence`
        (:`then_0`
          ;[1 1 1] Animation Rep
          (`/Engine/EditorBlueprintResources/ActorMacros.Switch Has Authority`
            (:`Authority`
              (`self.Throw Animation Multicast`))
            (:`Remote`
              (`self.Throw Animation Server`))))
        (:`then_1`
          (`self.StartReloadTimeline`)
          (`KismetSystemLibrary.Delay` (`self.Fire CoolDown`))
          (set `self.CanFire?` true :!label _label)))
      (else
        (`self.PlayNoAmmoSound`)
        (goto _label)))))

(event `self.ReceiveBeginPlay`
  (`parent.ReceiveBeginPlay`)
  (`KismetSystemLibrary.Delay` 0.2)
  (bind _asbp_char_raccoon (cast `/Game/Fadeout_Content/Core/Characters/BP_Char_Raccoon` (`self.GetOwner`)))
  (`self.ToolBoxColor` (`.ColorRGB_3_CE0A22804AA10303CF3F1F8E7359B3A0` (break `/Game/Fadeout_Content/Core/UI/Customize/CustomColor` (`/Game/Fadeout_Content/Core/Characters/BP_PlayerCharacter.HelmetColor` _asbp_char_raccoon)))))

(event `self.Throw Animation Server`
  (`self.Throw Animation Multicast`))

(event `self.OnAltFirePress`)

(event `Hologram Timer`
  (if (`self.showHologram?`)
    (`/Engine/EditorBlueprintResources/StandardMacros.IsValid` (`self.GetOwner`)
      (:`Is Valid`
        (`self.Cast Hologram`)))))

(event `self.OnDropped`
  ;[1 1 1] Kill on dropped
  (`parent.OnDropped`)
  (`self.K2_DestroyActor`))

(fn `ToolBoxColor`
  (params (InColor :type "Color Structure"))
  (bind _returnvalue (`KismetMaterialLibrary.CreateDynamicMaterialInstance` "/Game/Fadeout_Content/Core/FBX/Toolbox/M_Toolbox.M_Toolbox" "None"))
  (bind _output_get (set `self.DynamicMaterial` _returnvalue))
  (`PrimitiveComponent.SetMaterial` (`self.SkeletalMesh`) 0 _output_get)
  (`MaterialInstanceDynamic.SetVectorParameterValue` _output_get "TeamColor" (`KismetMathLibrary.Conv_ColorToLinearColor` InColor)))

(fn `UserConstructionScript`
  (`parent.UserConstructionScript`))