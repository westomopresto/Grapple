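; Hitscan gun Blueprint that fires shotgun-type point damage for BP_PlayerCharacter, only while aiming down sights.
; Alt-fire toggles ADS, the character's aim camera and tool swapping.
; Firing spends ammo, then runs multiple debug-drawn traces from the muzzle in a random spread cone toward the crosshair.
; Collected hits receive damage from the current ammo object; the impact effects function is an empty stub.
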(event `self.OnDropped`
  (if (`self.onGround?`) :!label _label
    (`SkinnedMeshComponent.SetPhysicsAsset` (`self.SkeletalMesh`) "/Game/Fadeout_Content/Libraries/FirstPerson/FPWeapon/Mesh/SK_FPGun_PhysicsAsset.SK_FPGun_PhysicsAsset" false)))

(event `self.ReceiveBeginPlay`
  (bind _returnvalue (`AddComponent|NODE_AddBP_BaseAmmo-0`))
  (set `self.currentAmmo` _returnvalue)
  (goto _label))

(event `self.OnFire`
  (bind _canfire (`self.CanWeaponFire`))
  (bind _output_get (set `self.CanFire?` _canfire))
  (if _output_get
    (if (`self.ADS`)
      (`self.DecrementAmmoCount`)
      (bind _asbp_player_character (cast `/Game/Fadeout_Content/Core/Characters/BP_PlayerCharacter` (`self.GetInstigator`)))
      (`/Game/Fadeout_Content/Core/Characters/BP_PlayerCharacter.PlayFireWeaponAnim` _asbp_player_character)
      (bind _crosshairworldspace (`/Game/Fadeout_Content/Core/Characters/BP_PlayerCharacter.GetCrosshairWorldSpace` _asbp_player_character))
      (bind _hitoccured (`self.DetermineHitObjects` _crosshairworldspace))
      (if _hitoccured
        (`self.ApplyDamageToHitActors`)
        (`self.PlayImpactEffects`)))))

(event `self.OnAltFire`
  (params (`MoveCamera?` :type Boolean))
  (bind _asbp_player_character (cast `/Game/Fadeout_Content/Core/Characters/BP_PlayerCharacter` (`self.GetInstigator`)))
  (set `/Game/Fadeout_Content/Core/Characters/BP_PlayerCharacter.canSwapTools?` false _asbp_player_character)
  (`/Game/Fadeout_Content/Core/Characters/BP_PlayerCharacter.releaseSlow` _asbp_player_character)
  (bind _asbp_player_character_2 (cast `/Game/Fadeout_Content/Core/Characters/BP_PlayerCharacter` (`self.GetInstigator`)))
  (set `/Game/Fadeout_Content/Core/Characters/BP_PlayerCharacter.canRun?` true _asbp_player_character_2)
  (`/Game/Fadeout_Content/Core/Characters/BP_PlayerCharacter.PlayChargeWeaponAnim` _asbp_player_character_2)
  (set `self.ADS` true)
  (`self.PlayNoAmmoSound`)
  (`/Game/Fadeout_Content/Core/Characters/BP_PlayerCharacter.toAimCam` _asbp_player_character_2 `MoveCamera?` true true))

(event `self.AltFireRelease`
  (bind _asbp_player_character (cast `/Game/Fadeout_Content/Core/Characters/BP_PlayerCharacter` (`self.GetInstigator`)))
  (set `/Game/Fadeout_Content/Core/Characters/BP_PlayerCharacter.canSwapTools?` true _asbp_player_character)
  (`/Game/Fadeout_Content/Core/Characters/BP_PlayerCharacter.releaseSlow` _asbp_player_character)
  (bind _asbp_player_character_2 (cast `/Game/Fadeout_Content/Core/Characters/BP_PlayerCharacter` (`self.GetInstigator`)))
  (set `/Game/Fadeout_Content/Core/Characters/BP_PlayerCharacter.canRun?` true _asbp_player_character_2)
  (`/Game/Fadeout_Content/Core/Characters/BP_PlayerCharacter.PlayChargeWeaponAnim` _asbp_player_character_2)
  (set `self.ADS` false)
  (`self.PlayNoAmmoSound`)
  (`/Game/Fadeout_Content/Core/Characters/BP_PlayerCharacter.toRearCam` _asbp_player_character_2))

(fn `ApplyDamageToHitActors`
  (bind _returnvalue (`self.GetInstigatorController`))
  (for _index (range (`KismetArrayLibrary.Array_Length` (`self.HitResults`)))
    (bind _output (`|GetArrayItem` (`self.HitResults`) _index))
    (bind (_bblockinghit _binitialoverlap _time _distance _location _impactpoint _normal _impactnormal _physmat _hitactor) (`GameplayStatics.BreakHitResult` _output))
    (`GameplayStatics.ApplyPointDamage` _hitactor (`/Game/Fadeout_Content/Core/Weapons/BP_BaseAmmo.BaseDamage` (`self.currentAmmo`)) (`KismetMathLibrary.GetForwardVector` (`KismetMathLibrary.FindLookAtRotation` _location (`self.K2_GetActorLocation` (`Controller.K2_GetPawn` _returnvalue)))) _output _returnvalue self "/Game/Fadeout_Content/Core/Weapons/DamageTypes/DT_Shotgun.DT_Shotgun_C")))

(fn `DetermineHitObjects`
  (params (CrosshairWorldSpace :type "Vector Structure"))
  (returns (HitOccured :type Boolean))
  (locals (ObjectHit :type Boolean))
  (bind _location (.location (`SceneComponent.GetSocketTransform` (`self.SkeletalMesh`) (`self.MuzzleSocket`) "RTS_World")))
  (`KismetArrayLibrary.Array_Clear` (`self.HitResults`))
  (for _ (range 1 (+ (`self.TracesUsed`) 1))
    (bind (_outhit _returnvalue) (`KismetSystemLibrary.LineTraceSingle` _location (+ _location (`KismetMathLibrary.GreaterGreater_VectorRotator` (* (`KismetMathLibrary.RandomUnitVectorInConeInRadians` (1.0 0.0 0.0) (`KismetMathLibrary.DegreesToRadians` (`self.Spread`))) (`self.Range`)) (`KismetMathLibrary.FindLookAtRotation` _location CrosshairWorldSpace))) "TraceTypeQuery1" true (`|MakeArray` (`self.GetInstigator`) :!type "Actor Object Reference") "ForDuration" true (struct :`R` 1.0 :`A` 1.0) (struct :`G` 1.0 :`A` 1.0) 0.5))
    (bind _output_get (set `local.ObjectHit` (or _returnvalue (`local.ObjectHit`))))
    (if _output_get
      (`KismetArrayLibrary.Array_Add` (`self.HitResults`) _outhit)))
  (return (`local.ObjectHit`)))

(fn `PlayImpactEffects`)

(fn `UserConstructionScript`
  (`parent.UserConstructionScript`))