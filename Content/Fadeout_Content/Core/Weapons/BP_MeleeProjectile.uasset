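; BP_MeleeProjectile is a melee hit actor that applies pick-type damage to whatever its sphere touches.
; Overlap and hit events share one server-authority path that prints the target's name, ignores the owning character and damages each actor only once via an already-hit list.
; Each new hit calls a multicast FX event that plays a pitch-randomized crack sound and spawns a small impact particle at the projectile's location.
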(event `self.Sphere.OnComponentBeginOverlap`
  (params (OverlappedComponent :type "PrimitiveComponent Object Reference") (OtherActor :type "Actor Object Reference") (OtherComp :type "PrimitiveComponent Object Reference") (OtherBodyIndex :type Integer) (bFromSweep :type Boolean) (SweepResult :type "HitResult Structure (by ref)"))
  (bind _instigator (`self.Instigator`))
  (bind _hit_actor (`self.hit actor`))
  (set `self.hit actor` OtherActor)
  (`/Engine/EditorBlueprintResources/ActorMacros.Switch Has Authority` :!label _label
    (:`Authority`
      (`KismetSystemLibrary.PrintString` (`KismetSystemLibrary.GetDisplayName` _hit_actor))
      (if (== (`self.owningCharacter`) _hit_actor)
        _
        (elif (not (`KismetArrayLibrary.Array_Contains` (`self.alreadyHitActors`) _hit_actor))
          (`GameplayStatics.ApplyDamage` _hit_actor (`self.damage`) (`self.GetInstigatorController` _instigator) _instigator "/Game/Fadeout_Content/Core/Weapons/DamageTypes/DT_Pick.DT_Pick_C")
          (`KismetArrayLibrary.Array_AddUnique` (`self.alreadyHitActors`) _hit_actor)
          (`self.spawnFXMulticast` (`self.K2_GetActorLocation`)))))))

(event `self.Sphere.OnComponentHit`
  (params (HitComponent :type "PrimitiveComponent Object Reference") (OtherActor :type "Actor Object Reference") (OtherComp :type "PrimitiveComponent Object Reference") (NormalImpulse :type "Vector Structure") (Hit :type "HitResult Structure (by ref)"))
  (set `self.hit actor` OtherActor)
  (goto _label))

(event `spawnFXMulticast`
  (params (Location :type "Vector Structure"))
  (`GameplayStatics.PlaySoundAtLocation` "/Game/Fadeout_Content/Core/Audio/Weapon_SFX/Unarmed/crack11_mp3.crack11_mp3" Location (struct) 1.0 (`KismetMathLibrary.RandomFloatInRange` 1.2 1.4) 0.0 "/Game/Fadeout_Content/Core/Characters/BulletHit_Attenuation.BulletHit_Attenuation" "/Game/Fadeout_Content/Core/Characters/ExplosionConcurrency.ExplosionConcurrency" null)
  (`GameplayStatics.SpawnEmitterAtLocation` "/Game/AnimeFX/Particles/HandDrawn/PS_Hit_04.PS_Hit_04" Location (struct) (0.5 0.5 0.5)))

(fn `UserConstructionScript`
  (`parent.UserConstructionScript`))