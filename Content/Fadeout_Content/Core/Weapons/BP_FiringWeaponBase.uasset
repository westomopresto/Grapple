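; BP_FiringWeaponBase is a base Blueprint for firing weapons, providing shared fire animation, sound and durability-check logic.
; FireAnimationEvent restarts the supplied animation on the mesh, while CanWeaponFire allows firing only while Durability is above zero.
; Fire sound gets slight random pitch and reuses footstep attenuation and concurrency settings; a separate function plays the no-ammo sound.
; DecrementAmmoCount and PlayMuzzleFlash are empty here.
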(event `Fire Animation Event`
  (params (NewAnimToPlay :type "AnimationAsset Object Reference"))
  (bind _mesh (`self.Mesh`))
  (`SkeletalMeshComponent.SetPosition` _mesh 0.0 false)
  (`SkeletalMeshComponent.PlayAnimation` _mesh NewAnimToPlay false))

(fn `CanWeaponFire`
  (returns (CanFire :type Boolean))
  (if (> (`self.Durability`) 0.0)
    (return true)
    (else
      (return false))))

(fn `DecrementAmmoCount`)

(fn `PlayFireSound`
  (`GameplayStatics.PlaySoundAtLocation` (`self.FireSound`) (`self.K2_GetActorLocation`) (struct) 1.0 (`KismetMathLibrary.RandomFloatInRange` 0.9 1.1) 0.0 "/Game/Fadeout_Content/Core/Characters/Footstep_Attenuation.Footstep_Attenuation" "/Game/Fadeout_Content/Core/Characters/FootStepConcurrency.FootStepConcurrency" null))

(fn `PlayMuzzleFlash`)

(fn `PlayNoAmmoSound`
  (`GameplayStatics.PlaySoundAtLocation` (`self.NoAmmoSound`) (`self.K2_GetActorLocation`) (struct) 1.0 1.0 0.0 null null null))

(fn `UserConstructionScript`)