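; Bolt pistol weapon that slams player characters it damages straight down.
; The AdditionalDamage event casts the victim to BP_PlayerCharacter and calls Plummet if CheckTeamDamage reports a different team or free-for-all.
; Plummet launches the victim downward, overriding its current velocity.
; Unconnected leftover nodes for spawning a trap projectile and attaching a slow DoT never run.
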(event `plummet`
  (params (`BP Player Character` :type "/Game/Fadeout_Content/Core/Characters/BP_PlayerCharacter Object Reference"))
  (`Character.LaunchCharacter` `BP Player Character` (0.0 0.0 -1850.0) true true))

(event `/Game/Fadeout_Content/Core/Weapons/BP_ProjectileGun.Additional Damage`
  (params (DamagedActor :type "Actor Object Reference") (BaseDamage :type "Float (single-precision)") (EventInstigator :type "Controller Object Reference") (DamageCauser :type "Actor Object Reference") (DamageTypeClass :type "DamageType Class Reference"))
  (bind _asbp_player_character (cast `/Game/Fadeout_Content/Core/Characters/BP_PlayerCharacter` DamagedActor))
  (bind (_sameteam _ffa_) (`/Game/Fadeout_Content/Core/Characters/BP_PlayerCharacter.CheckTeamDamage` _asbp_player_character (`self.GetInstigatorController`)))
  (if (or (not _sameteam) _ffa_)
    (`self.plummet` _asbp_player_character)))

(fn `UserConstructionScript`
  (`parent.UserConstructionScript`))