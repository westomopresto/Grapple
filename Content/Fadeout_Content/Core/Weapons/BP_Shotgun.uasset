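; BP_Shotgun is a shotgun weapon that extends a parent weapon Blueprint to fire several projectiles per shot in a fixed spread pattern.
; The construction script rebuilds the Spread array from the relative rotations of nine spread components, so the pattern follows their placement.
; When CanFire is true, firing calls the parent's fire event MaxFire times with skipped delays and per-index spread transforms, then spawns one shell-eject particle effect.
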(event `/Game/Fadeout_Content/Core/Weapons/BP_ProjectileGun.Fire Projectile Event`
  (params (skipDelays :type Boolean) (customSpread :type Boolean) (spreadTransform :type "Transform Structure"))
  (if (`self.CanFire?`)
    (for _index (range (`self.maxFire`))
      (`parent.Fire Projectile Event` true true (`|GetArrayItem` (`self.spread`) _index)))
    (`GameplayStatics.SpawnEmitterAttached` "/Game/Fadeout_Content/Core/FBX/Shotgun/P_ShotgunShell.P_ShotgunShell" (`self.shellsEject_0`) "None" (0.0 0.0 0.0) (struct) (1.5 1.5 1.5) "SnapToTargetIncludingScale")))

(fn `initSpreadCustomArray`
  (locals (arrows :type "Array of ArrowComponent Object Reference"))
  (bind _arrows (`local.arrows`))
  (`KismetArrayLibrary.Array_Clear` (`self.spread`))
  (`KismetArrayLibrary.Array_Clear` _arrows)
  (`KismetArrayLibrary.Array_Add` _arrows (`self.spread0`))
  (`KismetArrayLibrary.Array_Add` _arrows (`self.spread1`))
  (`KismetArrayLibrary.Array_Add` _arrows (`self.spread2`))
  (`KismetArrayLibrary.Array_Add` _arrows (`self.spread3`))
  (`KismetArrayLibrary.Array_Add` _arrows (`self.spread4`))
  (`KismetArrayLibrary.Array_Add` _arrows (`self.spread5`))
  (`KismetArrayLibrary.Array_Add` _arrows (`self.spread6`))
  (`KismetArrayLibrary.Array_Add` _arrows (`self.spread7`))
  (`KismetArrayLibrary.Array_Add` _arrows (`self.spread8`))
  (for _array_element (`local.arrows`)
    (`KismetArrayLibrary.Array_Add` (`self.spread`) (`KismetMathLibrary.MakeTransform` (0.0 0.0 0.0) (.rotation (`SceneComponent.GetRelativeTransform` _array_element)))))
  (return))

(fn `UserConstructionScript`
  (`parent.UserConstructionScript`)
  (`self.initSpreadCustomArray`))