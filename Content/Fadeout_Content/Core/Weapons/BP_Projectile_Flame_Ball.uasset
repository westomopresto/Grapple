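; Bouncing flame barrel projectile that damages on impact, spurts fire while active, then fades out, shrinks and self-destroys after a fixed lifetime.
; A server-side looping timer line-traces the spurt, damaging each hit actor once per tick.
; Incoming damage drains health and accumulates as stored damage that boosts emissive glow.
; At zero health a short fuse, paused by further hits, triggers radial damage scaled by stored damage and spawns eight flame projectiles.
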(event `self.OnProjectileHitEvent`
  (params (OtherActor :type "Actor Object Reference") (OtherComponent :type "PrimitiveComponent Object Reference") (HitResult :type "HitResult Structure (by ref)"))
  (`self.Damage Testing SERVER ONLY` HitResult OtherComponent OtherActor)
  (`self.SurfaceImpactEvent` HitResult false OtherActor)
  (if (>= (`KismetMathLibrary.VSize` (`self.GetVelocity` self)) 70.0)
    (`/Engine/EditorBlueprintResources/StandardMacros.DoOnce` false :!label _label
      (:`Completed`
        (`self.Bounce FX`)
        (`KismetSystemLibrary.Delay` 0.2)
        (goto _label :!via `Reset`)))))

(event `self.SurfaceImpactEvent`
  (params (HitResult :type "HitResult Structure") (`Hardsurface?` :type Boolean) (hitactor :type "Actor Object Reference"))
  (`self.PlayImpactEffects` HitResult `Hardsurface?`))

(event `self.ReceiveBeginPlay`
  (`parent.ReceiveBeginPlay`)
  (bind _returnvalue (`PrimitiveComponent.CreateDynamicMaterialInstance` (`self.Mesh`) 0 "/Game/Fadeout_Content/Core/FBX/FlameThrower/M_flame_Barrel.M_flame_Barrel" "None"))
  (set `self.barrel_dynamic` _returnvalue)
  (`/Engine/EditorBlueprintResources/ActorMacros.Switch Has Authority`
    (:`Authority`
      (bind _returnvalue_2 (`KismetSystemLibrary.K2_SetTimerDelegate` (delegate `Flame_Spurt`) 0.05 true 0.5))
      (set `self.SpurtTimer` _returnvalue_2))
    (:`Remote`
      _))
  (`self.K2_SetActorRotation` (struct))
  (`KismetSystemLibrary.Delay` 6.0)
  (`AudioComponent.FadeOut` (`self.fireAudio`) 0.5 0.0 "Linear")
  (`ActorComponent.Deactivate` (`self.trail`))
  (`ActorComponent.Deactivate` (`self.ParticleSystem`))
  (`KismetSystemLibrary.K2_PauseTimerHandle` (`self.SpurtTimer`))
  (bind (_direction _rotatealpha _sizealpha) (`Timeline|Timeline_0` :!via `PlayFromStart`)
    (:`Update`
      (`SceneComponent.SetRelativeScale3D` (`self.Mesh`) (`KismetMathLibrary.VLerp` (1.0 1.0 1.0) (0.05 0.05 0.05) _sizealpha))
      (set `RotatingMovementComponent.RotationRate` (`KismetMathLibrary.RLerp` (struct :`Pitch` 450.0) (struct) _rotatealpha) (`self.RotatingMovement`)))
    (:`Finished`
      (`self.K2_DestroyActor`))))

(event `Flame_Spurt`
  (bind _victims (`self.Victims`))
  (bind _owningweapon (`self.OwningWeapon`))
  (bind _returnvalue (`KismetSystemLibrary.IsValid` _owningweapon))
  (if _returnvalue
    (bind _asbp_player_character (cast `/Game/Fadeout_Content/Core/Characters/BP_PlayerCharacter` (`self.GetOwner` _owningweapon))))
  (bind _outhits (`KismetSystemLibrary.LineTraceMultiForObjects` (`SceneComponent.K2_GetComponentLocation` (`self.Transform`)) (`SceneComponent.K2_GetComponentLocation` (`self.end`)) (`|MakeArray` "ObjectTypeQuery3" "ObjectTypeQuery7" :!type "EObjectTypeQuery Enum") false (`|MakeArray` (select `bool` _returnvalue :`false` self :`true` _asbp_player_character :!type "Actor Object Reference") self :!type "Actor Object Reference") "ForDuration" true (struct :`R` 1.0 :`A` 1.0) (struct :`G` 1.0 :`A` 1.0) 0.05))
  (for _array_element _outhits
    (bind (_bblockinghit _binitialoverlap _time _distance _location _impactpoint _normal _impactnormal _physmat _hitactor) (`GameplayStatics.BreakHitResult` _array_element))
    (if (not (`KismetArrayLibrary.Array_Contains` _victims _hitactor))
      (`GameplayStatics.ApplyDamage` _hitactor 5.0 (`self.Instigator Controller`) (`self.OwningWeapon`) (`self.DamageType`))
      (`KismetArrayLibrary.Array_Add` _victims _hitactor)))
  (`KismetArrayLibrary.Array_Clear` _victims))

(event `Damage Effects`
  (params (StoredDamage :type "Float (double-precision)"))
  (`MaterialInstanceDynamic.SetScalarParameterValue` (`self.barrel_dynamic`) "Emission Boost" (`KismetMathLibrary.Lerp` 0.0 15.0 (`KismetMathLibrary.NormalizeToRange` StoredDamage 25.0 100.0))))

(event `DelayExplode`
  (bind _explodetimer (`self.explodeTimer`))
  (`KismetSystemLibrary.K2_PauseTimerHandle` _explodetimer)
  (`KismetSystemLibrary.RetriggerableDelay` 0.5)
  (`KismetSystemLibrary.K2_UnPauseTimerHandle` _explodetimer))

(event `self.ReceiveAnyDamage`
  (params (Damage :type "Float (single-precision)") (DamageType :type "DamageType Object Reference") (InstigatedBy :type "Controller Object Reference") (DamageCauser :type "Actor Object Reference"))
  (`self.DelayExplode`)
  (set `self.instigated_explode` InstigatedBy)
  (bind _output_get (set `self.health` (- (`self.health`) Damage)))
  (bind _output_get_2 (set `self.StoredDamage` (`KismetMathLibrary.FClamp` (+ (`self.StoredDamage`) Damage) 15.0 9999.0)))
  (`self.Damage Effects` _output_get_2)
  (if (and (not (`self.dead`)) (<= _output_get 0.0))
    (set `self.dead` true)
    (`/Engine/EditorBlueprintResources/StandardMacros.DoOnce` false
      (:`Completed`
        (bind _returnvalue (`KismetSystemLibrary.K2_SetTimerDelegate` (delegate `Exploding`) 0.4))
        (set `self.explodeTimer` _returnvalue)))))

(event `Exploding`
  (bind _instigated_explode (`self.instigated_explode`))
  (set `self.dead` true)
  (`KismetSystemLibrary.K2_ClearAndInvalidateTimerHandle` (`self.explodeTimer`))
  (`/Engine/EditorBlueprintResources/StandardMacros.IsValid` _instigated_explode
    (:`Is Valid`
      (set `self.Instigator` (`Controller.K2_GetPawn` _instigated_explode))
      (`self.Explode` (`self.StoredDamage`)))))

(event `Explode`
  (params (BaseDamage :type "Float (double-precision)" :default 25.0))
  (bind _returnvalue (`self.K2_GetActorLocation`))
  (bind _returnvalue_2 (* BaseDamage 0.5))
  (`self.Spawn Flames`)
  (`GameplayStatics.SpawnEmitterAtLocation` "/Game/StylizedVFX_Fire/Effects/P_FireExplosion_Medium.P_FireExplosion_Medium" (`self.K2_GetActorLocation`) (struct) (10.0 10.0 10.0))
  (`GameplayStatics.PlaySoundAtLocation` "/Game/Fadeout_Content/Core/Audio/Explosions/Explosion_5_W_Rubble_3.Explosion_5_W_Rubble_3" (`self.K2_GetActorLocation`) (struct) 1.25 (`KismetMathLibrary.RandomFloatInRange` 1.5 1.6) 0.0 "/Game/Fadeout_Content/Core/Characters/Footstep_Attenuation.Footstep_Attenuation" null null)
  (`|ExecutionSequence`
    (:`then_0`
      (`GameplayStatics.ApplyRadialDamage` :`BaseDamage` _returnvalue_2 :`Origin` _returnvalue :`DamageRadius` (`self.DamageRadius`) :`DamageTypeClass` "/Game/Fadeout_Content/Core/Weapons/DamageTypes/DT_TNT.DT_TNT_C" :`DamageCauser` self :`InstigatedByController` (`self.Instigator Controller`) :`bDoFullDamage` true))
    (:`then_1`
      (`GameplayStatics.ApplyRadialDamage` :`BaseDamage` _returnvalue_2 :`Origin` _returnvalue :`DamageRadius` (`self.DamageRadius`) :`DamageTypeClass` (`self.AOEDamageType`) :`DamageCauser` self :`InstigatedByController` (`self.Instigator Controller`) :`bDoFullDamage` true)
      (`ActorComponent.Deactivate` (`self.trail`))
      (`ActorComponent.Deactivate` (`self.ParticleSystem`))
      (`ActorComponent.Deactivate` (`self.fireAudio`))
      (`SceneComponent.SetVisibility` (`self.Mesh`) false false)
      (`PrimitiveComponent.SetCollisionResponseToAllChannels` (`self.CollisionSphere`) "ECR_Ignore")
      (bind _asbp_player_character (cast `/Game/Fadeout_Content/Core/Characters/BP_PlayerCharacter` (`self.GetOwner`)))
      (`KismetArrayLibrary.Array_RemoveItem` (`/Game/Fadeout_Content/Core/Characters/BP_PlayerCharacter.myOwnedProjectiles` _asbp_player_character) self))))

(event `Bounce FX`
  (`GameplayStatics.PlaySoundAtLocation` "/Game/PunchSoundPack/PunchSounds/Barrel_smack_random.Barrel_smack_random" (`self.K2_GetActorLocation`) (struct) 0.5 1.0 0.0 null null null)
  (bind (_direction _alpha) (`Timeline|BounceTimeline` :!via `PlayFromStart`)
    (:`Update`
      (`SceneComponent.SetRelativeScale3D` (`self.Mesh`) (`KismetMathLibrary.MakeVector` 1.0 _alpha 1.0)))))

(fn `Spawn Flames`
  (for _array_element (`|MakeArray` (`self.flame_spawn`) (`self.flame_spawn1`) (`self.flame_spawn2`) (`self.flame_spawn3`) (`self.flame_spawn5`) (`self.flame_spawn6`) (`self.flame_spawn7`) (`self.flame_spawn4`))
    (`|SpawnActorFromClass` "/Game/Fadeout_Content/Core/Weapons/BP_Projectile_Flame.BP_Projectile_Flame_C" (`SceneComponent.K2_GetComponentToWorld` _array_element) "Undefined" "OverrideRootScale" null (`self.OwningWeapon`) 1.0 false (`self.GetInstigator`)))
  (return))

(fn `UserConstructionScript`
  (`parent.UserConstructionScript`)
  (`MovementComponent.SetUpdatedComponent` (`self.RotatingMovement`) (`self.Mesh`)))