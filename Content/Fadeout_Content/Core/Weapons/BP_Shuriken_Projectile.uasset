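; Shuriken weapon projectile, a child of a base projectile Blueprint, that deals more damage to wounded players.
; On spawn it gives the mesh a random pitch, and it ignores hits against other shurikens.
; Each tick adds forward local velocity without delta-time scaling, so it keeps accelerating.
; The server damage event multiplies base damage up to tenfold by the player's missing health before calling the parent.
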(event `self.OnProjectileHitEvent`
  (params (OtherActor :type "Actor Object Reference") (OtherComponent :type "PrimitiveComponent Object Reference") (HitResult :type "HitResult Structure (by ref)") (fromHit :type Boolean))
  (if (not (== (`GameplayStatics.GetObjectClass` OtherActor) "BP_Shuriken_Projectile_C"))
    (`parent.OnProjectileHitEvent` OtherActor OtherComponent HitResult fromHit)))

(event `self.ReceiveBeginPlay`
  (`parent.ReceiveBeginPlay`)
  (`SceneComponent.K2_SetRelativeRotation` (`self.Mesh`) (`KismetMathLibrary.MakeRotator` 0.0 (`KismetMathLibrary.RandomFloatInRange` -90.0 90.0) -90.0) false false))

(event `self.Damage Testing SERVER ONLY`
  (params (Hit :type "HitResult Structure (by ref)") (`other Component` :type "PrimitiveComponent Object Reference") (`other actor` :type "Actor Object Reference"))
  (bind _asbp_player_character (cast `/Game/Fadeout_Content/Core/Characters/BP_PlayerCharacter` `other actor`)
    (:`then`
      (set `self.BaseDamage` (* (`self.BaseDamage`) (`KismetMathLibrary.Lerp` 1.0 10.0 (- 1.0 (/ (`/Game/Fadeout_Content/Core/Characters/BP_PlayerCharacter.health` _asbp_player_character) (`/Game/Fadeout_Content/Core/Characters/BP_PlayerCharacter.maxHealth` _asbp_player_character))))))
      (`parent.Damage Testing SERVER ONLY` Hit `other Component` `other actor`))
    (:`CastFailed`
      (`parent.Damage Testing SERVER ONLY` Hit `other Component` `other actor`))))

(event `self.ReceiveTick`
  (params (DeltaSeconds :type "Float (single-precision)"))
  (`parent.ReceiveTick` DeltaSeconds)
  (`ProjectileMovementComponent.SetVelocityInLocalSpace` (`self.ProjectileMovement`) (+ (`KismetMathLibrary.LessLess_VectorRotator` (`self.GetVelocity`) (`self.K2_GetActorRotation`)) (2000.0 0.0 0.0))))

(fn `UserConstructionScript`
  (`parent.UserConstructionScript`))