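; Alchemic weapon projectile, a child projectile that sets explode-on-impact with radial damage at half its base damage.
; Sphere overlaps trigger the hit event, sparing the owning player unless self-damage is allowed.
; Surface impacts play effects, disable collision and have the authority multicast a stop-and-attach to player bones, practice targets or other actors.
; It then throttles net updates, fades trail and audio, and destroys itself after a delay.
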(event `self.ReceiveBeginPlay`
  ;[1 1 1] Begin Play
  (`|ExecutionSequence`
    (:`then_0`
      (`PrimitiveComponent.IgnoreActorWhenMoving` (`self.Capsule`) self true)
      (`PrimitiveComponent.IgnoreActorWhenMoving` (`self.CollisionSphere`) self true)
      (`parent.ReceiveBeginPlay`)
      (`KismetSystemLibrary.Delay` 0.05)
      (`self.SetReplicateMovement` true))
    (:`then_1`
      ;[1 1 1] damage scale
      (bind _output_get (set `self.BaseDamage` 40.0))
      (set `self.explode on impact?` true)
      (set `self.AOEDamageType` (`self.DamageType`))
      (set `self.radialDamageAmount` (* _output_get 0.5)))))

(event `self.SurfaceImpactEvent`
  (params (HitResult :type "HitResult Structure") (`Hardsurface?` :type Boolean) (hitactor :type "Actor Object Reference"))
  (`self.onProjectileHit`)
  (`self.PlayImpactEffects` HitResult `Hardsurface?`)
  (`PrimitiveComponent.SetCollisionEnabled` (`self.CollisionSphere`) "NoCollision")
  (`PrimitiveComponent.SetCollisionEnabled` (`self.Capsule`) "NoCollision")
  (`/Engine/EditorBlueprintResources/ActorMacros.Switch Has Authority`
    (:`Authority`
      (`self.MultiCast Attach` HitResult))))

(event `self.CollisionSphere.OnComponentBeginOverlap`
  (params (OverlappedComponent :type "PrimitiveComponent Object Reference") (OtherActor :type "Actor Object Reference") (OtherComp :type "PrimitiveComponent Object Reference") (OtherBodyIndex :type Integer) (bFromSweep :type Boolean) (SweepResult :type "HitResult Structure (by ref)"))
  (bind _asbp_player_character (cast `/Game/Fadeout_Content/Core/Characters/BP_PlayerCharacter` OtherActor)
    (:`then`
      (if (== (`self.GetOwner`) _asbp_player_character)
        (if (`self.canhurtOwner`)
          (`self.OnProjectileHitEvent` OtherActor OtherComp SweepResult :!label _label))
        (else
          (goto _label))))
    (:`CastFailed`
      (`self.OnProjectileHitEvent` OtherActor OtherComp SweepResult))))

(event `MultiCast Attach`
  (params (HitResult :type "HitResult Structure"))
  (`|ExecutionSequence`
    (:`then_0`
      (`ProjectileMovementComponent.StopSimulating` (`self.ProjectileMovement`) HitResult)
      (if (not (`self.Attached`))
        (`self.ArrowAttach` HitResult)
        (`self.ForceNetUpdate`)))
    (:`then_1`
      (set `self.MinNetUpdateFrequency` 1.0)
      (set `self.NetUpdateFrequency` 1.0)
      (`ActorComponent.Deactivate` (`self.trail`))
      (`AudioComponent.FadeOut` (`self.Audio`) 0.25 0.0 "Linear")
      (`KismetSystemLibrary.Delay` (`self.DestroyDelayAfterImpact`))
      (`self.K2_DestroyActor`))))

(fn `ArrowAttach`
  (params (Hit :type "HitResult Structure (by ref)"))
  (bind (_bblockinghit _binitialoverlap _time _distance _location _impactpoint _normal _impactnormal _physmat _hitactor _hitcomponent _hitbonename) (`GameplayStatics.BreakHitResult` Hit))
  (`/Engine/EditorBlueprintResources/StandardMacros.IsValid` _hitactor
    (:`Is Valid`
      (if (!= _hitactor self)
        (cast `/Game/Fadeout_Content/Core/Characters/BP_PlayerCharacter` _hitactor
          (:`then`
            (`self.K2_AttachToComponent` _hitcomponent _hitbonename "SnapToTarget" "KeepWorld" "KeepWorld")
            (set `self.Attached` true)
            (return))
          (:`CastFailed`
            (bind _asbp_target_practice (cast `/Game/Fadeout_Content/Core/Debug/BP_TargetPractice` _hitactor)
              (:`then`
                (`self.K2_AttachToComponent` (`/Game/Fadeout_Content/Core/Debug/BP_TargetPractice.Offset` _asbp_target_practice) "None" "KeepWorld" "KeepWorld" "KeepWorld")
                (set `self.Attached` true)
                (return))
              (:`CastFailed`
                (`self.K2_AttachToActor` _hitactor "None" "KeepWorld" "KeepWorld" "KeepWorld")
                (set `self.Attached` true)
                (return)))))
        (else
          (`KismetSystemLibrary.PrintString` "COLLIDING WITH SELF SOMEHOW")
          (`KismetSystemLibrary.PrintString` (`KismetSystemLibrary.GetDisplayName` _hitcomponent))
          (return))))
    (:`Is Not Valid`
      (return))))

(fn `UserConstructionScript`
  (`parent.UserConstructionScript`))