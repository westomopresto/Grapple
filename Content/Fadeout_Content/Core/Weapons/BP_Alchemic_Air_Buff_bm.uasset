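; An alchemic air buff Blueprint that extends a parent class's weakness event with a change to the player's scale.
; After the parent logic runs, the server checks that the player is valid and plays a timeline that drives the player's uniform scale.
; When the timeline finishes, it resets the scale of the buff actor itself, rather than the player's, to one.
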(event `self.Apply Weakness Event`
  (`parent.Apply Weakness Event`)
  (`/Engine/EditorBlueprintResources/ActorMacros.Switch Has Authority`
    (:`Authority`
      (`self.Player`
        (:`then`
          (if true
            (bind (_direction _scale) (`Timeline|Timeline_1` :`NewTime` 5.0)
              (:`Update`
                (`self.SetActorScale3D` (`self.Player`) (`KismetMathLibrary.Conv_DoubleToVector` _scale)))
              (:`Finished`
                (`self.SetActorScale3D` (1.0 1.0 1.0))))))
        (:`else`)))))

(fn `UserConstructionScript`
  (`parent.UserConstructionScript`))