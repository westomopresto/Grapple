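; BP_MeleeBase is a melee weapon base that swings, traces and damages what it hits.
; OnFire routes through server and multicast events to play the owning character's windup and release, locking refire and tool swapping.
; A brief timed window enables per-Tick sphere traces between hitbox points, damaging each actor once per swing with pawn-specific impact sound and particles.
; Alt-fire is stubbed, and the knockback Impulse event is never called here.
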(event `self.OnAltFirePress`)

(event `AltFireRelease`)

(event `Effect Multicast`
  (`KismetArrayLibrary.Array_Clear` (`self.HitActors`))
  (bind _asbp_player_character (cast `/Game/Fadeout_Content/Core/Characters/BP_PlayerCharacter` (`self.GetOwner`)))
  (if (`self.CanFire?`)
    (`/Game/Fadeout_Content/Core/Characters/BP_PlayerCharacter.meleeWindup` _asbp_player_character)
    (set `self.CanFire?` false)
    (set `/Game/Fadeout_Content/Core/Characters/BP_PlayerCharacter.canSwapTools?` false _asbp_player_character)
    (`KismetSystemLibrary.Delay` 0.15)
    (`self.PlayFireSound_0`)
    (`/Game/Fadeout_Content/Core/Characters/BP_PlayerCharacter.meleeRelease` _asbp_player_character)
    (`KismetSystemLibrary.Delay` 0.05)
    (`self.Trace`)))

(event `Impulse`
  (params (Target :type "PrimitiveComponent Object Reference") (`hit normal` :type "Vector Structure") (`hit Location` :type "Vector Structure"))
  (if (`SceneComponent.IsSimulatingPhysics` Target "None")
    (`PrimitiveComponent.AddImpulseAtLocation` Target (* `hit normal` (* (`self.knockbackAmount`) -1.0)) `hit Location` "None")))

(event `OnFire`
  (`KismetSystemLibrary.RetriggerableDelay` 0.1)
  (`/Engine/EditorBlueprintResources/ActorMacros.Switch Has Authority`
    (:`Authority`
      (`self.Effect Multicast`))
    (:`Remote`
      (`self.Effect Server`))))

(event `Effect Server`
  (`self.Effect Multicast`))

(event `Effects`
  (params (Location :type "Vector Structure") (`hitPlayer?` :type Boolean))
  (bind _returnvalue (`KismetMathLibrary.SelectFloat` (`KismetMathLibrary.RandomFloatInRange` 1.2 1.5) 1.0 (`self.Sound_PitchVariance?`)))
  (if `hitPlayer?`
    (`GameplayStatics.PlaySoundAtLocation` (`self.HitPlayer_Sound`) Location (struct) 2.0 _returnvalue 0.0 null null null)
    (else
      (`GameplayStatics.PlaySoundAtLocation` (`self.HitElse_Sound`) Location (struct) 2.0 _returnvalue 0.0 null null null)))
  (`GameplayStatics.SpawnEmitterAtLocation` "/Game/AnimeFX/Particles/HandDrawn/PS_Hit01.PS_Hit01" Location (struct) (0.6 0.6 1.0)))

(event `CheckHits`
  (params (Hit :type "HitResult Structure (by ref)"))
  (bind (_bblockinghit _binitialoverlap _time _distance _location _impactpoint _normal _impactnormal _physmat _hitactor) (`GameplayStatics.BreakHitResult` Hit))
  (if (not (`KismetArrayLibrary.Array_Contains` (`self.HitActors`) _hitactor))
    (`GameplayStatics.ApplyDamage` _hitactor (`self.damage`) (`Pawn.GetController` (`Actor.Instigator` (`self.GetOwner`))) self (`self.Damage Type`))
    (`KismetArrayLibrary.Array_Add` (`self.HitActors`) _hitactor)
    (cast `Pawn` _hitactor
      (:`then`
        (`self.Effects` _impactpoint true))
      (:`CastFailed`
        (`self.Effects` _impactpoint)))))

(event `self.ReceiveTick`
  (params (DeltaSeconds :type "Float (single-precision)"))
  (`parent.ReceiveTick` DeltaSeconds)
  (if (`self.doTrace?`)
    ;[1 1 1] traces current
    (bind (_outhit _returnvalue) (`KismetSystemLibrary.SphereTraceSingle` (`SceneComponent.K2_GetComponentLocation` (`self.hitbox_start`)) (`SceneComponent.K2_GetComponentLocation` (`self.hitbox_end`)) 45.0 "TraceTypeQuery1" false (`|MakeArray` (`self.GetOwner`)) "None" true (struct :`R` 1.0 :`A` 1.0) (struct :`G` 1.0 :`A` 1.0) 0.2))
    (if _returnvalue
      (`self.CheckHits` _outhit))))

(event `self.Initialize`
  (`parent.Initialize`))

(event `Trace`
  (set `self.doTrace?` true)
  (`KismetSystemLibrary.Delay` 0.1)
  (set `self.doTrace?` false)
  (`KismetSystemLibrary.Delay` 0.1)
  (`self.FinishTrace`))

(event `FinishTrace`
  (bind _asbp_player_character (cast `/Game/Fadeout_Content/Core/Characters/BP_PlayerCharacter` (`self.GetOwner`)))
  (set `/Game/Fadeout_Content/Core/Characters/BP_PlayerCharacter.canSwapTools?` true _asbp_player_character)
  (set `self.CanFire?` true))

(fn `PlayAltFireSound_0`
  (`GameplayStatics.PlaySoundAtLocation` (`self.FireSound_0_0`) (`self.K2_GetActorLocation`) (struct) 1.0 1.0 0.0 null null null))

(fn `PlayFireSound_0`
  (`GameplayStatics.PlaySoundAtLocation` (`self.FireSound_0_0`) (`self.K2_GetActorLocation`) (struct) 1.0 (`KismetMathLibrary.RandomFloatInRange` 0.9 1.1) 0.0 null null null))

(fn `UserConstructionScript`)