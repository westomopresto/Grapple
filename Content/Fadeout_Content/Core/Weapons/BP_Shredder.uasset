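; BP_Shredder is a minigun weapon that fires faster the longer it spins and kicks its owner back with each shot.
; A looping Spin timer scales FireCoolDown within limits, driving animation play rate and rev sound pitch.
; Alt fire holds the spin; authority switches route sounds and blowback directly or through server events.
; The owner-slowdown branch is never reached.
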(event `Play Sound All`
  (params (Sound :type "SoundBase Object Reference"))
  (`GameplayStatics.PlaySoundAtLocation` Sound (`self.K2_GetActorLocation`) (struct) 1.0 1.0 0.0 null null null))

(event `Play Sound Server`
  (params (Sound :type "SoundBase Object Reference"))
  (`self.Play Sound All` Sound))

(event `self.Animation Sequence Multicast`
  (`GameplayStatics.SpawnEmitterAttached` (`self.muzzleEmitter`) (`self.muzzleParticle`) "None" (0.0 0.0 0.0) (struct) (1.0 1.0 1.0) "SnapToTargetIncludingScale"))

(event `self.Projectile Fire Sound ALt`
  (`GameplayStatics.PlaySoundAtLocation` "/Game/Fadeout_Content/Core/Audio/Weapon_SFX/Minigun/minigun_shot.minigun_shot" (`self.K2_GetActorLocation`) (struct) 1.0 1.0 0.0 null null null))

(event `self.OnFireRelease`
  (params (`charged?` :type Boolean))
  (`parent.OnFireRelease` `charged?`)
  (if (`self.AltFiring`)
    (`/Engine/EditorBlueprintResources/StandardMacros.DoOnce` false :!label _label
      (:`Completed`
        (if (`self.spinning`)
          (`/Engine/EditorBlueprintResources/ActorMacros.Switch Has Authority`
            (:`Authority`
              (`self.Play Sound All` "/Game/Fadeout_Content/Core/Audio/Weapon_SFX/Minigun/minigun_start.minigun_start"))
            (:`Remote`
              (`self.Play Sound Server` "/Game/Fadeout_Content/Core/Audio/Weapon_SFX/Minigun/minigun_start.minigun_start"))))))
    (else
      (`self.Set Spinning` false)
      (goto _label :!via `Reset`))))

(event `self.OnFirePress`
  (`parent.OnFirePress`)
  (`self.Set Spinning` true)
  (goto _label))

(event `SpinSounds Multi`
  (params (Condition :type Boolean) (Rate :type "Float (double-precision)"))
  (bind _minigun_rev (`self.minigun_rev`))
  (bind _returnvalue (`AudioComponent.IsPlaying` _minigun_rev))
  (`|ExecutionSequence`
    (:`then_0`
      (if Condition
        (if (not _returnvalue)
          (`AudioComponent.Play` _minigun_rev 0.0)
          (`GameplayStatics.PlaySoundAtLocation` "/Game/Fadeout_Content/Core/Audio/Weapon_SFX/Minigun/minigun_start.minigun_start" (`self.K2_GetActorLocation`) (struct) 1.0 1.0 0.0 null null null))
        (elif _returnvalue
          (`AudioComponent.FadeOut` _minigun_rev 0.5 0.0 "Linear")
          (`GameplayStatics.PlaySoundAtLocation` "/Game/Fadeout_Content/Core/Audio/Weapon_SFX/Minigun/minigun_end.minigun_end" (`self.K2_GetActorLocation`) (struct) 1.0 1.0 0.0 null null null))))
    (:`then_1`
      (if Condition
        (set `self.AnimPlayRate` (`KismetMathLibrary.MapRangeClamped` Rate 0.3 0.04 1.0 3.0))
        (else
          (set `self.AnimPlayRate` (`KismetMathLibrary.FClamp` (- (`self.AnimPlayRate`) 0.4) 0.0 3.0)))))
    (:`then_2`
      (`AudioComponent.SetPitchMultiplier` (`self.minigun_rev`) (`KismetMathLibrary.MapRangeClamped` (`self.AnimPlayRate`) 1.0 3.0 1.0 2.0)))))

(event `Set Spinning`
  (params (spinning :type Boolean))
  ;[1 1 1] Spinning set
  (set `self.spinning` spinning))

(event `self.ReceiveBeginPlay`
  (`parent.ReceiveBeginPlay`)
  (`KismetSystemLibrary.K2_SetTimerDelegate` (delegate `Spin`) 0.5 true))

(event `self.OnDropped`
  ;[1 1 1] Dropped
  (`parent.OnDropped`)
  (set `self.Fire CoolDown` 0.3))

(event `Spin`
  (bind _spinning (`self.spinning`))
  (if (not (`self.onGround?`))
    (`|ExecutionSequence`
      (:`then_0`
        (bind _output_get (set `self.Fire CoolDown` (`KismetMathLibrary.FClamp` (`KismetMathLibrary.SelectFloat` (* (`self.Fire CoolDown`) 0.8) (* (`self.Fire CoolDown`) 1.2) (`self.spinning`)) 0.075 0.3)))
        (`KismetSystemLibrary.RetriggerableDelay` 0.1)
        (`/Engine/EditorBlueprintResources/ActorMacros.Switch Has Authority`
          (:`Authority`
            (`self.SpinSounds Multi` _spinning _output_get))
          (:`Remote`
            (`self.SpinSounds Server` _output_get _spinning)))))))

(event `self.OnAltFirePress`
  (`self.Set Spinning` true)
  (set `self.AltFiring` true))

(event `SpinSounds Server`
  (params (Rate :type "Float (double-precision)") (Condition :type Boolean))
  (`self.SpinSounds Multi` Condition Rate))

(event `self.AltFireRelease`
  (`self.Set Spinning` false)
  (set `self.AltFiring` false))

(event `self.Initialize`
  (`parent.Initialize`)
  (`AudioComponent.FadeOut` (`self.minigun_rev`) 0.5 0.0 "Linear")
  (`self.Set Spinning` false)
  (set `self.AltFiring` false))

(event `Make Owner Slow Event`
  (params (Condition :type Boolean))
  (bind _asbp_player_character (cast `/Game/Fadeout_Content/Core/Characters/BP_PlayerCharacter` (`self.GetOwner`)))
  (if Condition
    (`/Game/Fadeout_Content/Core/Characters/BP_PlayerCharacter.slowMovement` _asbp_player_character (`/Game/Fadeout_Content/Core/Characters/BP_PlayerCharacter.walkSpeed` _asbp_player_character))
    (else
      (`/Game/Fadeout_Content/Core/Characters/BP_PlayerCharacter.releaseSlow` _asbp_player_character))))

(event `self.Fire Projectile Event`
  (params (skipDelays :type Boolean) (customSpread :type Boolean) (spreadTransform :type "Transform Structure"))
  (`parent.Fire Projectile Event` skipDelays customSpread spreadTransform)
  (bind (_locationvec _directionvec) (`self.getInstigatorCameraFVector`))
  (`/Engine/EditorBlueprintResources/ActorMacros.Switch Has Authority`
    (:`Authority`
      (`self.BlowBack` (`self.Blowback Amount`) _directionvec))
    (:`Remote`
      (`self.Blowback Server` (`self.Blowback Amount`) _directionvec))))

(event `Make Owner Slow`
  (params (Condition :type Boolean))
  (`self.Make Owner Slow Event` Condition))

(event `BlowBack`
  (params (Amount :type "Float (double-precision)") (Direction :type "Vector Structure"))
  (if (> Amount 0.0)
    (bind _asbp_player_character (cast `/Game/Fadeout_Content/Core/Characters/BP_PlayerCharacter` (`self.GetOwner`)))
    (`Character.LaunchCharacter` _asbp_player_character (* Direction (* Amount -1.0)) false false)))

(event `Blowback Server`
  (params (Amount :type "Float (double-precision)") (Direction :type "Vector Structure"))
  (`self.BlowBack` Amount Direction))

(fn `UserConstructionScript`
  (`parent.UserConstructionScript`))