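; Abby's shotgun weapon, with an alt fire that launches the player opposite the camera aim.
; Holding alt fire enables blowback mode, firing at once and repeating on a looping cooldown timer until release.
; Each fire press sets spread and recoil force from that mode, widening spread during blowback, then calls parent fire logic.
; Projectile firing applies the launch directly with authority or through BlowbackServer on remotes.
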(event `self.AltFireRelease`
  (set `self.blowbackMode` false)
  (`KismetSystemLibrary.K2_ClearAndInvalidateTimerHandle` (`self.triggerTimer`)))

(event `self.OnAltFirePress`
  (`KismetSystemLibrary.K2_ClearAndInvalidateTimerHandle` (`self.triggerTimer`))
  (bind _returnvalue (`KismetSystemLibrary.K2_SetTimerDelegate` (delegate `self.OnFirePress`) (+ (`self.Fire CoolDown`) (`GameplayStatics.GetWorldDeltaSeconds`)) true))
  (set `self.triggerTimer` _returnvalue)
  (set `self.blowbackMode` true)
  (if (`self.blowbackMode`) :!label _label
    (set `self.BlowbackAmount` 600.0)
    (set `self.INaccurateBulletSpread` 10.0)
    (else
      (set `self.BlowbackAmount` 0.0)
      (set `self.INaccurateBulletSpread` 3.0)))
  (`parent.OnFirePress`))

(event `self.OnFirePress`
  (goto _label))

(event `self.Fire Projectile Event`
  (params (skipDelays :type Boolean) (customSpread :type Boolean) (spreadTransform :type "Transform Structure"))
  (`parent.Fire Projectile Event` skipDelays customSpread spreadTransform)
  (bind (_locationvec _directionvec) (`self.getInstigatorCameraFVector`))
  (`/Engine/EditorBlueprintResources/ActorMacros.Switch Has Authority`
    (:`Authority`
      (`self.BlowBack` (`self.BlowbackAmount`) _directionvec))
    (:`Remote`
      (`self.Blowback Server` (`self.BlowbackAmount`) _directionvec))))

(event `BlowBack`
  (params (Amount :type "Float (double-precision)") (Direction :type "Vector Structure"))
  (if (> Amount 0.0)
    (bind _asbp_player_character (cast `/Game/Fadeout_Content/Core/Characters/BP_PlayerCharacter` (`self.GetOwner`)))
    (`Character.LaunchCharacter` _asbp_player_character (* Direction (* Amount -1.0)) false false)))

(event `Blowback Server`
  (params (Amount :type "Float (double-precision)") (Direction :type "Vector Structure"))
  (`self.BlowBack` Amount Direction))

(fn `UserConstructionScript`
  (`parent.UserConstructionScript`))