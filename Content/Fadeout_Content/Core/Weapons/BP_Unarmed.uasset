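; BP_Unarmed is the unarmed weapon Blueprint, handling aim-down-sights through alt fire on the player character.
; Pressing alt fire sets ADS and, when CanAltFire allows, enables firing, blocks tool swapping and switches the instigating BP_PlayerCharacter to a right-side aim camera with aim animation.
; Releasing it clears ADS and, under the same check, disables firing, restores tool swapping and returns to the rear camera.
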(event `self.OnAltFire`
  (params (`MoveCamera?` :type Boolean))
  (set `self.ADS` true)
  (if (`self.canAltFire?`)
    (set `self.CanFire?` true)
    (bind _asbp_player_character (cast `/Game/Fadeout_Content/Core/Characters/BP_PlayerCharacter` (`self.GetInstigator`)))
    (set `/Game/Fadeout_Content/Core/Characters/BP_PlayerCharacter.canSwapTools?` false _asbp_player_character)
    (`/Game/Fadeout_Content/Core/Characters/BP_PlayerCharacter.toAimCam` _asbp_player_character true true true)))

(event `self.AltFireRelease`
  (set `self.ADS` false)
  (if (`self.canAltFire?`)
    (set `self.CanFire?` false)
    (bind _asbp_player_character (cast `/Game/Fadeout_Content/Core/Characters/BP_PlayerCharacter` (`self.GetInstigator`)))
    (set `/Game/Fadeout_Content/Core/Characters/BP_PlayerCharacter.canSwapTools?` true _asbp_player_character)
    (`/Game/Fadeout_Content/Core/Characters/BP_PlayerCharacter.toRearCam` _asbp_player_character)))

(fn `UserConstructionScript`
  (`parent.UserConstructionScript`))