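; Base weapon projectile that deals hit damage, optional radial explosion damage and knockback, then destroys itself after a delay.
; Sphere hits and player overlaps share one handler, with a brief owner grace period on overlaps.
; Authority-only damage handles head-hitbox crits, per-actor deduplication, sphere-trace AoE with debug drawing, and physics impulses.
; Impacts play hard or body FX and sounds once and report AI noise; optional speed scaling adjusts velocity and gravity.
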(event `SurfaceImpactEvent`
  (params (HitResult :type "HitResult Structure") (`Hardsurface?` :type Boolean) (hitactor :type "Actor Object Reference"))
  (`self.onProjectileHit`)
  (`self.PlayImpactEffects` HitResult `Hardsurface?`)
  (`KismetSystemLibrary.Delay` (`self.DestroyDelayAfterImpact`))
  (`self.K2_DestroyActor`))

(event `Radial Damage`
  (params (Origin :type "Vector Structure (by ref)"))
  (bind _damagedactors_aoe (`self.DamagedActors_AoE`))
  (bind _damageradius (`self.DamageRadius`))
  (if (`self.explode on impact?`)
    (bind (_outhits _returnvalue) (`KismetSystemLibrary.SphereTraceMulti` Origin (+ Origin 0.1) _damageradius "TraceTypeQuery1"))
    (for _array_element _outhits
      (bind (_bblockinghit _binitialoverlap _time _distance _location _impactpoint _normal _impactnormal _physmat _hitactor) (`GameplayStatics.BreakHitResult` _array_element))
      (if (not (`KismetArrayLibrary.Array_Contains` _damagedactors_aoe _hitactor))
        (`KismetArrayLibrary.Array_AddUnique` _damagedactors_aoe _hitactor)
        (`GameplayStatics.ApplyDamage` _hitactor (`self.radialDamageAmount`) (`self.Instigator Controller`) self (`self.AOEDamageType`))
        (`self.damagedThisActor` _hitactor)))
    (`KismetSystemLibrary.DrawDebugSphere` Origin _damageradius 12 (select `bool` _returnvalue :`false` (struct :`R` 1.0 :`B` 0.215297 :`A` 1.0) :`true` (struct :`G` 0.927083 :`B` 0.618317 :`A` 1.0) :!type "LinearColor Structure") 5.0 0.25)))

(event `Launch Multicast`
  (params (`Target Character` :type "Character Object Reference") (LaunchVelocity :type "Vector Structure") (bXYOverride :type Boolean) (bZOverride :type Boolean))
  (`Character.LaunchCharacter` `Target Character` LaunchVelocity bXYOverride bZOverride))

(event `self.ReceiveBeginPlay`
  ;[1 1 1] Only two that matter
  (`PrimitiveComponent.IgnoreActorWhenMoving` (`self.CollisionSphere`) (`self.GetOwner`) true)
  (set `self.Instigator Controller` (`self.GetInstigatorController`))
  (set `self.SpawnLocation` (`self.K2_GetActorLocation`))
  (if (`self.Override Speed`)
    (`self.Speed Scale`))
  (`KismetSystemLibrary.Delay` 0.5)
  (set `self.canhurtOwner` true))

(event `OnProjectileHitEvent`
  (params (OtherActor :type "Actor Object Reference") (OtherComponent :type "PrimitiveComponent Object Reference") (HitResult :type "HitResult Structure (by ref)") (fromHit :type Boolean))
  (`self.Damage Testing SERVER ONLY` HitResult OtherComponent OtherActor)
  (`self.SurfaceImpactEvent` HitResult (not (`KismetMathLibrary.ClassIsChildOf` (`GameplayStatics.GetObjectClass` OtherActor) "/Script/Engine.Character")) OtherActor))

(event `self.CollisionSphere.OnComponentBeginOverlap`
  (params (OverlappedComponent :type "PrimitiveComponent Object Reference") (OtherActor :type "Actor Object Reference") (OtherComp :type "PrimitiveComponent Object Reference") (OtherBodyIndex :type Integer) (bFromSweep :type Boolean) (SweepResult :type "HitResult Structure (by ref)"))
  ;[1 1 1] Only two that matter
  (bind _asbp_player_character (cast `/Game/Fadeout_Content/Core/Characters/BP_PlayerCharacter` OtherActor))
  (if (== (`self.GetOwner`) _asbp_player_character)
    (if (`self.canhurtOwner`)
      (`self.OnProjectileHitEvent` OtherActor OtherComp SweepResult :!label _label))
    (else
      (goto _label))))

(event `self.CollisionSphere.OnComponentHit`
  (params (HitComponent :type "PrimitiveComponent Object Reference") (OtherActor :type "Actor Object Reference") (OtherComp :type "PrimitiveComponent Object Reference") (NormalImpulse :type "Vector Structure") (Hit :type "HitResult Structure (by ref)"))
  ;[1 1 1] Only two that matter
  (`self.OnProjectileHitEvent` OtherActor OtherComp Hit true))

(event `Damage Testing SERVER ONLY`
  (params (Hit :type "HitResult Structure (by ref)") (`other Component` :type "PrimitiveComponent Object Reference") (`other actor` :type "Actor Object Reference"))
  (bind (_bblockinghit _binitialoverlap _time _distance _location _impactpoint _normal _impactnormal _physmat _hitactor) (`GameplayStatics.BreakHitResult` Hit))
  (bind _instigator_controller (`self.Instigator Controller`))
  (bind _postmoddamage (`self.postModDamage`))
  (bind _returnvalue (> (`self.critMultiplier`) 1.0))
  (bind _returnvalue_2 (`KismetMathLibrary.GetDirectionUnitVector` (`self.K2_GetActorLocation` self) (`self.K2_GetActorLocation` `other actor`)))
  (`/Engine/EditorBlueprintResources/ActorMacros.Switch Has Authority`
    (:`Authority`
      (if (not (`KismetArrayLibrary.Array_Contains` (`self.DamagedActors`) `other actor`))
        (`KismetArrayLibrary.Array_AddUnique` (`self.DamagedActors`) `other actor`)
        (`self.Radial Damage` (+ _location (* _impactnormal 5.0)))
        (bind _ashit_box_capsule (cast `HitBoxCapsule` `other Component`)
          (:`then`
            ;[1 1 1] Can we even headshot
            (if _returnvalue
              (bind _returnvalue_3 (`KismetStringLibrary.Contains` (`HitBoxCapsule.HitBoxName` _ashit_box_capsule) "head"))
              (if _returnvalue_3
                (set `self.postModDamage` (* (`self.BaseDamage`) (`self.critMultiplier`)))
                (else
                  (set `self.postModDamage` (`self.BaseDamage`) :!label _label_2)))
              (else
                (goto _label_2))))
          (:`CastFailed`
            (goto _label_2)))
        (`GameplayStatics.ApplyDamage` _hitactor _postmoddamage _instigator_controller self (`self.DamageType`))
        (`self.damagedThisActor` _hitactor)
        (`AISense_Damage.ReportDamageEvent` _hitactor _instigator_controller _postmoddamage _location _impactpoint)
        (if (`KismetSystemLibrary.IsValid` _ashit_box_capsule)
          (if (and _returnvalue_3 _returnvalue)
            (bind _asbp_player_character (cast `/Game/Fadeout_Content/Core/Characters/BP_PlayerCharacter` _hitactor))
            (set `/Game/Fadeout_Content/Core/Characters/BP_PlayerCharacter.headShotted` true _asbp_player_character)))
        (`|ExecutionSequence`
          (:`then_0`
            (bind _asbp_player_character_2 (cast `/Game/Fadeout_Content/Core/Characters/BP_PlayerCharacter` _hitactor))
            (if (`Actor.bCanBeDamaged` _asbp_player_character_2)
              (`self.Launch Multicast` _asbp_player_character_2 (* _returnvalue_2 (`self.KnockbackPower`)))))
          (:`then_1`
            (bind _asstatic_mesh_component (cast `StaticMeshComponent` `other Component`))
            (if (`SceneComponent.IsSimulatingPhysics` _asstatic_mesh_component "None")
              (`PrimitiveComponent.AddImpulse` _asstatic_mesh_component (* _returnvalue_2 200.0) "None" true))))))))

(fn `Distance Damage Scale`
  (params (`Minimum Damage` :type "Float (double-precision)" :default 25.0) (`Max Damage` :type "Float (double-precision)" :default 60.0) (`Ideal Distance` :type "Float (double-precision)" :default 4000.0))
  (returns (`New Damage` :type "Float (double-precision)"))
  (return (`KismetMathLibrary.Lerp` `Minimum Damage` `Max Damage` (`KismetMathLibrary.FClamp` (/ (`KismetMathLibrary.Vector_Distance` (`self.SpawnLocation`) (`self.K2_GetActorLocation`)) `Ideal Distance`)))))

(fn `Play Bullet hit SFX`
  (params (Location :type "Vector Structure") (hardSurfaceHit :type Boolean))
  (bind _hardhitsounds (`self.HardhitSounds`))
  (bind _softhitsounds (`self.SofthitSounds`))
  (if hardSurfaceHit
    (`GameplayStatics.PlaySoundAtLocation` (`|GetArrayItem` _hardhitsounds (`KismetMathLibrary.RandomIntegerInRange` 0 (- (`KismetArrayLibrary.Array_Length` _hardhitsounds) 1))) Location (struct) 0.5 (`KismetMathLibrary.RandomFloatInRange` 0.9 1.1) 0.0 "/Game/Fadeout_Content/Core/Characters/BulletHit_Attenuation.BulletHit_Attenuation" "/Game/Fadeout_Content/Core/Characters/BulletHitConcurrency.BulletHitConcurrency" self)
    (`AISense_Hearing.ReportNoiseEvent` Location 1.0 (`self.GetInstigator`) 1000.0)
    (else
      (`GameplayStatics.PlaySoundAtLocation` (`|GetArrayItem` _softhitsounds (`KismetMathLibrary.RandomIntegerInRange` 0 (- (`KismetArrayLibrary.Array_Length` _softhitsounds) 1))) (0.0 0.0 0.0) (struct) 0.5 (`KismetMathLibrary.RandomFloatInRange` 0.9 1.1) 0.0 "/Game/Fadeout_Content/Core/Characters/BulletHit_Attenuation.BulletHit_Attenuation" "/Game/Fadeout_Content/Core/Characters/BulletHitConcurrency.BulletHitConcurrency" self)
      (`AISense_Hearing.ReportNoiseEvent` (0.0 0.0 0.0) 1.0 (`self.GetInstigator`) 1000.0))))

(fn `PlayImpactEffects`
  (params (HitResult :type "HitResult Structure") (`Hardsurface?` :type Boolean))
  (bind (_bblockinghit _binitialoverlap _time _distance _location _impactpoint _normal _impactnormal _physmat _hitactor _hitcomponent) (`GameplayStatics.BreakHitResult` HitResult))
  (bind _hardsurfacefxscale (`self.hardSurfaceFXScale`))
  (if (`self.alreadyPlayedImpactEffect`)
    (return)
    (else
      (set `self.alreadyPlayedImpactEffect` true)
      (if `Hardsurface?`
        (`GameplayStatics.SpawnEmitterAtLocation` (`self.HardSurface_ImpactEmitter`) _location (`KismetMathLibrary.MakeRotFromZ` _normal) _hardsurfacefxscale)
        (`self.Play Bullet hit SFX` _location `Hardsurface?`)
        (else
          (`GameplayStatics.SpawnEmitterAtLocation` (`self.Body_ImpactEmitter`) _location (`KismetMathLibrary.MakeRotFromZ` _normal) _hardsurfacefxscale)
          (`self.Play Bullet hit SFX` _location `Hardsurface?`)))
      (`/Engine/EditorBlueprintResources/StandardMacros.IsValid` _hitcomponent
        (:`Is Valid`
          (`PrimitiveComponent.AddRadialImpulse` _hitcomponent _location 50.0 4000.0 "RIF_Constant" false)
          (return))
        (:`Is Not Valid`
          (return))))))

(fn `Speed Scale`
  (bind _new_speed (`self.New Speed`))
  (bind _projectilemovement (`self.ProjectileMovement`))
  (set `ProjectileMovementComponent.ProjectileGravityScale` (/ (`ProjectileMovementComponent.ProjectileGravityScale` _projectilemovement) _new_speed) _projectilemovement)
  (`ProjectileMovementComponent.SetVelocityInLocalSpace` _projectilemovement (`KismetMathLibrary.MakeVector` (* _new_speed (`ProjectileMovementComponent.InitialSpeed` _projectilemovement))))
  (return))

(fn `UserConstructionScript`)