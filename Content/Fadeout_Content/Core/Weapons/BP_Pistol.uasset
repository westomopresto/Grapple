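; Pistol weapon Blueprint for the player character that fires projectiles only while aiming down sights.
; Alt fire toggles the aim camera, blocks tool swapping and arms firing when alt fire is allowed.
; Firing checks ammo, then spawns the projectile, plays animations and applies a short cooldown; no ammo or no aim plays an empty-clip sound.
; BeginPlay and dropping select an on-ground or in-hand physics asset.
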(event `self.OnAltFire`
  (params (`MoveCamera?` :type Boolean))
  (set `self.ADS` true)
  (if (`self.canAltFire?`)
    (set `self.CanFire?` true)
    (bind _asbp_player_character (cast `/Game/Fadeout_Content/Core/Characters/BP_PlayerCharacter` (`self.GetInstigator`)))
    (set `/Game/Fadeout_Content/Core/Characters/BP_PlayerCharacter.canSwapTools?` false _asbp_player_character)
    (`/Game/Fadeout_Content/Core/Characters/BP_PlayerCharacter.toAimCam` _asbp_player_character true true (`self.YawAimRighty?`))))

(event `self.AltFireRelease`
  (set `self.ADS` false)
  (if (`self.canAltFire?`)
    (set `self.CanFire?` false)
    (bind _asbp_player_character (cast `/Game/Fadeout_Content/Core/Characters/BP_PlayerCharacter` (`self.GetInstigator`)))
    (set `/Game/Fadeout_Content/Core/Characters/BP_PlayerCharacter.canSwapTools?` true _asbp_player_character)
    (`/Game/Fadeout_Content/Core/Characters/BP_PlayerCharacter.toRearCam` _asbp_player_character)))

(event `self.OnFire`
  (bind _asbp_player_character (cast `/Game/Fadeout_Content/Core/Characters/BP_PlayerCharacter` (`self.GetInstigator`)))
  (if (`/Game/Fadeout_Content/Core/Characters/BP_PlayerCharacter.weapon_ADS` _asbp_player_character)
    (if (`self.CanFire?`)
      (bind _firecostmet (`self.WeaponAmmoEvent`))
      (if _firecostmet
        (`self.FireProjectileEvent` true)
        (`self.Fire Animation Event` "/Game/Fadeout_Content/Core/FBX/Luger/luger_01_fire.luger_01_fire")
        (bind _asbp_player_character_2 (cast `/Game/Fadeout_Content/Core/Characters/BP_PlayerCharacter` (`self.GetInstigator`)))
        (`/Game/Fadeout_Content/Core/Characters/BP_PlayerCharacter.updateWeaponDetails` _asbp_player_character_2)
        (`KismetSystemLibrary.Delay` 0.05)
        (`Character.PlayAnimMontage` _asbp_player_character_2 "/Game/Fadeout_Content/Core/Characters/Kasparian_BP/Pistol/Pistol_Attack.Pistol_Attack" 1.0 "attack")
        (set `self.CanFire?` false)
        (`KismetSystemLibrary.Delay` 0.25)
        (set `self.CanFire?` true)
        (else
          (`GameplayStatics.PlaySound2D` "/Game/Fadeout_Content/Core/Audio/residue-sfx/emptyclip.emptyclip" 1.0 1.0 0.0 null null :!label _label))))
    (else
      (goto _label))))

(event `self.ReceiveBeginPlay`
  (bind _skeletalmesh (`self.SkeletalMesh`))
  (bind _skeletalmesh_2 (`self.SkeletalMesh`))
  (`parent.ReceiveBeginPlay`)
  (set `self.CanFire?` false)
  (bind _asbp_player_character (cast `/Game/Fadeout_Content/Core/Characters/BP_PlayerCharacter` (`self.GetInstigator`))
    (:`then`
      (set `self.playerCamera` (`/Game/Fadeout_Content/Core/Characters/BP_PlayerCharacter.TPCamera` _asbp_player_character))
      ;[1 1 1] Obtaining the pistol at spawn
      (if (`self.onGround?`)
        (`SkinnedMeshComponent.SetPhysicsAsset` _skeletalmesh "/Game/Fadeout_Content/Core/FBX/Luger/pistol_onGround.pistol_onGround" false)
        (else
          (`SkinnedMeshComponent.SetPhysicsAsset` _skeletalmesh "/Game/Fadeout_Content/Core/FBX/Luger/pistol_inHand.pistol_inHand" false))))
    (:`CastFailed`
      (if (`self.onGround?`)
        (`SkinnedMeshComponent.SetPhysicsAsset` _skeletalmesh_2 "/Game/Fadeout_Content/Core/FBX/Luger/pistol_onGround.pistol_onGround" false)
        (else
          (`SkinnedMeshComponent.SetPhysicsAsset` _skeletalmesh_2 "/Game/Fadeout_Content/Core/FBX/Luger/pistol_inHand.pistol_inHand" false))))))

(event `self.ReceiveTick`
  (params (DeltaSeconds :type "Float (single-precision)")))

(event `self.OnDropped`
  (bind _skeletalmesh (`self.SkeletalMesh`))
  ;[1 1 1] Dropping the pistol
  (`parent.OnDropped`)
  (if (`self.onGround?`)
    (`SkinnedMeshComponent.SetPhysicsAsset` _skeletalmesh "/Game/Fadeout_Content/Core/FBX/Luger/pistol_onGround.pistol_onGround" false)
    (else
      (`SkinnedMeshComponent.SetPhysicsAsset` _skeletalmesh "/Game/Fadeout_Content/Core/FBX/Luger/pistol_inHand.pistol_inHand" false))))

(fn `UserConstructionScript`
  (`parent.UserConstructionScript`))