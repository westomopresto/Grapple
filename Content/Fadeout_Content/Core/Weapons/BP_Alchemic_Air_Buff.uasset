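; Alchemic air buff that grants a temporary movement speed boost to friendly players, built on a parent weakness-effect class.
; The apply and revert overrides call the parent, then on the server add or subtract the speed bonus on the player's clamped speed modifier.
; Both paths call Sprint on the player right after changing the modifier, including on revert.
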(event `self.Apply Weakness Event`
  (bind _player (`self.Player`))
  (`parent.Apply Weakness Event`)
  (`/Engine/EditorBlueprintResources/ActorMacros.Switch Has Authority`
    (:`Authority`
      (`self.Player`
        (:`then`
          (if (`self.OnFriendly`)
            (set `/Game/Fadeout_Content/Core/Characters/BP_PlayerCharacter.SpeedMod` (`KismetMathLibrary.FClamp` (+ (`/Game/Fadeout_Content/Core/Characters/BP_PlayerCharacter.SpeedMod` _player) (`self.SpeedBuff_ToGive`)) 1.0 2.0) _player)
            (`/Game/Fadeout_Content/Core/Characters/BP_PlayerCharacter.Sprint` _player true)))
        (:`else`)))))

(event `self.Revert Weakness`
  (bind _player (`self.Player`))
  (`parent.Revert Weakness`)
  (`/Engine/EditorBlueprintResources/ActorMacros.Switch Has Authority`
    (:`Authority`
      (`self.Player`
        (:`then`
          (if (`self.OnFriendly`)
            (set `/Game/Fadeout_Content/Core/Characters/BP_PlayerCharacter.SpeedMod` (`KismetMathLibrary.FClamp` (- (`/Game/Fadeout_Content/Core/Characters/BP_PlayerCharacter.SpeedMod` _player) (`self.SpeedBuff_ToGive`)) 1.0 2.0) _player)
            (`/Game/Fadeout_Content/Core/Characters/BP_PlayerCharacter.Sprint` _player true)))
        (:`else`)))))

(fn `UserConstructionScript`
  (`parent.UserConstructionScript`))