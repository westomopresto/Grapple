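; Projectile gun weapon that fires either hitscan shots or spawned projectiles, depending on RaycastDamageFire.
; Aim traces from the owning player's third-person camera, then orients the shot from the muzzle socket toward that point.
; Hitscan sphere-traces to the target, spawns a dummy projectile and impact effect, and doubles damage on "head" HitBoxCapsules.
; Projectile shots pass through SpawnProjectileServer to SpawnProjectileMulticast, which spawns ProjectileToFire.
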(event `Raycast Damage`
  (params (InTransform :type "Transform Structure (by ref)") (DamagedActor :type "Actor Object Reference") (hitLocation :type "Vector Structure") (hitNormal :type "Vector Structure"))
  (bind _returnvalue (`self.GetInstigatorController` (`self.GetOwner`)))
  (bind _outhit (`KismetSystemLibrary.SphereTraceSingle` (.location InTransform) hitLocation 15.0 "TraceTypeQuery1" false (`|MakeArray` (`self.GetOwner`)) "None" true (struct :`R` 1.0 :`B` 0.792414 :`A` 1.0)))
  (`self.spawnDummy` InTransform)
  (bind (_bblockinghit _binitialoverlap _time _distance _location _impactpoint _normal _impactnormal _physmat _hitactor _hitcomponent) (`GameplayStatics.BreakHitResult` _outhit))
  (`self.SpawnEffectHit` _impactpoint _impactnormal)
  (`/Engine/EditorBlueprintResources/StandardMacros.IsValid` DamagedActor
    (:`Is Valid`
      (bind _ashit_box_capsule (cast `HitBoxCapsule` _hitcomponent)
        (:`then`
          (if (`KismetStringLibrary.Contains` (`HitBoxCapsule.HitBoxName` _ashit_box_capsule) "head")
            (set `self.postModDamage` (* (`self.rayCastDamage`) 2.0))
            (bind _asbp_player_character (cast `/Game/Fadeout_Content/Core/Characters/BP_PlayerCharacter` DamagedActor))
            (set `/Game/Fadeout_Content/Core/Characters/BP_PlayerCharacter.headShotted` true _asbp_player_character)
            (else
              (set `self.postModDamage` (`self.rayCastDamage`) :!label _label))))
        (:`CastFailed`
          (goto _label)))
      (bind _returnvalue_2 (`GameplayStatics.ApplyDamage` DamagedActor (`self.postModDamage`) _returnvalue self (`self.Damage Type`)))
      (`KismetSystemLibrary.PrintString` (`KismetStringLibrary.Concat_StrStr` "Ray Damage for: " (`KismetStringLibrary.Conv_DoubleToString` _returnvalue_2) "by: " (`KismetSystemLibrary.GetDisplayName` _returnvalue)) true true (struct :`R` 1.0 :`B` 0.921747 :`A` 1.0) 5.0))))

(event `spawnDummy`
  (params (SpawnTransform :type "Transform Structure"))
  (`|SpawnActorFromClass` (`self.raycastDummyProjectile`) SpawnTransform "AlwaysSpawn" "OverrideRootScale" null null))

(event `SpawnEffectHit`
  (params (Location :type "Vector Structure") (Normal :type "Vector Structure"))
  (`GameplayStatics.SpawnEmitterAtLocation` "/Game/Fadeout_Content/Core/FX/particle_fireCone.particle_fireCone" Location (`KismetMathLibrary.MakeRotFromZ` Normal)))

(event `Spawn Projectile Multicast`
  (params (SpawnTransform :type "Transform Structure") (OwningWeapon :type "/Game/Fadeout_Content/Core/Weapons/BP_weaponBase Object Reference"))
  ;[1 1 1] Normal Pattern
  (`self.Shoot Projectile` SpawnTransform OwningWeapon))

(event `Spawn Projectile`
  (params (SpawnTransform :type "Transform Structure") (OwningWeapon :type "/Game/Fadeout_Content/Core/Weapons/BP_weaponBase Object Reference"))
  (bind _shot_projectile (`self.Shoot Projectile` SpawnTransform OwningWeapon))
  (`PrimitiveComponent.IgnoreActorWhenMoving` (`/Game/Fadeout_Content/Core/Weapons/BP_ProjectileBase.CollisionSphere` _shot_projectile) (`Controller.K2_GetPawn` (`GameplayStatics.GetPlayerController` 0)) false)
  (set `self.LastProjectile` _shot_projectile)
  (set `self.CanFire?` true)
  (`self.UpdateInstigatorWeaponInfo`))

(event `Spawn Projectile Server`
  (params (SpawnTransform :type "Transform Structure") (OwningWeapon :type "/Game/Fadeout_Content/Core/Weapons/BP_weaponBase Object Reference"))
  ;[1 1 1] Normal Pattern
  (`self.Spawn Projectile Multicast` SpawnTransform OwningWeapon))

(event `Spawn Projectile SERVER_ONLY`
  (params (ShootTransform :type "Transform Structure") (OwningWeapon :type "/Game/Fadeout_Content/Core/Weapons/BP_weaponBase Object Reference"))
  (`self.Spawn Projectile` ShootTransform OwningWeapon))

(event `Fire Projectile Event`
  ;[1 1 1] Gets shoot transform locally
  (bind (_shootfromtransform _hitactor _hitlocation _impactnormal) (`self.Calculate Projectile Position` (`self.RaycastAim`)))
  (if (`self.raycastDamageFire`)
    (`self.Raycast Damage` _shootfromtransform _hitactor _hitlocation _impactnormal)
    (else
      (`self.Spawn Projectile Server` _shootfromtransform self))))

(event `Last Projectile Notify`)

(fn `Calculate Projectile Position`
  (params (raycastAim :type Boolean))
  (returns (ShootFromTransform :type "Transform Structure") (HitActor :type "Actor Object Reference") (hitLocation :type "Vector Structure") (ImpactNormal :type "Vector Structure"))
  (locals (ProjectileClass :type "/Game/Fadeout_Content/Core/Weapons/BP_ProjectileBase Class Reference"))
  (bind _traceloc (`self.traceLoc`))
  (bind _returnvalue (`SceneComponent.GetSocketLocation` (`self.SkeletalMesh`) (`self.MuzzleSocket`)))
  (bind (_locationvec _directionvec) (`self.getInstigatorCameraFVector`))
  (if raycastAim
    (bind (_outhit _returnvalue_2) (`KismetSystemLibrary.LineTraceSingle` (+ _locationvec (* _directionvec 300.0)) (+ _locationvec (* _directionvec (`self.vectorTraceDistance`))) "TraceTypeQuery1" false (`|MakeArray` (`self.GetOwner`)) "None" true (struct :`R` 1.0 :`G` 0.685576 :`A` 1.0) (struct :`G` 1.0 :`B` 0.065537 :`A` 1.0) 3.0))
    (if _returnvalue_2
      (bind (_bblockinghit _binitialoverlap _time _distance _location _impactpoint _normal _impactnormal _physmat _hitactor) (`GameplayStatics.BreakHitResult` _outhit))
      (bind _output_get (set `self.traceLoc` _impactpoint))
      (bind _output_get_2 (set `self.hitActor` _hitactor))
      (else
        (set `self.traceLoc` (+ _locationvec (* _directionvec 5000.0)) :!label _label)))
    (else
      (goto _label)))
  (return (`KismetMathLibrary.MakeTransform` (+ _returnvalue (* (`KismetMathLibrary.GetDirectionUnitVector` _returnvalue _traceloc) 10.0)) (`KismetMathLibrary.FindLookAtRotation` _returnvalue _traceloc)) _output_get_2 _output_get _impactnormal))

(fn `getInstigatorCameraFVector`
  (returns (LocationVec :type "Vector Structure") (DirectionVec :type "Vector Structure"))
  (bind _asbp_player_character (cast `/Game/Fadeout_Content/Core/Characters/BP_PlayerCharacter` (`self.GetOwner`)))
  (`/Engine/EditorBlueprintResources/StandardMacros.IsValid` _asbp_player_character
    (:`Is Valid`
      (bind _tpcamera (`/Game/Fadeout_Content/Core/Characters/BP_PlayerCharacter.TPCamera` _asbp_player_character))
      (return (`SceneComponent.K2_GetComponentLocation` _tpcamera) (`SceneComponent.GetForwardVector` _tpcamera)))))

(fn `OnRep_LastProjectile`
  (`self.Last Projectile Notify`))

(fn `playCharAttackAnim`
  (bind _asbp_player_character (cast `/Game/Fadeout_Content/Core/Characters/BP_PlayerCharacter` (`self.GetOwner`)))
  (`/Game/Fadeout_Content/Core/Characters/BP_PlayerCharacter.PlayGunAttackAnim` _asbp_player_character (`self.Inventory_Icon`)))

(fn `Shoot Projectile`
  (params (SpawnTransform :type "Transform Structure") (OwningWeapon :type "/Game/Fadeout_Content/Core/Weapons/BP_weaponBase Object Reference"))
  (returns (`Shot Projectile` :type "/Game/Fadeout_Content/Core/Weapons/BP_ProjectileBase Object Reference"))
  (bind _returnvalue (`|SpawnActorFromClass` (`self.ProjectileToFire`) SpawnTransform "Undefined" "OverrideRootScale" (`self.GetOwner`) OwningWeapon (`self.GetInstigator`)))
  (return _returnvalue))

(fn `UserConstructionScript`
  (`parent.UserConstructionScript`))