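; BP_Turret_Throw_Projectile is a thrown projectile that carries a turret and releases it on impact.
; On BeginPlay it spawns the turret at its collision sphere, passing on its own Instigator, and attaches it to itself.
; A hit on any actor other than itself or the turret detaches the turret in world space and destroys the projectile.
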(event `Attach Turret`
  (bind _returnvalue (`|SpawnActorFromClass` :`Class` "/Game/Fadeout_Content/Core/Characters/BP_Turret.BP_Turret_C" :`SpawnTransform` (`SceneComponent.K2_GetComponentToWorld` (`self.CollisionSphere`)) :`CollisionHandlingOverride` "AlwaysSpawn" :`TransformScaleMethod` "OverrideRootScale" :`Instigator` (`self.GetInstigator`)))
  (bind _output_get (set `self.Turret` _returnvalue))
  (`self.K2_AttachToActor` _output_get self "None" "KeepRelative" "KeepRelative" "KeepRelative" true))

(event `Detach Turret`
  (`self.K2_DetachFromActor` (`self.Turret`) "KeepWorld" "KeepWorld" "KeepWorld"))

(event `self.OnProjectileHitEvent`
  (params (OtherActor :type "Actor Object Reference") (OtherComponent :type "PrimitiveComponent Object Reference") (HitResult :type "HitResult Structure (by ref)"))
  (if (and (!= OtherActor self) (!= OtherActor (`self.Turret`)))
    (`self.Detach Turret`)
    (`self.K2_DestroyActor`)))

(event `self.ReceiveBeginPlay`
  (`parent.ReceiveBeginPlay`)
  (`self.Attach Turret`))

(fn `UserConstructionScript`
  (`parent.UserConstructionScript`))