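; Shotgun pellet projectile that bounces off surfaces and reports hits through a projectile hit event.
; It shuts off its trail, mesh and collision after four seconds or on the fourth surface impact, playing impact effects on each.
; Overlaps skip BP_ShotgunProjectile actors, and the owning player unless CanhurtOwner is set.
; Bounce-based damage and gravity scaling is present but disabled.
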(event `self.ReceiveBeginPlay`
  (`parent.ReceiveBeginPlay`)
  (`KismetSystemLibrary.Delay` 4.0)
  (`ActorComponent.Deactivate` (`self.trail`) :!label _label)
  (`SceneComponent.SetVisibility` (`self.Mesh`) false false)
  (`PrimitiveComponent.SetCollisionEnabled` (`self.CollisionSphere`) "NoCollision")
  (`KismetSystemLibrary.Delay` 1.0))

(event `self.SurfaceImpactEvent`
  (params (HitResult :type "HitResult Structure") (`Hardsurface?` :type Boolean) (hitactor :type "Actor Object Reference"))
  (`self.PlayImpactEffects` HitResult `Hardsurface?`)
  (`/Engine/EditorBlueprintResources/StandardMacros.IncrementInt` (`self.bounce counter`)
    (:`  `
      (if (>= (`self.bounce counter`) 4)
        (goto _label)))))

(event `self.CollisionSphere.OnComponentBeginOverlap`
  (params (OverlappedComponent :type "PrimitiveComponent Object Reference") (OtherActor :type "Actor Object Reference") (OtherComp :type "PrimitiveComponent Object Reference") (OtherBodyIndex :type Integer) (bFromSweep :type Boolean) (SweepResult :type "HitResult Structure (by ref)"))
  (bind _asbp_player_character (cast `/Game/Fadeout_Content/Core/Characters/BP_PlayerCharacter` OtherActor)
    (:`then`
      (if (== (`self.GetOwner`) _asbp_player_character)
        (if (`self.canhurtOwner`)
          (`self.OnProjectileHitEvent` OtherActor OtherComp SweepResult :!label _label_2))
        (else
          (goto _label_2))))
    (:`CastFailed`
      (cast `/Game/Fadeout_Content/Core/Weapons/BP_ShotgunProjectile` OtherActor
        (:`CastFailed`
          (`self.OnProjectileHitEvent` OtherActor OtherComp SweepResult))))))

(fn `UserConstructionScript`)