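; Networked physics ball that sticks to player characters it hits and drops off when the carrier takes damage.
; The server simulates physics and gives an upward impulse at start, while clients begin with simulation off.
; Server-detected hits call AttachMulticast, which attaches the ball, disables physics and binds the carrier's damage event to DetachMulticast, re-enabling physics.
; Point damage pushes the ball against the hit normal.
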(event `self.ReceiveBeginPlay`
  (bind _staticmesh (`self.StaticMesh`))
  (`/Engine/EditorBlueprintResources/ActorMacros.Switch Has Authority`
    (:`Authority`
      (`PrimitiveComponent.SetSimulatePhysics` _staticmesh true)
      (`PrimitiveComponent.AddImpulseAtLocation` (`self.StaticMesh`) (0.0 0.0 500.0) (`self.K2_GetActorLocation`) "None"))
    (:`Remote`
      (`PrimitiveComponent.SetSimulatePhysics` _staticmesh false))))

(event `AttachMulticast`
  (params (Object :type "Object Object Reference"))
  (bind _asbp_player_character (cast `/Game/Fadeout_Content/Core/Characters/BP_PlayerCharacter` Object))
  (`self.K2_AttachToActor` _asbp_player_character "None" "KeepWorld" "KeepWorld" "KeepWorld")
  (add `self.OnTakeAnyDamage` _asbp_player_character (delegate `DetachFromDamage`))
  (`PrimitiveComponent.SetSimulatePhysics` (`self.StaticMesh`) false))

(event `self.ReceivePointDamage`
  (params (Damage :type "Float (single-precision)") (DamageType :type "DamageType Object Reference") (HitLocation :type "Vector Structure") (HitNormal :type "Vector Structure") (HitComponent :type "PrimitiveComponent Object Reference") (BoneName :type Name) (ShotFromDirection :type "Vector Structure") (InstigatedBy :type "Controller Object Reference") (DamageCauser :type "Actor Object Reference") (HitInfo :type "HitResult Structure (by ref)"))
  (`PrimitiveComponent.AddImpulseAtLocation` (`self.StaticMesh`) (* HitNormal -200.0) HitLocation "None"))

(event `DetachFromDamage` :!signature `self.OnTakeAnyDamage`
  (params (DamagedActor :type "Actor Object Reference") (Damage :type "Float (double-precision)") (DamageType :type "DamageType Object Reference") (InstigatedBy :type "Controller Object Reference") (DamageCauser :type "Actor Object Reference"))
  (`self.DetachMulticast`))

(event `self.StaticMesh.OnComponentHit`
  (params (HitComponent :type "PrimitiveComponent Object Reference") (OtherActor :type "Actor Object Reference") (OtherComp :type "PrimitiveComponent Object Reference") (NormalImpulse :type "Vector Structure") (Hit :type "HitResult Structure (by ref)"))
  (`/Engine/EditorBlueprintResources/ActorMacros.Switch Has Authority`
    (:`Authority`
      (`self.AttachMulticast` OtherActor))))

(event `DetachMulticast`
  (`self.K2_DetachFromActor` "KeepWorld" "KeepWorld" "KeepWorld")
  (`PrimitiveComponent.SetSimulatePhysics` (`self.StaticMesh`) true))

(fn `UserConstructionScript`)