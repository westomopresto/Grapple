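; Global music actor that drives an audio component from the game mode's danger state and current area.
; Each tick it pushes the AreaID as the "area" parameter and checks DANGER for changes through a value-changed helper.
; A change sets the "combatswitch" parameter and restarts playback, while a timeline plays forward or in reverse, feeding the "combatfade" parameter.
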(event `self.ReceiveBeginPlay`
  (bind _asbp_game_mode (cast `/Game/Fadeout_Content/Core/GameModes/BP_GameMode` (`GameplayStatics.GetGameMode`)))
  (bind _output_get (set `self.danger?` (`/Game/Fadeout_Content/Core/GameModes/BP_GameMode.DANGER?` _asbp_game_mode)))
  (bind (_old_value _new_value) (`/Game/Fadeout_Content/Core/MacroLibrary.Value Changed` _output_get (`/Game/Fadeout_Content/Core/GameModes/BP_GameMode.DANGER?` (stale `self.ReceiveTick` _asbp_game_mode)) :!label _label)
    (:`Value changed`
      (if _new_value
        (`self.combatMusic`)
        (else
          (`self.normalMusic`))))))

(event `self.ReceiveTick`
  (params (DeltaSeconds :type "Float (single-precision)"))
  (bind _asbp_game_mode (cast `/Game/Fadeout_Content/Core/GameModes/BP_GameMode` (`GameplayStatics.GetGameMode`)))
  (`|ExecutionSequence`
    (:`then_0`
      (goto _label :!via `Check Change`))
    (:`then_1`
      (`self.areaSwitch` (`/Game/Fadeout_Content/Core/GameModes/BP_GameMode.areaID` _asbp_game_mode)))))

(event `areaSwitch`
  (params (areaID :type "Integer (by ref)"))
  (`AudioComponent.SetIntParameter` (`self.audio_component`) "area" areaID))

(event `combatMusic`
  (`self.start_combat`)
  (bind (_direction _fade) (`Timeline|combat` :!via `PlayFromStart` :!label _label_2)
    (:`Update`
      (`AudioComponent.SetFloatParameter` (`self.audio_component`) "combatfade" _fade))))

(event `normalMusic`
  (`self.end_combat`)
  (goto _label_2 :!via `ReverseFromEnd`))

(event `start_combat`
  (bind _audio_component (`self.audio_component`))
  (`AudioComponent.SetIntParameter` _audio_component "combatswitch" 0)
  (`AudioComponent.Play` _audio_component 0.0))

(event `end_combat`
  (bind _audio_component (`self.audio_component`))
  (`AudioComponent.SetIntParameter` _audio_component "combatswitch" 1)
  (`AudioComponent.Play` _audio_component 0.0))

(fn `UserConstructionScript`
  (`BillboardComponent.SetSprite` (`self.Billboard`) "/Engine/EditorResources/S_Pickup.S_Pickup"))