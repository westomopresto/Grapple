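; BP_Worker_Door is a door prop that opens and closes through Open and Close events, with an optional timed auto-close.
; Each event sets the Open flag on the door mesh's animation Blueprint, mirrors it into DoorOpen, and plays a matching metal-and-stone sound at the door's location.
; When TimedClose is set, opening starts a retriggerable delay that calls Close after Timer seconds.
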(event `Close`
  (bind _returnvalue (`self.K2_GetActorLocation`))
  (bind _asdoor_anim_bp (cast `/Game/Fadeout_Content/Core/FBX/worker_Door/door_animBP` (`SkeletalMeshComponent.GetAnimInstance` (`self.doorMesh`))))
  (bind _output_get (set `/Game/Fadeout_Content/Core/FBX/worker_Door/door_animBP.open?` false _asdoor_anim_bp))
  (set `self.doorOpen?` _output_get)
  (if (`self.doorOpen?`) :!label _label
    (`GameplayStatics.PlaySoundAtLocation` "/Game/Fadeout_Content/Core/Props/Doors/Rotating_Metal_and_Stone_Door_Open.Rotating_Metal_and_Stone_Door_Open" _returnvalue (struct) 1.0 1.0 0.0 "/Game/Fadeout_Content/Core/Props/Elevator_Attenuation.Elevator_Attenuation" "/Game/Fadeout_Content/Core/Characters/ExplosionConcurrency.ExplosionConcurrency" null)
    (if (`self.timedClose?`)
      (`KismetSystemLibrary.RetriggerableDelay` (`self.timer`))
      (`self.Close`))
    (else
      (`GameplayStatics.PlaySoundAtLocation` "/Game/Fadeout_Content/Core/Props/Doors/Rotating_Metal_and_Stone_Door_Close.Rotating_Metal_and_Stone_Door_Close" _returnvalue (struct) 1.0 1.0 0.0 "/Game/Fadeout_Content/Core/Props/Elevator_Attenuation.Elevator_Attenuation" "/Game/Fadeout_Content/Core/Characters/ExplosionConcurrency.ExplosionConcurrency" null))))

(event `Open`
  (bind _asdoor_anim_bp (cast `/Game/Fadeout_Content/Core/FBX/worker_Door/door_animBP` (`SkeletalMeshComponent.GetAnimInstance` (`self.doorMesh`))))
  (bind _output_get (set `/Game/Fadeout_Content/Core/FBX/worker_Door/door_animBP.open?` true _asdoor_anim_bp))
  (set `self.doorOpen?` _output_get)
  (goto _label))

(fn `UserConstructionScript`)