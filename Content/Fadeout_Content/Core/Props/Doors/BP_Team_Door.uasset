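; BP_Team_Door is a child door Blueprint that opens only for players on its team, or for everyone when set to "ffa".
; On the server, Box overlaps call the team check, then Open on entry or Close on exit.
; A looping one-second timer re-opens the door while an eligible player remains inside.
; TeamCheck compares the player state's team and passes anything that fails its casts, including non-player actors.
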(event `self.ReceiveBeginPlay`
  (`parent.ReceiveBeginPlay`)
  (set `SkeletalMeshComponent.GlobalAnimRateScale` 3.0 (`self.doorMesh`))
  (`/Engine/EditorBlueprintResources/ActorMacros.Switch Has Authority`
    (:`Authority`
      (`KismetSystemLibrary.K2_SetTimerDelegate` (delegate `DOORSTUCK`) 1.0 true))))

(event `DOORSTUCK`
  (bind _overlappingactors (`PrimitiveComponent.GetOverlappingActors` (`self.Box`) "/Game/Fadeout_Content/Core/Characters/BP_PlayerCharacter.BP_PlayerCharacter_C"))
  (if (> (`KismetArrayLibrary.Array_Length` _overlappingactors) 0)
    (for _array_element _overlappingactors
      (bind _allowed (`self.TeamCheck` _array_element))
      (if _allowed
        (`self.Open`)
        (break)))))

(event `self.Box.OnComponentBeginOverlap`
  (params (OverlappedComponent :type "PrimitiveComponent Object Reference") (OtherActor :type "Actor Object Reference") (OtherComp :type "PrimitiveComponent Object Reference") (OtherBodyIndex :type Integer) (bFromSweep :type Boolean) (SweepResult :type "HitResult Structure (by ref)"))
  (`/Engine/EditorBlueprintResources/ActorMacros.Switch Has Authority`
    (:`Authority`
      (bind _allowed (`self.TeamCheck` OtherActor))
      (if _allowed
        (`self.Open`)))))

(event `self.Box.OnComponentEndOverlap`
  (params (OverlappedComponent :type "PrimitiveComponent Object Reference") (OtherActor :type "Actor Object Reference") (OtherComp :type "PrimitiveComponent Object Reference") (OtherBodyIndex :type Integer))
  (`/Engine/EditorBlueprintResources/ActorMacros.Switch Has Authority`
    (:`Authority`
      (bind _allowed (`self.TeamCheck` OtherActor))
      (if _allowed
        (`self.Close`)))))

(fn `TeamCheck`
  (params (Object :type "Object Object Reference"))
  (returns (allowed :type Boolean))
  (bind _asbp_player_character (cast `/Game/Fadeout_Content/Core/Characters/BP_PlayerCharacter` Object)
    (:`then`
      (bind _asfo_player_state (cast `/Game/Fadeout_Content/Core/Support/Multiplayer_Support/FO_PlayerState` (`Pawn.PlayerState` _asbp_player_character))
        (:`then`
          (if (`KismetStringLibrary.EqualEqual_StrStr` (`self.team`) "ffa")
            (return true)
            (else
              (return (`KismetStringLibrary.EqualEqual_StrStr` (`/Game/Fadeout_Content/Core/Support/Multiplayer_Support/FO_PlayerState.Team` _asfo_player_state) (`self.team`))))))
        (:`CastFailed`
          (return true))))
    (:`CastFailed`
      (return true))))

(fn `UserConstructionScript`
  (`parent.UserConstructionScript`))