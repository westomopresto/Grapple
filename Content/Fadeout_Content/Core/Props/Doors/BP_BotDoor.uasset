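; BP_BotDoor is a simple door prop that appears or disappears instantly to block or clear a passage.
; Open and Close events set the DoorOpen flag and pass it to Toggle.
; Toggle hides the Cube and disables its collision when open, and shows it with query and physics collision when closed.
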(event `self.Open`
  (bind _output_get (set `self.doorOpen?` true))
  (`self.Toggle` _output_get))

(event `self.Close`
  (bind _output_get (set `self.doorOpen?` false))
  (`self.Toggle` _output_get))

(fn `Toggle`
  (params (Open :type Boolean))
  (bind _cube (`self.Cube`))
  (`SceneComponent.SetVisibility` _cube (not Open) false)
  (`PrimitiveComponent.SetCollisionEnabled` _cube (select `bool` Open :`false` "QueryAndPhysics" :`true` "NoCollision" :!type "ECollisionEnabled Enum")))

(fn `UserConstructionScript`
  (`parent.UserConstructionScript`))