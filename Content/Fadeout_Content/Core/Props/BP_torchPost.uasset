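; Torch post prop that starts unlit and catches flame when a lit lantern touches it.
; On BeginPlay it zeroes the Light intensity and hides the FlameParticle.
; When its Trigger overlaps a BP_Lantern_3 whose LanternOn is true, light_flame raises the light intensity and shows the flame.
; Nothing in this Blueprint extinguishes it again.
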(event `self.ReceiveBeginPlay`
  (`|ExecutionSequence`
    (:`then_0`
      (`LightComponent.SetIntensity` (`self.light`) 0.0))
    (:`then_1`
      (`SceneComponent.SetVisibility` (`self.flame particle`) false false))))

(event `light_flame`
  (`|ExecutionSequence`
    (:`then_0`
      (`LightComponent.SetIntensity` (`self.light`) 8.0))
    (:`then_1`
      (`SceneComponent.SetVisibility` (`self.flame particle`) true false))))

(event `self.trigger.OnComponentBeginOverlap`
  (params (OverlappedComponent :type "PrimitiveComponent Object Reference") (OtherActor :type "Actor Object Reference") (OtherComp :type "PrimitiveComponent Object Reference") (OtherBodyIndex :type Integer) (bFromSweep :type Boolean) (SweepResult :type "HitResult Structure (by ref)"))
  (bind _asbp_lantern_3 (cast `/Game/Fadeout_Content/Weapons/Lantern/BP_Lantern_3` OtherActor))
  (if (`/Game/Fadeout_Content/Weapons/Lantern/BP_Lantern_3.lanternOn?` _asbp_lantern_3)
    (`self.light_flame`)))

(fn `UserConstructionScript`)