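; BP_WorldPickup_Class is a world pickup prop with a physics-driven static mesh.
; On BeginPlay, a valid PuzzleWeight reference overrides the mesh mass with its Weight value.
; The noCollision event disables physics simulation and ignores all collision channels.
; The resetCollision event restores physics and blocks every channel except GameTraceChannel3, which stays ignored.
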(event `self.ReceiveBeginPlay`
  (bind _puzzleweight (`self.puzzleWeight`))
  (`/Engine/EditorBlueprintResources/StandardMacros.IsValid` _puzzleweight
    (:`Is Valid`
      (`PrimitiveComponent.SetMassOverrideInKg` (`self.StaticMeshComponent`) "None" (`KismetMathLibrary.Conv_IntToDouble` (`/Game/Fadeout_Content/Core/Props/puzzleWeight.Weight` _puzzleweight)) true))))

(event `resetCollision`
  (bind _staticmeshcomponent (`self.StaticMeshComponent`))
  (`PrimitiveComponent.SetCollisionResponseToAllChannels` _staticmeshcomponent "ECR_Block")
  (`PrimitiveComponent.SetCollisionResponseToChannel` _staticmeshcomponent "ECC_GameTraceChannel3" "ECR_Ignore")
  (`PrimitiveComponent.SetSimulatePhysics` (`self.StaticMeshComponent`) true))

(event `noCollision`
  (`PrimitiveComponent.SetCollisionResponseToAllChannels` (`self.StaticMeshComponent`) "ECR_Ignore")
  (`PrimitiveComponent.SetSimulatePhysics` (`self.StaticMeshComponent`) false))

(fn `UserConstructionScript`)