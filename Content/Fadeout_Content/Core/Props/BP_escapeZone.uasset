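; BP_escapeZone is an escape zone prop that registers allies reaching it as escaped.
; When a BP_Ally overlaps its collision component in a specific rescue state, it advances that ally's RescueState to another value.
; After a one-second delay, it calls UpdateEscapeCount on BP_GameMode through its updatePrisonerCount event.
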(event `updatePrisonerCount`
  (bind _asbp_game_mode (cast `/Game/Fadeout_Content/Core/GameModes/BP_GameMode` (`GameplayStatics.GetGameMode`)))
  (`/Game/Fadeout_Content/Core/GameModes/BP_GameMode.updateEscapeCount` _asbp_game_mode))

(event `self.CollisionComponent.OnComponentBeginOverlap`
  (params (OverlappedComponent :type "PrimitiveComponent Object Reference") (OtherActor :type "Actor Object Reference") (OtherComp :type "PrimitiveComponent Object Reference") (OtherBodyIndex :type Integer) (bFromSweep :type Boolean) (SweepResult :type "HitResult Structure (by ref)"))
  (bind _asbp_ally (cast `/Game/Fadeout_Content/Core/Characters/BP_Ally` OtherActor))
  (if (`|EnumEquality` (`/Game/Fadeout_Content/Core/Characters/BP_Ally.RescueState` _asbp_ally) "NewEnumerator4")
    (set `/Game/Fadeout_Content/Core/Characters/BP_Ally.RescueState` "NewEnumerator5" _asbp_ally)
    (`KismetSystemLibrary.Delay` 1.0)
    (`self.updatePrisonerCount`)))

(fn `UserConstructionScript`)