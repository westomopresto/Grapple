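; BP_Gate is a gate prop that slides between the first two points of its spline, playing a pitch-varied winch sound.
; BeginPlay detaches the spline and caches both world positions, which a timeline interpolates between.
; Push toggles direction through a FlipFlop when Pushable.
; With CloseOnDanger, Tick polls BP_GameMode's DANGER flag and, on change, plays the timeline forward for danger or reverses it otherwise.
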(event `self.ReceiveBeginPlay`
  (bind _spline (`self.Spline`))
  (`SceneComponent.K2_DetachFromComponent` _spline "KeepWorld" "KeepWorld" "KeepWorld" true)
  (set `self.startPoint` (`SplineComponent.GetLocationAtDistanceAlongSpline` _spline 0.0 "World"))
  (set `self.endPoint` (`SplineComponent.GetLocationAtDistanceAlongSpline` _spline (`SplineComponent.GetDistanceAlongSplineAtSplinePoint` _spline 1) "World"))
  (`self.initDanger`))

(event `Start`
  (`self.open sound`)
  (bind (_direction _alpha) (`Timeline|Timeline_0` :!label _label)
    (:`Update`
      (`self.K2_SetActorLocation` self (`KismetMathLibrary.VLerp` (`self.startPoint`) (`self.endPoint`) _alpha) false false))))

(event `Reverse`
  (`self.open sound`)
  (goto _label :!via `Reverse`))

(event `Push`
  (if (`self.pushable?`)
    (`/Engine/EditorBlueprintResources/StandardMacros.FlipFlop`
      (:`A`
        (`self.Start`))
      (:`B`
        (`self.Reverse`)))))

(event `self.ReceiveTick`
  (params (DeltaSeconds :type "Float (single-precision)"))
  (bind _in_danger_ (`self.In Danger?`))
  (if (`self.closeOnDanger?`)
    (bind _asbp_game_mode (cast `/Game/Fadeout_Content/Core/GameModes/BP_GameMode` (`GameplayStatics.GetGameMode`)))
    (set `self.In Danger?` (`/Game/Fadeout_Content/Core/GameModes/BP_GameMode.DANGER?` _asbp_game_mode))
    (goto _label_2 :!via `Check Change`)))

(event `initDanger`
  (bind _in_danger_ (`self.In Danger?`))
  (bind (_old_value _new_value) (`/Game/Fadeout_Content/Core/MacroLibrary.Value Changed` _in_danger_ _in_danger_ :!label _label_2)
    (:`Value changed`
      (if _new_value
        (`self.Start`)
        (else
          (`self.Reverse`))))))

(fn `open sound`
  (`GameplayStatics.PlaySoundAtLocation` "/Game/Fadeout_Content/Core/Audio/Chain_Winch/winch_-_Marker__7.winch_-_Marker__7" (`self.K2_GetActorLocation`) (struct) 0.5 (`KismetMathLibrary.RandomFloatInRange` 0.9 1.0) 1.0 "/Game/Fadeout_Content/Core/Props/Elevator_Attenuation.Elevator_Attenuation" null null))

(fn `UserConstructionScript`)