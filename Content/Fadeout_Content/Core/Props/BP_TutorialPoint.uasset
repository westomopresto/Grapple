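; Tutorial trigger actor that shows a text and texture popup on the player's combat UI when the player overlaps it, unless the game instance disables tutorials.
; Pausing popups show once, enable the mouse cursor and stop sprinting.
; Non-pausing popups hide on overlap end, repeating unless ShowOnce marks them seen.
; CustomCompletion marks the tutorial seen and hides it through the remembered player.
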(event `Custom Completion`
  (set `self.HasAlreadySeenThisTutorial` true)
  (`self.CompletionCheck`))

(event `CompletionCheck`
  (bind _asbp_player_character (cast `/Game/Fadeout_Content/Core/Characters/BP_PlayerCharacter` (`self.PlayerInMemory`)))
  (bind _aswbp_combat_base (cast `/Game/Fadeout_Content/Core/UI/WBP_CombatBase` (`/Game/Fadeout_Content/Core/Characters/BP_PlayerCharacter.inventoryUI` _asbp_player_character)))
  (if (`self.HasAlreadySeenThisTutorial`)
    (`/Game/Fadeout_Content/Core/UI/WBP_CombatBase.TutorialHide` _aswbp_combat_base false)))

(event `self.ReceiveActorEndOverlap`
  (params (OtherActor :type "Actor Object Reference"))
  (if (== (`GameplayStatics.GetObjectClass` OtherActor) "/Game/Fadeout_Content/Core/Characters/BP_PlayerCharacter.BP_PlayerCharacter_C")
    (if (not (`self.Pause Popup?`))
      (bind _asbp_player_character (cast `/Game/Fadeout_Content/Core/Characters/BP_PlayerCharacter` OtherActor))
      (bind _aswbp_combat_base (cast `/Game/Fadeout_Content/Core/UI/WBP_CombatBase` (`/Game/Fadeout_Content/Core/Characters/BP_PlayerCharacter.inventoryUI` _asbp_player_character)))
      (`/Game/Fadeout_Content/Core/UI/WBP_CombatBase.TutorialHide` _aswbp_combat_base false)
      (if (`self.show once?`)
        (set `self.HasAlreadySeenThisTutorial` true)))))

(event `self.ReceiveBeginPlay`)

(event `Get Tutorials Enabled?`
  (bind _asfadeout_game_instance (cast `/Game/Fadeout_GameInstance` (`GameplayStatics.GetGameInstance`)))
  (set `self.TutorialsDisabled` (`/Game/Fadeout_GameInstance.Disable Tutorials?` _asfadeout_game_instance)))

(event `self.ReceiveActorBeginOverlap`
  (params (OtherActor :type "Actor Object Reference"))
  (`self.Get Tutorials Enabled?`)
  (if (`self.TutorialsDisabled`)
    _
    (elif (== (`GameplayStatics.GetObjectClass` OtherActor) "/Game/Fadeout_Content/Core/Characters/BP_PlayerCharacter.BP_PlayerCharacter_C")
      (set `self.PlayerInMemory` OtherActor)
      (if (`self.Pause Popup?`)
        (if (not (`self.HasAlreadySeenThisTutorial`))
          (set `self.HasAlreadySeenThisTutorial` true)
          (`GameplayStatics.PlaySound2D` "/Game/Fadeout_Content/Core/Audio/residue-sfx/footsteps.footsteps" 1.0 1.0 0.0 null null)
          (bind _asbp_player_character (cast `/Game/Fadeout_Content/Core/Characters/BP_PlayerCharacter` OtherActor))
          (bind _aswbp_combat_base (cast `/Game/Fadeout_Content/Core/UI/WBP_CombatBase` (`/Game/Fadeout_Content/Core/Characters/BP_PlayerCharacter.inventoryUI` _asbp_player_character)))
          (`/Game/Fadeout_Content/Core/UI/WBP_CombatBase.TutorialPopUIp` _aswbp_combat_base (`KismetSystemLibrary.MakeLiteralText` (`self.Tutorial Text`)) true (`self.Blur Screen?`) (`self.Tutorial Texture`))
          (set `PlayerController.bShowMouseCursor` true (`GameplayStatics.GetPlayerController` (`/Game/Fadeout_Content/Core/Characters/BP_PlayerCharacter.PlayerInt` _asbp_player_character)))
          (`/Game/Fadeout_Content/Core/Characters/BP_PlayerCharacter.stopSprint` _asbp_player_character))
        (elif (not (`self.HasAlreadySeenThisTutorial`))
          (`GameplayStatics.PlaySound2D` "/Game/Fadeout_Content/Core/Audio/residue-sfx/footsteps.footsteps" 1.0 1.0 0.0 null null)
          (bind _asbp_player_character_2 (cast `/Game/Fadeout_Content/Core/Characters/BP_PlayerCharacter` OtherActor))
          (bind _aswbp_combat_base_2 (cast `/Game/Fadeout_Content/Core/UI/WBP_CombatBase` (`/Game/Fadeout_Content/Core/Characters/BP_PlayerCharacter.inventoryUI` _asbp_player_character_2)))
          (`/Game/Fadeout_Content/Core/UI/WBP_CombatBase.TutorialPopUIp` _aswbp_combat_base_2 (`KismetSystemLibrary.MakeLiteralText` (`self.Tutorial Text`)) false (`self.Blur Screen?`) (`self.Tutorial Texture`)))))))

(fn `UserConstructionScript`)