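; Bar bottle prop group that simulates physics on non-dedicated-server instances and periodically resets the bottles to their placed positions.
; The construction script caches child mesh transforms and sets their collision and decal settings.
; BeginPlay enables physics and starts a looping timer that freezes, teleports back and re-enables each mesh, skipping dedicated servers.
; A hit handler, with no binding shown, plays a high-pitched melee impact sound at the hit location.
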(event `RespawnTimer`
  (`self.Respawn Props`)
  (`KismetSystemLibrary.Delay` 0.1)
  (`self.SetPhys`))

(event `self.ReceiveBeginPlay`
  (if (not (`KismetSystemLibrary.IsDedicatedServer`))
    (`KismetSystemLibrary.K2_SetTimerDelegate` (delegate `RespawnTimer`) 60.0 true)
    (`self.SetPhys`)))

(event `WallHit_Event`
  (params (HitComponent :type "PrimitiveComponent Object Reference") (OtherActor :type "Actor Object Reference") (OtherComp :type "PrimitiveComponent Object Reference") (NormalImpulse :type "Vector Structure") (Hit :type "HitResult Structure (by ref)"))
  (`GameplayStatics.PlaySoundAtLocation` "/Game/Fadeout_Content/Core/Audio/Weapon_SFX/meleeHit_Sound.meleeHit_Sound" (`.Location` (`GameplayStatics.BreakHitResult` Hit)) (struct) 1.0 5.0 0.0 "/Game/Fadeout_Content/Core/Characters/BulletHit_Attenuation.BulletHit_Attenuation" "/Game/Fadeout_Content/Core/Characters/RagDoll_Hit_Concurrency.RagDoll_Hit_Concurrency" null))

(fn `Initialize`
  (bind _output_get (set `self.ourChildren` (`SceneComponent.GetChildrenComponents` (`self.Scene`) false)))
  (for (_array_element _array_index) _output_get
    (bind _asstatic_mesh_component (cast `StaticMeshComponent` _array_element))
    (`KismetArrayLibrary.Array_Set` (`self.childSpawns`) _array_index (`SceneComponent.K2_GetComponentToWorld` _asstatic_mesh_component) true)
    (`PrimitiveComponent.SetCollisionResponseToChannel` _asstatic_mesh_component "ECC_GameTraceChannel2" "ECR_Block")
    (`PrimitiveComponent.SetReceivesDecals` _asstatic_mesh_component false)
    (if (`KismetSystemLibrary.IsDedicatedServer`)
      (`PrimitiveComponent.SetSimulatePhysics` _asstatic_mesh_component false))))

(fn `Respawn Props`
  (for (_array_element _array_index) (`self.ourChildren`)
    (bind _asstatic_mesh_component (cast `StaticMeshComponent` _array_element))
    (`PrimitiveComponent.SetSimulatePhysics` _asstatic_mesh_component false)
    (`SceneComponent.K2_SetWorldTransform` _asstatic_mesh_component (`|GetArrayItem` (`self.childSpawns`) _array_index) false true))
  (return))

(fn `SetPhys`
  (for _array_element (`self.ourChildren`)
    (bind _asstatic_mesh_component (cast `StaticMeshComponent` _array_element))
    (`PrimitiveComponent.SetSimulatePhysics` _asstatic_mesh_component true))
  (return))

(fn `UserConstructionScript`
  (`self.Initialize`))