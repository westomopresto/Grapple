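; Interactable Wave Mode button that sells an action on its target actor, only proceeding when that target is a damaged BP_Tractor_Nexus.
; Its WaveModeBuySys component takes the configured cost at construction, and a widget displays that cost with flavor text.
; An action request from the signaling player attempts the purchase.
; Success sends a purchased-trigger message to the target, while failure shows that player a red "Not Enough Gold!" error.
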(event `Signal`
  (params (Player :type "/Game/Fadeout_Content/Core/Characters/BP_PlayerCharacter Object Reference"))
  (add `self.Action Requested` (delegate `Action Requested_Event`))
  (`parent.Signal` Player))

(event `self.ReceiveBeginPlay`
  (`parent.ReceiveBeginPlay`)
  (bind _aswm_cost_widget (cast `/Game/Fadeout_Content/Core/Support/Wave_Support/WM_CostWidget` (`WidgetComponent.GetUserWidgetObject` (`self.Widget`))))
  (set `/Game/Fadeout_Content/Core/Support/Wave_Support/WM_CostWidget.Cost` (`/Game/Fadeout_Content/Core/Support/Wave_Support/WaveMode_BuySys.CostOfThing` (`self.WaveMode_BuySys`)) _aswm_cost_widget)
  (set `/Game/Fadeout_Content/Core/Support/Wave_Support/WM_CostWidget.Flavor Text` (`self.FlavorText`) _aswm_cost_widget))

(event `Trigger Target`
  (params (NewParam :type "/Game/Fadeout_Content/Core/FO_PlayerController Object Reference"))
  (message `/Game/Fadeout_Content/Core/Support/Wave_Support/BPI_WaveModePurchases.PurchasedTrigger` (`self.Target Actor`)))

(event `Action Requested_Event` :!signature `self.Action Requested`
  (params (Player :type "/Game/Fadeout_Content/Core/Characters/BP_PlayerCharacter Object Reference"))
  (bind _wavemode_buysys (`self.WaveMode_BuySys`))
  (bind _asbp_tractor_nexus (cast `/Game/Fadeout_Content/Core/Support/Wave_Support/BP_Tractor_Nexus` (`self.Target Actor`)))
  (if (< (`/Game/Fadeout_Content/Core/Support/Wave_Support/BP_Tractor_Nexus.Health` _asbp_tractor_nexus) (`/Game/Fadeout_Content/Core/Support/Wave_Support/BP_Tractor_Nexus.MaxHealth` _asbp_tractor_nexus))
    (bind _asfo_player_controller (cast `/Game/Fadeout_Content/Core/FO_PlayerController` (`Pawn.GetController` Player)))
    (add `/Game/Fadeout_Content/Core/Support/Wave_Support/WaveMode_BuySys.PurchaseSuccess` _wavemode_buysys (delegate `Trigger Target`))
    (add `/Game/Fadeout_Content/Core/Support/Wave_Support/WaveMode_BuySys.PurchaseFail` _wavemode_buysys (delegate `ErrorPurchase`))
    (message `/Game/Fadeout_Content/Core/Support/Wave_Support/BPI_WaveModePurchases.AttemptPurchase` _wavemode_buysys _asfo_player_controller)))

(event `ErrorPurchase`
  (`/Game/Fadeout_Content/Core/FO_PlayerController.Error Message` (stale `Action Requested_Event` _asfo_player_controller) "Not Enough Gold!" (make `SlateColor` (struct :`R` 1.0 :`A` 1.0)) 3.0))

(fn `UserConstructionScript`
  (set `/Game/Fadeout_Content/Core/Support/Wave_Support/WaveMode_BuySys.CostOfThing` (`self.Cost`) (`self.WaveMode_BuySys`)))