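; BP_Billboard is a billboard prop with a configurable decal image and optional extra supports, built in the construction script.
; It applies the Texture variable to the decal through a dynamic material instance.
; With ExtraSupports on, a downward line trace estimates how many instanced meshes to stack below it, adjusted by ExtraLength.
; With ExtraSupports off, it destroys the instanced mesh component.
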(fn `UserConstructionScript`
  (bind _returnvalue (`self.K2_GetActorLocation`))
  (bind _instancedstaticmesh (`self.InstancedStaticMesh`))
  (bind _returnvalue_2 (`KismetMaterialLibrary.CreateDynamicMaterialInstance` (`DecalComponent.GetDecalMaterial` (`self.Decal`))))
  (`MaterialInstanceDynamic.SetTextureParameterValue` _returnvalue_2 "Texture" (`self.Texture`))
  (`DecalComponent.SetDecalMaterial` (`self.Decal`) _returnvalue_2)
  (if (`self.ExtraSupports`)
    (bind _outhit (`KismetSystemLibrary.LineTraceSingle` :`Start` _returnvalue :`End` (- _returnvalue (0.0 0.0 6000.0)) :`TraceChannel` "TraceTypeQuery1" :`bTraceComplex` true :`DrawDebugType` "ForOneFrame"))
    (`InstancedStaticMeshComponent.ClearInstances` _instancedstaticmesh)
    (for _index (range 1 (+ (+ (`KismetMathLibrary.FTrunc` (/ (`.Distance` (`GameplayStatics.BreakHitResult` _outhit)) 282.700012)) (`self.ExtraLength`)) 1))
      (`InstancedStaticMeshComponent.AddInstance` _instancedstaticmesh (`KismetMathLibrary.MakeTransform` (`KismetMathLibrary.MakeVector` 0.0 0.0 (* _index -223.0)))))
    (else
      (`ActorComponent.K2_DestroyComponent` (`self.InstancedStaticMesh`)))))