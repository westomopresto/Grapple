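; Conquest capture point that Red and Blue contest by standing in its zone, earning team score each second while held.
; On authority, timers box-trace for non-cloaked players, advance progress by the capped head-count difference, decay it otherwise, then switch control and credit capturers.
; Team color drives mesh vertex paint, hologram and rotating letter, while a material circle shows progress.
; A repeating game-state check shows the point only in Conquest.
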(event `Capture Progress`
  (params (Value :type "Float (double-precision)") (red :type Boolean) (blue :type Boolean))
  (bind _cappoint (`self.capPoint`))
  (bind _capture_m (`self.capture_m`))
  (`SceneComponent.SetVisibility` (`self.Plane`) (not (<= Value 0.0)) false)
  (if (or red blue)
    (`|ExecutionSequence`
      (:`then_0`
        (if (and (not (`self.red_captured`)) red)
          (`MaterialInstanceDynamic.SetVectorParameterValue` _capture_m "ProgressColor1" (`self.redColor`))
          (`MaterialInstanceDynamic.SetScalarParameterValue` _capture_m "Progress" Value)
          (`self.contested` true _cappoint)))
      (:`then_1`
        (if (and (not (`self.blue_captured`)) blue)
          (`MaterialInstanceDynamic.SetVectorParameterValue` _capture_m "ProgressColor1" (`self.blueColor`))
          (`MaterialInstanceDynamic.SetScalarParameterValue` _capture_m "Progress" Value)
          (`self.contested` true _cappoint))))
    (else
      (`MaterialInstanceDynamic.SetScalarParameterValue` _capture_m "Progress" Value)
      (`self.contested` false (`self.capPoint`)))))

(event `Enable Event`
  (params (Enable :type Boolean))
  ;[1 1 1] For the gamemode to hide/enable the point
  (`self.EnableToggle` Enable))

(event `self.ReceiveBeginPlay`
  (`|ExecutionSequence`
    (:`then_0`
      (`KismetSystemLibrary.K2_SetTimerDelegate` (delegate `Check Gamemode`) 2.0 true 2.0))
    (:`then_1`
      (`MovementComponent.SetUpdatedComponent` (`self.RotatingMovement`) (`self.letter`))
      (`/Engine/EditorBlueprintResources/ActorMacros.Switch Has Authority` :!label _label
        (:`Authority`
          (bind _returnvalue (`KismetSystemLibrary.K2_SetTimerDelegate` (delegate `Check for Overlap`) 1.0 true))
          (set `self.OVERLAP_TIMER` _returnvalue)
          (bind _returnvalue_2 (`KismetSystemLibrary.K2_SetTimerDelegate` (delegate `Award Tick`) 1.0 true 0.0 0.15))
          (set `self.AWARD_TIMER` _returnvalue_2)
          (`self.Change Color multi` (`self.ControllingTeam`)))))
    (:`then_2`
      (`KismetSystemLibrary.Delay` 3.0)
      (`self.teamChanged` (`self.capPoint`) (`self.ControllingTeam`) (`self.Capture Point Name`)))
    (:`then_3`
      (bind _returnvalue_3 (`PrimitiveComponent.CreateDynamicMaterialInstance` (`self.Plane`) 0 "/Game/RoboBars/Materials/M_Capture_Circle.M_Capture_Circle" "None"))
      (bind _output_get (set `self.capture_m` _returnvalue_3))
      (`MaterialInstanceDynamic.SetScalarParameterValue` _output_get "Progress" 1.0)
      (`MaterialInstanceDynamic.SetScalarParameterValue` _output_get "DivisionsCount" (`KismetMathLibrary.Conv_IntToDouble` (`self.TimeToCapture`))))))

(event `Start`
  (goto _label))

(event `Change Color multi`
  (params (Selection :type String))
  (bind _capture_m (`self.capture_m`))
  (set `self.red_captured` false)
  (set `self.blue_captured` false)
  (`self.Change Team Color` Selection)
  (`self.teamChanged` (`self.capPoint`) Selection (`self.Capture Point Name`))
  (switch `string` Selection
    (:`Default`
      (`/Engine/EditorBlueprintResources/StandardMacros.IsValid` _capture_m
        (:`Is Valid`
          (`MaterialInstanceDynamic.SetVectorParameterValue` _capture_m "ProgressColor1" (struct :`R` 1.0 :`G` 1.0 :`B` 1.0 :`A` 1.0)))))
    (:`red`
      (set `self.red_captured` true))
    (:`blue`
      (set `self.blue_captured` true))))

(event `Check Gamemode`
  ;[1 1 1] Check if conquest to enable or not
  (bind _asmultiplayer_game_state (cast `/Game/Fadeout_Content/Core/Support/Multiplayer_Support/Multiplayer_GameState` (`GameplayStatics.GetGameState`)))
  (`self.EnableToggle_client` (select `/Game/Fadeout_Content/Core/Support/Multiplayer_Support/DM_GameType` (`/Game/Fadeout_Content/Core/Support/Multiplayer_Support/Multiplayer_GameState.ModeType` _asmultiplayer_game_state) :`NewEnumerator3` true))
  (`self.Change Team Color` (`self.ControllingTeam`)))

(event `Check for Overlap`
  (bind _returnvalue (>= (`self.CaptureProgress`) (`self.TimeToCapture`)))
  (if (`self.enabled`)
    (bind _players1 (`self.TracePlayers`))
    (if (> (`KismetArrayLibrary.Array_Length` _players1) 0)
      (bind (_redcapturing _bluecapturing _playerstates _remainder) (`self.TeamControlCheck` _players1))
      (`|ExecutionSequence`
        (:`then_0`
          (if (or _redcapturing _bluecapturing)
            (bind _output_get (set `self.CaptureProgress` (+ (`self.CaptureProgress`) _remainder)))
            (`self.Capture Progress` (`KismetMathLibrary.FClamp` (* (`KismetMathLibrary.Conv_IntToDouble` _output_get) (/ 1.0 (`KismetMathLibrary.Conv_IntToDouble` (`self.TimeToCapture`))))) _redcapturing _bluecapturing)
            (else
              (`self.No one standing`))))
        (:`then_1`
          (if (and _redcapturing _returnvalue)
            (`self.AwardPlayerPointAndChangeControl` _playerstates "red")
            (set `self.CaptureProgress` 0)
            (`self.Capture Progress` 1.0)))
        (:`then_2`
          (if (and _bluecapturing _returnvalue)
            (`self.AwardPlayerPointAndChangeControl` _playerstates "blue")
            (set `self.CaptureProgress` 0)
            (`self.Capture Progress` 1.0))))
      (else
        (`self.No one standing`)))))

(event `Award Tick`
  ;[0 1 0.03815] AWARD TICK
  (`|ExecutionSequence`
    (:`then_0`
      (bind _asbp_multiplayer_gamemode (cast `/Game/Fadeout_Content/Core/GameModes/BP_MultiplayerGamemode` (`GameplayStatics.GetGameMode`)))
      (switch `string` (`self.ControllingTeam`)
        (:`red`
          (`/Game/Fadeout_Content/Core/GameModes/BP_MultiplayerGamemode.Add Teamscore` _asbp_multiplayer_gamemode 1 0))
        (:`blue`
          (`/Game/Fadeout_Content/Core/GameModes/BP_MultiplayerGamemode.Add Teamscore` _asbp_multiplayer_gamemode 0 1))))))

(event `All Player Announcement`
  (params (TEXT :type Text) (Color :type "SlateColor Structure"))
  ;[1 1 1] All player announce
  (bind _asbp_multiplayer_gamemode (cast `/Game/Fadeout_Content/Core/GameModes/BP_MultiplayerGamemode` (`GameplayStatics.GetGameMode`)))
  (for _array_element (`/Game/Fadeout_Content/Core/GameModes/BP_MultiplayerGamemode.ConnectedPlayers` _asbp_multiplayer_gamemode)
    (bind _asfo_player_controller (cast `/Game/Fadeout_Content/Core/FO_PlayerController` _array_element))
    (`/Game/Fadeout_Content/Core/FO_PlayerController.Error Message` _asfo_player_controller TEXT Color))
  (`/Game/Fadeout_Content/Core/Support/Multiplayer_Support/FO_Announcer.speak multi` (`/Game/Fadeout_Content/Core/GameModes/BP_MultiplayerGamemode.FO_Announcer` _asbp_multiplayer_gamemode) null null))

(fn `AwardPlayerPointAndChangeControl`
  (params (`player states` :type "Array of /Game/Fadeout_Content/Core/Support/Multiplayer_Support/FO_PlayerState Object Reference") (`team string` :type String))
  (if (`KismetStringLibrary.NotEqual_StrStr` (`self.ControllingTeam`) `team string`)
    (bind _output_get (set `self.ControllingTeam` `team string`))
    (for _array_element `player states`
      (`/Game/Fadeout_Content/Core/Support/Multiplayer_Support/FO_PlayerState.Add Capture` _array_element 1))
    (`self.Change Color multi` _output_get)
    (return)
    (else
      (return))))

(fn `Change Team Color`
  (params (Selection :type String))
  (bind _capturepointmesh (`self.CapturePointMesh`))
  (bind _letter_m (`self.letter_m`))
  (bind _hologram_m (`self.hologram_m`))
  (bind _chosencolor (`self.ChosenColor`))
  (switch `string` Selection
    (:`Default`
      (set `self.ChosenColor` (struct :`R` 1.0 :`G` 1.0 :`B` 1.0 :`A` 1.0) :!label _label))
    (:`red`
      (set `self.ChosenColor` (`self.redColor`)))
    (:`blue`
      (set `self.ChosenColor` (`self.blueColor`)))
    (:`neutral`
      (goto _label)))
  (if (not (`KismetSystemLibrary.IsDedicatedServer`))
    (`/Engine/EditorBlueprintResources/StandardMacros.IsValid` _capturepointmesh
      (:`Is Valid`
        (`MeshVertexPainterKismetLibrary.PaintVerticesSingleColor` _capturepointmesh _chosencolor)
        (`/Engine/EditorBlueprintResources/StandardMacros.IsValid` _letter_m
          (:`Is Valid`
            (`MaterialInstanceDynamic.SetVectorParameterValue` _letter_m "color" _chosencolor)
            (`/Engine/EditorBlueprintResources/StandardMacros.IsValid` _hologram_m
              (:`Is Valid`
                (`MaterialInstanceDynamic.SetVectorParameterValue` _hologram_m "color" (`self.ChosenColor`))))))))))

(fn `EnableToggle`
  (params (Enable :type Boolean))
  (bind _rotatingmovement (`self.RotatingMovement`))
  (bind _capturepointmesh (`self.CapturePointMesh`))
  (`|ExecutionSequence`
    (:`then_0`
      (`SceneComponent.SetVisibility` _capturepointmesh Enable false)
      (`SceneComponent.SetVisibility` (`self.hologram_mesh`) Enable false)
      (`SceneComponent.SetVisibility` (`self.letter`) Enable false)
      (`SceneComponent.SetVisibility` (`self.Plane`) Enable false)
      (`PrimitiveComponent.SetCollisionEnabled` _capturepointmesh (select `bool` Enable :`false` "NoCollision" :`true` "QueryAndPhysics" :!type "ECollisionEnabled Enum")))
    (:`then_1`
      (set `self.enabled` Enable))
    (:`then_2`
      (if Enable
        (set `self.ControllingTeam` "neutral")
        (`self.Start`)
        (else
          (`KismetSystemLibrary.K2_ClearAndInvalidateTimerHandle` (`self.AWARD_TIMER`))
          (`KismetSystemLibrary.K2_ClearAndInvalidateTimerHandle` (`self.OVERLAP_TIMER`)))))
    (:`then_3`
      (if Enable
        (`ActorComponent.Activate` _rotatingmovement false)
        (else
          (`ActorComponent.Deactivate` _rotatingmovement))))))

(fn `EnableToggle_client`
  (params (Enable :type Boolean))
  (bind _rotatingmovement (`self.RotatingMovement`))
  (bind _capturepointmesh (`self.CapturePointMesh`))
  (`|ExecutionSequence`
    (:`then_0`
      (`SceneComponent.SetVisibility` _capturepointmesh Enable false)
      (`SceneComponent.SetVisibility` (`self.hologram_mesh`) Enable false)
      (`SceneComponent.SetVisibility` (`self.letter`) Enable false)
      (`PrimitiveComponent.SetCollisionEnabled` _capturepointmesh (select `bool` Enable :`false` "NoCollision" :`true` "QueryAndPhysics" :!type "ECollisionEnabled Enum")))
    (:`then_1`
      (set `self.enabled` Enable))
    (:`then_3`
      (if Enable
        (`ActorComponent.Activate` _rotatingmovement false)
        (else
          (`ActorComponent.Deactivate` _rotatingmovement))))))

(fn `No one standing`
  (bind _output_get (set `self.CaptureProgress` (`KismetMathLibrary.Clamp` (- (`self.CaptureProgress`) 1) 0 (`self.TimeToCapture`))))
  (`self.Capture Progress` (`KismetMathLibrary.FClamp` (* (`KismetMathLibrary.Conv_IntToDouble` _output_get) (/ 1.0 (`KismetMathLibrary.Conv_IntToDouble` (`self.TimeToCapture`)))))))

(fn `TeamControlCheck`
  (params (Array :type "Array of /Game/Fadeout_Content/Core/Characters/BP_PlayerCharacter Object Reference"))
  (returns (RedCapturing :type Boolean) (BlueCapturing :type Boolean) (playerStates :type "Array of /Game/Fadeout_Content/Core/Support/Multiplayer_Support/FO_PlayerState Object Reference") (Remainder :type Integer))
  (locals (redPlayers :type Integer) (bluePlayers :type Integer) (redstates :type "Array of /Game/Fadeout_Content/Core/Support/Multiplayer_Support/FO_PlayerState Object Reference") (bluestates :type "Array of /Game/Fadeout_Content/Core/Support/Multiplayer_Support/FO_PlayerState Object Reference"))
  (bind _redplayers (`local.redPlayers`))
  (bind _blueplayers (`local.bluePlayers`))
  (bind _redplayers_2 (`local.redPlayers`))
  (bind _blueplayers_2 (`local.bluePlayers`))
  (for _array_element Array
    (if (not (`/Game/Fadeout_Content/Core/Characters/BP_PlayerCharacter.isCloaked` _array_element))
      (bind _asfo_player_state (cast `/Game/Fadeout_Content/Core/Support/Multiplayer_Support/FO_PlayerState` (`Pawn.PlayerState` _array_element)))
      (switch `string` (`/Game/Fadeout_Content/Core/Support/Multiplayer_Support/FO_PlayerState.Team` _asfo_player_state)
        (:`red`
          (`/Engine/EditorBlueprintResources/StandardMacros.IncrementInt` (`local.redPlayers`)
            (:`  `
              (`KismetArrayLibrary.Array_Add` (`local.redstates`) _asfo_player_state))))
        (:`blue`
          (`/Engine/EditorBlueprintResources/StandardMacros.IncrementInt` (`local.bluePlayers`)
            (:`  `
              (`KismetArrayLibrary.Array_Add` (`local.bluestates`) _asfo_player_state)))))))
  (`|ExecutionSequence`
    (:`then_0`
      ;[1 1 1] Red is capturing
      (if (> _redplayers_2 _blueplayers_2)
        (return true false (`local.redstates`) (`KismetMathLibrary.Clamp` (- _redplayers_2 _blueplayers_2) 0 3))))
    (:`then_1`
      ;[1 1 1] Blue is Capturing
      (if (> _blueplayers _redplayers)
        (return false true (`local.bluestates`) (`KismetMathLibrary.Clamp` (- _blueplayers _redplayers) 0 3))))
    (:`then_2`
      ;[1 1 1] No one is capturing
      (return false false _ 0))))

(fn `TracePlayers`
  (returns (Players1 :type "Array of /Game/Fadeout_Content/Core/Characters/BP_PlayerCharacter Object Reference"))
  (locals (Players :type "Array of /Game/Fadeout_Content/Core/Characters/BP_PlayerCharacter Object Reference"))
  (bind _players (`local.Players`))
  (bind _outhits (`KismetSystemLibrary.BoxTraceMultiForObjects` (`SceneComponent.K2_GetComponentLocation` (`self.ZoneStart`)) (`SceneComponent.K2_GetComponentLocation` (`self.ZoneEnd`)) (240.0 240.0 135.0) (struct) (`|MakeArray` "ObjectTypeQuery3" :!type "EObjectTypeQuery Enum")))
  (for _array_element _outhits
    (bind _asbp_player_character (cast `/Game/Fadeout_Content/Core/Characters/BP_PlayerCharacter` (`.HitActor` (`GameplayStatics.BreakHitResult` _array_element))))
    (`KismetArrayLibrary.Array_AddUnique` _players _asbp_player_character))
  (return _players))

(fn `UserConstructionScript`
  (bind _hologram_mesh (`self.hologram_mesh`))
  (bind _letter (`self.letter`))
  (bind _returnvalue (`PrimitiveComponent.CreateDynamicMaterialInstance` _hologram_mesh 0 "/Game/Fadeout_Content/Core/Props/Capture_Points/M_HoloGram_Vertex.M_hologram_Vertex" "None"))
  (bind _output_get (set `self.hologram_m` _returnvalue))
  (`PrimitiveComponent.SetMaterial` _hologram_mesh 0 _output_get)
  (`StaticMeshComponent.SetStaticMesh` _letter (`BlueprintMapLibrary.Map_Find` (`self.capLetters`) (`self.capPoint`)))
  (bind _returnvalue_2 (`PrimitiveComponent.CreateDynamicMaterialInstance` _letter 0 "/Game/Fadeout_Content/Core/Props/Capture_Points/M_Hololetters.M_Hololetters" "None"))
  (bind _output_get_2 (set `self.letter_m` _returnvalue_2))
  (`PrimitiveComponent.SetMaterial` _letter 0 _output_get_2)
  (`self.Change Team Color` (`self.ControllingTeam`)))