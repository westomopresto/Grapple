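; Team flag for capture-the-flag that enemies steal and teammates return by touch.
; Server-side overlap attaches it to the carrier, and carrier death or a drop event detaches it and starts a return countdown shown on its icon widget.
; Owning BP_FlagStand broadcasts throttled announcements, and a timer tracks an achievement window after leaving home.
; Tick periodically re-snaps the idle flag home, and heavy damage destroys it.
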(event `self.ReceiveAnyDamage`
  (params (Damage :type "Float (single-precision)") (DamageType :type "DamageType Object Reference") (InstigatedBy :type "Controller Object Reference") (DamageCauser :type "Actor Object Reference"))
  ;[1 1 1] Damage Taken
  (if (> Damage 400.0)
    (`self.DestroySelf`)))

(event `DestroySelf`
  ;[1 1 1] Damage Taken
  (`self.K2_DestroyActor`))

(event `ReturnTimer`
  ;[1 1 1] Return Timer
  (`|ExecutionSequence`
    (:`then_0`
      (bind (_direction _time) (`Timeline|Timer` :!via `SetNewTime` :!label _label)
        (:`Update`
          (bind _returnvalue (`KismetMathLibrary.FTrunc` _time))
          (bind _output_get (set `self.ReturnTimeLeft` _returnvalue))
          (set `/Game/Fadeout_Content/Core/Props/GameModeSupport/FlagIcon.TimeLeft` _output_get (cast `/Game/Fadeout_Content/Core/Props/GameModeSupport/FlagIcon` (`WidgetComponent.GetUserWidgetObject` (`self.FlagIconWidget`)) :!pure true)))
        (:`Finished`
          (bind _output_get_2 (set `self.ReturnTimeLeft` _returnvalue))
          (set `/Game/Fadeout_Content/Core/Props/GameModeSupport/FlagIcon.TimeLeft` _output_get_2 (cast `/Game/Fadeout_Content/Core/Props/GameModeSupport/FlagIcon` (`WidgetComponent.GetUserWidgetObject` (`self.FlagIconWidget`)) :!pure true))
          (`self.Respawn Flag`))))
    (:`then_1`
      (goto _label :!via `PlayFromStart`))))

(event `CancelReturn`
  ;[1 1 1] Return Timer
  (`|ExecutionSequence`
    (:`then_0`
      (goto _label :!via `Stop`))
    (:`then_1`
      (set `/Game/Fadeout_Content/Core/Props/GameModeSupport/FlagIcon.TimeLeft` 0 (cast `/Game/Fadeout_Content/Core/Props/GameModeSupport/FlagIcon` (`WidgetComponent.GetUserWidgetObject` (`self.FlagIconWidget`)) :!pure true)))))

(event `Respawn Flag`
  ;[1 1 1] Respawn Flag
  (`/Engine/EditorBlueprintResources/ActorMacros.Switch Has Authority`
    (:`Authority`
      (`self.K2_SetActorTransform` (`self.FlagTransform`) false true)
      (set `self.AtHome?` true))))

(event `self.ReceiveBeginPlay`
  ;[1 1 1] Begin Play
  (`|ExecutionSequence`
    (:`then_0`
      (`/Engine/EditorBlueprintResources/ActorMacros.Switch Has Authority`
        (:`Authority`
          (set `self.AtHome?` true))))
    (:`then_1`
      (if (not (`KismetSystemLibrary.IsDedicatedServer`))
        (`KismetSystemLibrary.Delay` 0.1)
        (switch `string` (`self.Team`)
          (:`Default`
            (set `self.ChosenColor` (`self.redColor`) :!label _label_2))
          (:`red`
            (goto _label_2))
          (:`blue`
            (set `self.ChosenColor` (`self.blueColor`))))
        (`MeshVertexPainterKismetLibrary.PaintVerticesSingleColor` (`self.Pole`) (`self.ChosenColor`))
        (`LightComponent.SetLightColor` (`self.PointLight`) (`self.ChosenColor`) true)
        (`UserWidget.SetColorAndOpacity` (`WidgetComponent.GetUserWidgetObject` (`self.FlagIconWidget`)) (`self.ChosenColor`))))))

(event `self.Box.OnComponentBeginOverlap`
  (params (OverlappedComponent :type "PrimitiveComponent Object Reference") (OtherActor :type "Actor Object Reference") (OtherComp :type "PrimitiveComponent Object Reference") (OtherBodyIndex :type Integer) (bFromSweep :type Boolean) (SweepResult :type "HitResult Structure (by ref)"))
  (bind _team (`self.Team`))
  ;[1 1 1] Player Overlap
  (`/Engine/EditorBlueprintResources/ActorMacros.Switch Has Authority`
    (:`Authority`
      (bind (_team_2 _valid_) (`self.GetPlayerTeam` OtherActor))
      (if (and (`KismetStringLibrary.NotEqual_StrStr` _team_2 _team) _valid_ (not (`self.AttachedToPlayer?`)))
        ;;[1 1 1] Pickup
        (bind _asbp_player_character (cast `/Game/Fadeout_Content/Core/Characters/BP_PlayerCharacter` OtherActor))
        (`self.FlagPickup` _asbp_player_character)
        (else
          ;;[1 1 1] Returns if its yours
          (if (and (`KismetStringLibrary.EqualEqual_StrStr` _team_2 _team) (not (`self.AttachedToPlayer?`)) (not (`self.AtHome?`)))
            (`self.CancelReturn`)
            (`self.Respawn Flag`)
            (`self.Flag Announcement` (select `bool` (`KismetStringLibrary.EqualEqual_StrStr` (`self.Team`) "red") :`false` "NewEnumerator0" :`true` "NewEnumerator1" :!type "/Game/Fadeout_Content/Core/Props/GameModeSupport/flagEventEnum Enum"))))))))

(event `self.ReceiveTick`
  (params (DeltaSeconds :type "Float (single-precision)"))
  ;[1 1 1] Carrier Alive Check
  (`|ExecutionSequence`
    (:`then_0`
      (if (and (`self.AttachedToPlayer?`) (`KismetSystemLibrary.IsValid` (`self.Carrier`)) (`self.HasAuthority`))
        (if (not (`/Game/Fadeout_Content/Core/Characters/BP_PlayerCharacter.alive?` (`self.Carrier`)))
          (`self.FlagDrop`))))
    (:`then_1`
      ;[1 1 1] Fixes movement bug at home
      (bind _output_get (set `self.Detla10` (+ DeltaSeconds (`self.Detla10`))))
      (if (and (`self.AtHome?`) (not (`self.AttachedToPlayer?`)) (>= _output_get 10.0))
        (`self.Respawn Flag`)
        (set `self.Detla10` 0.0)))))

(event `FlagPickup`
  (params (PlayerCharacter :type "/Game/Fadeout_Content/Core/Characters/BP_PlayerCharacter Object Reference"))
  ;[1 1 1] Flag Pickup
  (bind _output_get (set `self.Carrier` PlayerCharacter))
  (add `/Game/Fadeout_Content/Core/Characters/BP_PlayerCharacter.DropflagEvent` _output_get (delegate `DropFlagCommand`))
  (`self.K2_AttachToActor` self _output_get "None" "SnapToTarget" "SnapToTarget" "KeepWorld" true)
  (set `self.AttachedToPlayer?` true)
  (set `/Game/Fadeout_Content/Core/Characters/BP_PlayerCharacter.HasFlag?` true _output_get)
  (`self.K2_SetActorRelativeLocation` (`SceneComponent.RelativeLocation` (`/Game/Fadeout_Content/Core/Characters/BP_PlayerCharacter.FlagAttach` _output_get)) false true)
  (`self.CancelReturn`)
  (if (`self.AtHome?`)
    (`self.FromHomeTimer`))
  (set `self.AtHome?` false)
  (`/Engine/EditorBlueprintResources/StandardMacros.DoOnce` false :!label _label_3
    (:`Completed`
      (`self.Flag Announcement` (select `bool` (`KismetStringLibrary.EqualEqual_StrStr` (`self.Team`) "red") :`false` "NewEnumerator2" :`true` "NewEnumerator3" :!type "/Game/Fadeout_Content/Core/Props/GameModeSupport/flagEventEnum Enum"))
      (`KismetSystemLibrary.Delay` 10.0)
      (goto _label_3 :!via `Reset`))))

(event `DropFlagCommand`
  ;[1 1 1] Flag Pickup
  (`self.FlagDrop`))

(event `FromHomeTimer`
  ;[1 1 1] Achievement
  (bind _returnvalue (`KismetSystemLibrary.K2_SetTimerDelegate` (delegate `NoAchievement`) 20.0))
  (set `self.TimeFromHome` _returnvalue)
  (set `self.Achievo?` true))

(event `FlagDrop`
  (bind _pole (`self.Pole`))
  (bind _carrier (`self.Carrier`))
  ;[1 1 1] Flag Drop
  (`|ExecutionSequence`
    (:`then_0`
      (`/Engine/EditorBlueprintResources/StandardMacros.IsValid` _carrier
        (:`Is Valid`
          (set `/Game/Fadeout_Content/Core/Characters/BP_PlayerCharacter.HasFlag?` false _carrier))))
    (:`then_1`
      (`self.K2_DetachFromActor` self "KeepWorld" "KeepWorld" "KeepWorld")
      (remove `/Game/Fadeout_Content/Core/Characters/BP_PlayerCharacter.DropflagEvent` (`self.Carrier`) (delegate `DropFlagCommand`))
      (set `self.Carrier` null)
      (set `self.AttachedToPlayer?` false)
      (`PrimitiveComponent.SetEnableGravity` _pole true)
      (`PrimitiveComponent.SetSimulatePhysics` _pole true)
      (`self.K2_SetActorLocation` self (`SceneComponent.K2_GetComponentLocation` (`self.drop_world`)) false true))
    (:`then_2`
      (`self.ReturnTimer`))
    (:`then_3`
      (`/Engine/EditorBlueprintResources/StandardMacros.DoOnce` false :!label _label_4
        (:`Completed`
          (`self.Flag Announcement` (select `bool` (`KismetStringLibrary.EqualEqual_StrStr` (`self.Team`) "red") :`false` "NewEnumerator4" :`true` "NewEnumerator5" :!type "/Game/Fadeout_Content/Core/Props/GameModeSupport/flagEventEnum Enum"))
          (`KismetSystemLibrary.Delay` 10.0)
          (goto _label_4 :!via `Reset`))))))

(event `NoAchievement`
  ;[1 1 1] Achievement
  (set `self.Achievo?` false)
  (`KismetSystemLibrary.K2_ClearAndInvalidateTimerHandle` (`self.TimeFromHome`)))

(fn `Flag Announcement`
  (params (FlagEventMessage :type "/Game/Fadeout_Content/Core/Props/GameModeSupport/flagEventEnum Enum" :default "NewEnumerator0"))
  (locals (Phrase :type String :default "Returned!"))
  (bind _slatecolor (make `SlateColor` (struct :`R` 1.0 :`A` 1.0)))
  (bind _slatecolor_2 (make `SlateColor` (struct :`G` 0.2 :`B` 1.0 :`A` 1.0)))
  (bind _asbp_flag_stand (cast `/Game/Fadeout_Content/Core/Props/GameModeSupport/BP_FlagStand` (`self.GetOwner`)))
  (`/Game/Fadeout_Content/Core/Props/GameModeSupport/BP_FlagStand.All Player Announcement` _asbp_flag_stand (`KismetTextLibrary.Conv_StringToText` (select `/Game/Fadeout_Content/Core/Props/GameModeSupport/flagEventEnum` FlagEventMessage :`NewEnumerator0` "Blue Flag Returned!" :`NewEnumerator1` "Red Flag Returned!" :`NewEnumerator2` "Blue Flag Stolen!" :`NewEnumerator3` "Red Flag Stolen!" :`NewEnumerator4` "Blue Flag Dropped!" :`NewEnumerator5` "Red Flag Dropped!")) (select `/Game/Fadeout_Content/Core/Props/GameModeSupport/flagEventEnum` FlagEventMessage :`NewEnumerator0` _slatecolor_2 :`NewEnumerator1` _slatecolor :`NewEnumerator2` _slatecolor_2 :`NewEnumerator3` _slatecolor :`NewEnumerator4` _slatecolor_2 :`NewEnumerator5` _slatecolor) FlagEventMessage))

(fn `GetPlayerTeam`
  (params (BP_PlayerController :type "Object Object Reference"))
  (returns (Team :type String) (`Valid?` :type Boolean))
  (bind _asbp_player_character (cast `/Game/Fadeout_Content/Core/Characters/BP_PlayerCharacter` BP_PlayerController)
    (:`then`
      (bind _asfo_player_state (cast `/Game/Fadeout_Content/Core/Support/Multiplayer_Support/FO_PlayerState` (`Pawn.PlayerState` _asbp_player_character))
        (:`then`
          (bind _team (`/Game/Fadeout_Content/Core/Support/Multiplayer_Support/FO_PlayerState.Team` _asfo_player_state))
          (return _team (or (`KismetStringLibrary.EqualEqual_StrStr` _team "red") (`KismetStringLibrary.EqualEqual_StrStr` _team "blue"))))
        (:`CastFailed`
          _)))
    (:`CastFailed`
      _))
  (return "NULL" false))

(fn `UserConstructionScript`)