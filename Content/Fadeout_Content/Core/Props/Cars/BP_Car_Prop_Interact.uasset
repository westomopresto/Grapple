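; BP_Car_Prop_Interact is a car prop that rocks when it takes any damage.
; Its construction script applies the chosen car mesh to separate collision and display meshes, sets the wheel collision mesh, and tints a dynamic material through the TeamColor parameter.
; Shake picks a random direction and plays a timeline that pitches only the display mesh by ShakeAmount, leaving the collision meshes still.
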(event `Shake`
  (bind _shakeamount (`self.ShakeAmount`))
  (set `self.Direction` (`KismetMathLibrary.RandomBool`))
  (bind (_direction _alpha) (`Timeline|Timeline_0` :!via `PlayFromStart`)
    (:`Update`
      (`SceneComponent.K2_SetRelativeLocationAndRotation` (`self.DisplayMesh`) (0.0 0.0 0.0) (`KismetMathLibrary.MakeRotator` 0.0 (* _alpha (`KismetMathLibrary.SelectFloat` (* _shakeamount -1.0) _shakeamount (`self.Direction`)))) false false))))

(event `self.ReceiveAnyDamage`
  (params (Damage :type "Float (single-precision)") (DamageType :type "DamageType Object Reference") (InstigatedBy :type "Controller Object Reference") (DamageCauser :type "Actor Object Reference"))
  (`self.Shake`))

(fn `UserConstructionScript`
  (bind _carmesh (`self.CarMesh`))
  (`StaticMeshComponent.SetStaticMesh` (`self.CollisionMesh`) _carmesh)
  (`StaticMeshComponent.SetStaticMesh` (`self.DisplayMesh`) _carmesh)
  (`StaticMeshComponent.SetStaticMesh` (`self.Wheel_CollisionMesh`) (`self.WheelMesh`))
  (bind _returnvalue (`PrimitiveComponent.CreateDynamicMaterialInstance` (`self.DisplayMesh`) 0 (`StaticMesh.GetMaterial` (`self.CarMesh`) 0) "None"))
  (`MaterialInstanceDynamic.SetVectorParameterValue` _returnvalue "TeamColor" (`self.CarColor`)))