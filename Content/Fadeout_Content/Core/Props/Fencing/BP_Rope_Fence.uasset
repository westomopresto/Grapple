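; Rope fence prop that builds posts and ropes along a spline in the construction script.
; Each spline point gets a post, with a FlipFlop alternating its rotation and socket choice.
; A static mesh rope spans each pair of neighbouring posts, placed at the socket midpoint, aimed between them and scaled by distance over RopeLength.
; An unconnected skeletal rope setup with physics constraints remains in the graph but never runs.
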(event `self.ReceiveBeginPlay`)

(fn `UserConstructionScript`
  (bind _spline (`self.Spline`))
  (bind _location (.location (`SceneComponent.GetSocketTransform` (`self.nextPost`) (`self.nextSocket`) "RTS_Actor")))
  (bind _location_2 (.location (`SceneComponent.GetSocketTransform` (`self.lastPost`) (`self.nextSocket`) "RTS_Actor")))
  (for _index (range 1 (+ (`SplineComponent.GetNumberOfSplinePoints` _spline) 1))
    (`|ExecutionSequence`
      (:`then_0`
        (set `self.lastPost` (`self.nextPost`))
        (bind _returnvalue (- _index 1))
        ;[1 1 1] POST CREATION
        (bind _returnvalue_2 (`AddComponent|NODE_AddStaticMeshComponent-0` :`RelativeTransform` (`SplineComponent.GetTransformAtSplinePoint` _spline _returnvalue "Local" false)))
        (bind _output_get (set `self.nextPost` _returnvalue_2))
        (`/Engine/EditorBlueprintResources/StandardMacros.FlipFlop`
          (:`A`
            (`SceneComponent.K2_AddLocalRotation` _returnvalue_2 (struct :`Yaw` 90.0) false false)
            (set `self.firstSocket` "socket1")
            (set `self.nextSocket` "socket0"))
          (:`B`
            (`SceneComponent.K2_AddLocalRotation` _returnvalue_2 (struct :`Yaw` -90.0) false false)
            (set `self.firstSocket` "socket0")
            (set `self.nextSocket` "socket1")))
        (`StaticMeshComponent.SetStaticMesh` _output_get (`self.post_mesh`)))
      (:`then_1`
        ;[1 1 1] creates a Rope before the last post in a chain
        (if (> _returnvalue 0)
          (bind _returnvalue_3 (`AddComponent|NODE_AddStaticMeshComponent-3` :`RelativeTransform` (`KismetMathLibrary.MakeTransform` (/ (+ _location _location_2) 2.0) (`KismetMathLibrary.FindLookAtRotation` _location _location_2) (`KismetMathLibrary.MakeVector` 1.0 (* (/ (`KismetMathLibrary.Vector_Distance` _location _location_2) (`self.ropeLength`)) 2.0) 1.0))))
          (`SceneComponent.K2_AddLocalRotation` _returnvalue_3 (struct :`Yaw` 90.0) false false))))))