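; BP_Button is a networked prop button that controls either an elevator or a door, depending on its button type.
; Pushing routes through an authority check, sending remote calls to the server, which then multicasts the press.
; The multicast plays a beep at the button, then starts the elevator or toggles the door open or closed.
; The elevator reference is taken from the linked elevator track at BeginPlay.
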(event `self.ReceiveBeginPlay`
  (bind _elevator_track (`self.elevator_track`))
  (`/Engine/EditorBlueprintResources/StandardMacros.IsValid` _elevator_track
    (:`Is Valid`
      (set `self.elevator` (`/Game/Fadeout_Content/Core/Props/Elevator_Track.elevator` _elevator_track)))))

(event `Push Multicast`
  (bind _elevator (`self.elevator`))
  (bind _door (`self.door`))
  (`GameplayStatics.PlaySoundAtLocation` "/Game/Fadeout_Content/Core/Audio/Elevator/beep.beep" (`self.K2_GetActorLocation`) (struct) 2.0 1.0 0.0 "/Game/Fadeout_Content/Core/Characters/Footstep_Attenuation.Footstep_Attenuation" "/Game/Fadeout_Content/Core/Characters/ExplosionConcurrency.ExplosionConcurrency" null)
  (switch `/Game/Fadeout_Content/Core/Props/buttonTypes` (`self.button Type`)
    (:`NewEnumerator0`
      (`/Engine/EditorBlueprintResources/StandardMacros.IsValid` _elevator
        (:`Is Valid`
          (`/Game/Fadeout_Content/Core/Props/Elevator.startElevator` _elevator))))
    (:`NewEnumerator1`
      (`/Engine/EditorBlueprintResources/StandardMacros.IsValid` _door
        (:`Is Valid`
          (if (`/Game/Fadeout_Content/Core/Props/Doors/BP_Worker_Door.doorOpen?` _door)
            (`/Game/Fadeout_Content/Core/Props/Doors/BP_Worker_Door.Close` _door)
            (else
              (`/Game/Fadeout_Content/Core/Props/Doors/BP_Worker_Door.Open` _door))))))))

(event `push`
  (`/Engine/EditorBlueprintResources/ActorMacros.Switch Has Authority`
    (:`Authority`
      (`self.Push Multicast`))
    (:`Remote`
      (`self.Push Server`))))

(event `Push Server`
  (`self.Push Multicast`))

(fn `UserConstructionScript`)