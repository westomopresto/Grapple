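; Checkpoint prop that saves the game when the player character with PlayerInt 0 overlaps it.
; A gate opened half a second after BeginPlay lets overlaps through, ignoring any during startup.
; The save uses the game instance's chosen slot and passes the PlayerSpawnLoc transform as spawn override.
; Older GameMode current-checkpoint logic with sound and debug text remains but is unreachable.
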(event `self.ReceiveBeginPlay`
  (`KismetSystemLibrary.Delay` 0.5)
  (goto _label :!via `Open`))

(event `self.ReceiveActorBeginOverlap`
  (params (OtherActor :type "Actor Object Reference"))
  (`/Engine/EditorBlueprintResources/StandardMacros.Gate` true :!label _label
    (:`Exit`
      (bind _asbp_player_character (cast `/Game/Fadeout_Content/Core/Characters/BP_PlayerCharacter` OtherActor))
      (if (== (`/Game/Fadeout_Content/Core/Characters/BP_PlayerCharacter.PlayerInt` _asbp_player_character) 0)
        (bind _asfadeout_game_instance (cast `/Game/Fadeout_GameInstance` (`GameplayStatics.GetGameInstance`)))
        (`/Game/Fadeout_Content/Core/Characters/BP_PlayerCharacter.save_game` _asbp_player_character (`/Game/Fadeout_GameInstance.ChosenSaveSlot` _asfadeout_game_instance) 0 (`SceneComponent.K2_GetComponentToWorld` (`self.player_Spawn_Loc`)))))))

(fn `UserConstructionScript`)