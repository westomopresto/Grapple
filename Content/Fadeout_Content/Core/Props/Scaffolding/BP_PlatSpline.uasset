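; Scaffolding platform prop that lays spline mesh sections along an editable spline, with all logic in the construction script.
; It divides the spline into fixed-length sections scaled by the actor's X scale, leaving any shorter remainder uncovered.
; Each section takes local start and end points from the spline, with tangents clamped to half the section length to limit distortion.
; Sections are static, have query and physics collision, and block the Camera channel.
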(fn `UserConstructionScript`
  (bind _spline (`self.Spline`))
  (bind _spline_2 (`self.Spline`))
  (set `self.sectionLength` (* 621.0 (.x (`self.GetActorScale3D`))))
  (for _index (range (`KismetMathLibrary.FTrunc` (/ (`SplineComponent.GetSplineLength` (`self.Spline`)) (`self.sectionLength`))))
    (bind _returnvalue (`AddComponent|NODE_AddSplineMeshComponent-0`))
    (`SplineMeshComponent.SetForwardAxis` _returnvalue "X" true)
    (`PrimitiveComponent.SetCollisionEnabled` _returnvalue "QueryAndPhysics")
    (bind _returnvalue_2 (* _index (`self.sectionLength`)))
    (bind _returnvalue_3 (* (+ _index 1) (`self.sectionLength`)))
    (`SplineMeshComponent.SetStartAndEnd` _returnvalue (`SplineComponent.GetLocationAtDistanceAlongSpline` _spline_2 _returnvalue_2 "Local") (`KismetMathLibrary.ClampVectorSize` (`SplineComponent.GetTangentAtDistanceAlongSpline` _spline_2 _returnvalue_2 "Local") 0.0 (/ (`self.sectionLength`) 2.0)) (`SplineComponent.GetLocationAtDistanceAlongSpline` _spline _returnvalue_3 "Local") (`KismetMathLibrary.ClampVectorSize` (`SplineComponent.GetTangentAtDistanceAlongSpline` _spline _returnvalue_3 "Local") 0.0 (/ (`self.sectionLength`) 2.0)) true)
    (`SceneComponent.SetMobility` _returnvalue "Static")
    (`PrimitiveComponent.SetCollisionResponseToChannel` _returnvalue "ECC_Camera" "ECR_Block")))