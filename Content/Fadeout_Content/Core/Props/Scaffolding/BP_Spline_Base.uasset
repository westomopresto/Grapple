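; Base spline prop, filed under Scaffolding, that tiles a configurable mesh along a spline in the construction script.
; It adds one static, colliding spline mesh per whole section of actor-X-scaled length, leaving any remainder uncovered.
; Each segment takes position, roll and scale from the spline, with tangents clamped by section length, using different limits at start and end.
; The event graph has no runtime logic.
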(fn `UserConstructionScript`
  (bind _spline (`self.Spline`))
  (bind _spline_2 (`self.Spline`))
  (set `self.sectionLength` (* (`self.baseSectionLength`) (.x (`self.GetActorScale3D`))))
  (for _index (range (`KismetMathLibrary.FTrunc` (/ (`SplineComponent.GetSplineLength` (`self.Spline`)) (`self.sectionLength`))))
    (bind _returnvalue (`AddComponent|NODE_AddSplineMeshComponent-0`))
    (`StaticMeshComponent.SetStaticMesh` _returnvalue (`self.meshVar`))
    (`SplineMeshComponent.SetSplineUpDir` _returnvalue (`self.upDir`) true)
    (`SplineMeshComponent.SetForwardAxis` _returnvalue (`self.forwardAxis`) true)
    (`PrimitiveComponent.SetCollisionEnabled` _returnvalue "QueryAndPhysics")
    (bind _returnvalue_2 (* _index (`self.sectionLength`)))
    (bind _returnvalue_3 (* (+ _index 1) (`self.sectionLength`)))
    (`SplineMeshComponent.SetStartAndEnd` _returnvalue (`SplineComponent.GetLocationAtDistanceAlongSpline` _spline_2 _returnvalue_2 "Local") (`KismetMathLibrary.ClampVectorSize` (`SplineComponent.GetTangentAtDistanceAlongSpline` _spline_2 _returnvalue_2 "Local") 0.0 (/ (`self.sectionLength`) 0.5)) (`SplineComponent.GetLocationAtDistanceAlongSpline` _spline _returnvalue_3 "Local") (`KismetMathLibrary.ClampVectorSize` (`SplineComponent.GetTangentAtDistanceAlongSpline` _spline _returnvalue_3 "Local") 0.0 (/ (`self.sectionLength`) 4.0)) true)
    (bind _returnvalue_4 (* _index (`self.sectionLength`)))
    (`SplineMeshComponent.SetStartRoll` _returnvalue (.roll (`SplineComponent.GetRotationAtDistanceAlongSpline` _spline_2 _returnvalue_4 "Local")) true)
    (bind _returnvalue_5 (* (+ _index 1) (`self.sectionLength`)))
    (`SplineMeshComponent.SetEndRoll` _returnvalue (.roll (`SplineComponent.GetRotationAtDistanceAlongSpline` _spline_2 _returnvalue_5 "Local")) true)
    (`SplineMeshComponent.SetStartScale` _returnvalue (* (`KismetMathLibrary.MakeVector2D` (.y (`SplineComponent.GetScaleAtDistanceAlongSpline` _spline_2 _returnvalue_4)) (.z (`SplineComponent.GetScaleAtDistanceAlongSpline` _spline_2 _returnvalue_4))) (`self.scale`)) true)
    (`SplineMeshComponent.SetEndScale` _returnvalue (* (`KismetMathLibrary.MakeVector2D` (.y (`SplineComponent.GetScaleAtDistanceAlongSpline` _spline_2 _returnvalue_5)) (.z (`SplineComponent.GetScaleAtDistanceAlongSpline` _spline_2 _returnvalue_5))) (`self.scale`)) true)
    (`SceneComponent.SetMobility` _returnvalue "Static")
    (`PrimitiveComponent.SetCollisionResponseToChannel` _returnvalue "ECC_Camera" "ECR_Block")
    (`PrimitiveComponent.SetCollisionResponseToChannel` _returnvalue "ECC_Visibility" "ECR_Block")
    (`PrimitiveComponent.SetCollisionResponseToChannel` _returnvalue "ECC_GameTraceChannel7" "ECR_Block")))