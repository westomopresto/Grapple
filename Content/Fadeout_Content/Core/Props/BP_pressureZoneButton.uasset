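; Pressure zone button prop that drives a linked gate based on the mass of physics objects resting inside its trigger box.
; Box overlap begin and end events add or subtract each simulating component's mass, debug-printing the running weight.
; Reaching the weight threshold starts TargetGate and falling below reverses it, toggling the "active" material parameter to match.
; The construction script creates the dynamic material instance on the skeletal mesh.
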(event `self.ReceiveBeginPlay`)

(event `self.Box.OnComponentEndOverlap`
  (params (OverlappedComponent :type "PrimitiveComponent Object Reference") (OtherActor :type "Actor Object Reference") (OtherComp :type "PrimitiveComponent Object Reference") (OtherBodyIndex :type Integer))
  (bind _materialinstance (`self.materialInstance`))
  (bind _targetgate (`self.targetGate`))
  (if (`SceneComponent.IsAnySimulatingPhysics` OtherComp)
    (set `self.weight` (- (`self.weight`) (`PrimitiveComponent.GetMass` OtherComp)))
    (`KismetSystemLibrary.PrintString` (`KismetStringLibrary.Conv_DoubleToString` (`self.weight`)) :!label _label)
    (if (>= (`self.weight`) 1.0)
      (`/Game/Fadeout_Content/Core/Props/Gate/BP_Gate.Start` _targetgate)
      (`MaterialInstanceDynamic.SetScalarParameterValue` _materialinstance "active" 1.0)
      (else
        (`/Game/Fadeout_Content/Core/Props/Gate/BP_Gate.Reverse` _targetgate)
        (`MaterialInstanceDynamic.SetScalarParameterValue` _materialinstance "active" 0.0)))))

(event `self.Box.OnComponentBeginOverlap`
  (params (OverlappedComponent :type "PrimitiveComponent Object Reference") (OtherActor :type "Actor Object Reference") (OtherComp :type "PrimitiveComponent Object Reference") (OtherBodyIndex :type Integer) (bFromSweep :type Boolean) (SweepResult :type "HitResult Structure (by ref)"))
  (if (`SceneComponent.IsAnySimulatingPhysics` OtherComp)
    (set `self.weight` (+ (`self.weight`) (`PrimitiveComponent.GetMass` OtherComp)))
    (goto _label)))

(fn `UserConstructionScript`
  (bind _skeletalmeshcomponent (`self.SkeletalMeshComponent`))
  (bind _returnvalue (`PrimitiveComponent.CreateDynamicMaterialInstance` _skeletalmeshcomponent 0 (`PrimitiveComponent.GetMaterial` _skeletalmeshcomponent 0) "None"))
  (bind _output_get (set `self.materialInstance` _returnvalue))
  (`PrimitiveComponent.SetMaterial` _skeletalmeshcomponent 0 _output_get))