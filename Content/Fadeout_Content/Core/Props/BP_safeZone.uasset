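; BP_safeZone is a trigger prop that reacts when an allied BP_Ally character enters it, apparently as the drop-off point for rescues.
; On collision overlap it checks the ally's gameplay tags for Allied, then writes the Target component's world location to the AI blackboard's TargetDestination key.
; It then changes the ally's state and updates its RescueState.
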(event `self.CollisionComponent.OnComponentBeginOverlap`
  (params (OverlappedComponent :type "PrimitiveComponent Object Reference") (OtherActor :type "Actor Object Reference") (OtherComp :type "PrimitiveComponent Object Reference") (OtherBodyIndex :type Integer) (bFromSweep :type Boolean) (SweepResult :type "HitResult Structure (by ref)"))
  (bind _asbp_ally (cast `/Game/Fadeout_Content/Core/Characters/BP_Ally` OtherActor))
  (if (`BlueprintGameplayTagLibrary.MatchesAnyTags` (struct :`TagName` "allied") (`Character_w_Tags.GameplayTags` _asbp_ally))
    (`BlackboardComponent.SetValueAsVector` (`AIBlueprintHelperLibrary.GetBlackboard` (`AIBlueprintHelperLibrary.GetAIController` _asbp_ally)) "TargetDestination" (`SceneComponent.K2_GetComponentLocation` (`self.target`)))
    (`/Game/Fadeout_Content/Core/Characters/BP_Enemy.Change State` _asbp_ally "NewEnumerator2")
    (set `/Game/Fadeout_Content/Core/Characters/BP_Ally.RescueState` "NewEnumerator4" _asbp_ally)))

(fn `UserConstructionScript`)