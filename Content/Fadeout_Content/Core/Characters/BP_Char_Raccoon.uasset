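; BP_Char_Raccoon is the playable raccoon character Abby, extending a parent character with ammo regeneration, turret demolition and team-colored outfits.
; While player-controlled, its authority-side Tick timer periodically grants mixed ammo through the pickup logic and plays a pickup sound.
; The Character Special input destroys all owned structures with massive damage.
; After a short delay, ColorSet gives the current outfit's cosmetic a dynamic material tinted by HelmetColor.
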(event `RegenAmmo`
  (`self.PickUpItemBase _ USE` null 0 (make `/Game/Fadeout_Content/Core/Support/AmmoStruct` 1 30 0 5 5) true)
  (`self.PlayAmmoRegenFXLocal`))

(event `PlayAmmoRegenFXLocal`
  (`GameplayStatics.PlaySound2D` "/Game/Fadeout_Content/Core/Audio/residue-sfx/ammopickup_0.ammopickup_0" 1.0 1.0 0.0 null null))

(event `self.ReceiveTick`
  (params (DeltaSeconds :type "Float (single-precision)"))
  (`parent.ReceiveTick` DeltaSeconds)
  (if (and (`self.IsPlayerControlled`) (`self.HasAuthority`))
    (bind _output_get (set `self.Timer` (+ (`self.Timer`) DeltaSeconds)))
    (if (>= _output_get 10.0)
      (set `self.Timer` 0.0)
      (`self.RegenAmmo`))))

(event `self.Color Set`
  (bind _output (`|GetArrayItem` (`self.EquippedCosmetics`) (`KismetArrayLibrary.Array_Find` (`self.Equipped Cosmetic Reference`) "/Game/Fadeout_Content/Core/Characters/Raccoon/Outfits/abby_default.abby_default")))
  (bind _output_2 (`|GetArrayItem` (`self.EquippedCosmetics`) (`KismetArrayLibrary.Array_Find` (`self.Equipped Cosmetic Reference`) "/Game/Fadeout_Content/Core/Characters/Raccoon/Outfits/Scientist/scientist_outfit_b1.scientist_outfit_b1")))
  (bind _output_3 (`|GetArrayItem` (`self.EquippedCosmetics`) (`KismetArrayLibrary.Array_Find` (`self.Equipped Cosmetic Reference`) "/Game/Fadeout_Content/Core/Characters/Raccoon/Outfits/abby_pirate.abby_pirate")))
  (`KismetSystemLibrary.Delay` 0.2)
  (switch `/Game/Fadeout_Content/Core/UI/Customize/Abigail_Outfits` (cast `/Game/Fadeout_Content/Core/UI/Customize/Abigail_Outfits` (`self.current_outfit`))
    (:`NewEnumerator0`
      (`/Engine/EditorBlueprintResources/StandardMacros.IsValid` _output
        (:`Is Valid`
          (bind _returnvalue (`KismetMaterialLibrary.CreateDynamicMaterialInstance` (`PrimitiveComponent.GetMaterial` _output 0) "/Game/Fadeout_Content/Core/Characters/Raccoon/Materials/M_Abby_Clothing.M_Abby_Clothing" "None"))
          (bind _output_get (set `self.HelmetDynamic` _returnvalue))
          (`PrimitiveComponent.SetMaterial` _output 0 _output_get)
          (`MaterialInstanceDynamic.SetVectorParameterValue` _output_get "TeamColor" (`KismetMathLibrary.Conv_ColorToLinearColor` (`self.HelmetColor`))))))
    (:`NewEnumerator1`
      (`/Engine/EditorBlueprintResources/StandardMacros.IsValid` _output_3
        (:`Is Valid`
          (bind _returnvalue_2 (`KismetMaterialLibrary.CreateDynamicMaterialInstance` (`PrimitiveComponent.GetMaterial` _output_3 0) "/Game/Fadeout_Content/Core/Characters/Raccoon/Outfits/M_abby_pirate.M_abby_pirate" "None"))
          (bind _output_get_2 (set `self.HelmetDynamic` _returnvalue_2))
          (`PrimitiveComponent.SetMaterial` _output_3 0 _output_get_2)
          (`MaterialInstanceDynamic.SetVectorParameterValue` _output_get_2 "TeamColor" (`KismetMathLibrary.Conv_ColorToLinearColor` (`self.HelmetColor`))))))
    (:`NewEnumerator2`
      (`/Engine/EditorBlueprintResources/StandardMacros.IsValid` _output_2
        (:`Is Valid`
          (bind _returnvalue_3 (`KismetMaterialLibrary.CreateDynamicMaterialInstance` (`PrimitiveComponent.GetMaterial` _output_2 0) "/Game/Fadeout_Content/Core/Characters/Raccoon/Outfits/Scientist/M_Scientist_Outfit.M_Scientist_Outfit" "None"))
          (bind _output_get_3 (set `self.HelmetDynamic` _returnvalue_3))
          (`PrimitiveComponent.SetMaterial` _output_2 0 _output_get_3)
          (`MaterialInstanceDynamic.SetVectorParameterValue` _output_get_3 "TeamColor" (`KismetMathLibrary.Conv_ColorToLinearColor` (`self.HelmetColor`))))))))

(event `InputAction|Character Special`
  (params (Key :type "Key Structure"))
  (bind _returnvalue (`self.GetController` self))
  (:`Pressed`
    (`/Engine/EditorBlueprintResources/ActorMacros.Switch Has Authority`
      (:`Authority`
        (`self.Kill own turrets` _returnvalue self))
      (:`Remote`
        (`self.Kill own turrets` _returnvalue self)))))

(event `Kill own turrets`
  (params (EventInstigator :type "Controller Object Reference") (DamageCauser :type "Actor Object Reference"))
  (for _array_element (`self.OwnedStructures`)
    (`GameplayStatics.ApplyDamage` _array_element 9999999.0)))

(fn `UserConstructionScript`
  (`parent.UserConstructionScript`))