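; Mouse (Camille) character Blueprint that adds a remote TNT detonation special and team-colored outfit skins.
; Special routes to the server, which beeps and applies DT_TNT damage to each owned projectile, then clears the list.
; ColorSet creates dynamic materials tinted by team color for the current outfit, enabling the helmet spotlight for Miner and Midnight.
; The USB Mouse skin swaps in robot hurt sounds and binds a red emissive flash to the hurt dispatcher.
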(event `Detonate Server`
  ;[1 1 1] Detonate
  (`self.Special Detonate`))

(event `InputAction|Character Special`
  (params (Key :type "Key Structure"))
  ;[1 1 1] Detonate
  (:`Pressed`
    (`/Engine/EditorBlueprintResources/ActorMacros.Switch Has Authority`
      (:`Authority`
        (`self.Special Detonate`))
      (:`Remote`
        (`self.Detonate Server`)))))

(event `Special Detonate`
  (bind _myownedprojectiles (`self.myOwnedProjectiles`))
  ;[1 1 1] Detonate
  (if (> (`KismetArrayLibrary.Array_Length` _myownedprojectiles) 0)
    (`GameplayStatics.PlaySoundAtLocation` "/Game/Fadeout_Content/Core/Audio/Elevator/beep.beep" (`self.K2_GetActorLocation`) (struct) 1.0 1.5 0.0 null null null)
    (for _array_element _myownedprojectiles
      (bind _asbp_tnt_projectile (cast `/Game/Fadeout_Content/Weapons/Projectiles/BP_TNT_Projectile` _array_element))
      (`GameplayStatics.ApplyDamage` _asbp_tnt_projectile 5.0 null (`self.Instigator`) "/Game/Fadeout_Content/Core/Weapons/DamageTypes/DT_TNT.DT_TNT_C"))
    (`KismetArrayLibrary.Array_Clear` _myownedprojectiles)
    (else
      (`GameplayStatics.PlaySoundAtLocation` "/Game/Fadeout_Content/Core/Audio/short_beep.short_beep" (0.0 0.0 0.0) (struct) 1.0 1.0 0.0 null null null))))

(event `self.ReceiveBeginPlay`
  (`parent.ReceiveBeginPlay`)
  (`SceneComponent.SetVisibility` (`self.SpotLight`) false false))

(event `Miner Camille`
  (bind _equipped_cosmetic_reference (`self.Equipped Cosmetic Reference`))
  (bind _equippedcosmetics (`self.EquippedCosmetics`))
  (bind (_colorrgb _bonusmetallic) (break `/Game/Fadeout_Content/Core/UI/Customize/CustomColor` (`self.HelmetColor`)))
  (bind (_colorrgb_2 _bonusmetallic_2) (break `/Game/Fadeout_Content/Core/UI/Customize/CustomColor` (`self.HelmetColor`)))
  (bind _output (`|GetArrayItem` _equippedcosmetics (`KismetArrayLibrary.Array_Find` _equipped_cosmetic_reference "/Game/Fadeout_Content/Core/Characters/Kasparian_FBX/outfits/camille_v6_helmet.camille_v6_helmet")))
  (bind _output_2 (`|GetArrayItem` _equippedcosmetics (`KismetArrayLibrary.Array_Find` _equipped_cosmetic_reference "/Game/Fadeout_Content/Core/Characters/Kasparian_FBX/outfits/camille_v6_miningOutfit.camille_v6_miningOutfit")))
  (`|ExecutionSequence`
    (:`then_0`
      (`/Engine/EditorBlueprintResources/StandardMacros.IsValid` _output
        (:`Is Valid`
          (bind _returnvalue (`KismetMaterialLibrary.CreateDynamicMaterialInstance` (`PrimitiveComponent.GetMaterial` _output 0) "/Game/Fadeout_Content/Core/Characters/Kasparian_FBX/material/v4/M_helmet.M_helmet" "None"))
          (bind _output_get (set `self.HelmetDynamic` _returnvalue))
          (`PrimitiveComponent.SetMaterial` _output 0 _output_get)
          (`MaterialInstanceDynamic.SetVectorParameterValue` _output_get "TeamColor" (`KismetMathLibrary.Conv_ColorToLinearColor` _colorrgb_2))
          (`MaterialInstanceDynamic.SetScalarParameterValue` _output_get "BonusMetallic" _bonusmetallic_2)
          (`KismetSystemLibrary.Delay` 0.2)
          (`SceneComponent.SetVisibility` (`self.SpotLight`) true false))))
    (:`then_1`
      (`/Engine/EditorBlueprintResources/StandardMacros.IsValid` _output_2
        (:`Is Valid`
          (bind _returnvalue_2 (`KismetMaterialLibrary.CreateDynamicMaterialInstance` (`PrimitiveComponent.GetMaterial` _output_2 0) "/Game/Fadeout_Content/Core/Characters/Kasparian_FBX/material/v4/M_clothing.M_clothing" "None"))
          (bind _output_get_2 (set `self.Clothing Dynamic` _returnvalue_2))
          (`PrimitiveComponent.SetMaterial` _output_2 0 _output_get_2)
          (`MaterialInstanceDynamic.SetVectorParameterValue` _output_get_2 "TeamColor" (`KismetMathLibrary.Conv_ColorToLinearColor` _colorrgb))
          (`MaterialInstanceDynamic.SetScalarParameterValue` _output_get_2 "BonusMetallic" _bonusmetallic))))))

(event `Color Set`
  (bind (_colorrgb _bonusmetallic) (break `/Game/Fadeout_Content/Core/UI/Customize/CustomColor` (`self.HelmetColor`)))
  (bind (_colorrgb_2 _bonusmetallic_2) (break `/Game/Fadeout_Content/Core/UI/Customize/CustomColor` (`self.HelmetColor`)))
  (bind _output (`|GetArrayItem` (`self.EquippedCosmetics`) (`KismetArrayLibrary.Array_Find` (`self.Equipped Cosmetic Reference`) "/Game/Fadeout_Content/Core/Characters/Kasparian_FBX/outfits/camklle_sailor_v1.camklle_sailor_v1")))
  (bind _output_2 (`|GetArrayItem` (`self.EquippedCosmetics`) (`KismetArrayLibrary.Array_Find` (`self.Equipped Cosmetic Reference`) "/Game/Fadeout_Content/Core/Characters/Blaise/Skin/PJs/PJs_outfit.PJs_outfit")))
  (clear `self.HurtDispatcher`)
  (set `self.hurtSound` "/Game/Fadeout_Content/Core/Audio/Kasp_SFX/Female_Hurt_Cue.Female_Hurt_Cue")
  (`KismetSystemLibrary.Delay` 0.2)
  (`SceneComponent.SetVisibility` (`self.SpotLight`) false false)
  (switch `/Game/Fadeout_Content/Core/UI/Customize/Camille_Outfits` (cast `/Game/Fadeout_Content/Core/UI/Customize/Camille_Outfits` (`self.current_outfit`))
    (:`NewEnumerator0`
      (`self.Miner Camille`))
    (:`NewEnumerator1`
      (`/Engine/EditorBlueprintResources/StandardMacros.IsValid` _output
        (:`Is Valid`
          (bind _returnvalue (`KismetMaterialLibrary.CreateDynamicMaterialInstance` (`PrimitiveComponent.GetMaterial` _output 0) "/Game/Fadeout_Content/Core/Characters/Kasparian_FBX/outfits/M_Sailor_Camille.M_Sailor_Camille" "None"))
          (bind _output_get (set `self.HelmetDynamic` _returnvalue))
          (`PrimitiveComponent.SetMaterial` _output 0 _output_get)
          (`MaterialInstanceDynamic.SetVectorParameterValue` _output_get "TeamColor" (`KismetMathLibrary.Conv_ColorToLinearColor` _colorrgb))
          (`MaterialInstanceDynamic.SetScalarParameterValue` _output_get "BonusMetallic" _bonusmetallic))))
    (:`NewEnumerator2`
      (`self.Miner Camille`))
    (:`NewEnumerator3`
      (`/Engine/EditorBlueprintResources/StandardMacros.IsValid` _output_2
        (:`Is Valid`
          (bind _returnvalue_2 (`KismetMaterialLibrary.CreateDynamicMaterialInstance` (`PrimitiveComponent.GetMaterial` _output_2 0) "/Game/Fadeout_Content/Core/Characters/Blaise/Skin/PJs/M_PJs.M_PJs" "None"))
          (bind _output_get_2 (set `self.HelmetDynamic` _returnvalue_2))
          (`PrimitiveComponent.SetMaterial` _output_2 0 _output_get_2)
          (`MaterialInstanceDynamic.SetVectorParameterValue` _output_get_2 "TeamColor" (`KismetMathLibrary.Conv_ColorToLinearColor` _colorrgb_2))
          (`MaterialInstanceDynamic.SetScalarParameterValue` _output_get_2 "BonusMetallic" _bonusmetallic_2))))
    (:`NewEnumerator4`
      (`self.USB Mouse Skin`))))

(event `USBMouse_Hurt Event`
  (`MaterialInstanceDynamic.SetVectorParameterValue` (stale `USB Mouse Skin` _output_get) "EmissiveColorMod" (struct :`R` 15.0 :`A` 1.0))
  (`KismetSystemLibrary.Delay` 0.5)
  (`MaterialInstanceDynamic.SetVectorParameterValue` (stale `USB Mouse Skin` _output_get) "EmissiveColorMod" (struct :`R` 1.0 :`G` 1.0 :`B` 1.0 :`A` 1.0)))

(event `USB Mouse Skin`
  (bind _mesh (`self.Mesh`))
  (bind (_colorrgb _bonusmetallic) (break `/Game/Fadeout_Content/Core/UI/Customize/CustomColor` (`self.HelmetColor`)))
  (`/Engine/EditorBlueprintResources/StandardMacros.IsValid` _mesh
    (:`Is Valid`
      (bind _returnvalue (`KismetMaterialLibrary.CreateDynamicMaterialInstance` (`PrimitiveComponent.GetMaterial` _mesh 0) "/Game/Fadeout_Content/Core/Characters/Kasparian_FBX/outfits/ToyCamille/M_ToyCamille_Body.M_ToyCamille_Body" "None"))
      (bind _output_get (set `self.HelmetDynamic` _returnvalue))
      (`PrimitiveComponent.SetMaterial` _mesh 0 _output_get)
      (`MaterialInstanceDynamic.SetVectorParameterValue` _output_get "TeamColor" (`KismetMathLibrary.Conv_ColorToLinearColor` _colorrgb))
      (`MaterialInstanceDynamic.SetScalarParameterValue` _output_get "BonusMetallic" _bonusmetallic)
      (set `self.hurtSound` "/Game/Fadeout_Content/Core/Audio/Kasp_SFX/RobotFemale_hurt_Cue.RobotFemale_hurt_Cue")
      (add `self.HurtDispatcher` (delegate `USBMouse_Hurt Event`)))))

(fn `PlayHurtSounds`
  (params (`Damage TYpe` :type "DamageType Object Reference"))
  (`parent.PlayHurtSounds` `Damage TYpe`))

(fn `UserConstructionScript`
  (`parent.UserConstructionScript`))