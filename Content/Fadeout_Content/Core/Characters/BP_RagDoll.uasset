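; BP_RagDoll is a ragdoll actor that shows a character mesh collapsing under physics from a saved pose.
; On BeginPlay it applies the supplied mesh, enables gravity and passes the pose snapshot and a ragdoll flag to the kasp_animBP anim instance.
; It then simulates physics on the hips bone and all bodies below it, provided that anim Blueprint cast succeeds.
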(event `self.ReceiveBeginPlay`
  (bind _skeletalmesh (`self.SkeletalMesh`))
  (`SkinnedMeshComponent.SetSkinnedAssetAndUpdate` _skeletalmesh (`self.ragDollMesh`) true)
  (`PrimitiveComponent.SetEnableGravity` _skeletalmesh true)
  (bind _askasp_anim_bp (cast `/Game/Fadeout_Content/Core/Characters/Kasparian_BP/kasp_animBP` (`SkeletalMeshComponent.GetAnimInstance` (`self.SkeletalMesh`))))
  (set `/Game/Fadeout_Content/Core/Characters/Kasparian_BP/kasp_animBP.M Snapshot` (`self.poseSnapShot`) _askasp_anim_bp)
  (set `/Game/Fadeout_Content/Core/Characters/Kasparian_BP/kasp_animBP.ragDoll?` true _askasp_anim_bp)
  (`SkeletalMeshComponent.SetAllBodiesBelowSimulatePhysics` (`self.SkeletalMesh`) (`self.hipsPhysics`) true true))

(fn `UserConstructionScript`)