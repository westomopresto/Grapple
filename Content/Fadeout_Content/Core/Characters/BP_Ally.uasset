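; BP_Ally is a friendly AI character the player can command to stay put, follow or fight via a directional tag selection.
; Commands change its state, with stay and combat updating Blackboard locations and stay and follow playing voice lines.
; Perceiving the player triggers a DoOnce greeting with sound, wave and TargetActor update, re-armed once no actors are perceived.
; Taking damage switches it to the combat state.
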(event `taggedByPlayer`
  (params (Selection :type "/Game/Fadeout_Content/Core/Characters/D-Pad Enum" :default "NewEnumerator0"))
  (switch `/Game/Fadeout_Content/Core/Characters/D-Pad` Selection
    (:`NewEnumerator0`
      (`self.Command Stay Put`))
    (:`NewEnumerator1`
      (`self.Command Follow Player`))
    (:`NewEnumerator2`
      (`self.Command Combat`))))

(event `Command Combat`
  (bind _returnvalue (`AIBlueprintHelperLibrary.GetBlackboard` (`AIBlueprintHelperLibrary.GetAIController` self)))
  (`self.Change State` "NewEnumerator0")
  (`BlackboardComponent.SetValueAsVector` _returnvalue "Home" (`BlackboardComponent.GetValueAsVector` _returnvalue "TargetDestination")))

(event `Command Follow Player`
  (`self.Change State` "NewEnumerator1")
  (`self.sayFollowingYou`))

(event `Command Stay Put`
  (`self.Change State` "NewEnumerator2")
  (`self.sayStayingPut`)
  (`BlackboardComponent.SetValueAsVector` (`AIBlueprintHelperLibrary.GetBlackboard` null) "TargetDestination" (`self.K2_GetActorLocation`)))

(event `self.ReceiveBeginPlay`
  (`PrimitiveComponent.SetCollisionResponseToChannel` (`self.Mesh`) "ECC_GameTraceChannel5" "ECR_Block")
  (`parent.ReceiveBeginPlay`))

(event `sayStayingPut`
  (`GameplayStatics.SpawnSoundAttached` "/Game/Fadeout_Content/Core/Audio/Prisoners/stayingPut.stayingPut" (`self.CapsuleComponent`) "None" (0.0 0.0 0.0) (struct) "KeepRelativeOffset" true 1.0 1.0 0.0 null null))

(event `sayFollowingYou`
  (`GameplayStatics.SpawnSoundAttached` "/Game/Fadeout_Content/Core/Audio/Prisoners/okFollowingYou.okFollowingYou" (`self.CapsuleComponent`) "None" (0.0 0.0 0.0) (struct) "KeepRelativeOffset" true 1.0 1.0 0.0 null null))

(event `sayThankYou`
  (`GameplayStatics.SpawnSoundAttached` "/Game/Fadeout_Content/Core/Audio/Prisoners/thankYou.thankYou" (`self.CapsuleComponent`) "None" (0.0 0.0 0.0) (struct) "KeepRelativeOffset" true 1.0 1.0 0.0 null null))

(event `self.AIPerception_0.OnPerceptionUpdated`
  (params (UpdatedActors :type "Array of Actor Object Reference (by ref)"))
  (if (== (`KismetArrayLibrary.Array_Length` (`AIPerceptionComponent.GetKnownPerceivedActors` (`self.AIPerception`) null)) 0)
    (`self.resetHello`)))

(event `self.AIPerception_0.OnTargetPerceptionUpdated`
  (params (Actor :type "Actor Object Reference") (Stimulus :type "AIStimulus Structure"))
  (bind _returnvalue (`AIBlueprintHelperLibrary.GetBlackboard` null))
  (bind _asbp_player_character (cast `/Game/Fadeout_Content/Core/Characters/BP_PlayerCharacter` Actor))
  (`/Engine/EditorBlueprintResources/StandardMacros.DoOnce` false :!label _label
    (:`Completed`
      (`GameplayStatics.SpawnSoundAttached` "/Game/Fadeout_Content/Core/Audio/Prisoners/heyOverHere.heyOverHere" (`self.CapsuleComponent`) "None" (0.0 0.0 0.0) (struct) "KeepRelativeOffset" true 1.0 1.0 0.0 null null)
      (if (and (`KismetSystemLibrary.IsValid` _returnvalue) (`KismetSystemLibrary.IsValid` _asbp_player_character))
        (`BlackboardComponent.SetValueAsObject` _returnvalue "TargetActor" _asbp_player_character)
        (`self.PlayAnimMontage` "/Game/Fadeout_Content/Core/Characters/Kasparian_BP/Special/wave_montage.wave_montage")))))

(event `resetHello`
  (goto _label :!via `Reset`))

(event `self.ReceiveAnyDamage`
  (params (Damage :type "Float (single-precision)") (DamageType :type "DamageType Object Reference") (InstigatedBy :type "Controller Object Reference") (DamageCauser :type "Actor Object Reference"))
  (`parent.ReceiveAnyDamage` Damage DamageType InstigatedBy DamageCauser)
  (`self.Change State` "NewEnumerator0"))

(fn `UserConstructionScript`
  (`parent.UserConstructionScript`))