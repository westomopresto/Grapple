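; Opossum character Blueprint (Blaise) that adds outfit-specific team coloring and immunity to fire damage-over-time on top of its parent.
; ColorSet runs the parent logic, then switches on the current outfit to a matching event for the firefighter, sailor, miner or pajama look.
; Each event puts a dynamic material on the equipped cosmetic and feeds it the helmet color and metallic values.
; The AttachDoT override skips BP_Fire_DOT and forwards other classes to the parent.
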(event `Miner Blaise`
  (bind (_colorrgb _bonusmetallic) (break `/Game/Fadeout_Content/Core/UI/Customize/CustomColor` (`self.HelmetColor`)))
  (bind _output (`|GetArrayItem` (`self.EquippedCosmetics`) (`KismetArrayLibrary.Array_Find` (`self.Equipped Cosmetic Reference`) "/Game/Fadeout_Content/Core/Characters/Kasparian_FBX/outfits/camille_v6_miningOutfit.camille_v6_miningOutfit")))
  (`/Engine/EditorBlueprintResources/StandardMacros.IsValid` _output
    (:`Is Valid`
      (bind _returnvalue (`KismetMaterialLibrary.CreateDynamicMaterialInstance` (`PrimitiveComponent.GetMaterial` _output 0) "/Game/Fadeout_Content/Core/Characters/Kasparian_FBX/material/v4/M_clothing.M_clothing" "None"))
      (bind _output_get (set `self.HelmetDynamic` _returnvalue))
      (`PrimitiveComponent.SetMaterial` _output 0 _output_get)
      (`MaterialInstanceDynamic.SetVectorParameterValue` _output_get "TeamColor" (`KismetMathLibrary.Conv_ColorToLinearColor` _colorrgb))
      (`MaterialInstanceDynamic.SetScalarParameterValue` _output_get "BonusMetallic" _bonusmetallic))))

(event `FireFighter Blaise`
  (bind (_colorrgb _bonusmetallic) (break `/Game/Fadeout_Content/Core/UI/Customize/CustomColor` (`self.HelmetColor`)))
  (bind _output (`|GetArrayItem` (`self.EquippedCosmetics`) (`KismetArrayLibrary.Array_Find` (`self.Equipped Cosmetic Reference`) "/Game/Fadeout_Content/Core/Characters/Blaise/Skin/blaise_defaultSkin.blaise_defaultSkin")))
  (`/Engine/EditorBlueprintResources/StandardMacros.IsValid` _output
    (:`Is Valid`
      (bind _returnvalue (`KismetMaterialLibrary.CreateDynamicMaterialInstance` (`PrimitiveComponent.GetMaterial` _output 0) "/Game/Fadeout_Content/Core/Characters/Blaise/Skin/M_Blaise_Default.M_Blaise_Default" "None"))
      (bind _output_get (set `self.HelmetDynamic` _returnvalue))
      (`PrimitiveComponent.SetMaterial` _output 0 _output_get)
      (`MaterialInstanceDynamic.SetVectorParameterValue` _output_get "TeamColor" (`KismetMathLibrary.Conv_ColorToLinearColor` _colorrgb))
      (`MaterialInstanceDynamic.SetScalarParameterValue` _output_get "BonusMetallic" _bonusmetallic))))

(event `Color Set`
  (`parent.Color Set`)
  (switch `/Game/Fadeout_Content/Core/UI/Customize/Blaise_Outfits` (cast `/Game/Fadeout_Content/Core/UI/Customize/Blaise_Outfits` (`self.current_outfit`))
    (:`NewEnumerator2`
      (`self.FireFighter Blaise`))
    (:`NewEnumerator4`
      (`self.Sailor Blaise`))
    (:`NewEnumerator3`
      (`self.Miner Blaise`))
    (:`NewEnumerator6`
      (`self.PJ Outfit`))))

(event `Sailor Blaise`
  (bind (_colorrgb _bonusmetallic) (break `/Game/Fadeout_Content/Core/UI/Customize/CustomColor` (`self.HelmetColor`)))
  (bind _output (`|GetArrayItem` (`self.EquippedCosmetics`) (`KismetArrayLibrary.Array_Find` (`self.Equipped Cosmetic Reference`) "/Game/Fadeout_Content/Core/Characters/Kasparian_FBX/outfits/camklle_sailor_v1.camklle_sailor_v1")))
  (`/Engine/EditorBlueprintResources/StandardMacros.IsValid` _output
    (:`Is Valid`
      (bind _returnvalue (`KismetMaterialLibrary.CreateDynamicMaterialInstance` (`PrimitiveComponent.GetMaterial` _output 0) "/Game/Fadeout_Content/Core/Characters/Kasparian_FBX/outfits/M_Sailor_Camille.M_Sailor_Camille" "None"))
      (bind _output_get (set `self.HelmetDynamic` _returnvalue))
      (`PrimitiveComponent.SetMaterial` _output 0 _output_get)
      (`MaterialInstanceDynamic.SetVectorParameterValue` _output_get "TeamColor" (`KismetMathLibrary.Conv_ColorToLinearColor` _colorrgb))
      (`MaterialInstanceDynamic.SetScalarParameterValue` _output_get "BonusMetallic" _bonusmetallic))))

(event `PJ Outfit`
  (bind (_colorrgb _bonusmetallic) (break `/Game/Fadeout_Content/Core/UI/Customize/CustomColor` (`self.HelmetColor`)))
  (bind _output (`|GetArrayItem` (`self.EquippedCosmetics`) (`KismetArrayLibrary.Array_Find` (`self.Equipped Cosmetic Reference`) "/Game/Fadeout_Content/Core/Characters/Blaise/Skin/PJs/PJs_outfit.PJs_outfit")))
  (`/Engine/EditorBlueprintResources/StandardMacros.IsValid` _output
    (:`Is Valid`
      (bind _returnvalue (`KismetMaterialLibrary.CreateDynamicMaterialInstance` (`PrimitiveComponent.GetMaterial` _output 0) "/Game/Fadeout_Content/Core/Characters/Blaise/Skin/PJs/M_PJs.M_PJs" "None"))
      (bind _output_get (set `self.HelmetDynamic` _returnvalue))
      (`PrimitiveComponent.SetMaterial` _output 0 _output_get)
      (`MaterialInstanceDynamic.SetVectorParameterValue` _output_get "TeamColor" (`KismetMathLibrary.Conv_ColorToLinearColor` _colorrgb))
      (`MaterialInstanceDynamic.SetScalarParameterValue` _output_get "BonusMetallic" _bonusmetallic))))

(fn `Attach DoT `
  (params (Class :type "/Game/Fadeout_Content/Core/Weapons/BP_DoT_Effect_Damage_Over_Time Class Reference") (`Instigator Pawn` :type "Pawn Object Reference"))
  (returns (`Applied DoT` :type "/Game/Fadeout_Content/Core/Weapons/BP_DoT_Effect_Damage_Over_Time Object Reference"))
  (if (!= Class "/Game/Fadeout_Content/Core/Weapons/BP_Fire_DOT.BP_Fire_DOT_C")
    (bind _applied_dot (`parent.Attach DoT ` Class `Instigator Pawn`))
    (return _applied_dot)
    (else
      (return null))))

(fn `UserConstructionScript`
  (`parent.UserConstructionScript`))