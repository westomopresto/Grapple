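; BP_Char_Bunn is a playable character with three switchable outfits, a fast-fall move and a stomp attack.
; Outfit meshes follow the main Mesh as master pose, with visibility and body material chosen from the player state's favorite on possession.
; Fast fall replicates through server and multicast events, while falling stomps apply authority-only damage, play a bonk and bounce Bunn up.
; Bunny suit team color comes from the game instance in standalone, otherwise from player state.
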(event `self.Outfit Change Multicast`
  (params (InputPin :type Integer))
  (bind _mesh (`self.Mesh`))
  (set `self.chosenOutfit` InputPin)
  (`SceneComponent.SetVisibility` (`self.polygon`) false false :!label _label)
  (`SceneComponent.SetVisibility` (`self.bunnySuit`) false false)
  (`SceneComponent.SetVisibility` (`self.medicUniform`) false false)
  (`SceneComponent.SetVisibility` (`self.Mesh`) false false)
  (switch `int` (`self.chosenOutfit`)
    (:`0`
      (`SceneComponent.SetVisibility` _mesh true false)
      (`SceneComponent.SetVisibility` (`self.medicUniform`) true false)
      (`PrimitiveComponent.SetMaterial` _mesh 2 (`self.originalbody`)))
    (:`1`
      (`SceneComponent.SetVisibility` (`self.polygon`) true false))
    (:`2`
      (`SceneComponent.SetVisibility` (`self.bunnySuit`) true false)
      (`SceneComponent.SetVisibility` (`self.Mesh`) true false)
      (`PrimitiveComponent.SetMaterial` (`self.Mesh`) 2 (`self.fishnetbody`)))))

(event `fastFall Multicast`
  (`self.LaunchCharacter` (0.0 0.0 -500.0) true))

(event `self.Outfit Change Check LOCAL`
  (params (InputPin :type Integer))
  (set `self.chosenOutfit` InputPin)
  (goto _label))

(event `fastFall Server`
  (`self.fastFall Multicast`))

(event `InputAction|FastFall`
  (params (Key :type "Key Structure"))
  (:`Pressed`
    (if (`NavMovementComponent.IsFalling` (`self.CharacterMovement`))
      (`/Engine/EditorBlueprintResources/ActorMacros.Switch Has Authority`
        (:`Authority`
          (`self.fastFall Multicast`))
        (:`Remote`
          (`self.fastFall Server`))))))

(event `self.ReceiveBeginPlay`
  (`parent.ReceiveBeginPlay`)
  (`self.Outfit Change check`))

(event `self.stomphitbox.OnComponentBeginOverlap`
  (params (OverlappedComponent :type "PrimitiveComponent Object Reference") (OtherActor :type "Actor Object Reference") (OtherComp :type "PrimitiveComponent Object Reference") (OtherBodyIndex :type Integer) (bFromSweep :type Boolean) (SweepResult :type "HitResult Structure (by ref)"))
  (if (`NavMovementComponent.IsFalling` (`self.CharacterMovement`))
    (`/Engine/EditorBlueprintResources/ActorMacros.Switch Has Authority`
      (:`Authority`
        (if (!= OtherActor self)
          (bind _asbp_player_character (cast `/Game/Fadeout_Content/Core/Characters/BP_PlayerCharacter` OtherActor))
          (`GameplayStatics.ApplyDamage` _asbp_player_character 150.0 (`self.GetController`) null "/Game/Fadeout_Content/Core/Weapons/DamageTypes/DT_Pick.DT_Pick_C")
          (`self.stomp Effects` (`.Location` (`GameplayStatics.BreakHitResult` SweepResult)))
          (`self.BounceUp`))))))

(event `BounceUp`
  (`self.LaunchCharacter` (0.0 0.0 500.0) false true))

(event `stomp Effects`
  (params (Location :type "Vector Structure"))
  (`GameplayStatics.PlaySoundAtLocation` "/Game/Fadeout_Content/Core/Audio/Silly/coconut_bonk.coconut_bonk" Location (struct) 3.0 1.0 0.0 null null null))

(event `self.ReceivePossessed`
  (params (NewController :type "Controller Object Reference"))
  (`parent.ReceivePossessed` NewController)
  (bind _asfo_player_state (cast `/Game/Fadeout_Content/Core/Support/Multiplayer_Support/FO_PlayerState` (`Controller.PlayerState` NewController)))
  (`self.Outfit Change Multicast` (`KismetMathLibrary.Conv_ByteToInt` (`/Game/Fadeout_Content/Core/Support/Multiplayer_Support/FO_PlayerState.fav-outfit_Friday` _asfo_player_state))))

(event `self.update Color Local`
  (bind _bunnysuit (`self.bunnySuit`))
  (bind _helmetdynamic (`self.HelmetDynamic`))
  (if (`KismetSystemLibrary.IsStandalone`) :!label _label_2
    (bind _asfadeout_game_instance (cast `/Game/Fadeout_GameInstance` (`GameplayStatics.GetGameInstance`)))
    (set `self.HelmetColor` (`/Game/Fadeout_GameInstance.MultiplayerColor` _asfadeout_game_instance))
    (else
      (bind _asfo_player_state (cast `/Game/Fadeout_Content/Core/Support/Multiplayer_Support/FO_PlayerState` (`self.PlayerState`)))
      (set `self.HelmetColor` (`/Game/Fadeout_Content/Core/Support/Multiplayer_Support/FO_PlayerState.CustomColor` _asfo_player_state))))
  (`/Engine/EditorBlueprintResources/StandardMacros.IsValid` _helmetdynamic
    (:`Is Valid`
      _)
    (:`Is Not Valid`
      (bind _returnvalue (`KismetMaterialLibrary.CreateDynamicMaterialInstance` (`PrimitiveComponent.GetMaterial` _bunnysuit 0) "/Game/Fadeout_Content/Core/Characters/Bunn/outfits/m_bunnySuit.m_bunnySuit" "None"))
      (bind _output_get (set `self.HelmetDynamic` _returnvalue))
      (`PrimitiveComponent.SetMaterial` _bunnysuit 0 _output_get)))
  (`MaterialInstanceDynamic.SetVectorParameterValue` _helmetdynamic "TeamColor" (`KismetMathLibrary.Conv_ColorToLinearColor` (`self.HelmetColor`))))

(event `self.SetFavColor`
  (goto _label_2))

(fn `UserConstructionScript`
  (bind _mesh (`self.Mesh`))
  (`parent.UserConstructionScript`)
  (`SkinnedMeshComponent.SetLeaderPoseComponent` (`self.polygon`) _mesh true)
  (`SkinnedMeshComponent.SetLeaderPoseComponent` (`self.bunnySuit`) _mesh true)
  (`SkinnedMeshComponent.SetLeaderPoseComponent` (`self.medicUniform`) _mesh true)
  (bind _returnvalue (`PrimitiveComponent.CreateDynamicMaterialInstance` _mesh 2 (`PrimitiveComponent.GetMaterial` _mesh 2) "None"))
  (set `self.originalbody` _returnvalue)
  (bind _returnvalue_2 (`PrimitiveComponent.CreateDynamicMaterialInstance` _mesh 2 "/Game/Fadeout_Content/Core/Characters/Bunn/outfits/M_Friday_Body_fishnet.M_Friday_Body_fishnet" "None"))
  (set `self.fishnetbody` _returnvalue_2))