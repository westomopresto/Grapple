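; BP_snek_dummy is a dummy character that displays an outfit and can optionally hold a rifle.
; On BeginPlay it reads DaltonOutfit from the Fadeout game instance and passes it as an integer to OutfitChangeMulticast.
; When HoldingDummyRifle is set, the construction script adds a rifle skeletal mesh and attaches it to the body mesh's GunSocket.
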(event `self.ReceiveBeginPlay`
  (`parent.ReceiveBeginPlay`)
  (bind _asfadeout_game_instance (cast `/Game/Fadeout_GameInstance` (`GameplayStatics.GetGameInstance`)))
  (`self.Outfit Change Multicast` (`KismetMathLibrary.Conv_ByteToInt` (`/Game/Fadeout_GameInstance.daltonOutfit` _asfadeout_game_instance))))

(fn `UserConstructionScript`
  (bind _mesh (`self.Mesh`))
  (if (`self.holdingDummyRifle`)
    (bind _returnvalue (`AddComponent|NODE_AddSkeletalMeshComponent-0` :`RelativeTransform` (`SceneComponent.GetSocketTransform` _mesh "GunSocket" "RTS_Actor")))
    (`SkinnedMeshComponent.SetSkinnedAssetAndUpdate` _returnvalue "/Game/Fadeout_Content/Core/FBX/MAS_GUn/mas_rifle_f_01.mas_rifle_f_01" true)
    (`SceneComponent.K2_AttachToComponent` _returnvalue _mesh "GunSocket" "KeepWorld" "KeepWorld" "KeepWorld" true))
  (`parent.UserConstructionScript`))