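; BP_wolf_dummy is a wolf dummy character that arms itself with a dummy harpoon gun instead of starter weapons.
; EquipStarterWeapons is overridden empty; BeginPlay spawns Dummy_Harpoon_Gun firing BP_Harpoon_Projectile, then picks it up and equips it through inherited functions.
; It turns off replication on all equipment and destroys the spawned gun when its own play ends.
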(event `self.EquipStarter_Weapons`)

(event `self.ReceiveBeginPlay`
  (`parent.ReceiveBeginPlay`)
  (bind _returnvalue (`|SpawnActorFromClass` "/Game/Fadeout_Content/Core/Weapons/Dummy_Harpoon_Gun.Dummy_Harpoon_Gun_C" (`KismetMathLibrary.MakeTransform` (`self.K2_GetActorLocation`)) "Undefined" "OverrideRootScale" (`self.GetOwner`) "/Game/Fadeout_Content/Core/Weapons/BP_Harpoon_Projectile.BP_Harpoon_Projectile_C" true false null))
  (set `self.dummyWeapon` _returnvalue)
  (`self.weaponPickupFunction` _returnvalue)
  (add `self.OnEndPlay` (delegate `Destroy Our weapon`))
  (`self.EquipItemFunction` 0)
  (for _array_element (`self.equipment`)
    (`self.SetReplicates` _array_element false)))

(event `Destroy Our weapon` :!signature `self.OnEndPlay`
  (params (Actor :type "Actor Object Reference") (EndPlayReason :type "EEndPlayReason Enum" :default "Destroyed"))
  (bind _dummyweapon (`self.dummyWeapon`))
  (`/Engine/EditorBlueprintResources/StandardMacros.IsValid` _dummyweapon
    (:`Is Valid`
      (`self.K2_DestroyActor` _dummyweapon))))

(fn `UserConstructionScript`
  (`parent.UserConstructionScript`))