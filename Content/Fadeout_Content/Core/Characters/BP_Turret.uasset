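; Player-deployed AI turret character that takes its skin from the owner's outfit and its material tint from team or custom color.
; On spawn it starts a behavior tree as a non-patrolling hostile and culls the owner's structures beyond two.
; It self-destructs without a living owner, ignores owner damage up to 500, and faces other attackers.
; Perception updates refresh an enemy-only outline, while firing triggers alert and combat-loop audio through retriggerable delays.
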(event `Loop Sound kill`
  (bind _loopsound (`self.LoopSound`))
  ;[1 1 1] SFX
  (`/Engine/EditorBlueprintResources/StandardMacros.IsValid` _loopsound
    (:`Is Valid`
      (`AudioComponent.Stop` _loopsound))))

(event `Found you sound`
  ;[1 1 1] SFX
  (`GameplayStatics.PlaySoundAtLocation` "/Game/Fadeout_Content/Core/Audio/Weapon_SFX/Turret_SFX/Turret_Alert_V2.Turret_Alert_V2" (`self.K2_GetActorLocation`) (struct) 1.5 1.0 0.0 null null null))

(event `self.Fire Held Item`
  (`parent.Fire Held Item`)
  (`|ExecutionSequence`
    (:`then_0`
      (`/Engine/EditorBlueprintResources/StandardMacros.DoOnce` false :!label _label
        (:`Completed`
          (`self.Found you sound`))))
    (:`then_1`
      (`KismetSystemLibrary.RetriggerableDelay` 4.0)
      (goto _label :!via `Reset`))
    (:`then_2`
      (`self.Change Loop` true)
      (`KismetSystemLibrary.RetriggerableDelay` 3.0)
      (`self.Change Loop` false))))

(event `Change Loop`
  (params (`Combat?` :type Boolean))
  (bind _loopsound (`self.LoopSound`))
  ;[1 1 1] SFX
  (`/Engine/EditorBlueprintResources/StandardMacros.IsValid` _loopsound
    (:`Is Valid`
      (if `Combat?`
        (`AudioComponent.SetSound` _loopsound "/Game/Fadeout_Content/Core/Audio/Weapon_SFX/Turret_SFX/Turret_Active.Turret_Active")
        (else
          (`AudioComponent.SetSound` _loopsound "/Game/Fadeout_Content/Core/Audio/Weapon_SFX/Turret_SFX/Turret_V2.Turret_V2"))))))

(event `self.AIPerception.OnTargetPerceptionUpdated`
  (params (Actor :type "Actor Object Reference") (Stimulus :type "AIStimulus Structure"))
  (`self.EnemyCheck`))

(event `EnemyCheck`
  (bind _pixel_outline_controller (`self.Pixel_Outline_Controller`))
  (bind _playerstate (`Controller.PlayerState` (`GameplayStatics.GetPlayerController` 0)))
  ;[1 1 1] Enemy outline
  (`/Engine/EditorBlueprintResources/StandardMacros.IsValid` _playerstate
    (:`Is Valid`
      (bind (_triggered _team) (`self.IsEnemyToLocal` _playerstate))
      (bind _output_get (set `self.EnemyTurret` _triggered))
      (set `/Game/Fadeout_Content/Core/Post/Pixel_Outline_Controller.Enabled` _output_get _pixel_outline_controller)
      (set `/Game/Fadeout_Content/Core/Post/Pixel_Outline_Controller.team` _team _pixel_outline_controller))))

(event `self.ReceiveTick`
  (params (DeltaSeconds :type "Float (single-precision)"))
  (bind _instigator (`self.Instigator`))
  (`SceneComponent.K2_SetWorldRotation` (`self.turretBody_01`) (`KismetMathLibrary.FindLookAtRotation` (`KismetMathLibrary.MakeVector` 0.0) (`self.forwardVector`)) false false)
  (`/Engine/EditorBlueprintResources/ActorMacros.Switch Has Authority`
    (:`Authority`
      (`parent.ReceiveTick` DeltaSeconds)
      (if (`self.alive?`)
        (`/Engine/EditorBlueprintResources/StandardMacros.IsValid` _instigator
          (:`Is Valid`
            (bind _asbp_player_character (cast `/Game/Fadeout_Content/Core/Characters/BP_PlayerCharacter` _instigator))
            (if (not (`/Game/Fadeout_Content/Core/Characters/BP_PlayerCharacter.alive?` _asbp_player_character))
              (`GameplayStatics.ApplyDamage` self 999.0 :!label _label_2)))
          (:`Is Not Valid`
            (goto _label_2)))))))

(event `self.lerpCameraSocket`
  (params (cameraSocketSelection :type Integer))
  ;[1 1 1] Do nothing
)

(event `self.ZoomCamera`
  (params (`Zoom?` :type Boolean) (Scope :type Boolean))
  ;[1 1 1] Do nothing
)

(event `self.ReceiveAnyDamage`
  (params (Damage :type "Float (single-precision)") (DamageType :type "DamageType Object Reference") (InstigatedBy :type "Controller Object Reference") (DamageCauser :type "Actor Object Reference"))
  (bind _instigator (`self.Instigator`))
  (`/Engine/EditorBlueprintResources/StandardMacros.IsValid` _instigator
    (:`Is Valid`
      (if (== (`self.GetInstigatorController` _instigator) InstigatedBy)
        (`parent.ReceiveAnyDamage` (`KismetMathLibrary.SelectFloat` 0.0 Damage (<= Damage 500.0)) DamageType InstigatedBy DamageCauser)
        (else
          (`parent.ReceiveAnyDamage` Damage DamageType InstigatedBy DamageCauser :!label _label_3))))
    (:`Is Not Valid`
      (goto _label_3)))
  (`/Engine/EditorBlueprintResources/StandardMacros.IsValid` (`AIBlueprintHelperLibrary.GetBlackboard` (`self.GetController`))
    (:`Is Valid`
      (`/Engine/EditorBlueprintResources/StandardMacros.IsValid` InstigatedBy
        (:`Is Valid`
          (`AIController.K2_SetFocalPoint` (`AIBlueprintHelperLibrary.GetAIController` self) (`self.K2_GetActorLocation` (`Controller.K2_GetPawn` InstigatedBy))))))))

(event `self.Death Check`
  (bind _returnvalue (`AIBlueprintHelperLibrary.GetAIController` self))
  (if (not (`self.alive?`))
    (`GameplayStatics.SpawnEmitterAttached` "/Game/StylizedVFX_Fire/Effects/P_FireSmoke_Large.P_FireSmoke_Large" (`self.Mesh`) "None" (0.0 0.0 25.0) (struct) (2.0 2.0 2.0) "SnapToTarget")
    (`parent.Death Check`)
    (`/Engine/EditorBlueprintResources/StandardMacros.IsValid` _returnvalue
      (:`Is Valid`
        (`ActorComponent.Deactivate` (`AIController.BrainComponent` _returnvalue))))))

(event `Turret Skins`
  (bind _asbp_player_character (cast `/Game/Fadeout_Content/Core/Characters/BP_PlayerCharacter` (`self.Instigator`)))
  (bind _output_get (set `self.ThisTurretSkin` (cast `/Game/Fadeout_Content/Core/UI/Customize/Abigail_Outfits` (`/Game/Fadeout_Content/Core/Characters/BP_PlayerCharacter.current_outfit` _asbp_player_character))))
  (switch `/Game/Fadeout_Content/Core/UI/Customize/Abigail_Outfits` _output_get
    (:`NewEnumerator0`
      (bind _returnvalue (`PrimitiveComponent.CreateDynamicMaterialInstance` (`self.Mesh`) 0 "/Game/Fadeout_Content/Core/FBX/Turret/M_Turret.M_Turret" "None" :!label _label_4))
      (bind _output_get_2 (set `self.TurretMaterial` _returnvalue))
      (`PrimitiveComponent.SetMaterial` (`self.turretBody_01`) 0 _output_get_2))
    (:`NewEnumerator1`
      (`SkinnedMeshComponent.SetSkinnedAssetAndUpdate` (`self.Mesh`) "/Game/Fadeout_Content/Core/FBX/Turret/turret_Skins/turretHead_Pirate_01.turretHead_Pirate_01" true)
      (`StaticMeshComponent.SetStaticMesh` (`self.turretBody_01`) "/Game/Fadeout_Content/Core/FBX/Turret/turret_Skins/turretBody_Pirate_01.turretBody_Pirate_01")
      (bind _returnvalue_2 (`PrimitiveComponent.CreateDynamicMaterialInstance` (`self.Mesh`) 0 "/Game/Fadeout_Content/Core/FBX/Turret/turret_Skins/M_Turret1.M_Turret1" "None"))
      (bind _output_get_3 (set `self.TurretMaterial` _returnvalue_2))
      (`PrimitiveComponent.SetMaterial` (`self.turretBody_01`) 0 _output_get_3))
    (:`NewEnumerator2`
      (goto _label_4))
    (:`NewEnumerator3`
      (`SkinnedMeshComponent.SetSkinnedAssetAndUpdate` (`self.Mesh`) "/Game/Fadeout_Content/Core/FBX/Turret/turret_Skins/Groovy_head_rig.Groovy_head_rig" true)
      (`StaticMeshComponent.SetStaticMesh` (`self.turretBody_01`) "/Game/Fadeout_Content/Core/FBX/Turret/turret_Skins/Groovy_body_static.Groovy_body_static")
      (bind _returnvalue_3 (`PrimitiveComponent.CreateDynamicMaterialInstance` (`self.Mesh`) 0 "/Game/Fadeout_Content/Core/FBX/Turret/turret_Skins/M_turret_groovy.M_turret_groovy" "None"))
      (bind _output_get_4 (set `self.TurretMaterial` _returnvalue_3))
      (`PrimitiveComponent.SetMaterial` (`self.turretBody_01`) 0 _output_get_4)
      (`PrimitiveComponent.SetMaterial` (`self.Mesh`) 0 _output_get_4))))

(event `self.ReceiveBeginPlay`
  (bind _mesh (`self.Mesh`))
  (bind _turretmaterial (`self.TurretMaterial`))
  (bind _turretcolor (`self.turretColor`))
  (bind _returnvalue (`AIBlueprintHelperLibrary.GetBlackboard` (`self.GetController`)))
  (bind _returnvalue_2 (`AIBlueprintHelperLibrary.GetAIController` self))
  (`parent.ReceiveBeginPlay`)
  (set `self.forwardVector` (`self.GetActorForwardVector`))
  (`SceneComponent.K2_SetWorldRotation` (`self.turretBody_01`) (`KismetMathLibrary.FindLookAtRotation` (`KismetMathLibrary.MakeVector` 0.0) (`self.forwardVector`)) false false)
  (`self.Turret Skins`)
  (`self.EnemyCheck`)
  (set `self.OwningPlayerState` (`Pawn.PlayerState` (`self.Instigator`)))
  (`|ExecutionSequence`
    (:`then_0`
      (`GameplayStatics.SpawnSoundAttached` (select `/Game/Fadeout_Content/Core/UI/Customize/Abigail_Outfits` (`self.ThisTurretSkin`) :`NewEnumerator0` "/Game/Fadeout_Content/Core/Audio/Weapon_SFX/Turret_SFX/TurretBuild_V3.TurretBuild_V3" :`NewEnumerator1` "/Game/Fadeout_Content/Core/Audio/Weapon_SFX/Turret_SFX/TurretBuild_Alts/Pirate_Spawn.Pirate_Spawn" :`NewEnumerator2` "/Game/Fadeout_Content/Core/Audio/Weapon_SFX/Turret_SFX/TurretBuild_V3.TurretBuild_V3" :`NewEnumerator3` "/Game/Fadeout_Content/Core/Audio/Weapon_SFX/Turret_SFX/TurretTeleport/Turret_Teleport_Cue.Turret_Teleport_Cue" :!type "SoundBase Object Reference") _mesh "None" (0.0 0.0 0.0) (struct) "KeepRelativeOffset" true 1.0 1.0 0.0 null null))
    (:`then_1`
      (bind _returnvalue_3 (`GameplayStatics.SpawnEmitterAttached` "/Game/2dFX_Pack/Particles/P_BuildCircle.P_BuildCircle" _mesh "None" (0.0 0.0 40.0) (struct) (1.5 1.5 2.0)))
      (`KismetSystemLibrary.Delay` 1.0)
      (`/Engine/EditorBlueprintResources/StandardMacros.IsValid` _returnvalue_3
        (:`Is Valid`
          (`ActorComponent.Deactivate` _returnvalue_3)
          (`ActorComponent.Deactivate` (`self.ParticleSystem`)))
        (:`Is Not Valid`
          _))
      (`|ExecutionSequence`
        (:`then_0`
          (`self.SpawnLoopSound`))
        (:`then_1`
          (`/Engine/EditorBlueprintResources/ActorMacros.Switch Has Authority`
            (:`Authority`
              (`/Engine/EditorBlueprintResources/StandardMacros.IsValid` _returnvalue_2
                (:`Is Valid`
                  (`AIController.RunBehaviorTree` _returnvalue_2 (`self.Default Behavior_0`))
                  (`KismetSystemLibrary.Delay` 0.5)
                  (`/Engine/EditorBlueprintResources/StandardMacros.IsValid` _returnvalue
                    (:`Is Valid`
                      (`BlackboardComponent.SetValueAsVector` _returnvalue "Home" (`self.K2_GetActorLocation`))
                      (`BlackboardComponent.SetValueAsBool` _returnvalue "Patrols?" false)
                      (`BlackboardComponent.SetValueAsBool` _returnvalue "PlayerHostile?" true))))))))
        (:`then_2`
          (`KismetSystemLibrary.Delay` 0.1)
          (bind _asbp_player_character (cast `/Game/Fadeout_Content/Core/Characters/BP_PlayerCharacter` (`self.Instigator`)))
          (bind _ownedstructures (`/Game/Fadeout_Content/Core/Characters/BP_PlayerCharacter.OwnedStructures` _asbp_player_character))
          (`KismetArrayLibrary.Array_Add` _ownedstructures self)
          (if (> (`KismetArrayLibrary.Array_Length` _ownedstructures) 2)
            (for _array_element _ownedstructures
              (`GameplayStatics.ApplyDamage` _array_element 999.0 (`self.GetInstigatorController` (`self.OwningPlayerState`)) self)
              (if (<= (`KismetArrayLibrary.Array_Length` _ownedstructures) 2)
                (break)))))
        (:`then_3`
          (bind _asfo_player_state (cast `/Game/Fadeout_Content/Core/Support/Multiplayer_Support/FO_PlayerState` (`self.OwningPlayerState`)))
          (switch `string` (`/Game/Fadeout_Content/Core/Support/Multiplayer_Support/FO_PlayerState.Team` _asfo_player_state)
            (:`Default`
              (bind (_colorrgb _bonusmetallic) (break `/Game/Fadeout_Content/Core/UI/Customize/CustomColor` (`/Game/Fadeout_Content/Core/Support/Multiplayer_Support/FO_PlayerState.CustomColor` _asfo_player_state)))
              (set `self.turretColor` (`KismetMathLibrary.Conv_ColorToLinearColor` _colorrgb) :!label _label_5))
            (:`FFA`
              (goto _label_5))
            (:`red`
              (set `self.turretColor` (struct :`R` 1.0 :`A` 1.0)))
            (:`blue`
              (set `self.turretColor` (struct :`G` 0.067369 :`B` 1.0 :`A` 1.0))))
          (`/Engine/EditorBlueprintResources/StandardMacros.IsValid` _turretmaterial
            (:`Is Valid`
              _)
            (:`Is Not Valid`
              (`self.Turret Skins`)))
          (`MaterialInstanceDynamic.SetVectorParameterValue` _turretmaterial "TeamColor" _turretcolor)
          (`MaterialInstanceDynamic.SetScalarParameterValue` _turretmaterial "BonusMetallic" _bonusmetallic)
          (`MaterialInstanceDynamic.SetVectorParameterValue` _turretmaterial "EmissiveColorMod" _turretcolor))))))

(event `self.ConsumesOnDeath`
  (`parent.ConsumesOnDeath`)
  (`self.Loop Sound kill`)
  (`/Engine/EditorBlueprintResources/StandardMacros.IsValid` (`self.Instigator`)
    (:`Is Valid`
      (bind _asbp_player_character (cast `/Game/Fadeout_Content/Core/Characters/BP_PlayerCharacter` (`self.Instigator`)))
      (`KismetArrayLibrary.Array_RemoveItem` (`/Game/Fadeout_Content/Core/Characters/BP_PlayerCharacter.OwnedStructures` _asbp_player_character) self))))

(event `self.Notify_Controller_WeDied`
  (params (controllerForDeath :type "Controller Object Reference"))
  ;[1 1 1] commenting this out
)

(event `self.ReceiveUnpossessed`
  (params (OldController :type "Controller Object Reference"))
  (`|ExecutionSequence`
    (:`then_0`
      (bind _asaicontroller (cast `AIController` OldController))
      (bind _braincomponent (`AIController.BrainComponent` _asaicontroller))
      (`/Engine/EditorBlueprintResources/StandardMacros.IsValid` _braincomponent
        (:`Is Valid`
          (`ActorComponent.Deactivate` _braincomponent))))
    (:`then_1`
      (`self.DetachFromControllerPendingDestroy`))))

(event `self.Ragdoll Collide`
  (params (HitComponent :type "PrimitiveComponent Object Reference") (OtherActor :type "Actor Object Reference") (OtherComp :type "PrimitiveComponent Object Reference") (NormalImpulse :type "Vector Structure") (Hit :type "HitResult Structure (by ref)")))

(fn `IsEnemyToLocal`
  (params (`Player State` :type "PlayerState Object Reference"))
  (returns (Triggered :type Boolean) (Team :type String))
  (bind _playerstate (`Pawn.PlayerState` (`self.Instigator`)))
  (bind _returnvalue (!= (`PlayerState.PlayerId` `Player State`) (`PlayerState.PlayerId` _playerstate)))
  (`/Engine/EditorBlueprintResources/StandardMacros.IsValid` (`self.Instigator`)
    (:`Is Valid`
      (bind _asfo_player_state (cast `/Game/Fadeout_Content/Core/Support/Multiplayer_Support/FO_PlayerState` `Player State`))
      (bind _asfo_player_state_2 (cast `/Game/Fadeout_Content/Core/Support/Multiplayer_Support/FO_PlayerState` _playerstate))
      (bind _team (`/Game/Fadeout_Content/Core/Support/Multiplayer_Support/FO_PlayerState.Team` _asfo_player_state))
      (if (`KismetStringLibrary.NotEqual_StrStr` _team "FFA")
        (if (and (not (`KismetStringLibrary.EqualEqual_StrStr` _team (`/Game/Fadeout_Content/Core/Support/Multiplayer_Support/FO_PlayerState.Team` _asfo_player_state_2))) _returnvalue)
          _
          (else
            (return false _team)))
        (else
          ;[1 1 1] FFA
          (if _returnvalue
            _
            (else
              (return false _team)))))
      (return true _team))
    (:`Is Not Valid`
      (return false ""))))

(fn `SpawnLoopSound`
  (bind _returnvalue (`GameplayStatics.SpawnSoundAttached` "/Game/Fadeout_Content/Core/Audio/Weapon_SFX/Turret_SFX/Turret_V2.Turret_V2" (`self.Mesh`) "None" (0.0 0.0 0.0) (struct) "KeepRelativeOffset" true 1.0 1.0 0.0 "/Game/Fadeout_Content/Core/Characters/Turret_Attenuation.Turret_Attenuation" "/Game/Fadeout_Content/Core/Characters/quote_concurrency.quote_concurrency"))
  (set `self.LoopSound` _returnvalue))

(fn `UserConstructionScript`
  (`parent.UserConstructionScript`))