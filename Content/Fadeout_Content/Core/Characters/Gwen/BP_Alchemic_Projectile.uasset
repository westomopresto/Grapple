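; Gwen's alchemic projectile, which explodes on impact and applies an alchemic damage-over-time buff to damaged player characters.
; BuffCheck ends matching attached buffs, then attaches a fresh AlchemicBuff flagged for friendly targets, destroying the projectile when it ends.
; Overlaps respect CanhurtOwner; surface impacts trigger a multicast that stops, hides and delay-destroys it while lowering net update rates.
; Construction tints the trail with AlchemicColor; ArrowAttach is defined but uncalled here.
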(event `self.ReceiveBeginPlay`
  ;[1 1 1] Begin Play
  (add `self.damagedThisActor` (delegate `Buff Check`))
  (`|ExecutionSequence`
    (:`then_0`
      (`PrimitiveComponent.IgnoreActorWhenMoving` (`self.Capsule`) self true)
      (`PrimitiveComponent.IgnoreActorWhenMoving` (`self.CollisionSphere`) self true)
      (`parent.ReceiveBeginPlay`))
    (:`then_1`
      ;[1 1 1] damage scale
      (set `self.explode on impact?` true))))

(event `self.SurfaceImpactEvent`
  (params (HitResult :type "HitResult Structure") (`Hardsurface?` :type Boolean) (hitactor :type "Actor Object Reference"))
  (`self.onProjectileHit`)
  (`self.PlayImpactEffects` HitResult `Hardsurface?`)
  (`PrimitiveComponent.SetCollisionEnabled` (`self.CollisionSphere`) "NoCollision")
  (`PrimitiveComponent.SetCollisionEnabled` (`self.Capsule`) "NoCollision")
  (`/Engine/EditorBlueprintResources/ActorMacros.Switch Has Authority`
    (:`Authority`
      (`self.MultiCast Attach` HitResult))))

(event `MultiCast Attach`
  (params (HitResult :type "HitResult Structure"))
  (`|ExecutionSequence`
    (:`then_0`
      (`ProjectileMovementComponent.StopSimulating` (`self.ProjectileMovement`) HitResult)
      (`SceneComponent.SetVisibility` (`self.Mesh`) false true))
    (:`then_1`
      (set `self.MinNetUpdateFrequency` 1.0)
      (set `self.NetUpdateFrequency` 1.0)
      (`ActorComponent.Deactivate` (`self.K2_GetComponentsByClass` "/Script/Engine.ParticleSystemComponent"))
      (`AudioComponent.FadeOut` (`self.Audio`) 0.25 0.0 "Linear")
      (`KismetSystemLibrary.Delay` (`self.DestroyDelayAfterImpact`))
      (`self.K2_DestroyActor`))))

(event `self.CollisionSphere.OnComponentBeginOverlap`
  (params (OverlappedComponent :type "PrimitiveComponent Object Reference") (OtherActor :type "Actor Object Reference") (OtherComp :type "PrimitiveComponent Object Reference") (OtherBodyIndex :type Integer) (bFromSweep :type Boolean) (SweepResult :type "HitResult Structure (by ref)"))
  (bind _asbp_player_character (cast `/Game/Fadeout_Content/Core/Characters/BP_PlayerCharacter` OtherActor)
    (:`then`
      (if (== (`self.GetOwner`) _asbp_player_character)
        (if (`self.canhurtOwner`)
          (`self.OnProjectileHitEvent` OtherActor OtherComp SweepResult :!label _label))
        (else
          (goto _label))))
    (:`CastFailed`
      (`self.OnProjectileHitEvent` OtherActor OtherComp SweepResult))))

(event `Buff Check` :!signature `self.damagedThisActor`
  (params (CharacterDamaged :type "Actor Object Reference"))
  (bind _alchemicbuff (`self.AlchemicBuff`))
  (bind _asbp_player_character (cast `/Game/Fadeout_Content/Core/Characters/BP_PlayerCharacter` CharacterDamaged))
  (bind (_sameteam _ffa_ _valid) (`/Game/Fadeout_Content/Core/Characters/BP_PlayerCharacter.CheckTeamDamage` _asbp_player_character (`self.Instigator Controller`)))
  (if (`KismetSystemLibrary.IsValidClass` _alchemicbuff)
    (for _array_element (`self.GetAttachedActors` _asbp_player_character true)
      (bind _asbp_alchemic_buff_damage (cast `/Game/Fadeout_Content/Core/Weapons/BP_Alchemic_Buff_Damage` _array_element))
      (if (== (`GameplayStatics.GetObjectClass` _asbp_alchemic_buff_damage) (`self.AlchemicBuff`))
        (`/Game/Fadeout_Content/Core/Weapons/BP_DoT_Effect_Damage_Over_Time.earlyEnd` _asbp_alchemic_buff_damage)))
    (bind _returnvalue (and _sameteam (not _ffa_) _valid))
    (bind _applied_dot (`/Game/Fadeout_Content/Core/Characters/BP_PlayerCharacter.Attach DoT ` _asbp_player_character _alchemicbuff (`self.Instigator`) _returnvalue false))
    (add `/Game/Fadeout_Content/Core/Weapons/BP_DoT_Effect_Damage_Over_Time.DoT_Ended` _applied_dot (delegate `DoT_Ended_Event`))
    (if _returnvalue
      _)))

(event `DoT_Ended_Event`
  (`KismetSystemLibrary.Delay` 0.2)
  (`self.K2_DestroyActor`))

(fn `ArrowAttach`
  (params (Hit :type "HitResult Structure (by ref)"))
  (bind (_bblockinghit _binitialoverlap _time _distance _location _impactpoint _normal _impactnormal _physmat _hitactor _hitcomponent _hitbonename) (`GameplayStatics.BreakHitResult` Hit))
  (`/Engine/EditorBlueprintResources/StandardMacros.IsValid` _hitactor
    (:`Is Valid`
      (if (!= _hitactor self)
        (cast `/Game/Fadeout_Content/Core/Characters/BP_PlayerCharacter` _hitactor
          (:`then`
            (`self.K2_AttachToComponent` _hitcomponent _hitbonename "SnapToTarget" "KeepWorld" "KeepWorld")
            (set `self.Attached` true)
            (return))
          (:`CastFailed`
            (bind _asbp_target_practice (cast `/Game/Fadeout_Content/Core/Debug/BP_TargetPractice` _hitactor)
              (:`then`
                (`self.K2_AttachToComponent` (`/Game/Fadeout_Content/Core/Debug/BP_TargetPractice.Offset` _asbp_target_practice) "None" "KeepWorld" "KeepWorld" "KeepWorld")
                (set `self.Attached` true)
                (return))
              (:`CastFailed`
                (`self.K2_AttachToActor` _hitactor "None" "KeepWorld" "KeepWorld" "KeepWorld")
                (set `self.Attached` true)
                (return)))))
        (else
          (`KismetSystemLibrary.PrintString` "COLLIDING WITH SELF SOMEHOW")
          (`KismetSystemLibrary.PrintString` (`KismetSystemLibrary.GetDisplayName` _hitcomponent))
          (return))))
    (:`Is Not Valid`
      (return))))

(fn `UserConstructionScript`
  (`parent.UserConstructionScript`)
  (`FXSystemComponent.SetColorParameter` (`self.trail`) "ParticleColor" (`self.Alchemic_Color`)))