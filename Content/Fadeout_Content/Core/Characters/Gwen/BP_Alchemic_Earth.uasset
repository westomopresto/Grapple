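; Earth variant of Gwen's alchemic Blueprints, appearing as a rock that bursts on surface impact.
; On BeginPlay it randomly picks its mesh from three rock models, though the Length-1 bound on RandomInteger leaves the last one unused.
; On surface impact it spawns a scaled-down meteor explosion aligned to the hit normal, then passes the hit to the parent class's impact handling.
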(event `self.ReceiveBeginPlay`
  (bind _array (`|MakeArray` "/Game/Fadeout_Content/Core/Characters/Gwen/Element_Rocks_rock_01.Element_Rocks_rock_01" "/Game/Fadeout_Content/Core/Characters/Gwen/Element_Rocks_rock_02.Element_Rocks_rock_02" "/Game/Fadeout_Content/Core/Characters/Gwen/Element_Rocks_rock_03.Element_Rocks_rock_03" :!type "StaticMesh Object Reference"))
  (`parent.ReceiveBeginPlay`)
  (`StaticMeshComponent.SetStaticMesh` (`self.Mesh`) (`|GetArrayItem` _array (`KismetMathLibrary.RandomInteger` (- (`KismetArrayLibrary.Array_Length` _array) 1)))))

(event `self.SurfaceImpactEvent`
  (params (HitResult :type "HitResult Structure") (`Hardsurface?` :type Boolean) (hitactor :type "Actor Object Reference"))
  (bind (_bblockinghit _binitialoverlap _time _distance _location _impactpoint _normal) (`GameplayStatics.BreakHitResult` HitResult))
  (`GameplayStatics.SpawnEmitterAtLocation` "/Game/VFX_Toolkit_V1/ParticleSystems/356Days/Par_Meteora_Explode_02.Par_Meteora_Explode_02" _location (`KismetMathLibrary.MakeRotFromZ` _normal) (0.2 0.2 0.2))
  (`parent.SurfaceImpactEvent` HitResult `Hardsurface?` hitactor))

(fn `UserConstructionScript`
  (`parent.UserConstructionScript`))