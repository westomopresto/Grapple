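; Gwen's air alchemic projectile, which spawns a BP_Alchemic_Cyclone at its impact point.
; On the server, with a valid owning weapon, physical hits trigger it directly, while other contacts require a player passing the team-damage check (enemy or free-for-all).
; A DoOnce limits it to one cyclone, then the projectile forces a net update and destroys itself after a delay.
; The construction script tints the mesh with AlchemicColor.
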(event `self.OnProjectileHitEvent`
  (params (OtherActor :type "Actor Object Reference") (OtherComponent :type "PrimitiveComponent Object Reference") (HitResult :type "HitResult Structure (by ref)") (fromHit :type Boolean))
  (`parent.OnProjectileHitEvent` OtherActor OtherComponent HitResult fromHit)
  (`/Engine/EditorBlueprintResources/ActorMacros.Switch Has Authority`
    (:`Authority`
      (`self.OwningWeapon`
        (:`then`
          (if fromHit
            (`/Engine/EditorBlueprintResources/StandardMacros.DoOnce` false :!label _label
              (:`Completed`
                (`|SpawnActorFromClass` "/Game/Fadeout_Content/Core/Characters/Gwen/BP_Alchemic_Cyclone.BP_Alchemic_Cyclone_C" (`KismetMathLibrary.MakeTransform` (`.ImpactPoint` (`GameplayStatics.BreakHitResult` HitResult))) "AlwaysSpawn" "OverrideRootScale" (`self.GetOwner`) (`self.GetInstigator`))
                (`self.ForceNetUpdate`)
                (`KismetSystemLibrary.Delay` (`self.DestroyDelayAfterImpact`))
                (`self.K2_DestroyActor`)))
            (else
              (bind _asbp_player_character (cast `/Game/Fadeout_Content/Core/Characters/BP_PlayerCharacter` OtherActor))
              (bind (_sameteam _ffa_ _valid) (`/Game/Fadeout_Content/Core/Characters/BP_PlayerCharacter.CheckTeamDamage` _asbp_player_character (`self.Instigator Controller`)))
              (if (and (or (not _sameteam) _ffa_) _valid)
                (goto _label)))))
        (:`else`)))))

(fn `UserConstructionScript`
  (bind _mesh (`self.Mesh`))
  (`parent.UserConstructionScript`)
  (bind _returnvalue (`PrimitiveComponent.CreateDynamicMaterialInstance` _mesh 0 (`PrimitiveComponent.GetMaterial` _mesh 0) "None"))
  (`MaterialInstanceDynamic.SetVectorParameterValue` _returnvalue "Color" (`self.Alchemic_Color`)))