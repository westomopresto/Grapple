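; Gwen's alchemy bow weapon, which cycles through Fire, Electricity, Earth and Air on alt-fire with a short cooldown.
; Each element change swaps the projectile, charge particles and sound, plays a montage, fires an element-changed event and replaces the owner's self-buff, which a looping timer renews.
; Charge and fire montages fall back to generic bow animations for non-Gwen owners.
; BeginPlay defaults to Fire and creates a local-player element widget, removed on drop or EndPlay.
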(event `Switch Element Server`
  (`|ExecutionSequence`
    (:`then_0`
      (if (not (`KismetSystemLibrary.K2_IsTimerActiveHandle` (`self.elementSwitchCooldown`)))
        (`self.Switch Element`)
        (bind _returnvalue (`KismetSystemLibrary.K2_SetTimerDelegate` (delegate `elementSwitchCooldownOver`) 0.125))
        (set `self.elementSwitchCooldown` _returnvalue)))))

(event `self.Post Shot Mg`
  (params (Fired :type Boolean))
  (bind _returnvalue (`self.GetOwner`))
  (`parent.Post Shot Mg` Fired)
  (if Fired
    (`SkeletalMeshComponent.PlayAnimation` (`self.SkeletalMesh`) "/Game/Fadeout_Content/Core/FBX/Bow/Bow_Shoot.Bow_Shoot" false)
    (bind _asbp_char_gwen (cast `/Game/Fadeout_Content/Core/Characters/BP_Char_Gwen` _returnvalue)
      (:`then`
        (`Character.PlayAnimMontage` _asbp_char_gwen "/Game/Fadeout_Content/Core/Characters/Gwen/gwenCharge_Montage.gwenCharge_Montage" 1.5 "fire"))
      (:`CastFailed`
        (bind _asbp_player_character (cast `/Game/Fadeout_Content/Core/Characters/BP_PlayerCharacter` _returnvalue))
        (`Character.PlayAnimMontage` _asbp_player_character (`/Game/Fadeout_Content/Core/Characters/BP_PlayerCharacter.bow_fire_montage` _asbp_player_character) 1.0 "Default")))
    (`GameplayStatics.SpawnEmitterAttached` "/Game/AnimeFX/Particles/HandDrawn/PS_Circle02_01.PS_Circle02_01" (`self.SkeletalMesh`) "Muzzle" (0.0 0.0 0.0) (struct) (0.25 0.25 0.25))
    (else
      (bind _asbp_player_character_2 (cast `/Game/Fadeout_Content/Core/Characters/BP_PlayerCharacter` (`self.GetOwner`)))
      (`Character.StopAnimMontage` _asbp_player_character_2 (`/Game/Fadeout_Content/Core/Characters/BP_PlayerCharacter.bow_drawn_montage` _asbp_player_character_2)))))

(event `elementSwitchCooldownOver`)

(event `Element Change`
  (params (Index :type "/Game/Fadeout_Content/Core/Characters/Gwen/Gwen_Elements Enum" :default "NewEnumerator0"))
  (bind _output_get (set `self.current_gwen_element` Index))
  (set `self.ProjectileToFire` (select `/Game/Fadeout_Content/Core/Characters/Gwen/Gwen_Elements` _output_get :`NewEnumerator0` "/Game/Fadeout_Content/Core/Characters/Gwen/BP_Alchemic_Fire.BP_Alchemic_Fire_C" :`NewEnumerator1` "/Game/Fadeout_Content/Core/Characters/Gwen/BP_Alchemic_Bolt.BP_Alchemic_Bolt_C" :`NewEnumerator2` "/Game/Fadeout_Content/Core/Characters/Gwen/BP_Alchemic_Earth.BP_Alchemic_Earth_C" :`NewEnumerator3` "/Game/Fadeout_Content/Core/Characters/Gwen/BP_Alchemic_Air.BP_Alchemic_Air_C" :!type "/Game/Fadeout_Content/Core/Weapons/BP_ProjectileBase Class Reference"))
  (`ParticleSystemComponent.SetTemplate` (`self.ParticleSystem`) (select `/Game/Fadeout_Content/Core/Characters/Gwen/Gwen_Elements` _output_get :`NewEnumerator0` "/Game/StylizedVFX_Fire/Effects/P_FireBall_Charge.P_FireBall_Charge" :`NewEnumerator1` "/Game/VFX_Toolkit_V1/ParticleSystems/356Days/Par_FlashRing.Par_FlashRing" :`NewEnumerator2` "/Game/StylizedVFX_Fire/Effects/P_Earth_Charge.P_Earth_Charge" :`NewEnumerator3` "/Game/VFX_Toolkit_V1/ParticleSystems/356Days/Par_Matra_01b_Trail.Par_Matra_01b_Trail" :!type "ParticleSystem Object Reference"))
  (`self.ELEMENT_CHANGED` _output_get)
  (bind _asbp_player_character (cast `/Game/Fadeout_Content/Core/Characters/BP_PlayerCharacter` (`self.GetOwner`)))
  (`Character.PlayAnimMontage` _asbp_player_character "/Game/Fadeout_Content/Core/Characters/Gwen/gwen_montage_element.gwen_montage_element" 1.0 "start")
  (`|ExecutionSequence`
    (:`then_0`
      (bind _currentsoundobject (`self.currentSoundObject`)
        (:`then`
          (`AudioComponent.Stop` _currentsoundobject))
        (:`else`)))
    (:`then_1`
      (bind _returnvalue (`GameplayStatics.SpawnSoundAtLocation` (select `/Game/Fadeout_Content/Core/Characters/Gwen/Gwen_Elements` _output_get :`NewEnumerator0` "/Game/Fadeout_Content/Core/Audio/Character_VO/Gwen_VO/elements/gwen_fire_cue.gwen_fire_cue" :`NewEnumerator1` "/Game/Fadeout_Content/Core/Audio/Character_VO/Gwen_VO/elements/gwen_energy_cue1.gwen_energy_cue1" :`NewEnumerator2` "/Game/Fadeout_Content/Core/Audio/Character_VO/Gwen_VO/elements/gwen_earth_cue.gwen_earth_cue" :`NewEnumerator3` "/Game/Fadeout_Content/Core/Audio/Character_VO/Gwen_VO/elements/gwen_air_01_Cue.gwen_air_01_Cue" :!type "SoundBase Object Reference") (`self.K2_GetActorLocation` _asbp_player_character) (struct) 2.0 1.0 0.0 null null))
      (set `self.currentSoundObject` _returnvalue))))

(event `Switch Element`
  (bind _output_get (set `self.current_gwen_element` (select `/Game/Fadeout_Content/Core/Characters/Gwen/Gwen_Elements` (`self.current_gwen_element`) :`NewEnumerator0` "NewEnumerator1" :`NewEnumerator1` "NewEnumerator2" :`NewEnumerator2` "NewEnumerator3" :`NewEnumerator3` "NewEnumerator0" :!type "/Game/Fadeout_Content/Core/Characters/Gwen/Gwen_Elements Enum")))
  (`self.Element Change` _output_get)
  (`self.Buff Refresh` false)
  (`self.ELEMENT_CHANGED` _output_get))

(event `self.OnAltFirePress`
  (`parent.OnAltFirePress`)
  (`self.Switch Element Server`))

(event `self.Charge Start Multicast`
  (bind _returnvalue (`self.GetOwner`))
  (`parent.Charge Start Multicast`)
  (set `self.FireSound` (select `/Game/Fadeout_Content/Core/Characters/Gwen/Gwen_Elements` (`self.current_gwen_element`) :`NewEnumerator0` "/Game/Fadeout_Content/Core/Audio/magic/01_Fire_explosion_01_small.01_Fire_explosion_01_small" :`NewEnumerator1` "/Game/Fadeout_Content/Core/Audio/magic/lightmagic_cast.lightmagic_cast" :`NewEnumerator2` "/Game/Fadeout_Content/Core/Audio/magic/01_Fire_explosion_01_small.01_Fire_explosion_01_small" :`NewEnumerator3` "/Game/Fadeout_Content/Core/Audio/magic/lightmagic_cast.lightmagic_cast" :!type "SoundBase Object Reference"))
  (bind _asbp_char_gwen (cast `/Game/Fadeout_Content/Core/Characters/BP_Char_Gwen` _returnvalue)
    (:`then`
      (`Character.PlayAnimMontage` _asbp_char_gwen "/Game/Fadeout_Content/Core/Characters/Gwen/gwenCharge_Montage.gwenCharge_Montage" 1.0 "charge"))
    (:`CastFailed`
      (bind _asbp_player_character (cast `/Game/Fadeout_Content/Core/Characters/BP_PlayerCharacter` _returnvalue))
      (`Character.PlayAnimMontage` _asbp_player_character (`/Game/Fadeout_Content/Core/Characters/BP_PlayerCharacter.bow_drawn_montage` _asbp_player_character) 1.0 "Default"))))

(event `Buff Refresh`
  (params (auto :type Boolean))
  (bind _current_self_buff (`self.Current_Self_Buff`)
    (:`then`
      (`/Game/Fadeout_Content/Core/Weapons/BP_DoT_Effect_Damage_Over_Time.earlyEnd` _current_self_buff))
    (:`else`
      _))
  (bind _playerowner (`self.PlayerOwner`)
    (:`then`
      (bind _applied_dot (`/Game/Fadeout_Content/Core/Characters/BP_PlayerCharacter.Attach DoT ` _playerowner (select `/Game/Fadeout_Content/Core/Characters/Gwen/Gwen_Elements` (`self.current_gwen_element`) :`NewEnumerator0` "/Game/Fadeout_Content/Core/Weapons/BP_Alchemic_Fire_Buff.BP_Alchemic_Fire_Buff_C" :`NewEnumerator1` "/Game/Fadeout_Content/Core/Weapons/BP_Alchemic_Bolt_Buff.BP_Alchemic_Bolt_Buff_C" :`NewEnumerator2` "/Game/Fadeout_Content/Core/Weapons/BP_Alchemic_Earth_Buff.BP_Alchemic_Earth_Buff_C" :`NewEnumerator3` "/Game/Fadeout_Content/Core/Weapons/BP_Alchemic_Air_Buff.BP_Alchemic_Air_Buff_C" :!type "/Game/Fadeout_Content/Core/Weapons/BP_DoT_Effect_Damage_Over_Time Class Reference") _playerowner true true))
      (bind _asbp_alchemic_buff_damage (cast `/Game/Fadeout_Content/Core/Weapons/BP_Alchemic_Buff_Damage` _applied_dot))
      (set `self.Current_Self_Buff` _asbp_alchemic_buff_damage)
      (if (not auto)
        (bind _current_self_buff_2 (`self.Current_Self_Buff`)
          (:`then`
            (`/Game/Fadeout_Content/Core/Weapons/BP_Alchemic_Buff_Damage.Display Buff Message` _current_self_buff_2))
          (:`else`))))
    (:`else`)))

(event `Self Buff Refresher`
  (`self.Buff Refresh` true))

(event `self.ReceiveBeginPlay`
  (bind _playerowner (`self.PlayerOwner`))
  (`parent.ReceiveBeginPlay`)
  (`self.Element Change` "NewEnumerator0")
  (`self.Buff Refresh` false)
  (`KismetSystemLibrary.K2_SetTimerDelegate` (delegate `Self Buff Refresher`) 2.99 true)
  (`KismetSystemLibrary.Delay` 1.0)
  (bind _asfo_player_controller (cast `/Game/Fadeout_Content/Core/FO_PlayerController` (`Pawn.GetController` _playerowner)))
  (`|ExecutionSequence`
    (:`then_0`
      (if (`Controller.IsLocalPlayerController` _asfo_player_controller)
        (bind _returnvalue (`|CreateWidget` "/Game/Fadeout_Content/Core/Characters/Gwen/Widget_Gwen_Elements.Widget_Gwen_Elements_C" _asfo_player_controller self))
        (bind _output_get (set `self.GwenUI` _returnvalue))
        (set `/Game/Fadeout_Content/Core/UI/BP_HUD.GwenUI` _output_get (cast `/Game/Fadeout_Content/Core/UI/BP_HUD` (`PlayerController.GetHUD` _asfo_player_controller) :!pure true))
        (`UserWidget.AddToPlayerScreen` _output_get 1)
        (add `self.OnEndPlay` (delegate `Remove UI`))))
    (:`then_1`
      (bind _asbp_char_gwen (cast `/Game/Fadeout_Content/Core/Characters/BP_Char_Gwen` _playerowner))
      (`/Game/Fadeout_Content/Core/Characters/BP_Char_Gwen.StartListeningForForms` _asbp_char_gwen self))))

(event `Remove UI` :!signature `self.OnEndPlay`
  (params (Actor :type "Actor Object Reference") (EndPlayReason :type "EEndPlayReason Enum" :default "Destroyed"))
  (bind _gwenui (`self.GwenUI` :!label _label)
    (:`then`
      (`Widget.RemoveFromParent` _gwenui))
    (:`else`)))

(event `self.OnDropped`
  (`parent.OnDropped`)
  (goto _label))

(fn `UserConstructionScript`
  (`parent.UserConstructionScript`)
  (`SceneComponent.K2_AttachToComponent` (`self.HookDummy`) (`self.SkeletalMesh`) "arrowSocket" "SnapToTarget" "SnapToTarget" "SnapToTarget" true))