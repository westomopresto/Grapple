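; BP_Char_Wolf is a wolf player character that hunts bleeding enemies, changing its run speed by proximity to them.
; FindBleedingEnemy maintains the victim list, playing hit and howl-style sounds when one is added.
; After a one-second initial delay, Tick finds the nearest victim's distance and blends MaxWalkSpeed between a fixed close-range value and RunSpeed.
; ColorSet calls PackLeader, tinting default Hemlock outfit pieces with team color through dynamic materials.
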(event `Bleeding Enemy Distance`
  (set `self.BleedingLowestDistance` 9999999.0)
  (for _array_element (`self.Bleeding Enemies`)
    (`/Engine/EditorBlueprintResources/StandardMacros.IsValid` _array_element
      (:`Is Valid`
        (bind _returnvalue (`KismetMathLibrary.Vector_Distance` (`self.K2_GetActorLocation`) (`self.K2_GetActorLocation` _array_element)))
        (if (<= _returnvalue (`self.BleedingLowestDistance`))
          (set `self.BleedingLowestDistance` _returnvalue))))))

(event `Find Bleeding Enemy`
  (params (BP_Player :type "/Game/Fadeout_Content/Core/Characters/BP_PlayerCharacter Object Reference") (add :type Boolean))
  (if add
    (`KismetArrayLibrary.Array_Add` (`self.Bleeding Enemies`) BP_Player)
    (`GameplayStatics.PlaySoundAtLocation` "/Game/Fadeout_Content/Core/Audio/Wolf_Sounds/093998425-scary-drop-hit-sound-effect-ci.093998425-scary-drop-hit-sound-effect-ci" (`self.K2_GetActorLocation` BP_Player) (struct) 1.0 1.0 0.0 null null null)
    (`GameplayStatics.PlaySoundAtLocation` "/Game/Fadeout_Content/Core/Audio/Wolf_Sounds/067015201-animals-wolf-ext-medium-distan.067015201-animals-wolf-ext-medium-distan" (`self.K2_GetActorLocation`) (struct) 1.0 1.0 0.0 null null null)
    (else
      (`KismetArrayLibrary.Array_RemoveItem` (`self.Bleeding Enemies`) BP_Player))))

(event `self.ReceiveTick`
  (params (DeltaSeconds :type "Float (single-precision)"))
  (bind _bleedtick (`self.BleedTick`))
  (`parent.ReceiveTick` DeltaSeconds)
  (set `self.BleedTick` (+ _bleedtick DeltaSeconds))
  (if (>= _bleedtick 1.0)
    (`self.Bleeding Enemy Distance`)
    (set `CharacterMovementComponent.MaxWalkSpeed` (`KismetMathLibrary.Lerp` 1500.0 (`self.runSpeed`) (`KismetMathLibrary.FClamp` (`KismetMathLibrary.NormalizeToRange` (`self.BleedingLowestDistance`) 0.0 10000.0))) (`self.CharacterMovement`))))

(event `Pack Leader`
  (bind _equipped_cosmetic_reference (`self.Equipped Cosmetic Reference`))
  (bind _equippedcosmetics (`self.EquippedCosmetics`))
  (for _array_element (`|MakeArray` (`|GetArrayItem` _equippedcosmetics (`KismetArrayLibrary.Array_Find` _equipped_cosmetic_reference "/Game/Fadeout_Content/Core/Characters/Hemlock/hemlock_default_outfit.hemlock_default_outfit")) (`|GetArrayItem` _equippedcosmetics (`KismetArrayLibrary.Array_Find` _equipped_cosmetic_reference "/Game/Fadeout_Content/Core/Characters/Hemlock/hemlock_default_outfit_bottom.hemlock_default_outfit_bottom")))
    (`/Engine/EditorBlueprintResources/StandardMacros.IsValid` _array_element
      (:`Is Valid`
        (bind _returnvalue (`KismetMaterialLibrary.CreateDynamicMaterialInstance` (`PrimitiveComponent.GetMaterial` _array_element 0) "/Game/Fadeout_Content/Core/Characters/Hemlock/M_Hemlock_Default.M_Hemlock_Default" "None"))
        (bind _output_get (set `self.HelmetDynamic` _returnvalue))
        (`PrimitiveComponent.SetMaterial` _array_element 0 _output_get)
        (`MaterialInstanceDynamic.SetVectorParameterValue` _output_get "TeamColor" (`KismetMathLibrary.Conv_ColorToLinearColor` (`self.HelmetColor`)))))))

(event `self.Color Set`
  (switch `/Game/Fadeout_Content/Core/UI/Customize/Hemlock_Outfits` (cast `/Game/Fadeout_Content/Core/UI/Customize/Hemlock_Outfits` (`KismetMathLibrary.Conv_IntToByte` (`self.current_outfit`)))
    (:`NewEnumerator2`
      (`self.Pack Leader`))))

(fn `UserConstructionScript`
  (`parent.UserConstructionScript`))