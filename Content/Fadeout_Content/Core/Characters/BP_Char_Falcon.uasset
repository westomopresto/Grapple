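; Falcon's playable character Blueprint, a child class adding an air dodge into flight and a held fast fall.
; Dodge Roll passes airborne state to DodgeRollAction; AirDodgeServer spawns and possesses a BP_FlyingPawn, attaches the character to it and blends the camera over.
; Fast fall replicates through server and multicast events, with Tick repeatedly launching the character downward while falling.
; ColorSet calls the parent, then switches on Falcon outfits with empty branches.
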(event `InputAction|Dodge Roll`
  (params (Key :type "Key Structure"))
  (:`Pressed`
    (`self.Dodge Roll Action` (not (`NavMovementComponent.IsMovingOnGround` (`self.CharacterMovement`))))))

(event `self.airDodgeServer`
  (bind _returnvalue (`self.GetController`))
  (set `self.preventDespawn` true)
  (bind _returnvalue_2 (`|SpawnActorFromClass` "/Game/Fadeout_Content/Core/Vehicles/BP_FlyingPawn.BP_FlyingPawn_C" (`self.GetTransform`) "AlwaysSpawn" "OverrideRootScale" (`self.GetOwner`) self (`self.Instigator`)))
  (`Controller.Possess` _returnvalue _returnvalue_2)
  (`self.K2_AttachToActor` _returnvalue_2 "None" "KeepWorld" "KeepWorld" "KeepWorld")
  (bind _asplayer_controller (cast `PlayerController` (`self.GetController`)))
  (`PlayerController.SetViewTargetWithBlend` _asplayer_controller self 0.0 "VTBlend_Linear" 0.0 false)
  (bind _asplayer_controller_2 (cast `PlayerController` _returnvalue))
  (`PlayerController.SetViewTargetWithBlend` _asplayer_controller_2 _returnvalue_2 1.0 "VTBlend_EaseIn" 0.0 false))

(event `self.ReceiveTick`
  (params (DeltaSeconds :type "Float (single-precision)"))
  (`parent.ReceiveTick` DeltaSeconds)
  (if (`self.FastFalling`)
    (set `self.FastFallTick` (+ (`self.FastFallTick`) DeltaSeconds))
    (if (>= (`self.FastFallTick`) 0.1)
      (if (`NavMovementComponent.IsFalling` (`self.CharacterMovement`))
        (`self.LaunchCharacter` (0.0 0.0 -500.0))
        (set `self.FastFallTick` 0.0)
        (else
          (set `self.FastFalling` false))))
    (else
      (set `self.FastFallTick` 0.0))))

(event `fastFall Multicast`
  (params (FastFalling :type Boolean))
  (set `self.FastFalling` FastFalling))

(event `fastFall Server`
  (params (FastFalling :type Boolean))
  (`self.fastFall Multicast` FastFalling))

(event `InputAction|FastFall`
  (params (Key :type "Key Structure"))
  (:`Pressed`
    (`/Engine/EditorBlueprintResources/ActorMacros.Switch Has Authority`
      (:`Authority`
        (`self.fastFall Multicast` true))
      (:`Remote`
        (`self.fastFall Server` true))))
  (:`Released`
    (`/Engine/EditorBlueprintResources/ActorMacros.Switch Has Authority`
      (:`Authority`
        (`self.fastFall Multicast` false))
      (:`Remote`
        (`self.fastFall Server` false)))))

(event `self.Color Set`
  (`parent.Color Set`)
  (switch `/Game/Fadeout_Content/Core/UI/Customize/Falcon_Outfits` (cast `/Game/Fadeout_Content/Core/UI/Customize/Falcon_Outfits` (`self.current_outfit`))))

(fn `UserConstructionScript`
  (`parent.UserConstructionScript`))