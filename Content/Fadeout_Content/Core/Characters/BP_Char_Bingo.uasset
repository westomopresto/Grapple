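; Bingo, a playable stealth character that can cloak behind a smoke bomb and levels up its dagger through kills.
; Cloak toggles replicate via server and multicast events, swapping to a refraction material, hiding cosmetics and showing a combat-tinted decal locally.
; Cloak drains energy by combat and crouch state, breaking when energy runs out or combat begins.
; Dagger kills raise its form through three levels; Spy and Thief outfits get team-colored dynamic materials.
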(event `Force Exit Combat`
  (`KismetSystemLibrary.K2_ClearAndInvalidateTimerHandle` (`self.combatTimer`))
  (set `self.inCOMBAT` false))

(event `self.Kill Voice Line Client - Weapon`
  (params (`Weapon Used` :type "/Game/Fadeout_Content/Core/Weapons/DamageTypes Enum" :default "NewEnumerator0") (Headshot :type Boolean))
  (`parent.Kill Voice Line Client - Weapon` `Weapon Used` Headshot)
  (if (and (`|EnumEquality` `Weapon Used` "NewEnumerator10") (== (`GameplayStatics.GetObjectClass` (`self.CurrentWeapon`)) "/Game/Fadeout_Content/Weapons/BP_Melee_Dagger.BP_Melee_Dagger_C"))
    (`|ExecutionSequence`
      (:`then_0`
        (`/Engine/EditorBlueprintResources/ActorMacros.Switch Has Authority`
          (:`Authority`
            (set `self.dagger_level` (`KismetMathLibrary.Clamp` (+ (`self.dagger_level`) 1) 0 2)))))
      (:`then_1`
        (`self.DaggerLevelUP`)
        (`self.PlayAnimMontage` "/Game/Fadeout_Content/Core/Characters/Bingo/bingo_animations/bingo_levelup_montage.bingo_levelup_montage")
        (`GameplayStatics.PlaySoundAtLocation` "/Game/Fadeout_Content/Core/Audio/Weapon_SFX/CritMarker_V5.CritMarker_V5" (`self.K2_GetActorLocation`) (struct) 1.0 1.0 0.0 null null null)))))

(event `self.Enter_Combat`
  (`parent.Enter_Combat`)
  (`KismetSystemLibrary.Delay` 0.1)
  (`self.Cloak Toggle` false))

(event `self.ReceiveTick`
  (params (DeltaSeconds :type "Float (single-precision)"))
  (`parent.ReceiveTick` DeltaSeconds)
  (`self.Cloak Shimmer` (`self.inCOMBAT`))
  (`self.DecaleCombatColor`))

(event `self.Energy Regen`
  (bind _returnvalue (`KismetMathLibrary.SelectInt` 30 (`KismetMathLibrary.SelectInt` 10 20 (`self.Crouching_NET`)) (`self.inCOMBAT`)))
  (`parent.Energy Regen`)
  (if (`self.isCloaked`)
    (bind (_costmet _remainder) (`self.EnergyCost_Function` _returnvalue true))
    (`KismetSystemLibrary.PrintString` (`KismetStringLibrary.Conv_IntToString` _remainder))
    (if _costmet
      (`self.EnergyCost_Function` _returnvalue)
      (else
        (`self.Cloak Toggle` false)))))

(event `self.weaponPickupFunction`
  (params (weaponBaseActor :type "/Game/Fadeout_Content/Core/Weapons/BP_weaponBase Object Reference") (AmmoFromWeapon :type "/Game/Fadeout_Content/Core/Support/AmmoStruct Structure"))
  (bind _iscloaked (`self.isCloaked`))
  (`parent.weaponPickupFunction` weaponBaseActor AmmoFromWeapon)
  (`/Engine/EditorBlueprintResources/StandardMacros.IsValid` weaponBaseActor
    (:`Is Valid`
      (`/Engine/EditorBlueprintResources/ActorMacros.Switch Has Authority`
        (:`Authority`
          (`/Game/Fadeout_Content/Core/Weapons/BP_weaponBase.Cloak Weapon Multicast` weaponBaseActor _iscloaked))
        (:`Remote`
          (`/Game/Fadeout_Content/Core/Weapons/BP_weaponBase.Cloak Weapon Server` weaponBaseActor _iscloaked))))))

(event `Multicast Cloakmode`
  (params (Condition :type Boolean))
  (bind _capsulecomponent (`self.CapsuleComponent`))
  ;[1 1 1] Cloaking
  (if Condition
    (`GameplayStatics.SpawnEmitterAttached` "/Game/Fadeout_Content/Core/FX/p_smoke_bomb.p_smoke_bomb" _capsulecomponent "None" (0.0 0.0 -60.0))
    (`self.PlayAnimMontage` "/Game/Fadeout_Content/Core/Characters/Kasparian_BP/Goofy/bingo_stealth_enter_montage.bingo_stealth_enter_montage")
    (`GameplayStatics.SpawnSoundAttached` "/Game/Fadeout_Content/Core/Audio/Explosions/smoke_bomb_sfx_Cue.smoke_bomb_sfx_Cue" _capsulecomponent "None" (0.0 0.0 0.0) (struct) "KeepRelativeOffset" false 1.0 1.0 0.0 null null)
    (`KismetSystemLibrary.Delay` 0.1))
  (`self.Cloak Mode Function` Condition)
  (`self.Cloaked` Condition)
  (`self.ForceNetUpdate`))

(event `SpyOutfit`
  (bind (_colorrgb _bonusmetallic) (break `/Game/Fadeout_Content/Core/UI/Customize/CustomColor` (`self.HelmetColor`)))
  (bind _output (`|GetArrayItem` (`self.EquippedCosmetics`) (`KismetArrayLibrary.Array_Find` (`self.Equipped Cosmetic Reference`) "/Game/Fadeout_Content/Core/Characters/Bingo/Bingo_SpyOutfit.Bingo_SpyOutfit")))
  (`KismetSystemLibrary.PrintString` "spyoutfit" true true (struct :`R` 0.945955 :`G` 1.0 :`A` 1.0) 8.0)
  (`/Engine/EditorBlueprintResources/StandardMacros.IsValid` _output
    (:`Is Valid`
      (bind _returnvalue (`KismetMaterialLibrary.CreateDynamicMaterialInstance` (`PrimitiveComponent.GetMaterial` _output 0) "/Game/Fadeout_Content/Core/Characters/Bingo/M_Bingo_Spy.M_Bingo_Spy" "None"))
      (bind _output_get (set `self.HelmetDynamic` _returnvalue))
      (`PrimitiveComponent.SetMaterial` _output 0 _output_get)
      (`MaterialInstanceDynamic.SetVectorParameterValue` _output_get "TeamColor" (`KismetMathLibrary.Conv_ColorToLinearColor` _colorrgb))
      (`MaterialInstanceDynamic.SetScalarParameterValue` _output_get "BonusMetallic" _bonusmetallic))))

(event `Server Cloakmode`
  (params (Condition :type Boolean))
  ;[1 1 1] Cloaking
  (`self.Multicast Cloakmode` Condition))

(event `self.Color Set`
  (`parent.Color Set`)
  (switch `/Game/Fadeout_Content/Core/UI/Customize/Bingo_Outfits` (cast `/Game/Fadeout_Content/Core/UI/Customize/Bingo_Outfits` (`self.current_outfit`))
    (:`NewEnumerator2`
      (`self.SpyOutfit`))
    (:`NewEnumerator3`
      (`self.Theif Bingo`))))

(event `Cloak Toggle`
  (params (On :type Boolean))
  ;[1 1 1] Cloaking
  (`/Engine/EditorBlueprintResources/ActorMacros.Switch Has Authority`
    (:`Authority`
      (`self.Multicast Cloakmode` On))
    (:`Remote`
      (`self.Server Cloakmode` On))))

(event `Theif Bingo`
  (bind (_colorrgb _bonusmetallic) (break `/Game/Fadeout_Content/Core/UI/Customize/CustomColor` (`self.HelmetColor`)))
  (bind _output (`|GetArrayItem` (`self.EquippedCosmetics`) (`KismetArrayLibrary.Array_Find` (`self.Equipped Cosmetic Reference`) "/Game/Fadeout_Content/Core/Characters/Bingo/Outfits/Thief/Bingo_Thief_v1.Bingo_Thief_v1")))
  (`/Engine/EditorBlueprintResources/StandardMacros.IsValid` _output
    (:`Is Valid`
      (bind _returnvalue (`KismetMaterialLibrary.CreateDynamicMaterialInstance` (`PrimitiveComponent.GetMaterial` _output 0) "/Game/Fadeout_Content/Core/Characters/Bingo/Outfits/Thief/M_Bingo_Thief.M_Bingo_Thief" "None"))
      (bind _output_get (set `self.HelmetDynamic` _returnvalue))
      (`PrimitiveComponent.SetMaterial` _output 0 _output_get)
      (`MaterialInstanceDynamic.SetVectorParameterValue` _output_get "TeamColor" (`KismetMathLibrary.Conv_ColorToLinearColor` _colorrgb))
      (`MaterialInstanceDynamic.SetScalarParameterValue` _output_get "BonusMetallic" _bonusmetallic))))

(event `InputAction|Character Special`
  (params (Key :type "Key Structure"))
  ;[1 1 1] Cloaking
  (:`Pressed`
    (if (`self.isCloaked`)
      (`self.Cloak Toggle` false)
      (else
        (`self.Cloak Ability`)))))

(event `Cloak Ability`
  (if (>= (`.Energy_18_2D8D75E04E1979C951FEA185FE1A6270` (break `/Game/Fadeout_Content/Core/Support/AmmoStruct` (`self.HeldAmmo`))) 20)
    (`self.Cloak Toggle` true)))

(event `self.ReceiveBeginPlay`
  (`parent.ReceiveBeginPlay`)
  (`self.InitializeBingoStealthShader`)
  (set `self.oEnergyRegen` (`self.EnergyRegen`)))

(fn `Cloak Mode Function`
  (params (Condition :type Boolean))
  (bind _cloakdynamic (`self.CloakDynamic`))
  (bind _mesh (`self.Mesh`))
  (bind _equippedcosmetics (`self.EquippedCosmetics`))
  (bind _equippedcosmetics_2 (`self.EquippedCosmetics`))
  (`|ExecutionSequence`
    (:`then_0`
      (if (not (`KismetSystemLibrary.IsValid` (`self.Body Material with Mask`)))
        (`self.InitializeBingoStealthShader`)))
    (:`then_1`
      (if Condition
        (`SceneComponent.SetVisibility` _equippedcosmetics_2 false false)
        (`PrimitiveComponent.SetCastShadow` _equippedcosmetics_2 false)
        (`PrimitiveComponent.SetMaterial` _mesh 0 _cloakdynamic)
        (set `self.isCloaked` true)
        (`MaterialInstanceDynamic.SetScalarParameterValue` _cloakdynamic "Refraction Amount" 1.0)
        (if (`self.IsLocallyControlled`)
          (`SceneComponent.SetVisibility` (`self.Decal`) true false)
          (return)
          (else
            _))
        (else
          (`SceneComponent.SetVisibility` _equippedcosmetics true false)
          (`PrimitiveComponent.SetCastShadow` _equippedcosmetics true)
          (`PrimitiveComponent.SetMaterial` _mesh 0 (`self.Body Material with Mask`))
          (set `self.isCloaked` false)
          (if (`self.IsLocallyControlled`)
            (`SceneComponent.SetVisibility` (`self.Decal`) false false)
            (return)
            (else
              _))))
      (return))))

(fn `Cloak Shimmer`
  (params (combat :type Boolean))
  (bind _cloakdynamic (`self.CloakDynamic`))
  (`/Engine/EditorBlueprintResources/StandardMacros.IsValid` _cloakdynamic
    (:`Is Valid`
      (`MaterialInstanceDynamic.SetScalarParameterValue` _cloakdynamic "Refraction Amount" (`KismetMathLibrary.SelectFloat` 0.65 0.99 combat)))))

(fn `ComboStealth`
  (`self.Force Exit Combat`)
  (set `self.EnergyRegen` 9999)
  (`self.Energy Regen`)
  (set `self.EnergyRegen` (`self.oEnergyRegen`))
  (`self.Cloak Toggle` true)
  (return))

(fn `DaggerLevelUP`
  (bind _dagger_level (`self.dagger_level`))
  (bind _ourdagger (`self.ourDagger`))
  (`|ExecutionSequence`
    (:`then_0`
      (`/Engine/EditorBlueprintResources/StandardMacros.IsValid` (`self.ourDagger`)
        (:`Is Not Valid`
          (for _array_element (`self.equipment`)
            (if (== (`GameplayStatics.GetObjectClass` _array_element) "/Game/Fadeout_Content/Weapons/BP_Melee_Dagger.BP_Melee_Dagger_C")
              (set `self.ourDagger` _array_element)
              (break))))))
    (:`then_1`
      (`/Engine/EditorBlueprintResources/StandardMacros.IsValid` _ourdagger
        (:`Is Valid`
          (bind _asbp_melee_dagger (cast `/Game/Fadeout_Content/Weapons/BP_Melee_Dagger` _ourdagger))
          (set `/Game/Fadeout_Content/Weapons/BP_Melee_Dagger.daggerLevel` _dagger_level _asbp_melee_dagger)
          (set `/Game/Fadeout_Content/Core/Weapons/BP_weaponBase.Name` (`KismetStringLibrary.Conv_StringToName` (select `int` _dagger_level :`0` "Dagger lvl.1" :`1` "Dagger lvl.2" :`2` "Dagger lvl.3")) _ourdagger)
          (`/Game/Fadeout_Content/Weapons/BP_Melee_Dagger.DaggerFormChange` _asbp_melee_dagger))))))

(fn `DecaleCombatColor`
  (bind _decaldynamic (`self.decalDynamic`))
  (`/Engine/EditorBlueprintResources/StandardMacros.IsValid` _decaldynamic
    (:`Is Valid`
      (if (`self.inCOMBAT`)
        (`MaterialInstanceDynamic.SetVectorParameterValue` _decaldynamic "colorMult" (struct :`R` 1.0 :`A` 1.0))
        (else
          (`MaterialInstanceDynamic.SetVectorParameterValue` _decaldynamic "colorMult" (struct :`G` 1.0 :`B` 0.2 :`A` 1.0))))
      (return))
    (:`Is Not Valid`
      (return))))

(fn `InitializeBingoStealthShader`
  (`|ExecutionSequence`
    (:`then_0`
      (`/Engine/EditorBlueprintResources/StandardMacros.IsValid` (`self.CloakDynamic`)
        (:`Is Not Valid`
          (bind _returnvalue (`KismetMaterialLibrary.CreateDynamicMaterialInstance` "/Game/Fadeout_Content/Core/Shaders/M_Cloak_Instance.M_Cloak_Instance"))
          (set `self.CloakDynamic` _returnvalue))))
    (:`then_1`
      (`/Engine/EditorBlueprintResources/StandardMacros.IsValid` (`self.decalDynamic`)
        (:`Is Not Valid`
          (bind _returnvalue_2 (`DecalComponent.CreateDynamicMaterialInstance` (`self.Decal`)))
          (set `self.decalDynamic` _returnvalue_2))))))

(fn `UserConstructionScript`
  (`parent.UserConstructionScript`))