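; Snek character Blueprint that applies the character's team color to whichever outfit is equipped.
; It extends the parent's ColorSet event, then switches on the current outfit, read as a Dalton_Outfits enum.
; Depending on outfit, it creates dynamic materials on equipped cosmetic pieces or a body mesh slot, with Santa Dalton handled in its own event.
; Each material receives TeamColor and BonusMetallic from HelmetColor and is stored in the shared HelmetDynamic variable.
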(event `Color Set`
  (bind _mesh (`self.Mesh`))
  (bind _mesh_2 (`self.Mesh`))
  (bind _mesh_3 (`self.Mesh`))
  (bind _equipped_cosmetic_reference (`self.Equipped Cosmetic Reference`))
  (bind _equippedcosmetics (`self.EquippedCosmetics`))
  (bind (_colorrgb _bonusmetallic) (break `/Game/Fadeout_Content/Core/UI/Customize/CustomColor` (`self.HelmetColor`)))
  (bind (_colorrgb_2 _bonusmetallic_2) (break `/Game/Fadeout_Content/Core/UI/Customize/CustomColor` (`self.HelmetColor`)))
  (bind (_colorrgb_3 _bonusmetallic_3) (break `/Game/Fadeout_Content/Core/UI/Customize/CustomColor` (`self.HelmetColor`)))
  (bind (_colorrgb_4 _bonusmetallic_4) (break `/Game/Fadeout_Content/Core/UI/Customize/CustomColor` (`self.HelmetColor`)))
  (`parent.Color Set`)
  (switch `/Game/Fadeout_Content/Core/UI/Customize/Dalton_Outfits` (cast `/Game/Fadeout_Content/Core/UI/Customize/Dalton_Outfits` (`self.current_outfit`))
    (:`NewEnumerator0`
      (for _array_element (`|MakeArray` (`|GetArrayItem` _equippedcosmetics (`KismetArrayLibrary.Array_Find` _equipped_cosmetic_reference "/Game/Fadeout_Content/Core/Characters/Snake_FBX/outfits/snek_f_01_jacket.snek_f_01_jacket")) (`|GetArrayItem` _equippedcosmetics (`KismetArrayLibrary.Array_Find` _equipped_cosmetic_reference "/Game/Fadeout_Content/Core/Characters/Snake_FBX/outfits/snek_f_01_hlemet.snek_f_01_hlemet")))
        (`/Engine/EditorBlueprintResources/StandardMacros.IsValid` _array_element
          (:`Is Valid`
            (bind _returnvalue (`KismetMaterialLibrary.CreateDynamicMaterialInstance` (`PrimitiveComponent.GetMaterial` _array_element 0) "/Game/Fadeout_Content/Core/Characters/Snake_FBX/snek_Clothing_M.snek_Clothing_M" "None"))
            (bind _output_get (set `self.HelmetDynamic` _returnvalue))
            (`PrimitiveComponent.SetMaterial` _array_element 0 _output_get)
            (`MaterialInstanceDynamic.SetVectorParameterValue` _output_get "TeamColor" (`KismetMathLibrary.Conv_ColorToLinearColor` _colorrgb))
            (`MaterialInstanceDynamic.SetScalarParameterValue` _output_get "BonusMetallic" _bonusmetallic)))))
    (:`NewEnumerator1`
      (bind _returnvalue_2 (`KismetMaterialLibrary.CreateDynamicMaterialInstance` (`PrimitiveComponent.GetMaterial` _mesh_3 0) "/Game/Fadeout_Content/Core/Characters/Snake_FBX/snek_Body_M.snek_Body_M" "None"))
      (bind _output_get_2 (set `self.HelmetDynamic` _returnvalue_2))
      (`PrimitiveComponent.SetMaterial` _mesh_3 0 _output_get_2)
      (`MaterialInstanceDynamic.SetVectorParameterValue` _output_get_2 "TeamColor" (`KismetMathLibrary.Conv_ColorToLinearColor` _colorrgb_3))
      (`MaterialInstanceDynamic.SetScalarParameterValue` _output_get_2 "BonusMetallic" _bonusmetallic_3))
    (:`NewEnumerator2`
      (bind _returnvalue_3 (`KismetMaterialLibrary.CreateDynamicMaterialInstance` (`PrimitiveComponent.GetMaterial` _mesh 0) "/Game/Fadeout_Content/Core/Characters/Snake_FBX/outfits/FigureSkin_Snek/M_Figure_01.M_Figure_01" "None"))
      (bind _output_get_3 (set `self.HelmetDynamic` _returnvalue_3))
      (`PrimitiveComponent.SetMaterial` _mesh 0 _output_get_3)
      (`MaterialInstanceDynamic.SetVectorParameterValue` _output_get_3 "TeamColor" (`KismetMathLibrary.Conv_ColorToLinearColor` _colorrgb_4))
      (`MaterialInstanceDynamic.SetScalarParameterValue` _output_get_3 "BonusMetallic" _bonusmetallic_4))
    (:`NewEnumerator3`
      (`self.Santa Dalton`))
    (:`NewEnumerator4`
      (bind _returnvalue_4 (`KismetMaterialLibrary.CreateDynamicMaterialInstance` (`PrimitiveComponent.GetMaterial` _mesh_2 1) "/Game/Fadeout_Content/Core/Characters/Snake_FBX/outfits/Buff_Dalton/M_BuffDalton_TankTop.M_BuffDalton_TankTop" "None"))
      (bind _output_get_4 (set `self.HelmetDynamic` _returnvalue_4))
      (`PrimitiveComponent.SetMaterial` _mesh_2 1 _output_get_4)
      (`MaterialInstanceDynamic.SetVectorParameterValue` _output_get_4 "TeamColor" (`KismetMathLibrary.Conv_ColorToLinearColor` _colorrgb_2))
      (`MaterialInstanceDynamic.SetScalarParameterValue` _output_get_4 "BonusMetallic" _bonusmetallic_2))))

(event `Santa Dalton`
  (bind (_colorrgb _bonusmetallic) (break `/Game/Fadeout_Content/Core/UI/Customize/CustomColor` (`self.HelmetColor`)))
  (for _array_element (`|MakeArray` (`|GetArrayItem` (`self.EquippedCosmetics`) (`KismetArrayLibrary.Array_Find` (`self.Equipped Cosmetic Reference`) "/Game/Fadeout_Content/Core/Characters/Snake_FBX/outfits/Santa_Dalton/santa_dalton_01.santa_dalton_01")))
    (`/Engine/EditorBlueprintResources/StandardMacros.IsValid` _array_element
      (:`Is Valid`
        (bind _returnvalue (`KismetMaterialLibrary.CreateDynamicMaterialInstance` (`PrimitiveComponent.GetMaterial` _array_element 0) "/Game/Fadeout_Content/Core/Characters/Snake_FBX/outfits/Santa_Dalton/M_Santa_Dalton.M_Santa_Dalton" "None"))
        (bind _output_get (set `self.HelmetDynamic` _returnvalue))
        (`PrimitiveComponent.SetMaterial` _array_element 0 _output_get)
        (`MaterialInstanceDynamic.SetVectorParameterValue` _output_get "TeamColor" (`KismetMathLibrary.Conv_ColorToLinearColor` _colorrgb))
        (`MaterialInstanceDynamic.SetScalarParameterValue` _output_get "BonusMetallic" _bonusmetallic)))))

(fn `UserConstructionScript`
  (`parent.UserConstructionScript`))