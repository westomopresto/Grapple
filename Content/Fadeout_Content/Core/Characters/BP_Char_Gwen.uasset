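; Character Blueprint for Gwen, a child of a shared character base, adding her special action and outfit recoloring.
; Pressing Special casts the equipment at index 1 to her Alchemy item and asks the server to switch its element.
; ColorSet extends the parent: for the normal outfit, it applies a dynamic instance of her clothes material to the equipped clothing mesh, then passes it to RecolorMeshes.
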(event `InputAction|Character Special`
  (params (Key :type "Key Structure"))
  (:`Pressed`
    (bind _asbp_gwen_alchemy_01 (cast `/Game/Fadeout_Content/Core/Characters/Gwen/BP_Gwen_Alchemy_01` (`|GetArrayItem` (`self.equipment`) 1)))
    (`/Game/Fadeout_Content/Core/Characters/Gwen/BP_Gwen_Alchemy_01.Switch Element Server` _asbp_gwen_alchemy_01)))

(event `Color Set`
  (bind _output (`|GetArrayItem` (`self.EquippedCosmetics`) (`KismetArrayLibrary.Array_Find` (`self.Equipped Cosmetic Reference`) "/Game/Fadeout_Content/Core/Characters/Gwen/SK_Gwen_clothes.SK_Gwen_clothes")))
  (`parent.Color Set`)
  (switch `/Game/Fadeout_Content/Core/UI/Customize/Gwen_Outfits` (cast `/Game/Fadeout_Content/Core/UI/Customize/Gwen_Outfits` (`self.current_outfit`))
    (:`NewEnumerator0`
      ;[1 1 1] Normal Outfit
      (`/Engine/EditorBlueprintResources/StandardMacros.IsValid` _output
        (:`Is Valid`
          (bind _returnvalue (`KismetMaterialLibrary.CreateDynamicMaterialInstance` "/Game/Fadeout_Content/Core/Characters/Gwen/MI_Gwen_Clothes.MI_Gwen_Clothes" "None"))
          (bind _output_get (set `self.HelmetDynamic` _returnvalue))
          (`PrimitiveComponent.SetMaterial` _output 0 _output_get)
          (`self.RecolorMeshes` _output_get))))))

(fn `UserConstructionScript`
  (`parent.UserConstructionScript`))