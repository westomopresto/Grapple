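; Playable panda brawler Charlie, a child character Blueprint whose ability inputs equip and fire melee weapons from equipment slots.
; A short request cooldown and weapon dispatchers gate swapping, while unarmed attack indices select montages, including charge punch and flying chi launch.
; Unless disabled, its passive applies about half of non-lethal hits upfront and spawns damage-over-time for the rest, which cannot kill.
; It also recolors outfit materials and plays mega-weapon pickup voice lines.
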(event `InputAction|Fire`
  (params (Key :type "Key Structure"))
  (bind _returnvalue (`Controller.IsMoveInputIgnored` (`self.GetController`)))
  (:`Pressed`
    (`self.OnFireDispatcher` :!label _label)
    (cast `/Game/Fadeout_Content/Core/Weapons/Ability` (`self.CurrentWeapon`)
      (:`then`
        (if (not (`self.meleeAbilityRequested`))
          (if (not _returnvalue) :!label _label_2
            (`self.Fire Held Item`)
            (`self.MeleeAbilityRequestCD`))))
      (:`CastFailed`
        (goto _label_2))))
  (:`Released`
    (if (not _returnvalue) :!label _label_3
      (`self.Release Fire`))))

(event `InputAction|CharlieFire`
  (params (Key :type "Key Structure"))
  (:`Pressed`
    (goto _label))
  (:`Released`
    (goto _label_3)))

(event `Chi Launch`
  (bind _charactermovement (`self.CharacterMovement`))
  (`CharacterMovementComponent.SetMovementMode` _charactermovement "MOVE_Flying" 0)
  (`|PlayMontage` (`self.Mesh`) "/Game/Fadeout_Content/Core/Characters/Panda/Panda_Anims/chi_launch_montage.chi_launch_montage" 1.0 0.0 "Default"
    (:`then`
      (`KismetSystemLibrary.PrintString` "chi launch"))
    (:`OnCompleted`
      (`CharacterMovementComponent.SetMovementMode` _charactermovement "MOVE_Walking" 0 :!label _label_4))
    (:`OnBlendOut`
      (`CharacterMovementComponent.SetMovementMode` _charactermovement "MOVE_Walking" 0))
    (:`OnInterrupted`
      (goto _label_4))
    (:`OnNotifyEnd`
      (goto _label_4))))

(event `InputAction|CharlieAbility_1`
  (params (Key :type "Key Structure"))
  (:`Pressed`
    (if (`self.alive?`)
      (`self.Melee Ability` 0))))

(event `InputAction|QuickSwitch_1`
  (params (Key :type "Key Structure")))

(event `Key|One`
  (params (Key :type "Key Structure")))

(event `ChargePunch`
  (`|PlayMontage` (`self.Mesh`) "/Game/Fadeout_Content/Core/Characters/Bunn/attacks/unarmed/dashpunch_montage_2.dashpunch_montage_2" 1.25 0.0 "Default"
    (:`OnBlendOut`
      (`self.PlayAnimMontage` "/Game/Fadeout_Content/Core/Characters/Bunn/attacks/unarmed/dashpunch_montage_end.dashpunch_montage_end" 1.0 "Default"))))

(event `InputAction|CharlieAbility_2`
  (params (Key :type "Key Structure"))
  (:`Pressed`
    (if (`self.alive?`)
      (`self.Melee Ability` 1))))

(event `InputAction|QuickSwitch_2`
  (params (Key :type "Key Structure")))

(event `Key|Two`
  (params (Key :type "Key Structure")))

(event `InputAction|CharlieAbility_3`
  (params (Key :type "Key Structure"))
  (:`Pressed`
    (if (`self.alive?`)
      (`self.Melee Ability` 2))))

(event `InputAction|QuickSwitch_3`
  (params (Key :type "Key Structure")))

(event `Key|Three`
  (params (Key :type "Key Structure")))

(event `self.PlayerInputSwitchWeapon`
  (params (slot_index :type Integer) (IgnoreGCD :type Boolean))
  (`parent.PlayerInputSwitchWeapon` slot_index true))

(event `InputAction|QuickSwitch_4`
  (params (Key :type "Key Structure")))

(event `Key|Four`
  (params (Key :type "Key Structure")))

(event `InputAction|CharlieAbility_4`
  (params (Key :type "Key Structure"))
  (:`Pressed`
    (if (`self.alive?`)
      (`self.Melee Ability` 3))))

(event `InputAction|QuickSwitch_5`
  (params (Key :type "Key Structure")))

(event `Key|Five`
  (params (Key :type "Key Structure")))

(event `InputAction|CharlieAbility_5`
  (params (Key :type "Key Structure"))
  (:`Pressed`
    (if (`self.alive?`)
      (`self.Melee Ability` 4))))

(event `MeleeAbilityRequestCD`
  (set `self.meleeAbilityRequested` true)
  (`KismetSystemLibrary.K2_SetTimerDelegate` (delegate `MeleeAbilityCdEnded`) 0.1))

(event `MeleeAbilityCdEnded`
  (set `self.meleeAbilityRequested` false))

(event `Melee Ability`
  (params (`Dimension 1` :type Integer))
  (bind _output (`|GetArrayItem` (`self.equipment`) `Dimension 1`))
  (if (and (`self.canSwapTools?`) (not (`self.meleeAbilityRequested`)))
    (`self.MeleeAbilityRequestCD`)
    (`self.PlayerInputSwitchWeapon` `Dimension 1` true)
    (`self.EquipItemFunction` `Dimension 1`)
    (`self.ForceNetUpdate`)
    (bind _userwidget (message `/Game/Fadeout_Content/Core/UI/Interfaces/BPI_Get_GUIs.Get Combat Base` (`self.GetController`)))
    (`/Engine/EditorBlueprintResources/StandardMacros.IsValid` _userwidget
      (:`Is Valid`
        (`/Game/Fadeout_Content/Core/UI/WBP_CombatBase.gatherInventory` _userwidget (`self.equipment`) (`self.inventorySize`) `Dimension 1`))
      (:`Is Not Valid`
        _))
    (bind _asbp_melee_base (cast `/Game/Fadeout_Content/Core/Weapons/BP_MeleeBase` _output))
    (add `/Game/Fadeout_Content/Core/Weapons/BP_MeleeBase.Finish Trace Dispatcher` _asbp_melee_base (delegate `Can Swap Call`))
    (add `/Game/Fadeout_Content/Core/Weapons/BP_weaponBase.WeaponFiredEvent` _output (delegate `Success Fire`))
    (add `/Game/Fadeout_Content/Core/Weapons/BP_weaponBase.UpdateAmmoDispatch` _output (delegate `Success Fire`))
    (if (and (`self.canSwapTools?`) (`self.Can_GCD`))
      (`/Game/Fadeout_Content/Core/Weapons/BP_MeleeBase.OnFire` _asbp_melee_base))))

(event `Can Swap Call`
  (set `self.canSwapTools?` true))

(event `Success Fire`
  (set `self.canSwapTools?` false))

(event `self.Dodge Roll Action`
  (params (`Skip Ground Check` :type Boolean))
  (`parent.Dodge Roll Action` `Skip Ground Check`)
  (`self.Global CD`))

(event `self.ReceiveAnyDamage`
  (params (Damage :type "Float (single-precision)") (DamageType :type "DamageType Object Reference") (InstigatedBy :type "Controller Object Reference") (DamageCauser :type "Actor Object Reference"))
  (bind _returnvalue (`self.GetTransform`))
  (bind _returnvalue_2 (* Damage (`KismetMathLibrary.SelectFloat` 1.0 1.0 (`self.HasFlag?`))))
  (bind _returnvalue_3 (`KismetMathLibrary.FClamp` (/ (* _returnvalue_2 0.5) 3.0) 1.0 9999.0))
  (if (`self.bDisablePandaPassive`)
    (`parent.ReceiveAnyDamage` Damage DamageType InstigatedBy DamageCauser)
    (elif (!= (`GameplayStatics.GetObjectClass` DamageType) "/Game/Fadeout_Content/Core/Weapons/DamageTypes/DT_BrushOff.DT_BrushOff_C")
      ;[1 1 1] Regular Damage Type
      (`parent.ReceiveAnyDamage` (`KismetMathLibrary.SelectFloat` _returnvalue_2 (+ (* _returnvalue_2 0.5) 1.0) (<= (- (`self.health`) _returnvalue_2) 0.0)) DamageType InstigatedBy DamageCauser)
      (`/Engine/EditorBlueprintResources/StandardMacros.IsValid` InstigatedBy
        (:`Is Valid`
          (bind _returnvalue_4 (`|SpawnActorFromClass` "/Game/Fadeout_Content/Core/Weapons/BP_DoT_Effect_Damage_Over_Time.BP_DoT_Effect_Damage_Over_Time_C" _returnvalue "AlwaysSpawn" "OverrideRootScale" self _returnvalue_3 "/Game/Fadeout_Content/Core/Weapons/DamageTypes/DT_BrushOff.DT_BrushOff_C" false false false 3.0 false (`Controller.K2_GetPawn` InstigatedBy)))
          (`self.K2_AttachToActor` _returnvalue_4 self "None" "SnapToTarget" "SnapToTarget" "SnapToTarget" true))
        (:`Is Not Valid`
          (bind _returnvalue_5 (`|SpawnActorFromClass` "/Game/Fadeout_Content/Core/Weapons/BP_DoT_Effect_Damage_Over_Time.BP_DoT_Effect_Damage_Over_Time_C" _returnvalue "AlwaysSpawn" "OverrideRootScale" self _returnvalue_3 "/Game/Fadeout_Content/Core/Weapons/DamageTypes/DT_BrushOff.DT_BrushOff_C" false false false 3.0 false self))
          (`self.K2_AttachToActor` _returnvalue_5 self "None" "SnapToTarget" "SnapToTarget" "SnapToTarget" true)))
      (else
        ;[1 1 1] Brush off cant kill you
        (if (not (<= (- (`self.health`) _returnvalue_2) 1.0))
          (`parent.ReceiveAnyDamage` _returnvalue_2 DamageType InstigatedBy DamageCauser))))))

(event `self.Weapon Voice Event`
  (params (weapon :type "/Game/Fadeout_Content/Core/Weapons/BP_weaponBase Object Reference"))
  ;[1 1 1] mega weapon VO or weapon voice event override
)

(event `self.weaponBase_Pickup`
  (params (ActorObject :type "/Game/Fadeout_Content/Core/Weapons/BP_weaponBase Object Reference"))
  (bind _megaweapon_vo (`self.MegaWeapon_VO`))
  ;[1 1 1] mega weapon VO or weapon voice event override
  (`parent.weaponBase_Pickup` ActorObject)
  (for _array_element (`self.equipment`)
    (if (== (`GameplayStatics.GetObjectClass` _array_element) "/Game/Fadeout_Content/Core/Weapons/Abilities/Ability_Chi_Launch.Ability_Chi_Launch_C")
      (`/Engine/EditorBlueprintResources/StandardMacros.IsValid` _megaweapon_vo
        (:`Is Valid`
          (`self.SpeakQuote` _megaweapon_vo)
          (break))))))

(event `self.currentItemUIIndex`
  (params (`Instant?` :type Boolean))
  ;[1 1 1] instant item switch for UI
  (`parent.currentItemUIIndex` true))

(event `self.ReceiveBeginPlay`
  (`parent.ReceiveBeginPlay`)
  (`self.PlayerInputSwitchWeapon` 3 true))

(event `self.Color Set`
  (bind _output (`|GetArrayItem` (`self.EquippedCosmetics`) (`KismetArrayLibrary.Array_Find` (`self.Equipped Cosmetic Reference`) "/Game/Fadeout_Content/Core/Characters/Panda/Outfits/Pandan_Charlie/pandanCharlie_Skin_01.pandanCharlie_Skin_01")))
  (bind _output_2 (`|GetArrayItem` (`self.EquippedCosmetics`) (`KismetArrayLibrary.Array_Find` (`self.Equipped Cosmetic Reference`) "/Game/Fadeout_Content/Core/Characters/Panda/clothing_only.clothing_only")))
  (bind _output_3 (`|GetArrayItem` (`self.EquippedCosmetics`) (`KismetArrayLibrary.Array_Find` (`self.Equipped Cosmetic Reference`) "/Game/Fadeout_Content/Core/Characters/Panda/Outfits/Mafia_Charlie/mafiacharlie_01.mafiacharlie_01")))
  (`parent.Color Set`)
  (switch `/Game/Fadeout_Content/Core/UI/Customize/Charlie_Outfits` (cast `/Game/Fadeout_Content/Core/UI/Customize/Charlie_Outfits` (`self.current_outfit`))
    (:`NewEnumerator2`
      (`/Engine/EditorBlueprintResources/StandardMacros.IsValid` _output_2
        (:`Is Valid`
          (bind _returnvalue (`KismetMaterialLibrary.CreateDynamicMaterialInstance` (`PrimitiveComponent.GetMaterial` _output_2 0) "/Game/Fadeout_Content/Core/Characters/Panda/M_Panda_Clothing.M_Panda_Clothing" "None"))
          (bind _output_get (set `self.HelmetDynamic` _returnvalue))
          (`PrimitiveComponent.SetMaterial` _output_2 0 _output_get)
          (`self.RecolorMeshes` _output_get))))
    (:`NewEnumerator3`
      (`/Engine/EditorBlueprintResources/StandardMacros.IsValid` _output_3
        (:`Is Valid`
          (bind _returnvalue_2 (`KismetMaterialLibrary.CreateDynamicMaterialInstance` (`PrimitiveComponent.GetMaterial` _output_3 0) "/Game/Fadeout_Content/Core/Characters/Panda/Outfits/Mafia_Charlie/M_Mafia_Charlie.M_Mafia_Charlie" "None"))
          (bind _output_get_2 (set `self.HelmetDynamic` _returnvalue_2))
          (`PrimitiveComponent.SetMaterial` _output_3 0 _output_get_2)
          (`self.RecolorMeshes` _output_get_2))))
    (:`NewEnumerator4`
      (`/Engine/EditorBlueprintResources/StandardMacros.IsValid` _output
        (:`Is Valid`
          (bind _returnvalue_3 (`KismetMaterialLibrary.CreateDynamicMaterialInstance` (`PrimitiveComponent.GetMaterial` _output 0) "/Game/Fadeout_Content/Core/Characters/Panda/Outfits/Pandan_Charlie/M_Pandan_Skin.M_Pandan_Skin" "None"))
          (bind _output_get_3 (set `self.HelmetDynamic` _returnvalue_3))
          (`PrimitiveComponent.SetMaterial` _output 0 _output_get_3)
          (`self.RecolorMeshes` _output_get_3))))))

(fn `unarmed_Attacks`
  (params (attack :type Integer) (InPlayRate :type "Float (double-precision)"))
  (switch `int` attack
    (:`0`
      (`self.PlayAnimMontage` "/Game/Fadeout_Content/Core/Characters/Bunn/attacks/unarmed/panda_Fighter_ComboA_2_Montage.panda_Fighter_ComboA_2_Montage" InPlayRate "Default"))
    (:`1`
      (`self.ChargePunch`))
    (:`2`
      (`self.PlayAnimMontage` "/Game/Fadeout_Content/Core/Characters/Bunn/attacks/unarmed/panda_Fighter_Hammer_Montage.panda_Fighter_Hammer_Montage" InPlayRate "Default"))
    (:`3`
      (`self.PlayAnimMontage` "/Game/Fadeout_Content/Core/Characters/Bunn/attacks/unarmed/bunn_Kick_02_root_rootAction_Montage.bunn_Kick_02_root_rootAction_Montage" InPlayRate "Default"))
    (:`4`
      (`self.Chi Launch`))
    (:`5`
      (`self.PlayAnimMontage` "/Game/Fadeout_Content/Core/Characters/Bunn/attacks/unarmed/bunKick_Stationary_Montage.bunKick_Stationary_Montage" InPlayRate "Default"))))

(fn `UserConstructionScript`
  (`parent.UserConstructionScript`))