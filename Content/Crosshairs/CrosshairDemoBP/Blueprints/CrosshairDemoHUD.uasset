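; Demo HUD for browsing a crosshair pack with keyboard controls, creating the demo widget on BeginPlay and exposing the current name, index, size and texture through getters.
; Keys step the index by several increments, walk a shuffled index list built at startup, or resize the crosshair within limits.
; Index changes clamp to the DataTable row count and build a zero-padded row name to look up the texture.
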(event `self.ReceiveBeginPlay`
  (bind _randomizedcrosshairindices (`self.RandomizedCrosshairIndices`))
  (bind _crosshairdatatable (`self.CrosshairDataTable`))
  (`self.UpdateCrosshairTexture`)
  (`self.EnableInput` (`GameplayStatics.GetPlayerController` 0))
  (bind _returnvalue (`|CreateWidget` "/Game/Crosshairs/CrosshairDemoBP/Blueprints/CrosshairDemoWidget.CrosshairDemoWidget_C"))
  (`UserWidget.AddToViewport` _returnvalue 0)
  (`/Engine/EditorBlueprintResources/StandardMacros.IsValid` _crosshairdatatable
    (:`Is Valid`
      (bind _outrownames (`DataTableFunctionLibrary.GetDataTableRowNames` _crosshairdatatable))
      (for (_ _array_index) _outrownames
        (`KismetArrayLibrary.Array_Add` _randomizedcrosshairindices (+ _array_index 1)))
      (`KismetArrayLibrary.Array_Shuffle` _randomizedcrosshairindices))))

(event `Key|E`
  (params (Key :type "Key Structure"))
  (:`Pressed`
    (`self.IncrementRandomCrosshairIndex` -1)
    (`self.UpdateCrosshairTexture`)))

(event `Key|U`
  (params (Key :type "Key Structure"))
  (:`Pressed`
    (`self.IncrementCrosshairIndex` -100)))

(event `Key|I`
  (params (Key :type "Key Structure"))
  (:`Pressed`
    (`self.IncrementCrosshairIndex` 100)))

(event `Key|R`
  (params (Key :type "Key Structure"))
  (:`Pressed`
    (`self.IncrementRandomCrosshairIndex` 1)
    (`self.UpdateCrosshairTexture`)))

(event `Key|O`
  (params (Key :type "Key Structure"))
  (:`Pressed`
    (`self.IncrementCrosshairIndex` -10)))

(event `Key|P`
  (params (Key :type "Key Structure"))
  (:`Pressed`
    (`self.IncrementCrosshairIndex` 10)))

(event `Key|LeftBracket`
  (params (Key :type "Key Structure"))
  (:`Pressed`
    (`self.IncrementCrosshairIndex` -1)))

(event `Key|RightBracket`
  (params (Key :type "Key Structure"))
  (:`Pressed`
    (`self.IncrementCrosshairIndex` 1)))

(event `Key|PageUp`
  (params (Key :type "Key Structure"))
  (:`Pressed`
    (`self.AddToCrosshairSize` (`self.CrosshairSizeIncrement`))))

(event `Key|PageDown`
  (params (Key :type "Key Structure"))
  (:`Pressed`
    (`self.AddToCrosshairSize` (* (`self.CrosshairSizeIncrement`) -1.0))))

(fn `AddToCrosshairSize`
  (params (inValue :type "Float (double-precision)"))
  (bind (_x _y) (`KismetMathLibrary.BreakVector2D` (`self.CrosshairSizeLimits`)))
  (set `self.CrosshairSize` (`KismetMathLibrary.FClamp` (+ inValue (`self.CrosshairSize`)) _x _y)))

(fn `GetCrosshairIndex`
  (returns (OutIndex :type Integer))
  (return (`self.CrosshairIndex`)))

(fn `GetCrosshairName`
  (returns (OutString :type String))
  (return (`self.CrosshairName`)))

(fn `GetCrosshairSize`
  (returns (OutFloat :type "Float (double-precision)"))
  (return (`self.CrosshairSize`)))

(fn `GetCrosshairTexture`
  (returns (OutTexture :type "Texture Object Reference"))
  (return (`self.CrosshairTexture`)))

(fn `IncrementCrosshairIndex`
  (params (`Increment Value` :type Integer))
  (set `self.CrosshairIndex` (+ (`self.CrosshairIndex`) `Increment Value`))
  (`self.UpdateCrosshairTexture`))

(fn `IncrementRandomCrosshairIndex`
  (params (IncrementAmount :type Integer))
  (set `self.RandomCrosshairIndex` (`KismetMathLibrary.Clamp` (`self.RandomCrosshairIndex`) 0 (- (`KismetArrayLibrary.Array_Length` (`self.RandomizedCrosshairIndices`)) 1)))
  (if (`KismetArrayLibrary.Array_IsValidIndex` (`self.RandomizedCrosshairIndices`) (`self.RandomCrosshairIndex`))
    (set `self.CrosshairIndex` (`|GetArrayItem` (`self.RandomizedCrosshairIndices`) (`self.RandomCrosshairIndex`)))
    (set `self.RandomCrosshairIndex` (+ (`self.RandomCrosshairIndex`) IncrementAmount))))

(fn `PadNumber`
  (params (InNumber :type Integer))
  (returns (OutString :type String))
  (locals (OutputString :type String))
  (set `local.OutputString` "")
  (if (< InNumber 1000)
    (set `local.OutputString` (`KismetStringLibrary.Concat_StrStr` (`local.OutputString`) "0")))
  (if (< InNumber 100)
    (set `local.OutputString` (`KismetStringLibrary.Concat_StrStr` (`local.OutputString`) "0")))
  (if (< InNumber 10)
    (set `local.OutputString` (`KismetStringLibrary.Concat_StrStr` (`local.OutputString`) "0")))
  (bind _output_get (set `local.OutputString` (`KismetStringLibrary.Concat_StrStr` (`local.OutputString`) (`KismetStringLibrary.Conv_IntToString` InNumber))))
  (return _output_get))

(fn `UpdateCrosshairTexture`
  (locals (CrosshairIndexCount :type Integer))
  (`/Engine/EditorBlueprintResources/StandardMacros.IsValid` (`self.CrosshairDataTable`)
    (:`Is Valid`
      (bind _outrownames (`DataTableFunctionLibrary.GetDataTableRowNames` (`self.CrosshairDataTable`)))
      (set `local.CrosshairIndexCount` (`KismetArrayLibrary.Array_Length` _outrownames)))
    (:`Is Not Valid`
      (set `local.CrosshairIndexCount` 1)))
  (set `self.CrosshairIndex` (`KismetMathLibrary.Clamp` (`self.CrosshairIndex`) 1 (`local.CrosshairIndexCount`)))
  (bind _output_get (set `self.CrosshairName` (`KismetStringLibrary.Concat_StrStr` (`KismetStringLibrary.Concat_StrStr` "T_Crosshairs_S1_" (`self.PadNumber` (`self.CrosshairIndex`))) "_2048")))
  (bind _returnvalue (`|GetDataTableRow` (`self.CrosshairDataTable`) (`KismetStringLibrary.Conv_StringToName` _output_get))
    (:`then`
      (set `self.CrosshairTexture` (`.Texture_2_22B129064406D16B62AAE5B95DDC1F62` (break `/Game/Crosshairs/CrosshairPack/CrosshairManifestEntry` _returnvalue))))))

(fn `UserConstructionScript`)