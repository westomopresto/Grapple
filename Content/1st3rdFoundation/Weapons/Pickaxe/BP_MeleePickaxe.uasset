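; Pickaxe melee weapon Blueprint that sets its pick damage type on BeginPlay and relies on its parent for firing.
; On BeginPlay and when dropped, it swaps the skeletal mesh's physics asset between on-ground and in-hand versions based on OnGround.
; Release and alt-fire events are empty overrides.
; A charge-up attack, clamping Charge and passing a full-charge flag to the parent's release, remains in the graph but is disconnected.
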(event `self.OnRelease`
  (params (`charged?` :type Boolean)))

(event `self.OnFire`
  (`parent.OnFire`))

(event `self.ReceiveTick`
  (params (DeltaSeconds :type "Float (single-precision)"))
  (`parent.ReceiveTick` 0.0))

(event `self.OnDropped`
  (bind _skeletalmesh (`self.SkeletalMesh`))
  (if (`self.onGround?`) :!label _label
    (`SkinnedMeshComponent.SetPhysicsAsset` _skeletalmesh "/Game/1st3rdFoundation/Core/FBX/Pickaxe/pickaxe_onGround.pickaxe_onGround" false)
    (else
      (`SkinnedMeshComponent.SetPhysicsAsset` _skeletalmesh "/Game/1st3rdFoundation/Core/FBX/Pickaxe/pickaxe_inhand.pickaxe_inhand" false))))

(event `self.ReceiveBeginPlay`
  (set `self.Damage Type` "/Game/1st3rdFoundation/Core/Weapons/DamageTypes/DT_Pick.DT_Pick_C")
  (`parent.ReceiveBeginPlay`)
  (goto _label))

(event `self.OnAltFire`
  (params (`MoveCamera?` :type Boolean)))

(event `self.AltFireRelease`)

(fn `UserConstructionScript`
  (`parent.UserConstructionScript`))