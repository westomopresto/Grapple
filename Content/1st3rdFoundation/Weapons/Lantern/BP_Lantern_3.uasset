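; Lantern weapon that toggles two lights and a particle effect when fired and burns fuel while lit.
; Once-per-second fuel drain, skipped for post-mounted lanterns, syncs AmmoCount to the owning BP_PlayerCharacter's LanternFuel.
; A change watcher on HasFuel shuts the light off when fuel runs out.
; Placement flags choose ground or in-hand physics assets, and post lanterns not on the ground start lit with Stationary lights.
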(event `Oil Tick`
  (params (`Delta Time` :type "Float (double-precision)"))
  (if (not (`self.onPost?`))
    (set `self.tickFloat` (+ (`self.tickFloat`) `Delta Time`))
    (if (>= (`self.tickFloat`) 1.0)
      (set `self.tickFloat` 0.0)
      (bind _output_get (set `self.AmmoCount` (- (`self.AmmoCount`) (`self.FireCost`))))
      (`KismetSystemLibrary.PrintString` (`KismetStringLibrary.Conv_DoubleToString` _output_get))
      (`self.SetOrGetFuel` false)
      (if (<= _output_get 0.0)
        (set `self.AmmoCount` 0.0)
        (`self.SetOrGetFuel` false)))))

(event `self.OnDropped`
  (if (`self.onGround?`)
    (`SkinnedMeshComponent.SetPhysicsAsset` (`self.SkeletalMesh`) "/Game/1st3rdFoundation/Core/FBX/Lantern_Model/lantern_onGround.lantern_onGround" false)))

(event `self.ReceiveBeginPlay`
  (bind _hasfuel (`self.hasFuel`))
  (bind _skeletalmesh (`self.SkeletalMesh`))
  (`self.SetOrGetFuel` true)
  (bind (_old_value _new_value) (`/Game/1st3rdFoundation/Core/MacroLibrary.Value Changed` _hasfuel _hasfuel :!label _label)
    (:`Setup Complete`
      (if (`self.onGround?`)
        (`SkinnedMeshComponent.SetPhysicsAsset` _skeletalmesh "/Game/1st3rdFoundation/Core/FBX/Lantern_Model/lantern_onGround.lantern_onGround" false)
        (`self.turnOff`)
        (else
          (`SkinnedMeshComponent.SetPhysicsAsset` _skeletalmesh "/Game/1st3rdFoundation/Core/FBX/Lantern_Model/lantern_inHand.lantern_inHand" false)
          (if (`self.onPost?`)
            (`self.turnOn`)
            (`SceneComponent.SetMobility` (`self.PointLight1`) "Stationary")
            (`SceneComponent.SetMobility` (`self.meshShadow`) "Stationary")
            (else
              (`self.turnOff`))))))
    (:`Value changed`
      (if (not _new_value)
        (`self.turnOff`)))))

(event `self.ReceiveTick`
  (params (DeltaSeconds :type "Float (single-precision)"))
  (if (`self.lanternOn?`)
    (`self.Oil Tick` DeltaSeconds))
  (set `self.hasFuel` (> (`self.AmmoCount`) 0.0))
  (goto _label :!via `Check Change`))

(event `self.OnFire`
  (`self.SetOrGetFuel` true)
  (`/Engine/EditorBlueprintResources/StandardMacros.FlipFlop`
    (:`A`
      (set `self.lanternOn?` true)
      (`KismetSystemLibrary.PrintString` "lantern on")
      (if (> (`self.AmmoCount`) 0.0)
        (`self.turnOn`)))
    (:`B`
      (set `self.lanternOn?` false)
      (`KismetSystemLibrary.PrintString` "lantern off")
      (`self.turnOff`))))

(event `turnOn`
  (`LightComponent.SetIntensity` (`self.meshShadow`) 1000.0)
  (`LightComponent.SetIntensity` (`self.PointLight1`) 5502.0)
  (`ActorComponent.Activate` (`self.ParticleSystem`) false))

(event `turnOff`
  (`LightComponent.SetIntensity` (`self.meshShadow`) 0.0)
  (`LightComponent.SetIntensity` (`self.PointLight1`) 0.0)
  (`ActorComponent.Deactivate` (`self.ParticleSystem`)))

(fn `SetOrGetFuel`
  (params (GETorSET :type Boolean))
  (bind _returnvalue (`self.GetOwner`))
  (if GETorSET
    (bind _asbp_player_character (cast `/Game/1st3rdFoundation/Core/Characters/BP_PlayerCharacter` _returnvalue))
    (`/Engine/EditorBlueprintResources/StandardMacros.IsValid` _asbp_player_character
      (:`Is Valid`
        ;[1 1 1] get
        (set `self.AmmoCount` (`/Game/1st3rdFoundation/Core/Characters/BP_PlayerCharacter.lanternFuel` _asbp_player_character))))
    (else
      (bind _asbp_player_character_2 (cast `/Game/1st3rdFoundation/Core/Characters/BP_PlayerCharacter` _returnvalue))
      (`/Engine/EditorBlueprintResources/StandardMacros.IsValid` _asbp_player_character_2
        (:`Is Valid`
          ;[1 1 1] set
          (set `/Game/1st3rdFoundation/Core/Characters/BP_PlayerCharacter.lanternFuel` (`self.AmmoCount`) _asbp_player_character_2)))))
  (return))

(fn `UserConstructionScript`)