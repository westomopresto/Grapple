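; BP_Fuel is a pickup that refills the player's lantern fuel.
; Its PickedUp event casts the owning pawn to BP_PlayerCharacter, adds a fixed amount to LanternFuel with no clamp in this graph, and plays a bottle sound at the pickup's location.
; BeginPlay and the construction script only call their parent versions, and nothing here triggers PickedUp or removes the actor.
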(event `self.ReceiveBeginPlay`
  (`parent.ReceiveBeginPlay`))

(event `self.pickedUp`
  (params (owningPawn :type "Actor Object Reference"))
  (bind _asbp_player_character (cast `/Game/1st3rdFoundation/Core/Characters/BP_PlayerCharacter` owningPawn))
  (set `/Game/1st3rdFoundation/Core/Characters/BP_PlayerCharacter.lanternFuel` (+ (`/Game/1st3rdFoundation/Core/Characters/BP_PlayerCharacter.lanternFuel` _asbp_player_character) 50.0) _asbp_player_character)
  (`GameplayStatics.PlaySoundAtLocation` "/Game/1st3rdFoundation/Core/Audio/RPG_Sounds/inventory/bottle.bottle" (`self.K2_GetActorLocation`) (struct) 1.0 1.0 0.0 null null null))

(fn `UserConstructionScript`
  (`parent.UserConstructionScript`))