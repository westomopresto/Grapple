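; Grapple gun weapon Blueprint that fires a hook projectile after a full charge-up.
; Holding fire switches the player to aim camera, disables running and tool swapping, and builds a capped, frame-counted charge on Tick.
; Release fires only at full charge if the parent fire check passes, otherwise it cancels and restores player state.
; A Returned flag, set by hook return or dummy-hook visibility, gates reuse.
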(event `ReturnedHook`
  (set `self.Returned` true)
  (bind _asbp_player_character (cast `/Game/1st3rdFoundation/Core/Characters/BP_PlayerCharacter` (`GameplayStatics.GetPlayerPawn` 0)))
  (set `/Game/1st3rdFoundation/Core/Characters/BP_PlayerCharacter.canSwapTools?` true _asbp_player_character)
  (set `/Game/1st3rdFoundation/Core/Characters/BP_PlayerCharacter.canRun?` true _asbp_player_character)
  (`/Game/1st3rdFoundation/Core/Characters/BP_PlayerCharacter.toRearCam` _asbp_player_character))

(event `/Game/1st3rdFoundation/Core/Weapons/BP_weaponBase.OnFire`
  (bind _asbp_player_character (cast `/Game/1st3rdFoundation/Core/Characters/BP_PlayerCharacter` (`GameplayStatics.GetPlayerPawn` 0)))
  (set `/Game/1st3rdFoundation/Core/Characters/BP_PlayerCharacter.canSwapTools?` false _asbp_player_character)
  (`/Game/1st3rdFoundation/Core/Characters/BP_PlayerCharacter.releaseSlow` _asbp_player_character)
  (if (`self.Returned`)
    (bind _asbp_player_character_2 (cast `/Game/1st3rdFoundation/Core/Characters/BP_PlayerCharacter` (`GameplayStatics.GetPlayerPawn` 0)))
    (set `/Game/1st3rdFoundation/Core/Characters/BP_PlayerCharacter.canRun?` false _asbp_player_character_2)
    (`/Game/1st3rdFoundation/Core/Characters/BP_PlayerCharacter.PlayChargeWeaponAnim` _asbp_player_character_2)
    (set `self.Is Charging` true)
    (`self.PlayNoAmmoSound`)
    (`/Game/1st3rdFoundation/Core/Characters/BP_PlayerCharacter.toAimCam` _asbp_player_character_2)))

(event `/Game/1st3rdFoundation/Core/Weapons/BP_weaponBase.OnRelease`
  (if (`self.Returned`)
    (set `self.Is Charging` false)
    (`/Engine/EditorBlueprintResources/StandardMacros.CompareFloat` (`self.charge`) 60.0
      (:`>`
        (set `self.charge` 0.0 :!label _label)
        (`parent.OnFire`)
        (if (`self.CanFire?`)
          (`self.Fire Projectile`)
          (`self.PlayFireSound`)
          (bind _asbp_player_character (cast `/Game/1st3rdFoundation/Core/Characters/BP_PlayerCharacter` (`GameplayStatics.GetPlayerPawn` 0)))
          (`/Game/1st3rdFoundation/Core/Characters/BP_PlayerCharacter.PlayFireWeaponAnim` _asbp_player_character)
          (else
            (`self.PlayNoAmmoSound` :!label _label_2)
            (bind _asbp_player_character_2 (cast `/Game/1st3rdFoundation/Core/Characters/BP_PlayerCharacter` (`GameplayStatics.GetPlayerPawn` 0)))
            (`/Game/1st3rdFoundation/Core/Characters/BP_PlayerCharacter.StopChargingWeaponAnim` _asbp_player_character_2)
            (set `/Game/1st3rdFoundation/Core/Characters/BP_PlayerCharacter.canSwapTools?` true _asbp_player_character_2)
            (set `/Game/1st3rdFoundation/Core/Characters/BP_PlayerCharacter.canRun?` true _asbp_player_character_2)
            (`/Game/1st3rdFoundation/Core/Characters/BP_PlayerCharacter.toRearCam` _asbp_player_character_2)
            (`/Game/1st3rdFoundation/Core/Characters/BP_PlayerCharacter.releaseSlow` _asbp_player_character_2))))
      (:`==`
        (goto _label))
      (:`<`
        (set `self.charge` 0.0)
        (goto _label_2)))))

(event `self.ReceiveTick`
  (params (DeltaSeconds :type "Float (single-precision)"))
  (if (`self.Is Charging`)
    (bind _result (`/Engine/EditorBlueprintResources/StandardMacros.IncrementFloat` (`self.charge`))
      (:`  `
        (set `self.charge` (`KismetMathLibrary.FClamp` _result 0.0 60.0))))))

(fn `GetMuzzleLocation`
  (returns (MuzzleLocation :type "Vector Structure") (MuzzleTransform :type "Transform Structure"))
  (bind _muzzlesocket (`self.MuzzleSocket`))
  (return (`SceneComponent.GetSocketLocation` (`self.Mesh`) _muzzlesocket) (`SceneComponent.GetSocketTransform` (`self.Mesh`) _muzzlesocket "RTS_World")))

(fn `HideHookToggle`
  (params (visibility :type Boolean :default true))
  (bind _hookdummy (`self.HookDummy`))
  (`SceneComponent.SetVisibility` _hookdummy visibility false)
  (if (`SceneComponent.bVisible` _hookdummy)
    (set `self.Returned` true)
    (else
      (set `self.Returned` false))))

(fn `UserConstructionScript`
  (`parent.UserConstructionScript`))