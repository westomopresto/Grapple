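; Game mode that sets up local multiplayer by creating a configurable number of players at BeginPlay.
; SpawnPlayers first calls CreatePlayer for each controller ID with pawn spawning enabled.
; A second loop spawns a BP_PlayerCharacter per player at one fixed spot near the world origin, passes it the player index, and has the matching PlayerController possess it.
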(event `self.ReceiveBeginPlay`
  (`self.spawnPlayers`))

(fn `spawnPlayers`
  (bind _returnvalue (- (`self.numberOfPlayers`) 1))
  (for _index (range (+ _returnvalue 1))
    (`GameplayStatics.CreatePlayer` _index))
  (for _index_2 (range (+ _returnvalue 1))
    (bind _returnvalue_2 (`|SpawnActorFromClass` "/Game/1st3rdFoundation/Core/Characters/BP_PlayerCharacter.BP_PlayerCharacter_C" (`KismetMathLibrary.MakeTransform` (0.0 0.0 1.0)) "Undefined" "OverrideRootScale" null _index_2 null))
    (`Controller.Possess` (`GameplayStatics.GetPlayerController` _index_2) _returnvalue_2)))

(fn `UserConstructionScript`)