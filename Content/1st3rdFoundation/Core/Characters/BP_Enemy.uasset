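; Enemy AI character that runs BT_Enemy and can patrol along a spline path.
; BeginPlay starts it sprinting and stores its spawn location as the blackboard Home; taking damage sets the damage causer as TargetActor.
; Patrol start and pause events toggle sprint and a looping timer that advances a wrapping spline distance as the move goal.
; Death disables sight perception and clears the target.
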(event `self.ReceiveAnyDamage`
  (params (Damage :type "Float (single-precision)") (DamageType :type "DamageType Object Reference") (InstigatedBy :type "Controller Object Reference") (DamageCauser :type "Actor Object Reference"))
  (bind _returnvalue (`AIBlueprintHelperLibrary.GetBlackboard` (`self.GetController`)))
  (`parent.ReceiveAnyDamage` Damage DamageType InstigatedBy DamageCauser)
  (`KismetSystemLibrary.PrintString` (`KismetSystemLibrary.GetDisplayName` DamageCauser) true true (struct :`G` 0.66 :`B` 1.0 :`A` 1.0) 4.0)
  (`/Engine/EditorBlueprintResources/StandardMacros.IsValid` _returnvalue
    (:`Is Valid`
      (`BlackboardComponent.SetValueAsObject` _returnvalue "TargetActor" DamageCauser))))

(event `self.ReceiveBeginPlay`
  (set `self.HomeLocation` (`self.K2_GetActorLocation`))
  (`parent.ReceiveBeginPlay`)
  (`self.toSprint`)
  (`AIController.RunBehaviorTree` (`AIBlueprintHelperLibrary.GetAIController` self) "/Game/1st3rdFoundation/Core/Characters/BT_Enemy.BT_Enemy")
  (`BlackboardComponent.SetValueAsVector` (`AIBlueprintHelperLibrary.GetBlackboard` (`self.GetController`)) "Home" (`self.HomeLocation`)))

(event `self.ReceiveTick`
  (params (DeltaSeconds :type "Float (single-precision)"))
  (`parent.ReceiveTick` DeltaSeconds))

(event `pausePatrolling`
  (`KismetSystemLibrary.K2_PauseTimerHandle` (`self.Patrol Handle`))
  (`self.toSprint`))

(event `startPatrolling`
  (`self.stopSprint`)
  (`KismetSystemLibrary.K2_UnPauseTimerHandle` (`self.Patrol Handle`))
  (bind _returnvalue (`KismetSystemLibrary.K2_SetTimerDelegate` (delegate `Patrol`) 0.25 true))
  (set `self.Patrol Handle` _returnvalue))

(event `Patrol`
  (bind _returnvalue (`self.GetComponentByClass` (`self.patrolPath`) "/Script/Engine.SplineComponent"))
  (bind _returnvalue_2 (`SplineComponent.GetSplineLength` _returnvalue))
  (bind _output_get (set `self.splineDistance` (+ (`self.splineDistance`) (`self.patrolSpeed`))))
  (if (not (< _output_get _returnvalue_2))
    (set `self.splineDistance` (- (`self.splineDistance`) _returnvalue_2)))
  (bind _output_get_2 (set `self.Patrol Location` (`SplineComponent.GetLocationAtDistanceAlongSpline` _returnvalue (`self.splineDistance`) "World")))
  (`AIBlueprintHelperLibrary.SimpleMoveToLocation` (`self.GetController`) _output_get_2))

(event `self.Die`
  (bind _returnvalue (`AIBlueprintHelperLibrary.GetBlackboard` null))
  (`AIPerceptionComponent.SetSenseEnabled` (`self.AIPerception`) "/Script/AIModule.AISense_Sight" false)
  (`/Engine/EditorBlueprintResources/StandardMacros.IsValid` _returnvalue
    (:`Is Valid`
      (`BlackboardComponent.ClearValue` _returnvalue "TargetActor"))
    (:`Is Not Valid`
      _))
  (`parent.Die`))

(fn `UserConstructionScript`
  (`parent.UserConstructionScript`))