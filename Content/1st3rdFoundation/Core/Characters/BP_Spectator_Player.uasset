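; BP_Spectator_Player is a temporary spectator pawn that lets a player respawn by pressing Fire.
; On possession it prints an on-screen prompt explaining how to respawn.
; Fire spawns a BP_PlayerCharacter at the spectator's transform with rotation zeroed, passing on PlayerInt to keep the player's index.
; It then runs the character's spawn function, hands over possession, creates the combat HUD and destroys itself.
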(event `InputAction|Fire`
  (params (Key :type "Key Structure"))
  (bind _returnvalue (`KismetMathLibrary.MakeTransform` (.location (`SceneComponent.K2_GetComponentToWorld` (`self.RootComponent`))) (struct) (.scale (`SceneComponent.K2_GetComponentToWorld` (`self.RootComponent`)))))
  (:`Pressed`
    (bind _returnvalue_2 (`|SpawnActorFromClass` "/Game/1st3rdFoundation/Core/Characters/BP_PlayerCharacter.BP_PlayerCharacter_C" _returnvalue "Undefined" "OverrideRootScale" null (`self.PlayerInt`) null))
    (`/Game/1st3rdFoundation/Core/Characters/BP_PlayerCharacter.spawnFunction` _returnvalue_2 true _returnvalue)
    (`Controller.Possess` (stale `self.ReceivePossessed` NewController) _returnvalue_2)
    (`Controller.Possess` (`GameplayStatics.GetPlayerController` (`self.PlayerInt`)) _returnvalue_2)
    (`/Game/1st3rdFoundation/Core/Characters/BP_PlayerCharacter.create_combat_HUD` _returnvalue_2)
    (`self.K2_DestroyActor`)))

(event `self.ReceivePossessed`
  (params (NewController :type "Controller Object Reference"))
  (`KismetSystemLibrary.PrintString` "You are spectating. Click/Fire to respawn" true true (struct :`G` 0.66 :`B` 1.0 :`A` 1.0) 20.0))

(fn `UserConstructionScript`)