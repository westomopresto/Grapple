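; BP_DangerLight is a prop light that shows whether the game is in danger by switching its point light between reddish-orange and green.
; Each tick it copies the DANGER flag from BP_GameMode into InDanger by polling, then asks a valueChanged helper to check for a change.
; The helper, set up on BeginPlay, fires a callback that recolors the light only when the value changes.
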(event `self.ReceiveBeginPlay`
  (bind _pointlightcomponent (`self.PointLightComponent`))
  (bind _indanger_ (`self.inDanger?`))
  (bind (_old_value _new_value) (`/Game/1st3rdFoundation/Core/MacroLibrary.Value Changed` _indanger_ _indanger_ :!label _label)
    (:`Value changed`
      (if _new_value
        (`LightComponent.SetLightColor` _pointlightcomponent (struct :`R` 0.634375 :`G` 0.22225 :`B` 0.106387 :`A` 1.0) true)
        (else
          (`LightComponent.SetLightColor` _pointlightcomponent (struct :`R` 0.424692 :`G` 0.7375 :`B` 0.447592 :`A` 1.0) true))))))

(event `self.ReceiveTick`
  (params (DeltaSeconds :type "Float (single-precision)"))
  (bind _asbp_game_mode (cast `/Game/1st3rdFoundation/Core/GameModes/BP_GameMode` (`GameplayStatics.GetGameMode`)))
  (set `self.inDanger?` (`/Game/1st3rdFoundation/Core/GameModes/BP_GameMode.DANGER?` _asbp_game_mode))
  (goto _label :!via `Check Change`))

(fn `UserConstructionScript`)