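; Hitscan weapon Blueprint that extends a parent weapon's fire event with line traces and point damage.
; On fire, if allowed, it casts multiple traces from the muzzle socket toward the crosshair's world position, randomized within a spread cone and debug-drawn.
; Collected results receive point damage using the base damage of the ammo set at BeginPlay.
; The impact effects function is an empty stub.
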(event `self.ReceiveBeginPlay`
  (bind _returnvalue (`AddComponent|NODE_AddBP_BaseAmmo-0`))
  (set `self.CurrentAmmo` _returnvalue))

(event `self.OnFire`
  (params (CrosshairWorldSpace :type "Vector Structure"))
  (`parent.OnFire` CrosshairWorldSpace)
  (if (`self.CanFire?`)
    (bind _hitoccured (`self.DetermineHitObjects` CrosshairWorldSpace))
    (if _hitoccured
      (`self.ApplyDamageToHitActors`)
      (`self.PlayImpactEffects`))))

(fn `ApplyDamageToHitActors`
  (bind _returnvalue (`self.GetInstigatorController`))
  (for _index (range (`KismetArrayLibrary.Array_Length` (`self.HitResults`)))
    (bind _output (`|GetArrayItem` (`self.HitResults`) _index))
    (bind (_bblockinghit _binitialoverlap _time _distance _location _impactpoint _normal _impactnormal _physmat _hitactor) (`GameplayStatics.BreakHitResult` _output))
    (`GameplayStatics.ApplyPointDamage` _hitactor (`/Game/1st3rdFoundation/Core/Weapons/BP_BaseAmmo.BaseDamage` (`self.CurrentAmmo`)) (`KismetMathLibrary.GetForwardVector` (`KismetMathLibrary.FindLookAtRotation` _location (`self.K2_GetActorLocation` (`Controller.K2_GetPawn` _returnvalue)))) _output _returnvalue self)))

(fn `DetermineHitObjects`
  (params (CrosshairWorldSpace :type "Vector Structure"))
  (returns (HitOccured :type Boolean))
  (locals (ObjectHit :type Boolean))
  (bind _location (.location (`SceneComponent.GetSocketTransform` (`self.Mesh`) (`self.MuzzleSocket`) "RTS_World")))
  (`KismetArrayLibrary.Array_Clear` (`self.HitResults`))
  (for _ (range 1 (+ (`self.TracesUsed`) 1))
    (bind (_outhit _returnvalue) (`KismetSystemLibrary.LineTraceSingle` :`Start` _location :`End` (+ _location (`KismetMathLibrary.GreaterGreater_VectorRotator` (* (`KismetMathLibrary.RandomUnitVectorInConeInRadians` (1.0 0.0 0.0) (`KismetMathLibrary.DegreesToRadians` (`self.Spread`))) (`self.Range`)) (`KismetMathLibrary.FindLookAtRotation` _location CrosshairWorldSpace))) :`TraceChannel` "TraceTypeQuery1" :`DrawDebugType` "ForDuration"))
    (bind _output_get (set `local.ObjectHit` (or _returnvalue (`local.ObjectHit`))))
    (if _output_get
      (`KismetArrayLibrary.Array_Add` (`self.HitResults`) _outhit)))
  (return (`local.ObjectHit`)))

(fn `PlayImpactEffects`)

(fn `UserConstructionScript`
  (`parent.UserConstructionScript`))