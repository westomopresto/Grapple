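; Base item Blueprint with a skeletal mesh that grants health to the player when picked up.
; On BeginPlay it swaps the mesh's physics asset between on-ground and off-ground versions based on the OnGround flag.
; The pickedUp event casts the owning pawn to BP_PlayerCharacter and adds a fixed amount to Health, with no clamp or self-destruction here.
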(event `self.ReceiveBeginPlay`
  (bind _skeletalmesh (`self.SkeletalMesh`))
  (if (`self.onGround?`)
    (`SkinnedMeshComponent.SetPhysicsAsset` _skeletalmesh (`self.onGroundPHYS`) false)
    (else
      (`SkinnedMeshComponent.SetPhysicsAsset` _skeletalmesh (`self.offGroundPHYS`) false))))

(event `pickedUp`
  (params (owningPawn :type "Actor Object Reference"))
  (bind _asbp_player_character (cast `/Game/1st3rdFoundation/Core/Characters/BP_PlayerCharacter` owningPawn))
  (set `/Game/1st3rdFoundation/Core/Characters/BP_PlayerCharacter.health` (+ (`/Game/1st3rdFoundation/Core/Characters/BP_PlayerCharacter.health` _asbp_player_character) 20.0) _asbp_player_character))

(fn `UserConstructionScript`)