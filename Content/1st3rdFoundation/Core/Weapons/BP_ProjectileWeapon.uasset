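; Projectile weapon Blueprint that launches a grapple hook projectile when fired.
; On BeginPlay it caches the player index from its instigating BP_PlayerCharacter.
; OnFire runs the parent logic, then, if CanFire is set, spawns BP_GrappleHook_Projectile just ahead of the mesh's muzzle socket.
; The projectile is oriented along that player pawn's base aim rotation rather than the barrel and stored as ActiveProjectile.
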(event `self.ReceiveBeginPlay`
  (bind _asbp_player_character (cast `/Game/1st3rdFoundation/Core/Characters/BP_PlayerCharacter` (`self.GetInstigator`)))
  (set `self.playerInt` (`/Game/1st3rdFoundation/Core/Characters/BP_PlayerCharacter.PlayerInt` _asbp_player_character)))

(event `/Game/1st3rdFoundation/Core/Weapons/BP_weaponBase.OnFire`
  (`parent.OnFire`)
  (if (`self.CanFire?`)
    (`self.Fire Projectile`)))

(fn `Fire Projectile`
  (bind _mesh (`self.Mesh`))
  (bind _muzzlesocket (`self.MuzzleSocket`))
  (bind _returnvalue (`|SpawnActorFromClass` "/Game/1st3rdFoundation/Weapons/Projectiles/BP_GrappleHook_Projectile.BP_GrappleHook_Projectile_C" (`KismetMathLibrary.MakeTransform` (+ (`SceneComponent.GetSocketLocation` _mesh _muzzlesocket) (`KismetMathLibrary.Conv_RotatorToVector` (`SceneComponent.GetSocketRotation` _mesh _muzzlesocket))) (`Pawn.GetBaseAimRotation` (`GameplayStatics.GetPlayerPawn` (`self.playerInt`)))) "Undefined" "OverrideRootScale" self (`self.GetInstigator`)))
  (set `self.ActiveProjectile` _returnvalue))

(fn `UserConstructionScript`
  (`parent.UserConstructionScript`))