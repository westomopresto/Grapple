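; Base firing weapon Blueprint that provides shared ammo checks and audio helpers.
; OnFire only updates CanFire, which is true while both ammo and durability are above zero.
; Separate functions subtract a clamped fire cost with a debug print and play fire or empty sounds at the actor's location, but nothing here calls them.
; OnRelease and PlayMuzzleFlash are empty stubs.
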(event `self.OnFire`
  (bind _canfire (`self.CanWeaponFire`))
  (if _canfire
    (set `self.CanFire?` true)
    (else
      (set `self.CanFire?` false))))

(event `self.OnRelease`)

(fn `CanWeaponFire`
  (returns (CanFire :type Boolean))
  (if (> (`self.AmmoCount`) 0.0)
    (if (> (`self.Durability`) 0.0)
      (return true)
      (else
        _)))
  (return false))

(fn `DecrementAmmoCount`
  (bind _output_get (set `self.AmmoCount` (`KismetMathLibrary.FClamp` (- (`self.AmmoCount`) (`self.FireCost`)) 0.0 (`self.MaxAmmoCount`))))
  (`KismetSystemLibrary.PrintString` (`KismetStringLibrary.BuildString_Double` "" "Ammo Count" _output_get)))

(fn `PlayFireSound`
  (`GameplayStatics.PlaySoundAtLocation` (`self.FireSound`) (`self.K2_GetActorLocation`) (struct) 1.0 1.0 0.0 null null null))

(fn `PlayMuzzleFlash`)

(fn `PlayNoAmmoSound`
  (`GameplayStatics.PlaySoundAtLocation` (`self.NoAmmoSound`) (`self.K2_GetActorLocation`) (struct) 1.0 1.0 0.0 null null null))

(fn `UserConstructionScript`)