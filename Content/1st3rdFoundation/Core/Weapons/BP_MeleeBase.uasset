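; BP_MeleeBase is a melee weapon actor that forwards primary and alternate attack input to its instigating player's windup and release functions.
; A charged primary release opens a brief trace window, while an uncharged one cancels the montage.
; During that window, Tick sphere-traces at the mesh's "hitpoint" socket, applies damage and stops the swing on the first damaging hit.
; Primary attacks lock tool swapping until finished; alternate attacks never start the trace.
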(event `self.OnAltFire`
  (params (`MoveCamera?` :type Boolean))
  (`KismetSystemLibrary.PrintString` "Alternate Fire Pressed" false)
  (`/Game/1st3rdFoundation/Core/Characters/BP_PlayerCharacter.altMeleeWindup` (`self.Player`)))

(event `AltFireRelease`
  (`self.PlayAltFireSound`)
  (`/Game/1st3rdFoundation/Core/Characters/BP_PlayerCharacter.altMeleeRelease` (`self.Player`)))

(event `self.ReceiveBeginPlay`
  (bind _asbp_player_character (cast `/Game/1st3rdFoundation/Core/Characters/BP_PlayerCharacter` (`self.GetInstigator`)))
  (set `self.Player` _asbp_player_character)
  (`KismetSystemLibrary.PrintString` (`KismetStringLibrary.Concat_StrStr` "Player: " (`KismetStringLibrary.Conv_IntToString` (`/Game/1st3rdFoundation/Core/Characters/BP_PlayerCharacter.PlayerInt` _asbp_player_character)))))

(event `OnFire`
  (bind _player (`self.Player`))
  (`KismetSystemLibrary.PrintString` "Primary Fire Pressed" false)
  (`/Game/1st3rdFoundation/Core/Characters/BP_PlayerCharacter.meleeWindup` _player)
  (set `/Game/1st3rdFoundation/Core/Characters/BP_PlayerCharacter.canSwapTools?` false _player))

(event `self.OnRelease`
  (params (`charged?` :type Boolean))
  (bind _player (`self.Player`))
  (if `charged?`
    (`self.PlayFireSound`)
    (`/Game/1st3rdFoundation/Core/Characters/BP_PlayerCharacter.meleeRelease` _player)
    (`self.Trace`)
    (else
      (`/Game/1st3rdFoundation/Core/Characters/BP_PlayerCharacter.meleeRelease` _player)
      (bind _returnvalue (`Character.GetCurrentMontage` _player))
      (`Character.StopAnimMontage` _player _returnvalue)
      (set `/Game/1st3rdFoundation/Core/Characters/BP_PlayerCharacter.canSwapTools?` true (`self.Player`)))))

(event `self.ReceiveTick`
  (params (DeltaSeconds :type "Float (single-precision)"))
  (bind _hitlocation (`self.HitLocation`))
  (bind _player (`self.Player`))
  (set `self.HitLocation` (`SceneComponent.GetSocketLocation` (`self.SkeletalMesh`) "hitpoint"))
  (if (`self.doTrace?`)
    (bind _outhit (`KismetSystemLibrary.SphereTraceSingle` _hitlocation _hitlocation 25.0 "TraceTypeQuery2" false (`|MakeArray` (`self.GetInstigator`) :!type "Actor Object Reference") "ForDuration" true (struct :`R` 1.0 :`A` 1.0) (struct :`G` 1.0 :`A` 1.0) 0.1))
    (bind (_bblockinghit _binitialoverlap _time _distance _location _impactpoint _normal _impactnormal _physmat _hitactor) (`GameplayStatics.BreakHitResult` _outhit))
    (bind _returnvalue (`GameplayStatics.ApplyDamage` _hitactor (`self.damage`) null (`self.Player`) "/Script/Engine.DamageType"))
    (`KismetSystemLibrary.PrintString` (`KismetStringLibrary.BuildString_Object` (`KismetStringLibrary.BuildString_Double` (`KismetSystemLibrary.GetDisplayName` (`self.Player`)) " did " _returnvalue " damage to") "" _hitactor) false)
    (if (> _returnvalue 0.0)
      (set `self.doTrace?` false)
      (bind _returnvalue_2 (`Character.GetCurrentMontage` _player))
      (`Character.StopAnimMontage` _player _returnvalue_2))))

(event `Trace`
  (set `self.doTrace?` true)
  (`KismetSystemLibrary.Delay` 0.3)
  (set `self.doTrace?` false)
  (set `/Game/1st3rdFoundation/Core/Characters/BP_PlayerCharacter.canSwapTools?` true (`self.Player`)))

(fn `PlayAltFireSound`
  (`GameplayStatics.PlaySoundAtLocation` (`self.FireSound`) (`self.K2_GetActorLocation`) (struct) 1.0 1.0 0.0 null null null))

(fn `PlayFireSound`
  (`GameplayStatics.PlaySoundAtLocation` (`self.FireSound`) (`self.K2_GetActorLocation`) (struct) 1.0 (`KismetMathLibrary.RandomFloatInRange` 0.9 1.1) 0.0 null null null))

(fn `UserConstructionScript`)