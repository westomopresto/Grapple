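; BP_ProjectileGun is a weapon Blueprint that fires grapple hook projectiles.
; BeginPlay caches PlayerInt from the instigating BP_PlayerCharacter.
; OnFire calls FireProjectile when CanWeaponFire passes.
; FireProjectile spawns BP_GrappleHook_Projectile just ahead of the muzzle socket, oriented by the instigator's base aim with a slight yaw offset, and stores it as ActiveProjectile.
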(event `self.ReceiveBeginPlay`
  (bind _asbp_player_character (cast `/Game/1st3rdFoundation/Core/Characters/BP_PlayerCharacter` (`self.GetInstigator`)))
  (set `self.playerInt` (`/Game/1st3rdFoundation/Core/Characters/BP_PlayerCharacter.PlayerInt` _asbp_player_character)))

(event `self.OnFire`
  (bind _canfire (`self.CanWeaponFire`))
  (bind _output_get (set `self.CanFire?` _canfire))
  (if _output_get
    (`self.Fire Projectile`)))

(fn `Fire Projectile`
  (bind _mesh (`self.Mesh`))
  (bind _muzzlesocket (`self.MuzzleSocket`))
  (bind _returnvalue (`|SpawnActorFromClass` "/Game/1st3rdFoundation/Weapons/Projectiles/BP_GrappleHook_Projectile.BP_GrappleHook_Projectile_C" (`KismetMathLibrary.MakeTransform` (+ (`SceneComponent.GetSocketLocation` _mesh _muzzlesocket) (`KismetMathLibrary.Conv_RotatorToVector` (`SceneComponent.GetSocketRotation` _mesh _muzzlesocket))) (`KismetMathLibrary.MakeRotator` (.roll (`Pawn.GetBaseAimRotation` (`self.GetInstigator`))) (.pitch (`Pawn.GetBaseAimRotation` (`self.GetInstigator`))) (+ (.yaw (`Pawn.GetBaseAimRotation` (`self.GetInstigator`))) 3.0))) "Undefined" "OverrideRootScale" self (`self.GetInstigator`)))
  (set `self.ActiveProjectile` _returnvalue))

(fn `UserConstructionScript`
  (`parent.UserConstructionScript`))