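; Actor component that gives a character positional voice chat, with speaking toggle, local muting and cleanup on death.
; It creates a VOIP talker from the PlayerState, retrying until valid, attached to the capsule with attenuation.
; For the local player it adds a HUD and runs a looping timer that lists active speakers and shows their icons only with line of sight.
; Muting swaps attenuation assets; actors communicate through BP_VOIPInterface.
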(event `CreateVOIP`
  (bind _returnvalue (`self.GetOwner`))
  ;[1 1 1] Create VOIP
  (`/Engine/EditorBlueprintResources/StandardMacros.IsValid` _returnvalue :!label _label
    (:`Is Valid`
      (bind _ascharacter (cast `Character` _returnvalue)
        (:`then`
          (bind _playerstate (`Pawn.PlayerState` _ascharacter))
          (`/Engine/EditorBlueprintResources/StandardMacros.IsValid` _playerstate
            (:`Is Valid`
              (bind _returnvalue_2 (`VOIPTalker.CreateTalkerForPlayer` _playerstate))
              (set `self.MyVoiceRef` _returnvalue_2)
              (`VOIPStatics.SetMicThreshold` -5.0)
              (set `VOIPTalker.Settings` (make `VoiceSettings` (`Character.CapsuleComponent` _ascharacter) "/Game/AntizeVOIPSystem/Audio/SA_VOIPAttenuation.SA_VOIPAttenuation") (`self.MyVoiceRef`)))
            (:`Is Not Valid`
              (`KismetSystemLibrary.Delay` 0.2 :!label _label_2)
              (goto _label))))
        (:`CastFailed`
          (goto _label_2))))
    (:`Is Not Valid`
      (goto _label_2))))

(event `self.ReceiveBeginPlay`
  ;[1 1 1] OnConstruct
  (`KismetSystemLibrary.Delay` 2.0)
  (`self.CreateVOIP`)
  (`KismetSystemLibrary.ExecuteConsoleCommand` (select `bool` (`self.VOIPLoopBack?`) :`false` "OSS.VoiceLoopback 0" :`true` "OSS.VoiceLoopback 1") null)
  (bind _aspawn (cast `Pawn` (`self.GetOwner`)))
  ;;[1 1 1] Get Controller (if player), security to prevent looping for uncontrolled characters
  (if (`Pawn.IsLocallyControlled` _aspawn)
    (bind _returnvalue (`Pawn.GetController` _aspawn))
    (`/Engine/EditorBlueprintResources/StandardMacros.IsValid` _returnvalue :!label _label_3
      (:`Is Valid`
        (bind _asplayer_controller (cast `PlayerController` _returnvalue)
          (:`then`
            (set `self.ControllerRef` _asplayer_controller)
            ;[1 1 1] Loop check for VoIP icon visibility
            (bind _returnvalue_2 (`KismetSystemLibrary.K2_SetTimerDelegate` (delegate `CheckForVOIP`) 0.2 true))
            (set `self.Timer_CheckForLoop` _returnvalue_2)
            (bind _returnvalue_3 (`|CreateWidget` "/Game/AntizeVOIPSystem/Widgets/W_VOIPHUD.W_VOIPHUD_C"))
            (bind _output_get (set `self.W_VOIPHUDRef` _returnvalue_3))
            (`UserWidget.AddToViewport` _output_get 99))
          (:`CastFailed`
            (`KismetSystemLibrary.Delay` 0.2 :!label _label_4)
            (bind _result (`/Engine/EditorBlueprintResources/StandardMacros.IncrementInt` (`self.Attempt`))
              (:`  `
                (if (not (>= _result 25))
                  (goto _label_3)))))))
      (:`Is Not Valid`
        (goto _label_4)))))

(event `CheckForVOIP`
  (bind _returnvalue (`self.GetOwner`))
  (bind _w_voiphudref (`self.W_VOIPHUDRef`))
  ;[1 1 1] Loop check for VoIP icon visibility
  (cast `Pawn` _returnvalue)
  (bind _outactors (`GameplayStatics.GetAllActorsWithInterface` "/Game/AntizeVOIPSystem/Blueprints/BP_VOIPInterface.BP_VOIPInterface_C"))
  (for _array_element _outactors
    (`/Engine/EditorBlueprintResources/StandardMacros.IsValid` _array_element
      (:`Is Valid`
        (bind _activated_ (message `/Game/AntizeVOIPSystem/Blueprints/BP_VOIPInterface.MSG_GetIsVOIPActivated` _array_element))
        (`/Engine/EditorBlueprintResources/StandardMacros.IsValid` _w_voiphudref
          (:`Is Valid`
            (`/Game/AntizeVOIPSystem/Widgets/W_VOIPHUD.RefreshVOIPList` _w_voiphudref _activated_ _array_element))
          (:`Is Not Valid`
            _))
        (if _activated_
          (bind (_outhit _returnvalue_2) (`KismetSystemLibrary.LineTraceSingle` (`Actor.K2_GetActorLocation` _returnvalue) (`Actor.K2_GetActorLocation` _array_element) "TraceTypeQuery1"))
          (if _returnvalue_2
            (message `/Game/AntizeVOIPSystem/Blueprints/BP_VOIPInterface.MSG_SetVisibilityVOIPIcon` _array_element (== _array_element (`.HitActor` (`GameplayStatics.BreakHitResult` _outhit))))
            (else
              (message `/Game/AntizeVOIPSystem/Blueprints/BP_VOIPInterface.MSG_SetVisibilityVOIPIcon` _array_element false)))
          (else
            (message `/Game/AntizeVOIPSystem/Blueprints/BP_VOIPInterface.MSG_SetVisibilityVOIPIcon` _array_element false)))))))

(event `ActivateDeactivateVOIP`
  (params (`Activated?` :type Boolean))
  (bind _w_voiphudref (`self.W_VOIPHUDRef`))
  ;[1 1 1] Activate/Deactivate VoIP
  (`KismetSystemLibrary.ExecuteConsoleCommand` (select `bool` `Activated?` :`false` "ToggleSpeaking 0" :`true` "ToggleSpeaking 1") null)
  (message `/Game/AntizeVOIPSystem/Blueprints/BP_VOIPInterface.MSG_SetIsVOIPActivated` (`self.GetOwner`) `Activated?`)
  (`/Engine/EditorBlueprintResources/StandardMacros.IsValid` _w_voiphudref
    (:`Is Valid`
      (`/Game/AntizeVOIPSystem/Widgets/W_VOIPHUD.SetVOIPIconVisibility` _w_voiphudref `Activated?`))))

(event `SetVisibilityVOIPIcon`
  (params (`Visible?` :type Boolean))
  (bind _returnvalue (`self.GetOwner`))
  ;[1 1 1] Set WidgetVoice visibility
  (if (!= `Visible?` (`self.VOIPIconVisible?`))
    (set `self.VOIPIconVisible?` `Visible?`)
    (`/Engine/EditorBlueprintResources/StandardMacros.IsValid` _returnvalue
      (:`Is Valid`
        (bind _widgetvoiceref (message `/Game/AntizeVOIPSystem/Blueprints/BP_VOIPInterface.MSG_GetWidgetVoice` _returnvalue))
        (`SceneComponent.SetVisibility` _widgetvoiceref (`self.VOIPIconVisible?`) true)))))

(event `MuteTemplate`
  (params (PlayerIndex :type Integer))
  ;[1 1 1] (Local) Mute the player only at the one who called "MuteTemplate"
  (bind _outactors (`GameplayStatics.GetAllActorsWithInterface` "/Game/AntizeVOIPSystem/Blueprints/BP_VOIPInterface.BP_VOIPInterface_C"))
  (if (`KismetArrayLibrary.Array_IsValidIndex` _outactors PlayerIndex)
    (bind _output (`|GetArrayItem` _outactors PlayerIndex))
    (bind _ismuted_ (message `/Game/AntizeVOIPSystem/Blueprints/BP_VOIPInterface.MSG_GetIsMuted` _output))
    (message `/Game/AntizeVOIPSystem/Blueprints/BP_VOIPInterface.MSG_SetMute` _output (not _ismuted_))))

(event `SetIsMuted`
  (params (`Mute?` :type Boolean))
  ;[1 1 1] (Local) Mute/Unmute the player
  (bind _output_get (set `self.IsMuted?` `Mute?`))
  (bind _ascharacter (cast `Character` (`self.GetOwner`)))
  (set `VOIPTalker.Settings` (make `VoiceSettings` (`Character.CapsuleComponent` _ascharacter) (select `bool` _output_get :`false` "/Game/AntizeVOIPSystem/Audio/SA_VOIPAttenuation.SA_VOIPAttenuation" :`true` "/Game/AntizeVOIPSystem/Audio/SA_VOIPAttenuationMute.SA_VOIPAttenuationMute" :!type "SoundAttenuation Object Reference")) (`self.MyVoiceRef`))
  (bind (_success_ _username) (message `/Game/AntizeVOIPSystem/Blueprints/BP_VOIPInterface.MSG_GetPlayerUsername` (`self.GetOwner`)))
  (`KismetSystemLibrary.PrintString` (`KismetStringLibrary.Concat_StrStr` (`KismetTextLibrary.Conv_TextToString` _username) " -> " (select `bool` (`self.IsMuted?`) :`false` "Unmute" :`true` "Mute"))))

(event `OnDeath`
  (bind _w_voiphudref (`self.W_VOIPHUDRef`))
  ;[1 1 1] Disable VoIP, remove widget and invalidate timer on death
  (`self.ActivateDeactivateVOIP` false)
  (`KismetSystemLibrary.K2_ClearAndInvalidateTimerHandle` (`self.Timer_CheckForLoop`))
  (`/Engine/EditorBlueprintResources/StandardMacros.IsValid` _w_voiphudref
    (:`Is Valid`
      (`Widget.RemoveFromParent` _w_voiphudref))))