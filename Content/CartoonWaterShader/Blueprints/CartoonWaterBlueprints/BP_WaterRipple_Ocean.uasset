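; BP_WaterRipple_Ocean configures the look of ocean water ripples for the cartoon water shader.
; Its RippleParameters function writes its speed, X and Y tiling, pattern width and color variables into the MPC_RipplesDecal material parameter collection.
; The function runs in both the construction script and BeginPlay, so values apply in the editor and at runtime.
; Because the collection is global, these values are shared by every material that reads it.
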(event `self.ReceiveBeginPlay`
  (`self.Ripple Parameters`))

(fn `Ripple Parameters`
  ;[1 1 1] Ripple Parameters
  (`KismetMaterialLibrary.SetScalarParameterValue` "/Game/CartoonWaterShader/Materials/MaterialCollections/MPC_RipplesDecal.MPC_RipplesDecal" "Ripple Speed" (`self.Ripple Speed`))
  (`KismetMaterialLibrary.SetScalarParameterValue` "/Game/CartoonWaterShader/Materials/MaterialCollections/MPC_RipplesDecal.MPC_RipplesDecal" "Ripple X Tile" (`self.Ripple X Tile`))
  (`KismetMaterialLibrary.SetScalarParameterValue` "/Game/CartoonWaterShader/Materials/MaterialCollections/MPC_RipplesDecal.MPC_RipplesDecal" "Ripple Y Tile" (`self.Ripple Y Tile`))
  (`KismetMaterialLibrary.SetScalarParameterValue` "/Game/CartoonWaterShader/Materials/MaterialCollections/MPC_RipplesDecal.MPC_RipplesDecal" "Ripples Pattern Width" (`self.Ripple Pattern Width`))
  (`KismetMaterialLibrary.SetVectorParameterValue` "/Game/CartoonWaterShader/Materials/MaterialCollections/MPC_RipplesDecal.MPC_RipplesDecal" "Ripples Color" (`self.Ripple Color`)))

(fn `UserConstructionScript`
  (`self.Ripple Parameters`))