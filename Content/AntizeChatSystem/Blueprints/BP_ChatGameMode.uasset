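; Game mode for the Antize chat system that tracks connected players on the server for username lookups and private-message checks.
; PostLogin adds each controller to ConnectedPlayers and sends it the array index as its player ID; logout removes it.
; Message functions expose the list, resolve usernames to IDs and check whether a target ID is online.
; Other private-message requests return the default online flag, and the game mode's own ID, team and username getters are stubs.
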(event `self.K2_PostLogin`
  (params (NewPlayer :type "PlayerController Object Reference"))
  ;[1 1 1] Add player to PlayersConnected array
  (`/Engine/EditorBlueprintResources/ActorMacros.Switch Has Authority`
    (:`Authority`
      (`/Engine/EditorBlueprintResources/StandardMacros.IsValid` NewPlayer
        (:`Is Valid`
          (bind _returnvalue (`KismetArrayLibrary.Array_AddUnique` (`self.ConnectedPlayers`) NewPlayer))
          (message `/Game/AntizeChatSystem/Blueprints/BP_AntizeChatInterface.MSG_SetPlayerID` NewPlayer _returnvalue))))))

(event `self.K2_OnLogout`
  (params (ExitingController :type "Controller Object Reference"))
  ;[1 1 1] Remove player from PlayersConnected array
  (`/Engine/EditorBlueprintResources/ActorMacros.Switch Has Authority`
    (:`Authority`
      (`KismetArrayLibrary.Array_RemoveItem` (`self.ConnectedPlayers`) ExitingController))))

(fn `MSG_GetConnectedPlayers`
  (returns (Players :type "Array of Controller Object Reference"))
  (return (`self.ConnectedPlayers`)))

(fn `MSG_GetPlayerID`
  (returns (PlayerID :type Integer))
  (return 0))

(fn `MSG_GetPlayerIDFromUsername`
  (params (Username :type Text))
  (returns (PlayerID :type Integer))
  (locals (Local_PlayerID :type Integer :default -1))
  (for _array_element (`self.ConnectedPlayers`)
    (bind (_success_ _username) (message `/Game/AntizeChatSystem/Blueprints/BP_AntizeChatInterface.MSG_GetUsername` _array_element))
    (if _success_
      (if (`KismetTextLibrary.EqualEqual_TextText` _username Username)
        (bind _playerid (message `/Game/AntizeChatSystem/Blueprints/BP_AntizeChatInterface.MSG_GetPlayerID` _array_element))
        (set `local.Local_PlayerID` _playerid)
        (break))))
  (return (`local.Local_PlayerID`)))

(fn `MSG_GetTeamID`
  (returns (TeamID :type Integer))
  (return 0))

(fn `MSG_GetUsername`
  (returns (`Success?` :type Boolean) (Username :type Text))
  (return false ""))

(fn `MSG_RequestPrivateMessage`
  (params (Request :type "/Game/AntizeChatSystem/Logics/E_PrivateMEssage Enum" :default "NewEnumerator1") (ToPlayerID :type Integer) (Username :type Text) (Message :type Text))
  (returns (`Online?` :type Boolean))
  (locals (`Local_Online?` :type Boolean))
  (if (>= ToPlayerID 0)
    (switch `/Game/AntizeChatSystem/Logics/E_PrivateMEssage` Request
      (:`NewEnumerator1`
        _)
      (:`NewEnumerator3`
        _)
      (:`NewEnumerator0`
        (for _array_element (`self.ConnectedPlayers`)
          (bind _playerid (message `/Game/AntizeChatSystem/Blueprints/BP_AntizeChatInterface.MSG_GetPlayerID` _array_element))
          (if (== _playerid ToPlayerID)
            (set `local.Local_Online?` true)
            (break)))
        (return (`local.Local_Online?`)))
      (:`NewEnumerator4`
        _))
    (return (`local.Local_Online?`))
    (else
      (return (`local.Local_Online?`)))))

(fn `UserConstructionScript`)